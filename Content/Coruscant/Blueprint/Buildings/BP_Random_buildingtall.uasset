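; Construction-script Blueprint for a randomized tall building in the Coruscant content.
; It gives each of its four static mesh components an independently random mesh from the first seven entries of the RandomMesh array.
; The picks use unseeded random integers, so the combination can change whenever construction reruns, and the event graph holds no active logic.
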(event EventBeginPlay)

(event Collision|EventActorBeginOverlap
  (params (OtherActor :type Actor%20Object%20Reference)))

(event EventTick
  (params (DeltaSeconds :type Float%20%28single-precision%29)))

(fn ConstructionScript
  (Components|StaticMesh|SetStaticMesh (Variables|Default|GetStaticMesh) (Utilities|Array|Get(acopy) (Variables|Default|GetRandomMesh) (Math|Random|RandomIntegerinRange 0 6)))
  (Components|StaticMesh|SetStaticMesh (Variables|Default|GetStaticMesh2) (Utilities|Array|Get(acopy) (Variables|Default|GetRandomMesh) (Math|Random|RandomIntegerinRange 0 6)))
  (Components|StaticMesh|SetStaticMesh (Variables|Default|GetStaticMesh3) (Utilities|Array|Get(acopy) (Variables|Default|GetRandomMesh) (Math|Random|RandomIntegerinRange 0 6)))
  (Components|StaticMesh|SetStaticMesh (Variables|Default|GetStaticMesh4) (Utilities|Array|Get(acopy) (Variables|Default|GetRandomMesh) (Math|Random|RandomIntegerinRange 0 6))))