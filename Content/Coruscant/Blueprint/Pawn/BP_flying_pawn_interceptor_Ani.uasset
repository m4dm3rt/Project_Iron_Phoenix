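; Player-flown interceptor pawn with physics-driven flight, switchable first-person, third-person and alternate cameras.
; Thrust input eases forward speed with camera shake, and Tick overwrites mesh velocity with it plus faked gravity that grows below a speed threshold.
; Axis inputs apply pitch, yaw and roll torque, with control-rotation roll held at zero.
; Hits rotate the craft using the surface normal, and the construction script resets the world origin from its current location.
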(event EventBeginPlay
  ;[1 1 1] Initialzing speed
  (Variables|Default|SetThrust (/ (Variables|Default|GetMax_thrust) 15.0)))

(event Collision|EventHit
  (params (MyComp :type Primitive%20Component%20Object%20Reference) (Other :type Actor%20Object%20Reference) (OtherComp :type Primitive%20Component%20Object%20Reference) (bSelfMoved :type Boolean) (HitLocation :type Vector :default "0, 0, 0") (HitNormal :type Vector :default "0, 0, 0") (NormalImpulse :type Vector :default "0, 0, 0") (Hit :type Hit%20Result%20Structure%20%28by%20ref%29))
  ;[1 1 1] Deflect when colliding
  (Transformation|SetActorRotation (Math|Rotator|Lerp(Rotator) (Transformation|GetActorRotation) (Math|Conversions|RotationFromXVector HitNormal) 1.5e+03 true)))

(event EventTick
  (params (DeltaSeconds :type Float%20%28single-precision%29))
  ;[1 1 1] gravity
  (Utilities|FlowControl|Sequence
    (:then_0
      (Physics|SetPhysicsLinearVelocity (Variables|Default|GetStaticMesh) (+ (Variables|Default|GetForwardVel) (Variables|Default|GetUpvel)) false "None")
      (if (< (Math|Vector|VectorLength (Variables|Default|GetForwardVel)) (Variables|Default|GetGravity_threshold))
        (Variables|Default|SetUpvel (* (Math|Vector|UnrotateVector (Transformation|GetActorUpVector) (Transformation|GetActorRotation)) (Math|Float|Lerp 0.0 -9.8e+02 (- 1.0 (/ (Math|Vector|VectorLength (Variables|Default|GetForwardVel)) (Variables|Default|GetGravity_threshold))))))
        (else
          (Variables|Default|SetUpvel (Math|Interpolation|VInterpTo (Variables|Default|GetUpvel) "0, 0, 0" (Utilities|Time|GetWorldDeltaSeconds) 2e+01)))))))

(event Input|ActionEvents|InputActionChange_camera
  (params (Key :type Key%20Structure))
  ;[1 1 1] Change Camera
  (:Pressed
    (Utilities|FlowControl|FlipFlop
      (:A
        (Components|Activation|SetActive (Variables|Default|GetFPP) true true)
        (Components|Activation|SetActive (Variables|Default|GetTPP) false false))
      (:B
        (Components|Activation|SetActive (Variables|Default|GetFPP) false false)
        (Components|Activation|SetActive (Variables|Default|GetTPP) true true)))))

(event Input|ActionEvents|InputActionChange_camera_back
  (params (Key :type Key%20Structure))
  (:Pressed
    (Utilities|FlowControl|FlipFlop
      (:A
        (Components|Activation|SetActive (Variables|Default|GetTPP1) true true)
        (Components|Activation|SetActive (Variables|Default|GetTPP) false false)
        (Components|Activation|SetActive (Variables|Default|GetFPP) false false))
      (:B
        (Components|Activation|SetActive (Variables|Default|GetTPP1) false false)
        (Components|Activation|SetActive (Variables|Default|GetTPP) true true)
        (Components|Activation|SetActive (Variables|Default|GetFPP) true false)))))

(event Input|AxisEvents|InputAxisMoveUp
  (params (AxisValue :type Float%20%28single-precision%29))
  ;[1 1 1] Movement
  (Class|PrimitiveComponent|AddTorqueinDegrees (Variables|Default|GetStaticMesh) (* (Transformation|GetActorRightVector) (* AxisValue 1.5e+02)) "None" true))

(event Input|AxisEvents|InputAxisMoveRight
  (params (AxisValue :type Float%20%28single-precision%29))
  ;[1 1 1] Movement
  (Class|PrimitiveComponent|AddTorqueinDegrees (Variables|Default|GetStaticMesh) (* (Transformation|GetActorUpVector) (* AxisValue 1e+02)) "None" true))

(event Input|AxisEvents|InputAxisroll
  (params (AxisValue :type Float%20%28single-precision%29))
  (bind _returnvalue (Pawn|GetControlRotation :!class /Script/Engine.Pawn))
  ;[1 1 1] Movement
  (Class|PrimitiveComponent|AddTorqueinDegrees (Variables|Default|GetStaticMesh) (* (Transformation|GetActorForwardVector) (* AxisValue 5e+02)) "None" true)
  (Pawn|Input|AddControllerYawInput 0.0)
  (Pawn|SetControlRotation (Game|GetPlayerController 0) (Math|Rotator|MakeRotator 0.0 (.pitch _returnvalue) (.yaw _returnvalue))))

(event Input|AxisEvents|InputAxisThrust
  (params (AxisValue :type Float%20%28single-precision%29))
  ;[1 1 1] calculating_foraward_thrust
  (Utilities|FlowControl|Sequence
    (:then_0
      (if (not (Math|Float|NearlyEqual(Float) AxisValue 0.0 0.1))
        (Variables|Default|SetThrust (Math|Interpolation|FInterpTo (Variables|Default|GetThrust) (Math|Float|Lerp 0.0 (Variables|Default|GetMax_thrust) (/ (+ AxisValue 1.0) 2.0)) (Utilities|Time|GetWorldDeltaSeconds) 0.25))
        (Camera|PlayWorldCameraShake 0 (Transformation|GetActorLocation) 0.0 5e+02)))
    (:then_1
      (Variables|Default|SetForwardVel (* (Transformation|GetActorForwardVector) (Variables|Default|GetThrust))))))

(fn ConstructionScript
  (CallFunction|ZeroWorldOrigin (Math|Conversions|ToVector(Float) (Class|GameplayStatics|GetWorldOriginLocation))))

(fn ZeroWorldOrigin
  (params (New%200 :type Vector))
  (bind _returnvalue (Class|GameplayStatics|GetWorldOriginLocation))
  (bind (_x _y _z) (Math|Vector|BreakVector New%200))
  (bind (_x_2 _y_2 _z_2) (Utilities|Struct|BreakIntVector _returnvalue))
  (Class|GameplayStatics|SetWorldOriginLocation (Utilities|Struct|MakeIntVector (+ (Math|Float|Truncate _x) _x_2) (+ (Math|Float|Truncate _y) _y_2) (+ (Math|Float|Truncate _z) _z_2))))