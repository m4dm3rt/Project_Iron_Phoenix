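; Single-player character Blueprint in a developer folder that holds the player's health, shield, boost and XP stat logic.
; Each resource has decrease, regenerate and max-increase functions, with regeneration capped at the maximum and booleans reporting depletion or full shield.
; Health only drops when the NoShield input is true.
; XP gains notify the player HUD, and reaching MaxXP increments Level in MainGameInstance, resets XP and raises the threshold.
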(fn ConstructionScript)

(fn DecreaseHealth
  (params (NoShield :type Boolean) (Damage%20Received :type Float%20%28double-precision%29))
  (if NoShield
    (bind _output_get (Variables|Backend|Conditions|Stats|SetCurrentHealth (- (Variables|Backend|Conditions|Stats|GetCurrentHealth) Damage%20Received)))
    (if (<= (/ _output_get (Variables|Backend|Conditions|Stats|GetMaxHealth)) 0.0)
      (return true)
      (else
        (return false)))))

(fn RegenerateHealth
  (params (Health%20Increase :type Float%20%28double-precision%29))
  (bind _output_get (Variables|Backend|Conditions|Stats|SetCurrentHealth (+ (Variables|Backend|Conditions|Stats|GetCurrentHealth) Health%20Increase)))
  (if (> _output_get (Variables|Backend|Conditions|Stats|GetMaxHealth))
    (bind _output_get_2 (Variables|Backend|Conditions|Stats|SetCurrentHealth (Variables|Backend|Conditions|Stats|GetMaxHealth)))))

(fn IncreaseMaxHealth
  (params (Max%20Health%20Increase :type Float%20%28double-precision%29))
  (Variables|Backend|Conditions|Stats|SetMaxHealth (+ (Variables|Backend|Conditions|Stats|GetMaxHealth) Max%20Health%20Increase)))

(fn DecreaseShield
  (params (Damage%20Received :type Float%20%28double-precision%29))
  (if (<= (/ (Variables|Backend|Conditions|Stats|GetCurrentShield) (Variables|Backend|Conditions|Stats|GetMaxShield)) 0.0)
    (return true)
    (else
      (Variables|Backend|Conditions|Stats|SetCurrentShield (- (Variables|Backend|Conditions|Stats|GetCurrentShield) Damage%20Received))
      (return false))))

(fn RegenerateShield
  (params (Shield%20Recovery :type Float%20%28double-precision%29))
  (bind _maxshield (Variables|Backend|Conditions|Stats|GetMaxShield))
  (bind _output_get (Variables|Backend|Conditions|Stats|SetCurrentShield (+ (Variables|Backend|Conditions|Stats|GetCurrentShield) Shield%20Recovery)))
  (if (> _output_get _maxshield)
    (bind _output_get_2 (Variables|Backend|Conditions|Stats|SetCurrentShield (Variables|Backend|Conditions|Stats|GetMaxShield))))
  (if (== _output_get_2 _maxshield)
    (return true)
    (else
      (return false))))

(fn IncreaseMaxShield
  (params (Max%20Shield%20Increase :type Float%20%28double-precision%29))
  (Variables|Backend|Conditions|Stats|SetMaxShield (+ (Variables|Backend|Conditions|Stats|GetMaxShield) Max%20Shield%20Increase)))

(fn DecreaseBoost
  (params (Boost%20Decrease :type Float%20%28double-precision%29))
  (bind _output_get (Variables|Backend|Conditions|Stats|SetCurrentBoost (- (Variables|Backend|Conditions|Stats|GetCurrentBoost) Boost%20Decrease)))
  (if (<= (/ _output_get (Variables|Backend|Conditions|Stats|GetMaxBoost)) 0.0)
    (return true)
    (else
      (return false))))

(fn RegenerateBoost
  (params (Boost%20Increase :type Float%20%28double-precision%29))
  (bind _output_get (Variables|Backend|Conditions|Stats|SetCurrentBoost (+ (Variables|Backend|Conditions|Stats|GetCurrentBoost) Boost%20Increase)))
  (if (> _output_get (Variables|Backend|Conditions|Stats|GetMaxBoost))
    (Variables|Backend|Conditions|Stats|SetCurrentBoost (Variables|Backend|Conditions|Stats|GetMaxBoost))))

(fn IncreaseMaxBoost
  (params (Max%20Boost%20Increase :type Float%20%28double-precision%29))
  (Variables|Backend|Conditions|Stats|SetMaxBoost (+ (Variables|Backend|Conditions|Stats|GetMaxBoost) Max%20Boost%20Increase)))

(fn IncreaseXP
  (params (Add%20XP :type Float%20%28double-precision%29))
  (bind _playerhud_ref (Variables|Backend|References|GetPlayerHUD%20REF))
  (bind _output_get (Variables|Backend|Conditions|Stats|SetCurrentXP (+ (Variables|Backend|Conditions|Stats|GetCurrentXP) Add%20XP)))
  (if (>= _output_get (Variables|Backend|Conditions|Stats|GetMaxXP))
    (Default|LevelUp _playerhud_ref)
    (LevelSystem|IncreaseLevel)
    (else
      (Default|XPUp _playerhud_ref Add%20XP))))

(fn IncreaseLevel
  (bind _asmain_game_instance (Utilities|Casting|CastToMainGameInstance (Game|GetGameInstance)))
  (bind _output_get (Variables|Backend|Conditions|Stats|SetLevel (+ (Variables|/Game/Devs/PRO_Mert/BluePrints/Player/MISC/MainGameInstance.MainGameInstance_C|GetLevel _asmain_game_instance) 1.0)))
  (Variables|/Game/Devs/PRO_Mert/BluePrints/Player/MISC/MainGameInstance.MainGameInstance_C|SetLevel _asmain_game_instance _output_get)
  (Variables|Backend|Conditions|Stats|SetMaxXP (+ (Variables|Backend|Conditions|Stats|GetMaxXP) 5e+01))
  (Variables|Backend|Conditions|Stats|SetCurrentXP 0.0))