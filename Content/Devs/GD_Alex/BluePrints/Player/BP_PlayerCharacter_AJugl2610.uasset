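; Player-controlled spaceship with physics flight, two switchable repeat-fire guns, boost, regenerating shield, health and collision damage.
; Looping timers ramp throttle, strafe and rise counters from input flags, which Speed lerps into the physics body's velocity on Tick.
; Tick also damps spin with counter-torque, widens FOV with throttle and capsule-traces from the crosshair to flag enemy lock-on.
; Input graphs handle look, roll, aim zoom, camera distance and a HUD-hiding spectator camera.
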(event EventBeginPlay
  (|CGraphBeginPlay))

(event EventTick
  (params (DeltaSeconds :type Float%20%28single-precision%29))
  (bind _crosshair (Variables|Default|GetCrosshair))
  (bind _followcamera (Variables|Default|GetFollowCamera))
  (bind _driverphsysics (Variables|Default|GetDriverPhsysics))
  (bind _returnvalue (Transformation|GetWorldLocation _crosshair))
  (Utilities|FlowControl|Delay 0.001)
  (CallFunction|Speed)
  (Class|PrimitiveComponent|AddTorqueinDegrees _driverphsysics (/ (Math|Vector|NegateVector (Physics|GetPhysicsAngularVelocityinDegrees _driverphsysics "None")) 0.5) "None" true)
  (bind _returnvalue_2 (Physics|GetPhysicsLinearVelocity _driverphsysics "None"))
  (Physics|SetPhysicsLinearVelocity _driverphsysics _returnvalue_2 false "None")
  (if (Variables|Player|Conditions|GetAiming)
    _
    (else
      (Camera|SetFieldOfView _followcamera (Math|Interpolation|FInterpTo (Variables|/Script/Engine.CameraComponent|GetFieldOfView _followcamera) (Math|Float|SelectFloat 1.2e+02 1e+02 (> (Variables|Player|Conditions|GetThrottleAmount) 50)) (Utilities|Time|GetWorldDeltaSeconds) 1.0))))
  (bind (_outhit _returnvalue_3) (Collision|CapsuleTraceByChannel _returnvalue (+ _returnvalue (* (* (Math|Vector|GetForwardVector (Transformation|GetWorldRotation _crosshair)) -1.0) 3e+05)) (Variables|Player|Settings|Combat|GetTargetRadius) 0.0 "TraceTypeQuery1" false 0 "None"))
  (if _returnvalue_3
    (if (not (Variables|Player|Conditions|GetTargetLocked))
      (Utilities|Casting|CastToBP_EnemyCharacter1 (.HitActor (Collision|BreakHitResult _outhit)))
      (Utilities|FlowControl|Delay 0.5)
      (Utilities|Casting|CastToBP_EnemyCharacter1 (.HitActor (Collision|BreakHitResult _outhit)))
      (Variables|Player|Conditions|SetTargetLocked true)
      (Audio|PlaySound2D "/Game/Devs/GD_Alex/Sounds/ShootingSFX/HitEnemySound/PewCut.PewCut" 0.5 1.5 0.4 0 0 false)
      (goto _label Reset))
    (else
      (Utilities|FlowControl|DoOnce true :!label _label
        (:Completed
          (Utilities|FlowControl|Delay 0.5)
          (Variables|Player|Conditions|SetTargetLocked false)
          (Audio|PlaySound2D "/Game/Devs/GD_Alex/Sounds/ShootingSFX/HitEnemySound/PewCut.PewCut" 0.5 0.5 0.3 0 0 false))))))

(fn ConstructionScript)

(fn Throttle
  (if (Variables|Player|Conditions|GetThrottleUp)
    (bind _result (Math|Integer|IncrementInt (Variables|Player|Conditions|GetThrottleAmount))
      (:%20%20
        (Variables|Player|Conditions|SetThrottleAmount (Math|Integer|Clamp(Integer) _result (Variables|Player|Conditions|GetThrottleMin) (Variables|Player|Conditions|GetThrottleMax)))
        (Development|SetHiddeninGame (Variables|Default|GetBP_VorwardVFX) false false)))
    (else
      (Development|SetHiddeninGame (Variables|Default|GetBP_VorwardVFX) true false)
      (if (Variables|Player|Conditions|GetThrottleDown)
        (bind _result_2 (Math|Integer|DecrementInt (Variables|Player|Conditions|GetThrottleAmount))
          (:%20%20
            (bind _output_get (Variables|Player|Conditions|SetThrottleAmount (Math|Integer|Clamp(Integer) _result_2 (Variables|Player|Conditions|GetThrottleMin) (Variables|Player|Conditions|GetThrottleMax))))
            (if (== _output_get 0)
              (Variables|Player|Conditions|SetThrottleDown false))))
        (else
          (bind _result_3 (Math|Integer|DecrementInt (Variables|Player|Conditions|GetThrottleAmount))
            (:%20%20
              (Variables|Player|Conditions|SetThrottleAmount (Math|Integer|Clamp(Integer) _result_3 0 (Variables|Player|Conditions|GetThrottleMax))))))))))

(fn Speed
  (bind _strafevalue (Variables|Player|Conditions|GetStrafeValue))
  (bind _strafevalue_2 (Variables|Player|Conditions|GetStrafeValue))
  (bind _driverphsysics (Variables|Default|GetDriverPhsysics))
  (bind _rise_lowvalue (Variables|Player|Conditions|GetRise/LowValue))
  (bind _rise_lowvalue_2 (Variables|Player|Conditions|GetRise/LowValue))
  (bind _boostvelocity (Variables|Player|Settings|Movement|GetBoostVelocity))
  (bind _throttlevalue (Variables|Player|Conditions|GetThrottleValue))
  (bind _returnvalue (Physics|GetPhysicsLinearVelocity _driverphsysics "None"))
  (Physics|SetPhysicsLinearVelocity (Variables|Default|GetDriverPhsysics) (Math|Vector|Lerp(Vector) _returnvalue (* (Math|Vector|GetForwardVector _driverphsysics) (+ (Math|Float|Clamp(Float) (* (Variables|Player|Conditions|GetThrottleAmount) _throttlevalue) -1e+04 (Math|Conversions|ToFloat(Integer) (* _throttlevalue 50))) (Math|Float|Clamp(Float) (* (Variables|Player|Conditions|GetBoostAmount) _boostvelocity) 0.0 (Math|Conversions|ToFloat(Integer) (* _boostvelocity 50))))) (Variables|Player|Settings|Movement|GetAccelerationVelocity)) false "None")
  (Utilities|FlowControl|Sequence
    (:then_0
      (if (Variables|Player|Conditions|GetStrafingRight)
        (Physics|SetPhysicsLinearVelocity (Variables|Default|GetDriverPhsysics) (Math|Vector|Lerp(Vector) _returnvalue (* (Math|Vector|GetRightVector (Variables|Default|GetDriverPhsysics)) (Math|Float|Clamp(Float) (* (Variables|Player|Conditions|GetStrafeAmount) _strafevalue) 0.0 (Math|Conversions|ToFloat(Integer) (* _strafevalue 1)))) (Variables|Player|Settings|Movement|GetStrafeVelocity)) false "None")))
    (:then_1
      (if (Variables|Player|Conditions|GetStrafingLeft)
        (Physics|SetPhysicsLinearVelocity (Variables|Default|GetDriverPhsysics) (Math|Vector|Lerp(Vector) _returnvalue (* (Math|Vector|GetRightVector (Variables|Default|GetDriverPhsysics)) (Math|Float|Clamp(Float) (* (Variables|Player|Conditions|GetStrafeAmount) _strafevalue_2) 0.0 (Math|Conversions|ToFloat(Integer) (* _strafevalue_2 -1)))) (Variables|Player|Settings|Movement|GetStrafeVelocity)) false "None")))
    (:then_2
      (if (Variables|Player|Conditions|GetRising)
        (Physics|SetPhysicsLinearVelocity (Variables|Default|GetDriverPhsysics) (Math|Vector|Lerp(Vector) _returnvalue (* (Math|Vector|GetUpVector (Variables|Default|GetDriverPhsysics)) (Math|Float|Clamp(Float) (* (Variables|Player|Conditions|GetRise/LowAmount) _rise_lowvalue) 0.0 (Math|Conversions|ToFloat(Integer) (* _rise_lowvalue 50)))) (Variables|Player|Settings|Movement|GetRise/LowerVelocity)) false "None")))
    (:then_3
      (if (Variables|Player|Conditions|GetLowering)
        (Physics|SetPhysicsLinearVelocity (Variables|Default|GetDriverPhsysics) (Math|Vector|Lerp(Vector) _returnvalue (* (Math|Vector|GetUpVector (Variables|Default|GetDriverPhsysics)) (Math|Float|Clamp(Float) (* (Variables|Player|Conditions|GetRise/LowAmount) _rise_lowvalue_2) 0.0 (Math|Conversions|ToFloat(Integer) (* _rise_lowvalue_2 -50)))) (Variables|Player|Settings|Movement|GetRise/LowerVelocity)) false "None")))))

(fn StrafeRight
  (if (Variables|Player|Conditions|GetStrafingRight)
    (bind _result (Math|Integer|IncrementInt (Variables|Player|Conditions|GetStrafeAmount))
      (:%20%20
        (Variables|Player|Conditions|SetStrafeAmount (Math|Integer|Clamp(Integer) _result 0 (Variables|Player|Conditions|GetStrafeMax)))
        (Development|SetHiddeninGame (Variables|Default|GetPointLight3) false false)))
    (else
      (Development|SetHiddeninGame (Variables|Default|GetPointLight3) true false)
      (bind _result_2 (Math|Integer|DecrementInt (Variables|Player|Conditions|GetStrafeAmount))
        (:%20%20
          (Variables|Player|Conditions|SetStrafeAmount (Math|Integer|Clamp(Integer) _result_2 0 (Variables|Player|Conditions|GetStrafeMax))))))))

(fn StrafeLeft
  (if (Variables|Player|Conditions|GetStrafingLeft)
    (bind _result (Math|Integer|IncrementInt (Variables|Player|Conditions|GetStrafeAmount))
      (:%20%20
        (Variables|Player|Conditions|SetStrafeAmount (Math|Integer|Clamp(Integer) _result 0 (Variables|Player|Conditions|GetStrafeMax)))
        (Development|SetHiddeninGame (Variables|Default|GetPointLight4) false false)))
    (else
      (Development|SetHiddeninGame (Variables|Default|GetPointLight4) true false)
      (bind _result_2 (Math|Integer|DecrementInt (Variables|Player|Conditions|GetStrafeAmount))
        (:%20%20
          (Variables|Player|Conditions|SetStrafeAmount (Math|Integer|Clamp(Integer) _result_2 0 (Variables|Player|Conditions|GetStrafeMax))))))))

(fn Rise
  (if (Variables|Player|Conditions|GetRising)
    (bind _result (Math|Integer|IncrementInt (Variables|Player|Conditions|GetRise/LowAmount))
      (:%20%20
        (bind _result_2 (Math|Integer|IncrementInt _result)
          (:%20%20
            (bind _result_3 (Math|Integer|IncrementInt _result_2)
              (:%20%20
                (bind _result_4 (Math|Integer|IncrementInt _result_3)
                  (:%20%20
                    (Variables|Player|Conditions|SetRise/LowAmount (Math|Integer|Clamp(Integer) _result_4 0 (Variables|Player|Conditions|GetRise/LowMax)))))))))))
    (else
      (bind _result_5 (Math|Integer|DecrementInt (Variables|Player|Conditions|GetRise/LowAmount))
        (:%20%20
          (Variables|Player|Conditions|SetRise/LowAmount (Math|Integer|Clamp(Integer) _result_5 0 (Variables|Player|Conditions|GetRise/LowMax))))))))

(event Input|ActionEvents|InputActionStrafeLeft
  (params (Key :type Key%20Structure :default "None"))
  (:Pressed
    (Variables|Player|Conditions|SetStrafingLeft true))
  (:Released
    (Variables|Player|Conditions|SetStrafingLeft false)))

(event Input|ActionEvents|InputActionStrafeRight
  (params (Key :type Key%20Structure :default "None"))
  (:Pressed
    (Variables|Player|Conditions|SetStrafingRight true))
  (:Released
    (Variables|Player|Conditions|SetStrafingRight false)))

(event Input|AxisEvents|InputAxisStrafe
  (params (AxisValue :type Float%20%28single-precision%29))
  (bind _strafevalue (Variables|Player|Conditions|GetStrafeValue))
  (Physics|SetPhysicsLinearVelocity (Variables|Default|GetDriverPhsysics) (Math|Vector|Lerp(Vector) "0, 0, 0" (* (* (* AxisValue (Variables|Player|Settings|Movement|GetGravityControl)) (Math|Vector|GetRightVector (Variables|Default|GetDriverPhsysics))) (Math|Float|Clamp(Float) (* (Variables|Player|Conditions|GetStrafeAmount) _strafevalue) 0.0 (Math|Conversions|ToFloat(Integer) _strafevalue))) 0.01) true "None"))

(event Custom|ShieldRecovery
  (Utilities|FlowControl|Delay 4.0)
  (if (not (Variables|Player|Conditions|GetPlayerDamaged)) :!label _label
    (if (< (Variables|Player|Settings|GetShield) 1.0)
      (Utilities|FlowControl|Delay 0.002)
      (Variables|Player|Settings|SetShield (+ (Variables|Player|Settings|GetShield) 0.004))
      (goto _label))))

(event Custom|GotHit
  (Audio|PlaySound2D "/Game/Devs/GD_Alex/Sounds/ShootingSFX/HitEnemySound/Pew01.Pew01" 1.0 1.2 0.0 0 0 false)
  (Variables|Player|Conditions|SetPlayerDamaged true)
  (bind _output_get (Variables|Player|Settings|SetShield (- (Variables|Player|Settings|GetShield) (Variables|Player|Conditions|GetDamageReceived))))
  (if (< _output_get 0.001)
    (bind _output_get_2 (Variables|Player|Settings|SetHealth (- (Variables|Player|Settings|GetHealth) (Variables|Player|Conditions|GetDamageReceived))))
    (if (< _output_get_2 0.001)
      (Actor|DestroyActor)
      (else
        (Utilities|FlowControl|Delay 0.2)
        (Variables|Player|Conditions|SetPlayerDamaged false)
        (CallFunction|ShieldRecovery)))))

(event Input|ActionEvents|InputActionSwitchCameras
  (params (Key :type Key%20Structure :default "None"))
  (bind _spectatecamera (Variables|Default|GetSpectateCamera))
  (bind _followcamera (Variables|Default|GetFollowCamera))
  (bind _playerhud_ref (Variables|Player|References|GetPlayerHUD%20ref))
  (:Pressed
    (Utilities|FlowControl|FlipFlop
      (:A
        (Components|Activation|SetActive _followcamera false false)
        (Components|Activation|SetActive _spectatecamera true false)
        (Widget|RemovefromParent _playerhud_ref)
        (Variables|Player|Conditions|SetSpectating true))
      (:B
        (Components|Activation|SetActive _followcamera true false)
        (Components|Activation|SetActive _spectatecamera false false)
        (UserInterface|Viewport|AddtoViewport _playerhud_ref 0)
        (Variables|Player|Conditions|SetSpectating false)))))

(event Input|ActionEvents|InputActionRoll
  (params (Key :type Key%20Structure :default "None"))
  (:Pressed
    (Variables|Player|Conditions|SetRolling true))
  (:Released
    (Variables|Player|Conditions|SetRolling false)))

(event Input|AxisEvents|InputAxisRoll
  (params (AxisValue :type Float%20%28single-precision%29))
  (if (Variables|Player|Conditions|GetRolling)
    (Class|PrimitiveComponent|AddTorqueinDegrees (Variables|Default|GetDriverPhsysics) (Math|Vector|Lerp(Vector) "0, 0, 0" (* (Math|Vector|GetForwardVector (Variables|Default|GetDriverPhsysics)) (* AxisValue (Variables|Player|Settings|Movement|GetGravityControl))) (Variables|Player|Settings|Movement|GetRollVelocity)) "None" true)))

(event Input|ActionEvents|InputActionSwitchWeapons
  (params (Key :type Key%20Structure :default "None"))
  (:Pressed
    (if (not (Variables|Player|Conditions|GetShooting))
      (if (Variables|Player|Conditions|GetGun1)
        (Variables|Player|Conditions|SetGun2 true)
        (Variables|Player|Conditions|SetGun1 false)
        (Audio|PlaySound2D "/Game/Devs/GD_Alex/Sounds/ShootingSFX/HitEnemySound/PewCut.PewCut" 0.5 1.1 0.1 0 0 false)
        (elif (Variables|Player|Conditions|GetGun2)
          (Variables|Player|Conditions|SetGun2 false)
          (Variables|Player|Conditions|SetGun1 true)
          (Audio|PlaySound2D "/Game/Devs/GD_Alex/Sounds/ShootingSFX/HitEnemySound/PewCut.PewCut" 0.5 0.9 0.1 0 0 false))))))

(event Input|AxisEvents|InputAxisLookUp
  (params (AxisValue :type Float%20%28single-precision%29))
  (Default|Pitch (Variables|Default|GetBP_EZDOF_Component) (* AxisValue 0.3)))

(event Input|AxisEvents|InputAxisLookRight
  (params (AxisValue :type Float%20%28single-precision%29))
  (Default|Yaw (Variables|Default|GetBP_EZDOF_Component) (* AxisValue 0.3)))

(event Input|ActionEvents|InputActionRise
  (params (Key :type Key%20Structure :default "None"))
  (:Pressed
    (Variables|Player|Conditions|SetRising true))
  (:Released
    (Variables|Player|Conditions|SetRising false)))

(event Input|ActionEvents|InputActionLower
  (params (Key :type Key%20Structure :default "None"))
  (:Pressed
    (Variables|Player|Conditions|SetLowering true))
  (:Released
    (Variables|Player|Conditions|SetLowering false)))

(event Collision|EventHit
  (params (MyComp :type Primitive%20Component%20Object%20Reference) (Other :type Actor%20Object%20Reference) (OtherComp :type Primitive%20Component%20Object%20Reference) (bSelfMoved :type Boolean) (HitLocation :type Vector :default "0, 0, 0") (HitNormal :type Vector :default "0, 0, 0") (NormalImpulse :type Vector :default "0, 0, 0") (Hit :type Hit%20Result%20Structure%20%28by%20ref%29))
  (Utilities|FlowControl|Sequence
    (:then_0
      (Utilities|FlowControl|DoOnce false :!label _label
        (:Completed
          (Variables|Player|Conditions|SetThrottleAmount 0)
          (Components|Activation|Activate (Variables|Default|GetP_Default) false)
          (bind _output_get (Variables|Player|Settings|SetHealth (- (Variables|Player|Settings|GetHealth) (Variables|Player|Settings|Combat|GetCollisionDamage))))
          (if (< _output_get 0.001)
            (Actor|DestroyActor)))))
    (:then_1
      (Utilities|FlowControl|Delay 0.5)
      (goto _label Reset))))

(event Custom|BoostRecovery
  (Utilities|FlowControl|Delay 4.0)
  (if (not (Variables|Player|Conditions|GetBoosting))
    (Variables|Player|Conditions|SetBoostAmount 0)
    (if (not (Variables|Player|Conditions|GetBoosting)) :!label _label
      (if (< (Variables|Player|Settings|GetBoost) 1.0)
        (Utilities|FlowControl|Delay 0.002)
        (Variables|Player|Settings|SetBoost (+ (Variables|Player|Settings|GetBoost) 0.004))
        (goto _label)))))

(event Input|ActionEvents|InputActionBoost
  (params (Key :type Key%20Structure :default "None"))
  (:Pressed
    (Variables|Player|Conditions|SetBoosting true)
    (Development|SetHiddeninGame (Variables|Default|GetStaticMesh6) false false)
    (Utilities|FlowControl|Sequence
      (:then_0
        (bind _output_get (Variables|Player|Settings|SetBoost (- (Variables|Player|Settings|GetBoost) 0.01) :!label _label))
        (if (> _output_get 0.0)
          (if (Variables|Player|Conditions|GetBoosting)
            (Utilities|FlowControl|Sequence
              (:then_0
                (if (< (Variables|Player|Conditions|GetBoostAmount) 100)
                  (bind _result (Math|Integer|IncrementInt (Variables|Player|Conditions|GetBoostAmount))
                    (:%20%20
                      (Variables|Player|Conditions|SetBoostAmount _result))))
                (Utilities|FlowControl|Delay (Variables|Player|Conditions|GetBoostTime))
                (goto _label))
              (:then_1
                (Utilities|FlowControl|DoOnce false :!label _label_2
                  (:Completed
                    (Audio|PlaySound2D "/Game/Devs/GD_Alex/Sounds/ShootingSFX/HitEnemySound/PewCut.PewCut" 0.5 1.0 0.0 0 0 false)))))
            (else
              (Utilities|FlowControl|DoOnce false :!label _label_3
                (:Completed
                  (Audio|PlaySound2D "/Game/Devs/GD_Alex/Sounds/ShootingSFX/HitEnemySound/PewCut.PewCut" 0.5 0.6 0.0 0 0 false)
                  (CallFunction|BoostRecovery)
                  (goto _label_2 Reset)))))
          (else
            (goto _label_3))))
      (:then_1
        (goto _label_3 Reset))))
  (:Released
    (Variables|Player|Conditions|SetBoosting false)
    (Development|SetHiddeninGame (Variables|Default|GetStaticMesh5) true false)
    (goto _label_3)))

(event Input|ActionEvents|InputActionShoot
  (params (Key :type Key%20Structure :default "None"))
  (bind _gun1location (Variables|Default|GetGun1Location))
  (bind _gun2location (Variables|Default|GetGun2Location))
  (bind _gun1class (Variables|Player|References|GetGun1Class))
  (bind _gun2class (Variables|Player|References|GetGun2Class))
  (:Pressed
    (Variables|Player|Conditions|SetShooting true)
    (if (Variables|Player|Conditions|GetGun1)
      (bind _outactors (Actor|GetAllActorsOfClass _gun1class))
      (Game|SpawnActorfromClass _gun1class (Math|Transform|MakeTransform (Transformation|GetWorldLocation _gun1location) (Transformation|GetWorldRotation _gun1location) (.scale (Transformation|GetActorTransform (Utilities|Array|Get(acopy) _outactors)))) "Undefined" "MultiplyWithRoot" 0 0 :!label _label)
      (Audio|PlaySound2D "/Game/Devs/GD_Alex/Sounds/ShootingSFX_Pitch/SFX_Laser_Big.SFX_Laser_Big" 0.25 0.9 0.0 0 0 false)
      (Utilities|FlowControl|Delay (Variables|Player|Settings|Combat|GetProjectile%201%20Cooldown))
      (if (Variables|Player|Conditions|GetShooting)
        (goto _label))
      (elif (Variables|Player|Conditions|GetGun2)
        (bind _outactors_2 (Actor|GetAllActorsOfClass _gun2class))
        (Game|SpawnActorfromClass _gun2class (Math|Transform|MakeTransform (Transformation|GetWorldLocation _gun2location) (Transformation|GetWorldRotation _gun2location) (.scale (Transformation|GetActorTransform (Utilities|Array|Get(acopy) _outactors_2)))) "Undefined" "MultiplyWithRoot" 0 0 :!label _label_2)
        (Audio|PlaySound2D "/Game/Devs/GD_Alex/Sounds/ShootingSFX_Pitch/SFX_Kinetic_Small.SFX_Kinetic_Small" 0.5 1.0 0.0 0 0 false)
        (Utilities|FlowControl|Delay (Variables|Player|Settings|Combat|GetProjectile%202%20Cooldown))
        (if (Variables|Player|Conditions|GetShooting)
          (goto _label_2)))))
  (:Released
    (Variables|Player|Conditions|SetShooting false)))

(event Input|ActionEvents|InputActionThrottleUp
  (params (Key :type Key%20Structure :default "None"))
  (:Pressed
    (Variables|Player|Conditions|SetThrottleUp true))
  (:Released
    (Variables|Player|Conditions|SetThrottleUp false)))

(event Input|ActionEvents|InputActionThrottleDown
  (params (Key :type Key%20Structure :default "None"))
  (:Pressed
    (Variables|Player|Conditions|SetThrottleDown true))
  (:Released
    (Variables|Player|Conditions|SetThrottleDown false)
    (Utilities|FlowControl|Delay 2.0)))

(event Input|ActionEvents|InputActionAim
  (params (Key :type Key%20Structure :default "None"))
  (bind _crosshair (Variables|Default|GetCrosshair))
  (bind _crosshairaim (Variables|Default|GetCrosshairAim))
  (bind _followcamera (Variables|Default|GetFollowCamera))
  (:Pressed
    (Variables|Player|Conditions|SetAiming true)
    (bind _newtrack_0 (Timeline|Timeline PlayFromStart)
      (:Update
        (Camera|SetFieldOfView _followcamera (Math|Float|Lerp 9e+01 6e+01 _newtrack_0))
        (Development|SetHiddeninGame _crosshair true false)
        (Development|SetHiddeninGame _crosshairaim false false))))
  (:Released
    (Variables|Player|Conditions|SetAiming false)
    (bind _newtrack_0_2 (Timeline|Timeline_0 PlayFromStart)
      (:Update
        (Camera|SetFieldOfView _followcamera (Math|Float|Lerp 6e+01 9e+01 _newtrack_0_2))
        (Development|SetHiddeninGame _crosshair false false)
        (Development|SetHiddeninGame _crosshairaim true false)))))

(event Input|AxisEvents|InputAxisCameraDistance
  (params (AxisValue :type Float%20%28single-precision%29))
  (bind _cameraspringarm (Variables|Default|GetCameraSpringArm))
  (if (< (Variables|/Script/Engine.SpringArmComponent|GetTargetArmLength _cameraspringarm) 1e+03)
    (if (> (Variables|/Script/Engine.SpringArmComponent|GetTargetArmLength _cameraspringarm) 4e+02)
      (Variables|/Script/Engine.SpringArmComponent|SetTargetArmLength _cameraspringarm (+ (* AxisValue 1e+01) (Variables|/Script/Engine.SpringArmComponent|GetTargetArmLength _cameraspringarm)))
      (else
        (Variables|/Script/Engine.SpringArmComponent|SetTargetArmLength _cameraspringarm 401.0)))
    (else
      (Variables|/Script/Engine.SpringArmComponent|SetTargetArmLength _cameraspringarm 999.0))))