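; World border actor whose sphere kills the single-player character if they stay outside too long.
; Leaving creates a countdown HUD widget polled every 0.2 seconds until it triggers death; re-entering fades and removes it.
; Paired DoOnce gates prevent repeat triggers.
; Overlaps also write enemy out-of-border flags, though on exit only Swarm is set true; Sniper and Bomber are set false.
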(event OnComponentBeginOverlap(SphereCollision)
  (params (OverlappedComponent :type Primitive%20Component%20Object%20Reference) (OtherActor :type Actor%20Object%20Reference) (OtherComp :type Primitive%20Component%20Object%20Reference) (OtherBodyIndex :type Integer) (bFromSweep :type Boolean) (SweepResult :type Hit%20Result%20Structure%20%28by%20ref%29))
  ;[1 1 1] Collision if Player is in Range
  (Utilities|FlowControl|Sequence
    (:then_0
      _)
    (:then_1
      (bind _asbp_enemy_swarm (Utilities|Casting|CastToBP_EnemySwarm OtherActor)
        (:then
          (Variables|/Game/Devs/PRO_Mert/BluePrints/Enemies/Actors/BP_EnemySwarm.BP_EnemySwarm_C|SetOutOufBorder _asbp_enemy_swarm false))
        (:CastFailed
          _)))
    (:then_2
      (bind _asbp_enemy_sniper (Utilities|Casting|CastToBP_EnemySniper OtherActor)
        (:then
          (Variables|/Game/Devs/PRO_Mert/BluePrints/Enemies/Actors/BP_EnemySniper.BP_EnemySniper_C|SetOutOufBorder _asbp_enemy_sniper false))
        (:CastFailed
          _)))
    (:then_3
      (bind _asbp_enemy_bomber (Utilities|Casting|CastToBP_EnemyBomber OtherActor)
        (:then
          (Variables|/Game/Devs/PRO_Mert/BluePrints/Enemies/Actors/BP_EnemyBomber.BP_EnemyBomber_C|SetOutOufBorder _asbp_enemy_bomber false))
        (:CastFailed
          _))))
  (Utilities|Casting|CastToBP_SingleplayerCharacter OtherActor)
  (Variables|Default|SetOutOfBounds false)
  (Default|FadeOut (Variables|Default|GetWorldBorder%20HUD%20REF))
  (Utilities|FlowControl|DoOnce false
    (:Completed
      (Utilities|FlowControl|Delay 0.5)
      (Widget|RemovefromParent (Variables|Default|GetWorldBorder%20HUD%20REF))
      (Default|ResetCountdown (Variables|Default|GetWorldBorder%20HUD%20REF))
      (Utilities|FlowControl|DoOnce false) ; enters at Reset
    )))

(event OnComponentEndOverlap(SphereCollision)
  (params (OverlappedComponent :type Primitive%20Component%20Object%20Reference) (OtherActor :type Actor%20Object%20Reference) (OtherComp :type Primitive%20Component%20Object%20Reference) (OtherBodyIndex :type Integer))
  ;[1 1 1] Collision if Player is in Range
  (Utilities|FlowControl|Sequence
    (:then_0
      _)
    (:then_1
      (bind _asbp_enemy_swarm (Utilities|Casting|CastToBP_EnemySwarm OtherActor)
        (:then
          (Variables|/Game/Devs/PRO_Mert/BluePrints/Enemies/Actors/BP_EnemySwarm.BP_EnemySwarm_C|SetOutOufBorder _asbp_enemy_swarm true))
        (:CastFailed
          _)))
    (:then_2
      (bind _asbp_enemy_sniper (Utilities|Casting|CastToBP_EnemySniper OtherActor)
        (:then
          (Variables|/Game/Devs/PRO_Mert/BluePrints/Enemies/Actors/BP_EnemySniper.BP_EnemySniper_C|SetOutOufBorder _asbp_enemy_sniper false))
        (:CastFailed
          _)))
    (:then_3
      (bind _asbp_enemy_bomber (Utilities|Casting|CastToBP_EnemyBomber OtherActor)
        (:then
          (Variables|/Game/Devs/PRO_Mert/BluePrints/Enemies/Actors/BP_EnemyBomber.BP_EnemyBomber_C|SetOutOufBorder _asbp_enemy_bomber false))
        (:CastFailed
          _))))
  (bind _asbp_singleplayer_character (Utilities|Casting|CastToBP_SingleplayerCharacter OtherActor))
  (if (not (Variables|/Game/Devs/PRO_Mert/BluePrints/Player/MISC/BP_SingleplayerCharacter.BP_SingleplayerCharacter_C|GetisDead _asbp_singleplayer_character))
    (Variables|Default|SetOutOfBounds true)
    (Utilities|FlowControl|DoOnce false
      (:Completed
        (CallFunction|Timer)
        (bind _returnvalue (UserInterface|CreateWidget "/Game/Devs/PRO_Alex/Blueprints/Widgets/WorldBorder_HUD.WorldBorder_HUD_C"))
        (bind _output_get (Variables|Default|SetWorldBorder%20HUD%20REF _returnvalue))
        (UserInterface|Viewport|AddtoViewport _output_get 0)
        (Utilities|FlowControl|DoOnce false) ; enters at Reset
      ))))

(event Custom|Timer
  (bind _worldborder_hud_ref (Variables|Default|GetWorldBorder%20HUD%20REF))
  ;[1 1 1] Counting Timer
  (Default|CountingtoZero _worldborder_hud_ref)
  (if (Variables|/Game/Devs/PRO_Alex/Blueprints/Widgets/WorldBorder_HUD.WorldBorder_HUD_C|GetPlayerGone _worldborder_hud_ref) :!label _label
    (CallFunction|DestroyPlayer)
    (elif (Variables|Default|GetOutOfBounds)
      (Utilities|FlowControl|Delay 0.2)
      (goto _label))))

(event Custom|DestroyPlayer
  ;[1 1 1] Kill Player
  (bind _outactors (Actor|GetAllActorsOfClass "/Game/Devs/PRO_Mert/BluePrints/Player/MISC/BP_SingleplayerCharacter.BP_SingleplayerCharacter_C"))
  (Default|PlayerDies (Utilities|Array|Get(acopy) _outactors)))

(fn ConstructionScript)