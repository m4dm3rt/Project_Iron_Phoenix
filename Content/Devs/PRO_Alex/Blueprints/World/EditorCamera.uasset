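; Pawn that serves as the orbit camera for a ship editor.
; On BeginPlay it shows the mouse cursor and adds the ShipEditor_HUD widget to the viewport.
; Holding the right mouse button turns mouse movement into controller yaw and pitch, with yaw inverted and roll reset to zero on horizontal movement.
; The mouse wheel zooms by changing the spring arm length in fixed, unclamped steps.
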(event EventBeginPlay
  ;[0.4179 0.6584 1] HUD
  (Variables|/Script/Engine.PlayerController|SetbShowMouseCursor (Game|GetPlayerController 0) true)
  (bind _returnvalue (UserInterface|CreateWidget "/Game/Devs/PRO_Alex/Blueprints/Widgets/ShipEditor_HUD.ShipEditor_HUD_C"))
  (UserInterface|Viewport|AddtoViewport _returnvalue 0))

(event Input|MouseEvents|MouseX
  (params (AxisValue :type Float%20%28single-precision%29))
  (bind _returnvalue (Pawn|GetControlRotation :!class /Script/Engine.Pawn))
  ;[0.4179 0.6584 1] Camera Rotation
  (if (Game|Player|IsInputKeyDown (Game|GetPlayerController 0) "RightMouseButton")
    (Pawn|Input|AddControllerYawInput (* AxisValue -1.0))
    (Pawn|SetControlRotation (Game|GetPlayerController 0) (Math|Rotator|MakeRotator 0.0 (.pitch _returnvalue) (.yaw _returnvalue)))))

(event Input|MouseEvents|MouseY
  (params (AxisValue :type Float%20%28single-precision%29))
  ;[0.4179 0.6584 1] Camera Rotation
  (if (Game|Player|IsInputKeyDown (Game|GetPlayerController 0) "RightMouseButton")
    (Pawn|Input|AddControllerPitchInput AxisValue)))

(event Input|MouseEvents|MouseWheelDown
  (params (Key :type Key%20Structure :default "None"))
  (bind _springarm (Variables|Default|GetSpringArm))
  ;[0.4163 0.6612 1] Camera Zoom
  (:Pressed
    (Variables|/Script/Engine.SpringArmComponent|SetTargetArmLength _springarm (- (Variables|/Script/Engine.SpringArmComponent|GetTargetArmLength _springarm) -2e+01))))

(event Input|MouseEvents|MouseWheelUp
  (params (Key :type Key%20Structure :default "None"))
  (bind _springarm (Variables|Default|GetSpringArm))
  ;[0.4163 0.6612 1] Camera Zoom
  (:Pressed
    (Variables|/Script/Engine.SpringArmComponent|SetTargetArmLength _springarm (- (Variables|/Script/Engine.SpringArmComponent|GetTargetArmLength _springarm) 2e+01))))

(fn ConstructionScript)