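; EditorCamera is the player camera for the main menu and editor mode, with mouse orbit while the right button is held.
; BeginPlay spawns the main menu widget, stores the player name in the game instance, adds an FMOD audio component and destroys any session.
; EditorMode and MenuMode switch input modes and play or reverse a timeline blending spring arm and FOV.
; MenuMode also eases control rotation back to its starting value.
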(event Custom|EditorMode
  (bind _springarm (Variables|Default|GetSpringArm))
  ;[0.4179 0.6584 1] Editor HUD
  (Input|SetInputModeGameandUI (Game|GetPlayerController 0) 0 "LockInFullscreen" true false)
  (bind _smooth (Timeline|Timeline Play)
    (:Update
      (Variables|/Script/Engine.SpringArmComponent|SetTargetArmLength _springarm (Math|Float|Lerp 2.5e+02 4e+02 _smooth))
      (Variables|/Script/Engine.SpringArmComponent|SetSocketOffset _springarm (Math|Vector|MakeVector 0.0 0.0 (Math|Float|Lerp 5e+01 1e+02 _smooth)))
      (Camera|SetFieldOfView (Variables|Default|GetCamera) (Math|Float|Lerp 1e+02 8e+01 _smooth)))))

(event Custom|MenuMode
  (bind _springarm (Variables|Default|GetSpringArm))
  ;[0.2941 0.3804 1] Menu HUD
  (Input|SetInputModeUIOnly (Game|GetPlayerController 0) 0 "LockInFullscreen" false)
  (Utilities|FlowControl|Sequence
    (:then_0
      (bind _smooth (Timeline|Timeline_0 PlayFromStart)
        (:Update
          (Pawn|SetControlRotation (Game|GetPlayerController 0) (Math|Rotator|Lerp(Rotator) (Pawn|GetControlRotation (Game|GetPlayerController 0) :!class /Script/Engine.Controller) (Variables|Default|GetStartRotation) _smooth true)))))
    (:then_1
      ;[0.4179 0.6584 1] Editor HUD
      (bind _smooth_2 (Timeline|Timeline Reverse)
        (:Update
          (Variables|/Script/Engine.SpringArmComponent|SetTargetArmLength _springarm (Math|Float|Lerp 2.5e+02 4e+02 _smooth_2))
          (Variables|/Script/Engine.SpringArmComponent|SetSocketOffset _springarm (Math|Vector|MakeVector 0.0 0.0 (Math|Float|Lerp 5e+01 1e+02 _smooth_2)))
          (Camera|SetFieldOfView (Variables|Default|GetCamera) (Math|Float|Lerp 1e+02 8e+01 _smooth_2)))))))

(event EventBeginPlay
  (bind _returnvalue (Game|GetPlayerController 0))
  ;[0.2941 0.3804 1] Begin Play
  (bind _returnvalue_2 (UserInterface|CreateWidget "/Game/Devs/PRO_Mert/BluePrints/UI/Menu/MainMenu_W.MainMenu_W_C"))
  (bind _output_get (Variables|Default|SetMainMenuWidgetRef _returnvalue_2))
  (UserInterface|Viewport|AddtoViewport _output_get 0)
  (Variables|Default|SetStartRotation (Pawn|GetControlRotation (Game|GetPlayerController 0) :!class /Script/Engine.Controller))
  (Variables|/Script/Engine.PlayerController|SetbShowMouseCursor _returnvalue true)
  (Input|SetInputModeUIOnly _returnvalue 0 "DoNotLock" false)
  (bind _asmain_game_instance (Utilities|Casting|CastToMainGameInstance (Game|GetGameInstance)))
  (Variables|/Game/Devs/PRO_Mert/BluePrints/Player/MISC/MainGameInstance.MainGameInstance_C|SetPlayerName _asmain_game_instance (Utilities|Text|ToText(String) (Class|AdvancedSessionsLibrary|GetPlayerName (Game|GetPlayerController 0))))
  (AddComponent|AddFMODAudioComponent false) ; FMOD Music Menu
  (|DestroySession (Game|GetPlayerController 0)))

(event Input|AxisEvents|InputAxisLookUp/Down
  (params (AxisValue :type Float%20%28single-precision%29))
  ;[0.4179 0.6584 1] Camera Rotation
  (if (Game|Player|IsInputKeyDown (Game|GetPlayerController 0) "RightMouseButton")
    (Pawn|Input|AddControllerPitchInput (* AxisValue -1.0))))

(event Input|AxisEvents|InputAxisLookRight/Left
  (params (AxisValue :type Float%20%28single-precision%29))
  ;[0.4179 0.6584 1] Camera Rotation
  (if (Game|Player|IsInputKeyDown (Game|GetPlayerController 0) "RightMouseButton")
    (Pawn|Input|AddControllerYawInput (* AxisValue -1.0))))

(fn ConstructionScript)