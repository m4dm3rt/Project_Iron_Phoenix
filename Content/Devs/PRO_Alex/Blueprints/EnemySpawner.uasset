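; Enemy spawner that holds a queue of enemy classes and spawns them one at a time at its own transform.
; A looping two-second timer spawns the next queued class and removes it from the queue.
; EnemyToQ appends a class and spawns immediately unless enough enemies overlap the sphere to cover the new queue index.
; Spawned enemies get a destroy-event binding, and EnemyDefeated notifies BP_ThirdPersonGameMode.
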(event Custom|TryToSpawn
  (CallFunction|SpawnEnemy))

(event Custom|EnemyDefeated
  (bind _asbp_third_person_game_mode (Utilities|Casting|CastToBP_ThirdPersonGameMode (Game|GetGameMode)))
  (Default|OnEnemyDefeated _asbp_third_person_game_mode))

(event EventBeginPlay
  (Utilities|Time|SetTimerbyEvent (delegate Custom|TryToSpawn) 2.0 true))

(fn ConstructionScript)

(fn SpawnEnemy
  (if (Utilities|Array|IsValidIndex (Variables|Default|GetEnemyQueue))
    (bind _returnvalue (Game|SpawnActorfromClass (Utilities|Array|Get(acopy) (Variables|Default|GetEnemyQueue)) (Transformation|GetActorTransform) "AdjustIfPossibleButAlwaysSpawn" "MultiplyWithRoot" 0 0))
    (EventDispatchers|BindEventtoAlexonDestroyed _returnvalue (EventDispatchers|CreateEvent :!event Custom|EnemyDefeated))
    (Utilities|Array|RemoveIndex (Variables|Default|GetEnemyQueue))
    (return true)
    (else
      (return false))))

(fn EnemytoQ
  (params (EnemyClass :type BP%20Enemy%20Character%20Class%20Reference%20%28by%20ref%29))
  (bind _returnvalue (Utilities|Array|Add (Variables|Default|GetEnemyQueue) EnemyClass))
  (if (not (Utilities|Array|IsValidIndex (Collision|GetOverlappingActors (Variables|Default|GetSphere) "/Game/Devs/PRO_Mert/BluePrints/Enemies/BP_EnemyCharacter.BP_EnemyCharacter_C" :!class /Script/Engine.PrimitiveComponent) _returnvalue))
    (CallFunction|SpawnEnemy)))