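; Enemy spawner that releases two waves of enemies, capped at five and then ten, each spawn at one of three randomly chosen location components.
; BeginPlay starts a looping spawn timer, then polls EnemyKilled with a Delay loop until it equals five and starts a second timer.
; Wave2 resets EnemyCount once; the first timer is never cleared, and EnemyKilled is not updated in this graph.
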(event Custom|Wave2
  ;[1 1 1] Wave2
  (Utilities|FlowControl|Sequence
    (:then_0
      (Utilities|FlowControl|DoOnce false
        (:Completed
          (Variables|Default|SetEnemyCount 0.0))))
    (:then_1
      ;;[1 0.04092 0.07036] MaxEnemyInWave
      (if (< (Variables|Default|GetEnemyCount) 1e+01)
        (switch int (Math|Random|RandomIntegerinRange 0 2)
          (:0
            (bind _output_get (Variables|Default|SetEnemySpawnLocation (Transformation|GetWorldLocation (Variables|Default|GetEnemySpawnLocationComponent))))
            (Game|SpawnActorfromClass (Variables|Default|GetEnemyClass) (Math|Conversions|ToTransform(Vector) _output_get) "AdjustIfPossibleButAlwaysSpawn" "MultiplyWithRoot" 0 0))
          (:1
            (bind _output_get_2 (Variables|Default|SetEnemySpawnLocation (Transformation|GetWorldLocation (Variables|Default|GetEnemySpawnLocationComponent1))))
            (Game|SpawnActorfromClass (Variables|Default|GetEnemyClass) (Math|Conversions|ToTransform(Vector) _output_get_2) "AdjustIfPossibleButAlwaysSpawn" "MultiplyWithRoot" 0 0))
          (:2
            (bind _output_get_3 (Variables|Default|SetEnemySpawnLocation (Transformation|GetWorldLocation (Variables|Default|GetEnemySpawnLocationComponent2))))
            (Game|SpawnActorfromClass (Variables|Default|GetEnemyClass) (Math|Conversions|ToTransform(Vector) _output_get_3) "AdjustIfPossibleButAlwaysSpawn" "MultiplyWithRoot" 0 0)))
        ;;[1 0.04092 0.07036] AddEnemyCount
        (Variables|Default|SetEnemyCount (+ (Variables|Default|GetEnemyCount) 1.0))))))

(event Custom|Wave1
  ;[1 1 1] Wave1
  ;;[1 0.04092 0.07036] Max Enemy In Wave
  (if (< (Variables|Default|GetEnemyCount) 5.0)
    (switch int (Math|Random|RandomIntegerinRange 0 2)
      (:0
        (bind _output_get (Variables|Default|SetEnemySpawnLocation (Transformation|GetWorldLocation (Variables|Default|GetEnemySpawnLocationComponent))))
        (Game|SpawnActorfromClass (Variables|Default|GetEnemyClass) (Math|Conversions|ToTransform(Vector) _output_get) "AdjustIfPossibleButAlwaysSpawn" "MultiplyWithRoot" 0 0))
      (:1
        (bind _output_get_2 (Variables|Default|SetEnemySpawnLocation (Transformation|GetWorldLocation (Variables|Default|GetEnemySpawnLocationComponent1))))
        (Game|SpawnActorfromClass (Variables|Default|GetEnemyClass) (Math|Conversions|ToTransform(Vector) _output_get_2) "AdjustIfPossibleButAlwaysSpawn" "MultiplyWithRoot" 0 0))
      (:2
        (bind _output_get_3 (Variables|Default|SetEnemySpawnLocation (Transformation|GetWorldLocation (Variables|Default|GetEnemySpawnLocationComponent2))))
        (Game|SpawnActorfromClass (Variables|Default|GetEnemyClass) (Math|Conversions|ToTransform(Vector) _output_get_3) "AdjustIfPossibleButAlwaysSpawn" "MultiplyWithRoot" 0 0)))
    ;;[1 0.04092 0.07036] Add Enemy To Count
    (Variables|Default|SetEnemyCount (+ (Variables|Default|GetEnemyCount) 1.0))))

(event EventBeginPlay
  ;[1 1 1] BeginPlay
  (Utilities|Time|SetTimerbyEvent (EventDispatchers|CreateEvent :!event Custom|Wave1) 3.0 true)
  (if (== (Variables|Default|GetEnemyKilled) 5.0) :!label _label
    (Utilities|Time|SetTimerbyEvent (EventDispatchers|CreateEvent :!event Custom|Wave2) 3.0 true)
    (else
      (Utilities|FlowControl|Delay 5.0)
      (goto _label))))

(fn ConstructionScript)