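; World border actor that kills the player after roughly ten seconds outside its sphere.
; Sphere overlaps toggle OutOfBounds for BP_PlayerCharacter, and each exit also adds a new WaveModeHUD widget.
; A DoOnce-gated Timer event, not called within this graph, counts BoundsTimer down through chained one-second delays.
; Re-entry resets the countdown at the next check; otherwise DestroyPlayer zeroes Health and destroys the pawn.
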(event OnComponentEndOverlap(Sphere)
  (params (OverlappedComponent :type Primitive%20Component%20Object%20Reference) (OtherActor :type Actor%20Object%20Reference) (OtherComp :type Primitive%20Component%20Object%20Reference) (OtherBodyIndex :type Integer))
  (Utilities|Casting|CastToBP_PlayerCharacter OtherActor)
  (Variables|Default|SetOutOfBounds true)
  (bind _returnvalue (UserInterface|CreateWidget "/Game/Devs/PRO_Alex/Blueprints/WaveModeHUD.WaveModeHUD_C"))
  (UserInterface|Viewport|AddtoViewport _returnvalue 0))

(event OnComponentBeginOverlap(Sphere)
  (params (OverlappedComponent :type Primitive%20Component%20Object%20Reference) (OtherActor :type Actor%20Object%20Reference) (OtherComp :type Primitive%20Component%20Object%20Reference) (OtherBodyIndex :type Integer) (bFromSweep :type Boolean) (SweepResult :type Hit%20Result%20Structure%20%28by%20ref%29))
  (Utilities|Casting|CastToBP_PlayerCharacter OtherActor)
  (Variables|Default|SetOutOfBounds false))

(event Custom|Timer
  (Utilities|FlowControl|DoOnce false :!label _label
    (:Completed
      (Utilities|FlowControl|Delay 1.0)
      (if (Variables|Default|GetOutOfBounds)
        (Variables|Default|SetBoundsTimer 9)
        (Utilities|FlowControl|Delay 1.0)
        (if (Variables|Default|GetOutOfBounds)
          (Variables|Default|SetBoundsTimer 8)
          (Utilities|FlowControl|Delay 1.0)
          (if (Variables|Default|GetOutOfBounds)
            (Variables|Default|SetBoundsTimer 7)
            (Utilities|FlowControl|Delay 1.0)
            (if (Variables|Default|GetOutOfBounds)
              (Variables|Default|SetBoundsTimer 6)
              (Utilities|FlowControl|Delay 1.0)
              (if (Variables|Default|GetOutOfBounds)
                (Variables|Default|SetBoundsTimer 5)
                (Utilities|FlowControl|Delay 1.0)
                (if (Variables|Default|GetOutOfBounds)
                  (Variables|Default|SetBoundsTimer 4)
                  (Utilities|FlowControl|Delay 1.0)
                  (if (Variables|Default|GetOutOfBounds)
                    (Variables|Default|SetBoundsTimer 3)
                    (Utilities|FlowControl|Delay 1.0)
                    (if (Variables|Default|GetOutOfBounds)
                      (Variables|Default|SetBoundsTimer 2)
                      (Utilities|FlowControl|Delay 1.0)
                      (if (Variables|Default|GetOutOfBounds)
                        (Variables|Default|SetBoundsTimer 1)
                        (Utilities|FlowControl|Delay 1.0)
                        (if (Variables|Default|GetOutOfBounds)
                          (Variables|Default|SetBoundsTimer 0)
                          (CallFunction|DestroyPlayer)
                          (else
                            (Variables|Default|SetBoundsTimer 10 :!label _label_2)
                            (goto _label Reset)))
                        (else
                          (goto _label_2)))
                      (else
                        (goto _label_2)))
                    (else
                      (goto _label_2)))
                  (else
                    (goto _label_2)))
                (else
                  (goto _label_2)))
              (else
                (goto _label_2)))
            (else
              (goto _label_2)))
          (else
            (goto _label_2)))
        (else
          (goto _label_2))))))

(event Custom|DestroyPlayer
  (bind _asbp_player_character (Utilities|Casting|CastToBP_PlayerCharacter (Game|Player|GetPlayerPawn 0)))
  (Variables|/Game/Devs/PRO_Mert/BluePrints/Player/BP_PlayerCharacter.BP_PlayerCharacter_C|SetHealth _asbp_player_character 0.0)
  (Actor|DestroyActor _asbp_player_character))

(fn ConstructionScript)