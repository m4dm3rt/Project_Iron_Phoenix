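; Player ship Blueprint that swaps visible wing, engine and body parts for ship customization.
; Each part has its own event that hides the default and alternative parts in its category, then shows itself through a DoOnce.
; Showing a part calls its siblings' Reset events to re-arm their DoOnce gates.
; Only the Butterfly and Defense wing events update selection flags; the main EventGraph and construction script are empty.
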(fn ConstructionScript)

(event Custom|Reset%20Butterfly
  ;[0.4039 0.06274 0.09412] Butterfly Wings
  (Utilities|FlowControl|DoOnce false) ; enters at Reset
)

(event Custom|Butterfly%20Wings
  ;[0.4039 0.06274 0.09412] Butterfly Wings
  (Rendering|SetVisibility (Variables|Default|GetLeftWing) false false)
  (Variables|Default|SetDefenseW%20Selected false)
  (Variables|Default|SetGunShipW%20Selected false)
  (Utilities|FlowControl|DoOnce false
    (:Completed
      (Rendering|SetVisibility (Variables|Default|GetButterflyW) true false)
      (Variables|Default|SetButterflyW%20Selected true)
      (CallFunction|ResetDefense)
      (CallFunction|ResetGunShip)
      (CallFunction|ResetHero)
      (CallFunction|ResetMegaSpeed)
      (CallFunction|ResetX-W))))

(event Custom|ResetBooster
  ;[0.4039 0.06274 0.09412] Booster Engine
  (Utilities|FlowControl|DoOnce false) ; enters at Reset
)

(event Custom|Booster%20Engine
  ;[0.4039 0.06274 0.09412] Booster Engine
  (Rendering|SetVisibility (Variables|Default|GetRectanE) false true)
  (Utilities|FlowControl|DoOnce false
    (:Completed
      (Rendering|SetVisibility (Variables|Default|GetBoosterE) true true)
      (CallFunction|ResetPower)
      (CallFunction|ResetRectan))))

(event Custom|ResetPower
  ;[0.4039 0.06274 0.09412] Power Engine
  (Utilities|FlowControl|DoOnce false) ; enters at Reset
)

(event Custom|Power%20Engine
  ;[0.4039 0.06274 0.09412] Power Engine
  (Rendering|SetVisibility (Variables|Default|GetRectanE) false true)
  (Utilities|FlowControl|DoOnce false
    (:Completed
      (Rendering|SetVisibility (Variables|Default|GetPowerE) true true)
      (CallFunction|ResetBooster)
      (CallFunction|ResetRectan))))

(event Custom|Reset%20Rectan
  ;[0.4039 0.06274 0.09412] Rectan Engine
  (Utilities|FlowControl|DoOnce false) ; enters at Reset
)

(event Custom|Rectan%20Engine
  ;[0.4039 0.06274 0.09412] Rectan Engine
  (Rendering|SetVisibility (Variables|Default|GetPowerE) false true)
  (Utilities|FlowControl|DoOnce false
    (:Completed
      (Rendering|SetVisibility (Variables|Default|GetRectanE) true true)
      (CallFunction|ResetBooster)
      (CallFunction|ResetPower))))

(event Custom|Reset%20Defense
  ;[0.4039 0.06274 0.09412] Defense Wings
  (Utilities|FlowControl|DoOnce false) ; enters at Reset
)

(event Custom|Defense%20Wings
  ;[0.4039 0.06274 0.09412] Defense Wings
  (Rendering|SetVisibility (Variables|Default|GetLeftWing) false false)
  (Variables|Default|SetButterflyW%20Selected false)
  (Variables|Default|SetGunShipW%20Selected false)
  (Utilities|FlowControl|DoOnce false
    (:Completed
      (Rendering|SetVisibility (Variables|Default|GetDefenseW) true false)
      (Variables|Default|SetDefenseW%20Selected true)
      (CallFunction|ResetButterfly)
      (CallFunction|ResetGunShip)
      (CallFunction|ResetHero)
      (CallFunction|ResetMegaSpeed)
      (CallFunction|ResetX-W))))

(event Custom|GunShip%20Wings
  ;[0.4039 0.06274 0.09412] GunShip Wings
  (Rendering|SetVisibility (Variables|Default|GetLeftWing) false false)
  (Utilities|FlowControl|DoOnce false
    (:Completed
      (Rendering|SetVisibility (Variables|Default|GetGunShipW) true false)
      (CallFunction|ResetButterfly)
      (CallFunction|ResetDefense)
      (CallFunction|ResetHero)
      (CallFunction|ResetMegaSpeed)
      (CallFunction|ResetX-W))))

(event Custom|Reset%20GunShip
  ;[0.4039 0.06274 0.09412] GunShip Wings
  (Utilities|FlowControl|DoOnce false) ; enters at Reset
)

(event Custom|Hero%20Wings
  ;[0.4039 0.06274 0.09412] Hero Wings
  (Rendering|SetVisibility (Variables|Default|GetLeftWing) false false)
  (Utilities|FlowControl|DoOnce false
    (:Completed
      (Rendering|SetVisibility (Variables|Default|GetHeroW) true false)
      (CallFunction|ResetButterfly)
      (CallFunction|ResetDefense)
      (CallFunction|ResetGunShip)
      (CallFunction|ResetMegaSpeed)
      (CallFunction|ResetX-W))))

(event Custom|Reset%20Hero
  ;[0.4039 0.06274 0.09412] Hero Wings
  (Utilities|FlowControl|DoOnce false) ; enters at Reset
)

(event Custom|Reset%20X-W
  ;[0.4039 0.06274 0.09412] X-Wings
  (Utilities|FlowControl|DoOnce false) ; enters at Reset
)

(event Custom|X-Wings
  ;[0.4039 0.06274 0.09412] X-Wings
  (Rendering|SetVisibility (Variables|Default|GetButterflyW) false false)
  (Utilities|FlowControl|DoOnce false
    (:Completed
      (Rendering|SetVisibility (Variables|Default|GetX-W) true false)
      (CallFunction|ResetButterfly)
      (CallFunction|ResetDefense)
      (CallFunction|ResetGunShip)
      (CallFunction|ResetHero)
      (CallFunction|ResetMegaSpeed))))

(event Custom|Reset%20MegaSpeed
  ;[0.4039 0.06274 0.09412] MegaSpeed Wings
  (Utilities|FlowControl|DoOnce false) ; enters at Reset
)

(event Custom|MegaSpeed%20Wings
  ;[0.4039 0.06274 0.09412] MegaSpeed Wings
  (Rendering|SetVisibility (Variables|Default|GetButterflyW) false false)
  (Utilities|FlowControl|DoOnce false
    (:Completed
      (Rendering|SetVisibility (Variables|Default|GetMegaSpeedW) true false)
      (CallFunction|ResetButterfly)
      (CallFunction|ResetDefense)
      (CallFunction|ResetGunShip)
      (CallFunction|ResetHero)
      (CallFunction|ResetX-W))))

(event Custom|ResetLightB
  ;[0.4039 0.06274 0.09412] Light Body
  (Utilities|FlowControl|DoOnce false) ; enters at Reset
)

(event Custom|Light%20Body
  ;[0.4039 0.06274 0.09412] Light Body
  (Rendering|SetVisibility (Variables|Default|GetBody) false false)
  (Utilities|FlowControl|DoOnce false
    (:Completed
      (Rendering|SetVisibility (Variables|Default|GetLightB) true false)
      (CallFunction|ResetHeavy)
      (CallFunction|ResetTankB))))

(event Custom|ResetHeavy
  ;[0.4039 0.06274 0.09412] Heavy Body
  (Utilities|FlowControl|DoOnce false) ; enters at Reset
)

(event Custom|Heavy%20Body
  ;[0.4039 0.06274 0.09412] Heavy Body
  (Rendering|SetVisibility (Variables|Default|GetBody) false false)
  (Utilities|FlowControl|DoOnce false
    (:Completed
      (Rendering|SetVisibility (Variables|Default|GetHeavyB) true false)
      (CallFunction|ResetLightB)
      (CallFunction|ResetTankB))))

(event Custom|ResetTankB
  ;[0.4039 0.06274 0.09412] Tank Body
  (Utilities|FlowControl|DoOnce false) ; enters at Reset
)

(event Custom|Tank%20Body
  ;[0.4039 0.06274 0.09412] Tank Body
  (Rendering|SetVisibility (Variables|Default|GetBody) false false)
  (Utilities|FlowControl|DoOnce false
    (:Completed
      (Rendering|SetVisibility (Variables|Default|GetTankB) true false)
      (CallFunction|ResetHeavy)
      (CallFunction|ResetLightB))))