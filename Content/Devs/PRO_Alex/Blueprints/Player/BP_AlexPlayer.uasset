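; Player flight pawn with physics-driven six-axis movement, boost, two switchable auto-fire guns, recharging shield, health and collision damage.
; Input sets flags, and looping timers ramp throttle, strafe and rise amounts that Speed blends into DriverPhsysics velocity each Tick, alongside counter-torque damping spin.
; BPEZDOFComponent handles pitch and yaw, while roll adds torque.
; Also manages the HUD, aim zoom, camera distance and spectate toggle; mouse look-at is never run.
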(event EventBeginPlay
  (|CGraphBeginPlay))

(event EventTick
  (params (DeltaSeconds :type Float%20%28single-precision%29))
  (bind _driverphsysics (Variables|Default|GetDriverPhsysics))
  (Utilities|FlowControl|Delay 0.001)
  (CallFunction|Speed)
  (Class|PrimitiveComponent|AddTorqueinDegrees _driverphsysics (/ (Math|Vector|NegateVector (Physics|GetPhysicsAngularVelocityinDegrees _driverphsysics "None")) 0.5) "None" true)
  (bind _returnvalue (Physics|GetPhysicsLinearVelocity _driverphsysics "None"))
  (Physics|SetPhysicsLinearVelocity _driverphsysics _returnvalue false "None"))

(fn ConstructionScript)

(fn Throttle
  (if (Variables|PlayerConditions|GetThrottleUp)
    (bind _result (Math|Integer|IncrementInt (Variables|PlayerConditions|GetThrottleAmount))
      (:%20%20
        (bind _result_2 (Math|Integer|IncrementInt _result)
          (:%20%20
            (Variables|PlayerConditions|SetThrottleAmount (Math|Integer|Clamp(Integer) _result_2 0 (Variables|PlayerSettings|GetThrottleMax)))
            (Development|SetHiddeninGame (Variables|Default|GetBP_VorwardVFX) false false)))))
    (else
      (Development|SetHiddeninGame (Variables|Default|GetBP_VorwardVFX) true false)
      (if (Variables|PlayerConditions|GetThrottleDown)
        (bind _result_3 (Math|Integer|DecrementInt (Variables|PlayerConditions|GetThrottleAmount))
          (:%20%20
            (bind _result_4 (Math|Integer|DecrementInt _result_3)
              (:%20%20
                (Variables|PlayerConditions|SetThrottleAmount (Math|Integer|Clamp(Integer) _result_4 0 (Variables|PlayerSettings|GetThrottleMax)))))))))))

(fn Speed
  (bind _strafevalue (Variables|PlayerSettings|GetStrafeValue))
  (bind _strafevalue_2 (Variables|PlayerSettings|GetStrafeValue))
  (bind _driverphsysics (Variables|Default|GetDriverPhsysics))
  (bind _rise_lowvalue (Variables|PlayerSettings|GetRise/LowValue))
  (bind _rise_lowvalue_2 (Variables|PlayerSettings|GetRise/LowValue))
  (bind _boostvalue (Variables|PlayerSettings|GetBoostValue))
  (bind _throttlevalue (Variables|PlayerSettings|GetThrottleValue))
  (bind _returnvalue (Physics|GetPhysicsLinearVelocity _driverphsysics "None"))
  (Physics|SetPhysicsLinearVelocity (Variables|Default|GetDriverPhsysics) (Math|Vector|Lerp(Vector) _returnvalue (* (Math|Vector|GetForwardVector _driverphsysics) (+ (Math|Float|Clamp(Float) (* (Variables|PlayerConditions|GetThrottleAmount) _throttlevalue) 0.0 (Math|Conversions|ToFloat(Integer) (* _throttlevalue 100))) (Math|Float|Clamp(Float) (* (Variables|PlayerConditions|GetBoostAmount) _boostvalue) 0.0 (Math|Conversions|ToFloat(Integer) (* _boostvalue 100))))) (Variables|PlayerSettings|GetAccelerationVelocity)) false "None")
  (Utilities|FlowControl|Sequence
    (:then_0
      (if (Variables|PlayerConditions|GetStrafingRight)
        (Physics|SetPhysicsLinearVelocity (Variables|Default|GetDriverPhsysics) (Math|Vector|Lerp(Vector) _returnvalue (* (Math|Vector|GetRightVector (Variables|Default|GetDriverPhsysics)) (Math|Float|Clamp(Float) (* (Variables|PlayerConditions|GetStrafeAmount) _strafevalue) 0.0 (Math|Conversions|ToFloat(Integer) (* _strafevalue 10)))) (Variables|PlayerSettings|GetStrafeVelocity)) false "None")))
    (:then_1
      (if (Variables|PlayerConditions|GetStrafingLeft)
        (Physics|SetPhysicsLinearVelocity (Variables|Default|GetDriverPhsysics) (Math|Vector|Lerp(Vector) _returnvalue (* (Math|Vector|GetRightVector (Variables|Default|GetDriverPhsysics)) (Math|Float|Clamp(Float) (* (Variables|PlayerConditions|GetStrafeAmount) _strafevalue_2) 0.0 (Math|Conversions|ToFloat(Integer) (* _strafevalue_2 -10)))) (Variables|PlayerSettings|GetStrafeVelocity)) false "None")))
    (:then_2
      (if (Variables|PlayerConditions|GetRising)
        (Physics|SetPhysicsLinearVelocity (Variables|Default|GetDriverPhsysics) (Math|Vector|Lerp(Vector) _returnvalue (* (Math|Vector|GetUpVector (Variables|Default|GetDriverPhsysics)) (Math|Float|Clamp(Float) (* (Variables|PlayerConditions|GetRise/LowAmount) _rise_lowvalue) 0.0 (Math|Conversions|ToFloat(Integer) (* _rise_lowvalue 100)))) (Variables|PlayerSettings|GetRise/LowerVelocity)) false "None")))
    (:then_3
      (if (Variables|PlayerConditions|GetLowering)
        (Physics|SetPhysicsLinearVelocity (Variables|Default|GetDriverPhsysics) (Math|Vector|Lerp(Vector) _returnvalue (* (Math|Vector|GetUpVector (Variables|Default|GetDriverPhsysics)) (Math|Float|Clamp(Float) (* (Variables|PlayerConditions|GetRise/LowAmount) _rise_lowvalue_2) 0.0 (Math|Conversions|ToFloat(Integer) (* _rise_lowvalue_2 -100)))) (Variables|PlayerSettings|GetRise/LowerVelocity)) false "None")))))

(fn StrafeRight
  (if (Variables|PlayerConditions|GetStrafingRight)
    (bind _result (Math|Integer|IncrementInt (Variables|PlayerConditions|GetStrafeAmount))
      (:%20%20
        (Variables|PlayerConditions|SetStrafeAmount (Math|Integer|Clamp(Integer) _result 0 (Variables|PlayerSettings|GetStrafeMax)))
        (Development|SetHiddeninGame (Variables|Default|GetPointLight3) false false)))
    (else
      (Development|SetHiddeninGame (Variables|Default|GetPointLight3) true false)
      (bind _result_2 (Math|Integer|DecrementInt (Variables|PlayerConditions|GetStrafeAmount))
        (:%20%20
          (Variables|PlayerConditions|SetStrafeAmount (Math|Integer|Clamp(Integer) _result_2 0 (Variables|PlayerSettings|GetStrafeMax))))))))

(fn StrafeLeft
  (if (Variables|PlayerConditions|GetStrafingLeft)
    (bind _result (Math|Integer|IncrementInt (Variables|PlayerConditions|GetStrafeAmount))
      (:%20%20
        (Variables|PlayerConditions|SetStrafeAmount (Math|Integer|Clamp(Integer) _result 0 (Variables|PlayerSettings|GetStrafeMax)))
        (Development|SetHiddeninGame (Variables|Default|GetPointLight4) false false)))
    (else
      (Development|SetHiddeninGame (Variables|Default|GetPointLight4) true false)
      (bind _result_2 (Math|Integer|DecrementInt (Variables|PlayerConditions|GetStrafeAmount))
        (:%20%20
          (Variables|PlayerConditions|SetStrafeAmount (Math|Integer|Clamp(Integer) _result_2 0 (Variables|PlayerSettings|GetStrafeMax))))))))

(fn Rise
  (if (Variables|PlayerConditions|GetRising)
    (bind _result (Math|Integer|IncrementInt (Variables|PlayerConditions|GetRise/LowAmount))
      (:%20%20
        (bind _result_2 (Math|Integer|IncrementInt _result)
          (:%20%20
            (bind _result_3 (Math|Integer|IncrementInt _result_2)
              (:%20%20
                (bind _result_4 (Math|Integer|IncrementInt _result_3)
                  (:%20%20
                    (Variables|PlayerConditions|SetRise/LowAmount (Math|Integer|Clamp(Integer) _result_4 0 (Variables|PlayerSettings|GetRise/LowMax)))))))))))
    (else
      (bind _result_5 (Math|Integer|DecrementInt (Variables|PlayerConditions|GetRise/LowAmount))
        (:%20%20
          (Variables|PlayerConditions|SetRise/LowAmount (Math|Integer|Clamp(Integer) _result_5 0 (Variables|PlayerSettings|GetRise/LowMax))))))))

(event Input|ActionEvents|InputActionStrafeLeft
  (params (Key :type Key%20Structure))
  (:Pressed
    (Variables|PlayerConditions|SetStrafingLeft true))
  (:Released
    (Variables|PlayerConditions|SetStrafingLeft false)))

(event Input|ActionEvents|InputActionStrafeRight
  (params (Key :type Key%20Structure))
  (:Pressed
    (Variables|PlayerConditions|SetStrafingRight true))
  (:Released
    (Variables|PlayerConditions|SetStrafingRight false)))

(event Input|AxisEvents|InputAxisStrafe
  (params (AxisValue :type Float%20%28single-precision%29))
  (bind _strafevalue (Variables|PlayerSettings|GetStrafeValue))
  (Physics|SetPhysicsLinearVelocity (Variables|Default|GetDriverPhsysics) (Math|Vector|Lerp(Vector) "0, 0, 0" (* (* (* AxisValue (Variables|PlayerSettings|GetAirControl)) (Math|Vector|GetRightVector (Variables|Default|GetDriverPhsysics))) (Math|Float|Clamp(Float) (* (Variables|PlayerConditions|GetStrafeAmount) _strafevalue) 0.0 (Math|Conversions|ToFloat(Integer) (* _strafevalue 2)))) 0.01) true "None"))

(event Custom|ShieldRecovery
  (Utilities|FlowControl|Delay 4.0)
  (if (not (Variables|PlayerConditions|GetPlayerDamaged)) :!label _label
    (if (< (Variables|PlayerSettings|GetShield) 1.0)
      (Utilities|FlowControl|Delay 0.002)
      (Variables|PlayerSettings|SetShield (+ (Variables|PlayerSettings|GetShield) 0.004))
      (goto _label))))

(event Custom|GotHit
  (Audio|PlaySound2D "/Game/Devs/GD_Alex/Sounds/ShootingSFX/HitEnemySound/Pew01.Pew01" 1.0 1.2 0.0 0 0 false)
  (Variables|PlayerConditions|SetPlayerDamaged true)
  (bind _output_get (Variables|PlayerSettings|SetShield (- (Variables|PlayerSettings|GetShield) (Variables|PlayerConditions|GetDamageReceived))))
  (if (< _output_get 0.001)
    (bind _output_get_2 (Variables|PlayerSettings|SetHealth (- (Variables|PlayerSettings|GetHealth) (Variables|PlayerConditions|GetDamageReceived))))
    (if (< _output_get_2 0.001)
      (Actor|DestroyActor)
      (else
        (Utilities|FlowControl|Delay 0.2)
        (Variables|PlayerConditions|SetPlayerDamaged false)
        (CallFunction|ShieldRecovery)))))

(event Input|ActionEvents|InputActionSwitchCameras
  (params (Key :type Key%20Structure))
  (bind _spectatecamera (Variables|Default|GetSpectateCamera))
  (bind _followcamera (Variables|Default|GetFollowCamera))
  (bind _playerhud_ref (Variables|PlayerReferences|GetPlayerHUD%20ref))
  (:Pressed
    (Utilities|FlowControl|FlipFlop
      (:A
        (Components|Activation|SetActive _followcamera false false)
        (Components|Activation|SetActive _spectatecamera true false)
        (Widget|RemovefromParent _playerhud_ref)
        (Variables|PlayerConditions|SetSpectating true))
      (:B
        (Components|Activation|SetActive _followcamera true false)
        (Components|Activation|SetActive _spectatecamera false false)
        (UserInterface|Viewport|AddtoViewport _playerhud_ref 0)
        (Variables|PlayerConditions|SetSpectating false)))))

(event Input|ActionEvents|InputActionRoll
  (params (Key :type Key%20Structure))
  (:Pressed
    (Variables|PlayerConditions|SetRolling true))
  (:Released
    (Variables|PlayerConditions|SetRolling false)))

(event Input|AxisEvents|InputAxisRoll
  (params (AxisValue :type Float%20%28single-precision%29))
  (if (Variables|PlayerConditions|GetRolling)
    (Class|PrimitiveComponent|AddTorqueinDegrees (Variables|Default|GetDriverPhsysics) (Math|Vector|Lerp(Vector) "0, 0, 0" (* (Math|Vector|GetForwardVector (Variables|Default|GetDriverPhsysics)) (* AxisValue (Variables|PlayerSettings|GetAirControl))) (Variables|PlayerSettings|GetRollVelocity)) "None" true)))

(event Input|ActionEvents|InputActionSwitchWeapons
  (params (Key :type Key%20Structure))
  (:Pressed
    (if (not (Variables|PlayerConditions|GetShooting))
      (if (Variables|PlayerConditions|GetGun1)
        (Variables|PlayerConditions|SetGun2 true)
        (Variables|PlayerConditions|SetGun1 false)
        (Audio|PlaySound2D "/Game/Devs/GD_Alex/Sounds/ShootingSFX/HitEnemySound/PewCut.PewCut" 0.5 1.1 0.1 0 0 false)
        (elif (Variables|PlayerConditions|GetGun2)
          (Variables|PlayerConditions|SetGun2 false)
          (Variables|PlayerConditions|SetGun1 true)
          (Audio|PlaySound2D "/Game/Devs/GD_Alex/Sounds/ShootingSFX/HitEnemySound/PewCut.PewCut" 0.5 0.9 0.1 0 0 false))))))

(event Input|AxisEvents|InputAxisLookUp
  (params (AxisValue :type Float%20%28single-precision%29))
  (bind _returnvalue (Transformation|GetActorRotation))
  (Default|Pitch (Variables|Default|GetBP_EZDOF_Component) (.pitch (Math|Interpolation|RInterpTo (Math|Rotator|MakeRotator 0.0 (.pitch _returnvalue) (.yaw _returnvalue)) (Math|Rotator|MakeRotator 0.0 AxisValue (stale Input|AxisEvents|InputAxisLookRight AxisValue)) 0.5 1e+01))))

(event Input|AxisEvents|InputAxisLookRight
  (params (AxisValue :type Float%20%28single-precision%29))
  (bind _returnvalue (Transformation|GetActorRotation))
  (Default|Yaw (Variables|Default|GetBP_EZDOF_Component) (.yaw (Math|Interpolation|RInterpTo (Math|Rotator|MakeRotator 0.0 (.pitch _returnvalue) (.yaw _returnvalue)) (Math|Rotator|MakeRotator 0.0 (stale Input|AxisEvents|InputAxisLookUp AxisValue) AxisValue) 0.5 1e+01))))

(event Input|ActionEvents|InputActionRise
  (params (Key :type Key%20Structure))
  (:Pressed
    (Variables|PlayerConditions|SetRising true))
  (:Released
    (Variables|PlayerConditions|SetRising false)))

(event Input|ActionEvents|InputActionLower
  (params (Key :type Key%20Structure))
  (:Pressed
    (Variables|PlayerConditions|SetLowering true))
  (:Released
    (Variables|PlayerConditions|SetLowering false)))

(event Collision|EventHit
  (params (MyComp :type Primitive%20Component%20Object%20Reference) (Other :type Actor%20Object%20Reference) (OtherComp :type Primitive%20Component%20Object%20Reference) (bSelfMoved :type Boolean) (HitLocation :type Vector :default "0, 0, 0") (HitNormal :type Vector :default "0, 0, 0") (NormalImpulse :type Vector :default "0, 0, 0") (Hit :type Hit%20Result%20Structure%20%28by%20ref%29))
  (Utilities|FlowControl|Sequence
    (:then_0
      (Utilities|FlowControl|DoOnce false :!label _label
        (:Completed
          (Variables|PlayerConditions|SetThrottleAmount 0)
          (Components|Activation|Activate (Variables|Default|GetP_Default) false)
          (bind _output_get (Variables|PlayerSettings|SetHealth (- (Variables|PlayerSettings|GetHealth) (Variables|PlayerSettings|GetCollisionDamage))))
          (if (< _output_get 0.001)
            (Actor|DestroyActor)))))
    (:then_1
      (Utilities|FlowControl|Delay 0.5)
      (goto _label Reset))))

(event Custom|BoostRecovery
  (Utilities|FlowControl|Delay 4.0)
  (if (not (Variables|PlayerConditions|GetBoosting))
    (Variables|PlayerConditions|SetBoostAmount 0)
    (if (not (Variables|PlayerConditions|GetBoosting)) :!label _label
      (if (< (Variables|PlayerSettings|GetBoost) 1.0)
        (Utilities|FlowControl|Delay 0.002)
        (Variables|PlayerSettings|SetBoost (+ (Variables|PlayerSettings|GetBoost) 0.004))
        (goto _label)))))

(event Input|ActionEvents|InputActionBoost
  (params (Key :type Key%20Structure))
  (:Pressed
    (Variables|PlayerConditions|SetBoosting true)
    (Development|SetHiddeninGame (Variables|Default|GetStaticMesh6) false false)
    (Utilities|FlowControl|Sequence
      (:then_0
        (bind _output_get (Variables|PlayerSettings|SetBoost (- (Variables|PlayerSettings|GetBoost) 0.01) :!label _label))
        (if (> _output_get 0.0)
          (if (Variables|PlayerConditions|GetBoosting)
            (Utilities|FlowControl|Sequence
              (:then_0
                (bind _result (Math|Integer|IncrementInt (Variables|PlayerConditions|GetBoostAmount))
                  (:%20%20
                    (bind _result_2 (Math|Integer|IncrementInt _result)
                      (:%20%20
                        (Variables|PlayerConditions|SetBoostAmount _result_2)
                        (Utilities|FlowControl|Delay 0.02)
                        (goto _label))))))
              (:then_1
                (Utilities|FlowControl|DoOnce false :!label _label_2
                  (:Completed
                    (Audio|PlaySound2D "/Game/Devs/GD_Alex/Sounds/ShootingSFX/HitEnemySound/PewCut.PewCut" 0.5 1.0 0.0 0 0 false)))))
            (else
              (Utilities|FlowControl|DoOnce false :!label _label_3
                (:Completed
                  (Audio|PlaySound2D "/Game/Devs/GD_Alex/Sounds/ShootingSFX/HitEnemySound/PewCut.PewCut" 0.5 0.6 0.0 0 0 false)
                  (CallFunction|BoostRecovery)
                  (goto _label_2 Reset)))))
          (else
            (goto _label_3))))
      (:then_1
        (goto _label_3 Reset))))
  (:Released
    (Variables|PlayerConditions|SetBoosting false)
    (Development|SetHiddeninGame (Variables|Default|GetStaticMesh5) true false)
    (goto _label_3)))

(event Input|ActionEvents|InputActionShoot
  (params (Key :type Key%20Structure))
  (bind _gun1location (Variables|Default|GetGun1Location))
  (bind _gun2location (Variables|Default|GetGun2Location))
  (bind _gun1class (Variables|PlayerReferences|GetGun1Class))
  (bind _gun2class (Variables|PlayerReferences|GetGun2Class))
  (:Pressed
    (Variables|PlayerConditions|SetShooting true)
    (if (Variables|PlayerConditions|GetGun1)
      (bind _outactors (Actor|GetAllActorsOfClass _gun1class))
      (Game|SpawnActorfromClass _gun1class (Math|Transform|MakeTransform (Transformation|GetWorldLocation _gun1location) (Transformation|GetWorldRotation _gun1location) (.scale (Transformation|GetActorTransform (Utilities|Array|Get(acopy) _outactors)))) "Undefined" "MultiplyWithRoot" 0 0 :!label _label)
      (Audio|PlaySound2D "/Game/Devs/GD_Alex/Sounds/ShootingSFX/Laser/LaserShoot2.LaserShoot2" 0.25 0.9 0.0 0 0 false)
      (Utilities|FlowControl|Delay (Variables|PlayerSettings|GetProjectile%201%20Cooldown))
      (if (Variables|PlayerConditions|GetShooting)
        (goto _label))
      (elif (Variables|PlayerConditions|GetGun2)
        (bind _outactors_2 (Actor|GetAllActorsOfClass _gun2class))
        (Game|SpawnActorfromClass _gun2class (Math|Transform|MakeTransform (Transformation|GetWorldLocation _gun2location) (Transformation|GetWorldRotation _gun2location) (.scale (Transformation|GetActorTransform (Utilities|Array|Get(acopy) _outactors_2)))) "Undefined" "MultiplyWithRoot" 0 0 :!label _label_2)
        (Audio|PlaySound2D "/Game/Devs/GD_Alex/Sounds/ShootingSFX/Laser/LaserShoot.LaserShoot" 0.5 1.0 0.0 0 0 false)
        (Utilities|FlowControl|Delay (Variables|PlayerSettings|GetProjectile%202%20Cooldown))
        (if (Variables|PlayerConditions|GetShooting)
          (goto _label_2)))))
  (:Released
    (Variables|PlayerConditions|SetShooting false)))

(event Input|ActionEvents|InputActionThrottleUp
  (params (Key :type Key%20Structure))
  (:Pressed
    (Variables|PlayerConditions|SetThrottleUp true))
  (:Released
    (Variables|PlayerConditions|SetThrottleUp false)))

(event Input|ActionEvents|InputActionThrottleDown
  (params (Key :type Key%20Structure))
  (:Pressed
    (Variables|PlayerConditions|SetThrottleDown true))
  (:Released
    (Variables|PlayerConditions|SetThrottleDown false)))

(event Input|ActionEvents|InputActionAim
  (params (Key :type Key%20Structure))
  (bind _crosshair (Variables|Default|GetCrosshair))
  (bind _crosshairaim (Variables|Default|GetCrosshairAim))
  (bind _followcamera (Variables|Default|GetFollowCamera))
  (:Pressed
    (bind _newtrack_0 (Timeline|Timeline PlayFromStart)
      (:Update
        (Camera|SetFieldOfView _followcamera (Math|Float|Lerp 9e+01 6e+01 _newtrack_0))
        (Development|SetHiddeninGame _crosshair true false)
        (Development|SetHiddeninGame _crosshairaim false false))))
  (:Released
    (bind _newtrack_0_2 (Timeline|Timeline_0 PlayFromStart)
      (:Update
        (Camera|SetFieldOfView _followcamera (Math|Float|Lerp 6e+01 9e+01 _newtrack_0_2))
        (Development|SetHiddeninGame _crosshair false false)
        (Development|SetHiddeninGame _crosshairaim true false)))))

(event Input|AxisEvents|InputAxisCameraDistance
  (params (AxisValue :type Float%20%28single-precision%29))
  (bind _cameraspringarm (Variables|Default|GetCameraSpringArm))
  (if (< (Variables|/Script/Engine.SpringArmComponent|GetTargetArmLength _cameraspringarm) 1e+03)
    (if (> (Variables|/Script/Engine.SpringArmComponent|GetTargetArmLength _cameraspringarm) 4e+02)
      (Variables|/Script/Engine.SpringArmComponent|SetTargetArmLength _cameraspringarm (+ (* AxisValue 1e+01) (Variables|/Script/Engine.SpringArmComponent|GetTargetArmLength _cameraspringarm)))
      (else
        (Variables|/Script/Engine.SpringArmComponent|SetTargetArmLength _cameraspringarm 401.0)))
    (else
      (Variables|/Script/Engine.SpringArmComponent|SetTargetArmLength _cameraspringarm 999.0))))