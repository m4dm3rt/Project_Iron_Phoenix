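; A laser gun projectile that damages asteroids and enemy characters on contact.
; On sphere overlap it casts the other actor to AsteroidMert, then BP_EnemyCharacter, subtracts Damage from Health and destroys itself.
; Targets whose health drops to near zero are destroyed directly by the projectile.
; An enemy kill also increments EnemyKilled on the first EnemySpawner1 found in the level.
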(event OnComponentBeginOverlap(SphereCollision)
  (params (OverlappedComponent :type Primitive%20Component%20Object%20Reference) (OtherActor :type Actor%20Object%20Reference) (OtherComp :type Primitive%20Component%20Object%20Reference) (OtherBodyIndex :type Integer) (bFromSweep :type Boolean) (SweepResult :type Hit%20Result%20Structure%20%28by%20ref%29))
  (Utilities|FlowControl|Sequence
    (:then_0
      (bind _asasteroid_mert (Utilities|Casting|CastToAsteroidMert OtherActor))
      (bind _output_get (Variables|/Game/Devs/PRO_Mert/BluePrints/Environment/AsteroidMert.AsteroidMert_C|SetHealth _asasteroid_mert (- (Variables|/Game/Devs/PRO_Mert/BluePrints/Environment/AsteroidMert.AsteroidMert_C|GetHealth _asasteroid_mert) (Variables|Default|GetDamage))))
      (Actor|DestroyActor)
      (if (< _output_get 0.01)
        (Actor|DestroyActor _asasteroid_mert)))
    (:then_1
      (bind _asbp_enemy_character (Utilities|Casting|CastToBP_EnemyCharacter OtherActor))
      (bind _output_get_2 (Variables|/Game/Devs/PRO_Mert/BluePrints/Enemies/BP_EnemyCharacter.BP_EnemyCharacter_C|SetHealth _asbp_enemy_character (- (Variables|/Game/Devs/PRO_Mert/BluePrints/Enemies/BP_EnemyCharacter.BP_EnemyCharacter_C|GetHealth _asbp_enemy_character) (Variables|Default|GetDamage))))
      (Actor|DestroyActor)
      (if (< _output_get_2 0.001)
        (Actor|DestroyActor _asbp_enemy_character)
        (bind _outactors (Actor|GetAllActorsOfClass "/Game/Devs/PRO_Alex/Blueprints/EnemySpawner1.EnemySpawner1_C"))
        (Variables|/Game/Devs/PRO_Alex/Blueprints/EnemySpawner1.EnemySpawner1_C|SetEnemyKilled (Utilities|Array|Get(acopy) _outactors) (+ (Variables|/Game/Devs/PRO_Alex/Blueprints/EnemySpawner1.EnemySpawner1_C|GetEnemyKilled (Utilities|Array|Get(acopy) _outactors)) 1.0))))))

(fn ConstructionScript)