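; Asteroid ring actor that procedurally fills a band around its origin with hierarchical instanced static meshes.
; The construction script sets mesh and cull distances, then loops over length and width to add instances, scaled by width index rather than randomly.
; AsteroidTransformation spreads them around Z, using a random stream for position jitter and blending ring-aligned with random rotations.
; Tick applies a speed-based local rotation, but its zero axis yields no visible spin.
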(event EventTick
  (params (DeltaSeconds :type Float%20%28single-precision%29))
  (Transformation|AddActorLocalRotation (Math|Vector|RotatorfromAxisandAngle "0, 0, 0" (* DeltaSeconds (Variables|Animation|GetRotationSpeed))) false false))

(fn ConstructionScript
  (bind _hierarchicalinstancedstaticspawn (Variables|Default|GetHierarchicalInstancedStaticSpawn))
  (bind _instancecountbylenght (Variables|Instances|GetInstanceCountbyLenght))
  (bind _instancecountbywidth (Variables|Instances|GetInstanceCountbyWidth))
  (Utilities|FlowControl|Sequence
    (:then_0
      (Components|StaticMesh|SetStaticMesh _hierarchicalinstancedstaticspawn (Variables|Instances|GetInstanceMesh)))
    (:then_1
      (Components|InstancedStaticMesh|SetCullDistances _hierarchicalinstancedstaticspawn (Variables|Performance|GetCullingNear) (Variables|Performance|GetCullingFar)))
    (:then_2
      (for _index (range 0 (- _instancecountbylenght 1))
        (for _index_2 (range 0 (- _instancecountbywidth 1))
          (bind (_outlocation _outrotating) (CallFunction|AsteroidTransformation _index_2 _instancecountbywidth _index _instancecountbylenght))
          (Components|InstancedStaticMesh|AddInstance (Variables|Default|GetHierarchicalInstancedStaticSpawn) (Math|Transform|MakeTransform _outlocation _outrotating (Math|Conversions|ToVector(Float) (* _index_2 (Variables|Transform|GetRandomScaleMinium)))) false))))))

(fn AsteroidTransformation
  (params (Index%20From%20Width%20Loop :type Integer) (Number%20of%20Instance%20by%20Width :type Integer) (Index%20from%20Lenght%20Loop :type Integer) (Number%20of%20Instances%20By%20Lenght :type Integer))
  (bind _returnvalue (Math|Vector|MakeVector 0.0 0.0 1.0))
  (bind _returnvalue_2 (Math|Conversions|ToFloat(Integer) Number%20of%20Instances%20By%20Lenght))
  (bind _returnvalue_3 (Math|Conversions|ToFloat(Integer) Index%20from%20Lenght%20Loop))
  (bind _returnvalue_4 (Math|Conversions|ToFloat(Integer) Index%20From%20Width%20Loop))
  (bind _returnvalue_5 (Math|Conversions|ToFloat(Integer) Number%20of%20Instance%20by%20Width))
  (bind _returnvalue_6 (Math|Float|MakeLiteralFloat 3.6e+02))
  (bind _transformrandom (Variables|Transform|GetTransformRandom))
  (bind _randomizeposition (Variables|Transform|GetRandomizePosition))
  (bind _randomizezaxisposition (Variables|Transform|GetRandomizeZAxisPosition))
  (bind _ringwidth (Variables|Instances|GetRingWidth))
  (bind _ringwidth_2 (Variables|Instances|GetRingWidth))
  (bind _ringradius (Variables|Instances|GetRingRadius))
  (bind _returnvalue_7 (Math|Random|RandomFloatfromStream _transformrandom))
  (bind _returnvalue_8 (Math|Random|RandomUnitVectorfromStream _transformrandom))
  (bind _returnvalue_9 (/ _returnvalue_4 _returnvalue_5))
  (bind _returnvalue_10 (/ _returnvalue_3 _returnvalue_2))
  (bind _returnvalue_11 (* _returnvalue_8 _randomizeposition))
  (bind _returnvalue_12 (* _returnvalue_10 _returnvalue_6))
  (bind _returnvalue_13 (- _returnvalue_7 0.5))
  (bind _returnvalue_14 (- _returnvalue_9 0.5))
  (bind _returnvalue_15 (* _returnvalue_13 _randomizezaxisposition _ringwidth))
  (bind _returnvalue_16 (* _returnvalue_14 _ringwidth_2))
  (bind _returnvalue_17 (+ _ringradius _returnvalue_16))
  (bind _returnvalue_18 (+ _returnvalue_15 _returnvalue_11))
  (bind _returnvalue_19 (Math|Vector|MakeVector 0.0 _returnvalue_17 0.0))
  (bind _returnvalue_20 (+ _returnvalue_18 _returnvalue_19))
  (bind _returnvalue_21 (Math|Vector|RotateVectorAroundAxis _returnvalue_20 _returnvalue_12 _returnvalue))
  (return _returnvalue_21 (Math|Rotator|Lerp(Rotator) (Class|KismetMathLibrary|MakeRotfromYZ (Math|Vector|CrossProduct _returnvalue _returnvalue_21) _returnvalue) (Class|KismetMathLibrary|RandomRotatorfromStream (Variables|Transform|GetTransformRandom) true) (Variables|Transform|GetRandomizeRotation) true)))