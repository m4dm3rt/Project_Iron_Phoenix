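; Black hole actor that exposes the look of its material as editable variables on the actor.
; The construction script pushes those variables into the BlackHole component's materials as scalar parameters plus a disk color vector, covering the rings, event horizon, Doppler intensity, emission and quality steps.
; The event graph holds only disabled default events, so the Blueprint runs no gameplay logic.
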(event EventBeginPlay)

(event Collision|EventActorBeginOverlap
  (params (OtherActor :type Actor%20Object%20Reference)))

(event EventTick
  (params (DeltaSeconds :type Float%20%28single-precision%29)))

(fn ConstructionScript
  (Utilities|FlowControl|Sequence
    (:then_0
      (Rendering|Material|SetScalarParameterValueonMaterials (Variables|Default|GetBlackHole) "maxrot" (Variables|Disk|GetRingRotation))
      (Rendering|Material|SetScalarParameterValueonMaterials (Variables|Default|GetBlackHole) "EmissionIntensity" (Variables|GlobalScalarParameters|GetEmissionIntensity))
      (Rendering|Material|SetScalarParameterValueonMaterials (Variables|Default|GetBlackHole) "BlackHoleSize" (Variables|GlobalSettings|GetBlackholeSize))
      (Rendering|Material|SetVectorParameterValueonMaterials (Variables|Default|GetBlackHole) "DiskColor" (Variables|Disk|GetColor)))
    (:then_1
      (Rendering|Material|SetScalarParameterValueonMaterials (Variables|Default|GetBlackHole) "RingIntensity" (Variables|Disk|GetRingIntensity))
      (Rendering|Material|SetScalarParameterValueonMaterials (Variables|Default|GetBlackHole) "iring" (Variables|GlobalScalarParameters|Getiring))
      (Rendering|Material|SetScalarParameterValueonMaterials (Variables|Default|GetBlackHole) "QualitySteps" (Variables|GlobalSettings|GetQualitySteps)))
    (:then_2
      (Rendering|Material|SetScalarParameterValueonMaterials (Variables|Default|GetBlackHole) "RingIntensityFallOff" (Variables|Disk|GetRingIntensityFallOff))
      (Rendering|Material|SetScalarParameterValueonMaterials (Variables|Default|GetBlackHole) "rfac" (Variables|GlobalScalarParameters|Getrfac))
      (Rendering|Material|SetScalarParameterValueonMaterials (Variables|Default|GetBlackHole) "DopplerIntensity" (Variables|HoleSettings|GetDopplerIntensity)))
    (:then_3
      (Rendering|Material|SetScalarParameterValueonMaterials (Variables|Default|GetBlackHole) "RingRadius" (Variables|Disk|GetRingRadius))
      (Rendering|Material|SetScalarParameterValueonMaterials (Variables|Default|GetBlackHole) "rint" (Variables|GlobalScalarParameters|Getrint))
      (Rendering|Material|SetScalarParameterValueonMaterials (Variables|Default|GetBlackHole) "EventHorizonSize" (Variables|HoleSettings|GetEventHorizonSize)))
    (:then_4
      (Rendering|Material|SetScalarParameterValueonMaterials (Variables|Default|GetBlackHole) "RingSpeed" (Variables|Disk|GetRingSpeed))
      (Rendering|Material|SetScalarParameterValueonMaterials (Variables|Default|GetBlackHole) "rrad" (Variables|GlobalScalarParameters|Getrrad)))
    (:then_5
      (Rendering|Material|SetScalarParameterValueonMaterials (Variables|Default|GetBlackHole) "TextureStrecht" (Variables|Disk|GetTextureStrecht))
      (Rendering|Material|SetScalarParameterValueonMaterials (Variables|Default|GetBlackHole) "rv" (Variables|GlobalScalarParameters|Getrv)))))