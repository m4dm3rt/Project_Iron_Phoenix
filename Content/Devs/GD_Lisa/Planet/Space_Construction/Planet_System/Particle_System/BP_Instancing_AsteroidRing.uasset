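; Asteroid ring actor that spawns an instanced mesh belt around its center and spins it about its local Z axis on Tick.
; The construction script fills HierarchicalInstanceSpawner over a length-by-width grid, setting mesh and cull distances.
; CalculateAsteroidTransformation maps grid indices onto the ring, using a random stream to jitter position and rotation, while scale grows with width index.
; An experimental per-instance spin loop is left unconnected.
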(event EventBeginPlay)

(event Collision|EventActorBeginOverlap
  (params (OtherActor :type Actor%20Object%20Reference)))

(event EventTick
  (params (DeltaSeconds :type Float%20%28single-precision%29))
  (Transformation|AddActorLocalRotation (Math|Vector|RotatorfromAxisandAngle "0, 0,1.000000" (* DeltaSeconds (Variables|Animation|GetRotationSpeed))) false false))

(fn ConstructionScript
  (bind _hierarchicalinstancespawner (Variables|Default|GetHierarchicalInstanceSpawner))
  (bind _instancecountbylength (Variables|Instances|GetInstanceCountByLength))
  (bind _instancecountbywidth (Variables|Instances|GetInstanceCountByWidth))
  (Utilities|FlowControl|Sequence
    (:then_0
      (Components|StaticMesh|SetStaticMesh _hierarchicalinstancespawner (Variables|Instances|GetInstanceMesh)) ; Set the mesh to be cloned
    )
    (:then_1
      (Components|InstancedStaticMesh|SetCullDistances _hierarchicalinstancespawner (Variables|Performance|GetCullingNear) (Variables|Performance|GetCulling%20Far)) ; Visibility distances
    )
    (:then_2
      (for _index (range 0 (- _instancecountbylength 1))
        (for _index_2 (range 0 (- _instancecountbywidth 1))
          (bind (_outlocation _outrotator) (CallFunction|CalculateAsteroidTransformation _index_2 _instancecountbywidth _index _instancecountbylength))
          (Components|InstancedStaticMesh|AddInstance (Variables|Default|GetHierarchicalInstanceSpawner) (Math|Transform|MakeTransform _outlocation _outrotator (Math|Conversions|ToVector(Float) (* _index_2 (Variables|Transform|GetRandomScaleMinimum)))) false))))))

(fn CalculateAsteroidTransformation
  (params (IndexFromWidthLoop :type Integer) (NumberOfInstancesByWidth :type Integer) (IndexFromLengthLoop :type Integer) (NumberOfInstancesByLength :type Integer))
  (bind _returnvalue (Math|Float|MakeLiteralFloat 3.6e+02))
  (bind _returnvalue_2 (Math|Conversions|ToFloat(Integer) IndexFromLengthLoop))
  (bind _returnvalue_3 (Math|Conversions|ToFloat(Integer) NumberOfInstancesByLength))
  (bind _returnvalue_4 (Math|Vector|MakeVector 0.0 0.0 1.0))
  (bind _returnvalue_5 (Math|Conversions|ToFloat(Integer) IndexFromWidthLoop))
  (bind _returnvalue_6 (Math|Conversions|ToFloat(Integer) NumberOfInstancesByWidth))
  (bind _ringradius (Variables|Instances|GetRingRadius))
  (bind _ringwidth (Variables|Instances|GetRingWidth))
  (bind _ringwidth_2 (Variables|Instances|GetRingWidth))
  (bind _transformrandom (Variables|Transform|GetTransformRandom))
  (bind _randomizeposition (Variables|Transform|GetRandomizePosition))
  (bind _randomizeupaxisposition (Variables|Transform|GetRandomizeUpAxisPosition))
  (bind _returnvalue_7 (/ _returnvalue_2 _returnvalue_3))
  (bind _returnvalue_8 (/ _returnvalue_5 _returnvalue_6))
  (bind _returnvalue_9 (Math|Random|RandomUnitVectorfromStream _transformrandom))
  (bind _returnvalue_10 (Math|Random|RandomFloatfromStream _transformrandom))
  (bind _returnvalue_11 (- _returnvalue_8 0.5))
  (bind _returnvalue_12 (* _returnvalue_9 _randomizeposition))
  (bind _returnvalue_13 (- _returnvalue_10 0.5))
  (bind _returnvalue_14 (* _returnvalue_7 _returnvalue))
  (bind _returnvalue_15 (* _returnvalue_11 _ringwidth_2))
  (bind _returnvalue_16 (* _returnvalue_13 _randomizeupaxisposition _ringwidth))
  (bind _returnvalue_17 (Math|Vector|MakeVector 0.0 0.0 _returnvalue_16))
  (bind _returnvalue_18 (+ _ringradius _returnvalue_15))
  (bind _returnvalue_19 (Math|Vector|MakeVector 0.0 _returnvalue_18 0.0))
  (bind _returnvalue_20 (+ _returnvalue_17 _returnvalue_12))
  (bind _returnvalue_21 (+ _returnvalue_20 _returnvalue_19))
  (bind _returnvalue_22 (Math|Vector|RotateVectorAroundAxis _returnvalue_21 _returnvalue_14 _returnvalue_4))
  (return _returnvalue_22 (Math|Rotator|Lerp(Rotator) (Class|KismetMathLibrary|MakeRotfromYZ (Math|Vector|CrossProduct _returnvalue_4 _returnvalue_22) _returnvalue_4) (Class|KismetMathLibrary|RandomRotatorfromStream (Variables|Transform|GetTransformRandom) true) (Variables|Transform|GetRandomizeRotation) true)))