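; Asteroid belt actor that builds a ring of instanced meshes around its local Z axis in the construction script.
; Nested length and width loops call AsteroidTransform, which spreads points around and across the ring with stream-driven position jitter and blends ring-aligned rotation toward random.
; Each instance goes to one of two HISMs by an unseeded random pick, scaled by width index times RandomScaleMin, so the first row has zero scale.
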(fn ConstructionScript
  (bind _instancecountbywidth (Variables|Instance|GetInstanceCountByWidth))
  (bind _instancecountbylength (Variables|Instance|GetInstanceCountByLength))
  (Utilities|FlowControl|Sequence
    (:then_0
      (Components|StaticMesh|SetStaticMesh (Variables|Default|GetHISM00) (Variables|Instance|GetInstanceMesh00)))
    (:then_1
      (Components|StaticMesh|SetStaticMesh (Variables|Default|GetHISM01) (Variables|Instance|GetInstanceMesh01)))
    (:then_2
      (for _index (range 0 (- _instancecountbylength 1))
        (for _index_2 (range 0 (- _instancecountbywidth 1))
          (bind (_outpos _outrot) (CallFunction|AsteroidTransform _index_2 _instancecountbywidth _index _instancecountbylength))
          (Components|InstancedStaticMesh|AddInstance (Utilities|Select :Index (Math|Random|RandomIntegerinRange 0 1) :Option%200 (Variables|Default|GetHISM00) :Option%201 (Variables|Default|GetHISM01)) (Math|Transform|MakeTransform _outpos _outrot (Math|Conversions|ToVector(Float) (* _index_2 (Variables|Transform|GetRandomScaleMin)))) false))))))

(fn AsteroidTransform
  (params (IndexFromWidthLoop :type Integer) (NumberOfInstanceByWidth :type Integer) (IndexFromLengthLoop :type Integer) (NumberOfInstanceByLength :type Integer))
  (bind _returnvalue (Math|Conversions|ToFloat(Integer) NumberOfInstanceByWidth))
  (bind _returnvalue_2 (Math|Conversions|ToFloat(Integer) IndexFromWidthLoop))
  (bind _returnvalue_3 (Math|Conversions|ToFloat(Integer) IndexFromLengthLoop))
  (bind _returnvalue_4 (Math|Conversions|ToFloat(Integer) NumberOfInstanceByLength))
  (bind _returnvalue_5 (Math|Vector|MakeVector 0.0 0.0 1.0))
  (bind _returnvalue_6 (Math|Float|MakeLiteralFloat 3.6e+02))
  (bind _ringradius (Variables|Instance|GetRingRadius))
  (bind _ringwidth (Variables|Instance|GetRingWidth))
  (bind _ringwidth_2 (Variables|Instance|GetRingWidth))
  (bind _randomisezaxispos (Variables|Transform|GetRandomiseZAxisPos))
  (bind _randomisepos (Variables|Transform|GetRandomisePos))
  (bind _transformrandom (Variables|Transform|GetTransformRandom))
  (bind _returnvalue_7 (Math|Random|RandomFloatfromStream _transformrandom))
  (bind _returnvalue_8 (Math|Random|RandomUnitVectorfromStream _transformrandom))
  (bind _returnvalue_9 (/ _returnvalue_2 _returnvalue))
  (bind _returnvalue_10 (/ _returnvalue_3 _returnvalue_4))
  (bind _returnvalue_11 (- _returnvalue_7 0.5))
  (bind _returnvalue_12 (- _returnvalue_9 0.5))
  (bind _returnvalue_13 (* _returnvalue_8 _randomisepos))
  (bind _returnvalue_14 (* _returnvalue_10 _returnvalue_6))
  (bind _returnvalue_15 (* _returnvalue_11 _randomisezaxispos _ringwidth))
  (bind _returnvalue_16 (* _returnvalue_12 _ringwidth_2))
  (bind _returnvalue_17 (+ _returnvalue_15 _returnvalue_13))
  (bind _returnvalue_18 (+ _ringradius _returnvalue_16))
  (bind _returnvalue_19 (Math|Vector|MakeVector 0.0 _returnvalue_18 0.0))
  (bind _returnvalue_20 (+ _returnvalue_17 _returnvalue_19))
  (bind _returnvalue_21 (Math|Vector|RotateVectorAroundAxis _returnvalue_20 _returnvalue_14 _returnvalue_5))
  (return _returnvalue_21 (Math|Rotator|Lerp(Rotator) (Class|KismetMathLibrary|MakeRotfromYZ (Math|Vector|CrossProduct _returnvalue_5 _returnvalue_21) _returnvalue_5) (Class|KismetMathLibrary|RandomRotatorfromStream (Variables|Transform|GetTransformRandom) true) (Variables|Transform|GetRandomiseRot) true)))