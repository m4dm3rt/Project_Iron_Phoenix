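; Flying bomber enemy that hunts the single-player character, firing projectiles on random cooldowns once in range.
; Each tick it aims at the player's velocity-predicted position, closes to attack distance, then strafes along timer-randomized axes.
; Damage drains shield before health with laser/ballistic multipliers, updating HUD bars and target widgets, with logic for shield regeneration.
; Death notifies the wave spawner, awards XP and spawns an explosion.
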(event EventBeginPlay
  ;[1 0 0 0.25 40] Initial Events
  (|CG-BeginPlay))

(event EventTick
  (params (DeltaSeconds :type Float%20%28single-precision%29))
  ;[1 0 0 0.25 40] Initial Events
  (|CG-EventTick))

(fn ConstructionScript
  (bind _hitbox_scale (Variables|Enemy|Settings|Combat|GetHitbox%20Scale))
  (bind _charactermovement (Variables|Character|GetCharacterMovement))
  (Variables|/Script/Engine.CharacterMovementComponent|SetMaxFlySpeed _charactermovement (Variables|Enemy|Settings|Movement|GetAcceleration))
  (Variables|/Script/Engine.CharacterMovementComponent|SetBrakingDecelerationFlying _charactermovement (Variables|Enemy|Settings|Movement|GetDecelaration))
  (Transformation|SetRelativeScale3D (Variables|Default|GetHitSphere) (Math|Vector|MakeVector _hitbox_scale _hitbox_scale _hitbox_scale)))

(event Custom|SetShieldHealthReticle
  (bind _player_character_ref (Variables|Enemy|References|GetPlayer%20Character%20REF))
  (bind _playerhud_ref (Variables|/Game/Devs/PRO_Mert/BluePrints/Player/MISC/BP_SingleplayerCharacter.BP_SingleplayerCharacter_C|GetPlayerHUD%20REF _player_character_ref))
  (Progress|SetPercent (Variables|/Game/Devs/PRO_Mert/BluePrints/UI/HUD/PlayerHUD_W.PlayerHUD_W_C|GetEnemy_ShieldBar _playerhud_ref) (/ (Variables|Enemy|Settings|General|GetShield) 1e+02))
  (Progress|SetPercent (Variables|/Game/Devs/PRO_Mert/BluePrints/UI/HUD/PlayerHUD_W.PlayerHUD_W_C|GetEnemy_HealthBar _playerhud_ref) (/ (Variables|Enemy|Settings|General|GetHealth) 1e+02))
  (Variables|/Game/Devs/PRO_Mert/BluePrints/UI/HUD/PlayerHUD_W.PlayerHUD_W_C|SetEnemyBomberHealth _playerhud_ref true)
  (Variables|/Game/Devs/PRO_Mert/BluePrints/UI/HUD/PlayerHUD_W.PlayerHUD_W_C|SetEnemyREF _playerhud_ref (Utilities|GetDisplayName self))
  (if (Variables|Enemy|Conditions|GetShield%20Regenerated) :!label _label
    (Variables|/Game/Devs/PRO_Mert/BluePrints/UI/HUD/PlayerHUD_W.PlayerHUD_W_C|SetEnemyBomberHealth _playerhud_ref false)
    (else
      (Utilities|FlowControl|Delay 0.2)
      (goto _label))))

(event Custom|HideHealthReticle
  (Variables|/Game/Devs/PRO_Mert/BluePrints/UI/HUD/PlayerHUD_W.PlayerHUD_W_C|SetEnemyBomberHealth (Variables|/Game/Devs/PRO_Mert/BluePrints/Player/MISC/BP_SingleplayerCharacter.BP_SingleplayerCharacter_C|GetPlayerHUD%20REF (Variables|Enemy|References|GetPlayer%20Character%20REF)) false))

(event Custom|ShootProjectile
  (bind _returnvalue (Transformation|GetActorTransform))
  (bind _enemygunclass_ref (Variables|Enemy|References|GetEnemyGunClass%20REF))
  ;[1 1 1] Get & Shoot Projectile
  (Utilities|FlowControl|Delay (Math|Random|RandomFloatinRange (Variables|Enemy|Settings|Combat|GetShot%20Cooldown%20Min) (Variables|Enemy|Settings|Combat|GetShot%20Cooldown%20Max))) ; Cooldown Time
  (bind _outactors (Actor|GetAllActorsOfClass _enemygunclass_ref))
  (Game|SpawnActorfromClass _enemygunclass_ref (Math|Transform|MakeTransform (.location _returnvalue) (.rotation _returnvalue) (.scale (Transformation|GetActorTransform (Utilities|Array|Get(acopy) _outactors)))) "Undefined" "MultiplyWithRoot" 0 0))

(event Custom|ShieldRecovery
  ;[1 1 1] Shield Regeneration
  (if (Variables|Enemy|Conditions|GetShield%20Regenerated) :!label _label
    (Variables|Enemy|Conditions|SetShield%20Regenerated true :!label _label_2)
    (if (not (< (Variables|Enemy|Settings|General|GetHealth) 1e+02))
      (Default|StopHighlight (Variables|/Game/Devs/PRO_Mert/BluePrints/Enemies/MISC/BP_IndicatorComponent.BP_IndicatorComponent_C|GetEnemyIndicator_W%20REF (Variables|Default|GetBP_IndicatorComponent)))
      (CallFunction|StopTargeting))
    (else
      (CallFunction|ShieldVisual)
      (Utilities|FlowControl|Sequence
        (:then_0
          (if (not (Variables|Enemy|Conditions|GetDamaged))
            (if (< (Variables|Enemy|Settings|General|GetShield) 1e+02)
              (Utilities|FlowControl|Delay 0.002)
              (Variables|Enemy|Settings|General|SetShield (+ (Variables|Enemy|Settings|General|GetShield) (Variables|Enemy|Settings|Combat|GetShield%20Regen%20Value)))
              (goto _label)
              (else
                (goto _label_2)))))
        (:then_1
          (if (Utilities|Enum|Equal(Enum) (Variables|/Game/Devs/PRO_Mert/BluePrints/UI/HUD/PlayerHUD_W.PlayerHUD_W_C|GetEnemyREF (Variables|/Game/Devs/PRO_Mert/BluePrints/Player/MISC/BP_SingleplayerCharacter.BP_SingleplayerCharacter_C|GetPlayerHUD%20REF (Variables|Enemy|References|GetPlayer%20Character%20REF))) (Utilities|GetDisplayName self)) ; Check if HUD Health is this Enemy
            (CallFunction|SetShieldHealthReticle)))))))

(event Custom|EnemyDeath
  (bind _returnvalue (Transformation|GetActorTransform))
  (bind _player_character_ref (Variables|Enemy|References|GetPlayer%20Character%20REF))
  ;[1 1 1] WaveSpawner count
  (bind _outactors (Actor|GetAllActorsOfClass "/Game/Devs/PRO_Alex/Blueprints/World/EnemySpawner.EnemySpawner_C"))
  (Default|EnemyKillCounter (Utilities|Array|Get(acopy) _outactors))
  ;[1 1 1] Give Player Points according to Reward
  (Variables|/Game/Devs/PRO_Mert/BluePrints/Player/MISC/BP_SingleplayerCharacter.BP_SingleplayerCharacter_C|SetReceivedXP_0 _player_character_ref (Variables|Enemy|Settings|General|GetXP%20Reward))
  ;[1 1 1] Player Points Count
  (Default|AddXP _player_character_ref)
  (Default|DestroySFX _player_character_ref)
  ;[1 1 1] Death
  (Actor|DestroyActor)
  (Game|SpawnActorfromClass "/Game/Devs/DA_Leo/Leo_BluePrints/Leo_Enemies/BP_EnemyExplosion.BP_EnemyExplosion_C" (Math|Transform|MakeTransform (.location _returnvalue) (.rotation _returnvalue) "3.000000,3.000000,3.000000") "Undefined" "MultiplyWithRoot" 0 0))

(event Custom|ShieldVisual
  (bind _widgettargetballistic (Variables|Default|GetWidgetTargetBallistic))
  (bind _widgettargetlaser (Variables|Default|GetWidgetTargetLaser))
  (if (<= (Variables|Enemy|Settings|General|GetShield) 0.0)
    (Rendering|SetVisibility _widgettargetballistic true false)
    (Rendering|SetVisibility _widgettargetlaser false false)
    (else
      (Rendering|SetVisibility _widgettargetballistic false false)
      (Rendering|SetVisibility _widgettargetlaser true false))))

(event Game|Damage|EventAnyDamage
  (params (Damage :type Float%20%28single-precision%29) (DamageType :type Damage%20Type%20Object%20Reference) (InstigatedBy :type Controller%20Object%20Reference) (DamageCauser :type Actor%20Object%20Reference))
  (bind _output_get (Variables|Enemy|References|SetDamageType DamageType))
  (bind _damagetype (Class|BaseDamage|ProccessDamage(Message) _output_get Damage))
  (if (Utilities|Enum|Equal(Enum) _damagetype "LaserBattery")
    (Components|Activation|Activate (Variables|Default|GetNS_Hit_LaserBattery) true)
    (elif (Utilities|Enum|Equal(Enum) _damagetype "LaserCutter")
      (Components|Activation|Activate (Variables|Default|GetNS_Hit_LaserCutter) true)
      (elif (Utilities|Enum|Equal(Enum) _damagetype "KineticCanon")
        (Components|Activation|Activate (Variables|Default|GetNS_Hit_KineticCanon) true)
        (elif (Utilities|Enum|Equal(Enum) _damagetype "KineticMinigun")
          (Components|Activation|Activate (Variables|Default|GetNS_Hit_KineticMinigun) true)))))
  (Variables|Enemy|Conditions|SetDamage%20Received Damage)
  (Variables|Enemy|Conditions|SetDamaged true)
  (Variables|Enemy|Conditions|SetShield%20Regenerated false)
  (bind _output_get_2 (Variables|Enemy|Settings|General|SetShield (- (Variables|Enemy|Settings|General|GetShield) (/ (Math|Float|SelectFloat (* (Variables|Enemy|Settings|Combat|GetLaser%20Damage%20Multiplier) (Variables|Enemy|Conditions|GetDamage%20Received)) (Variables|Enemy|Conditions|GetDamage%20Received) (Variables|/Game/Devs/PRO_Mert/BluePrints/Player/MISC/BP_SingleplayerCharacter.BP_SingleplayerCharacter_C|GetLaserGun (.AsBP%20Singleplayer%20Character (Utilities|Casting|CastToBP_SingleplayerCharacter (Game|Player|GetPlayerPawn 0))))) 1.8)))) ; Decrease Shield
  (CallFunction|ShieldVisual)
  (Default|HighlightEnemy (Variables|/Game/Devs/PRO_Mert/BluePrints/Enemies/MISC/BP_IndicatorComponent.BP_IndicatorComponent_C|GetEnemyIndicator_W%20REF (Variables|Default|GetBP_IndicatorComponent)))
  (if (<= _output_get_2 0.0) ; Check if Shield is active
    (bind _output_get_3 (Variables|Enemy|Settings|General|SetHealth (- (Variables|Enemy|Settings|General|GetHealth) (/ (Math|Float|SelectFloat (* (Variables|Enemy|Settings|Combat|GetBallistic%20Damage%20Multiplier) (Variables|Enemy|Conditions|GetDamage%20Received)) (Variables|Enemy|Conditions|GetDamage%20Received) (Variables|/Game/Devs/PRO_Mert/BluePrints/Player/MISC/BP_SingleplayerCharacter.BP_SingleplayerCharacter_C|GetKineticGun (.AsBP%20Singleplayer%20Character (Utilities|Casting|CastToBP_SingleplayerCharacter (Game|Player|GetPlayerPawn 0))))) 1.8)))) ; Decrease Health
    (if (<= _output_get_3 0.0)
      (CallFunction|EnemyDeath)
      (CallFunction|HideHealthReticle)
      (else
        (CallFunction|SetShieldHealthReticle :!label _label)
        (Utilities|Time|SetTimerbyEvent (EventDispatchers|CreateEvent :!event Custom|ShieldRecovery) (Variables|Enemy|Settings|Combat|GetShield%20Regen%20Delay))
        (Utilities|FlowControl|Delay 0.2)
        (Variables|Enemy|Conditions|SetDamaged false)))
    (else
      (goto _label))))

(event Custom|StrafeDirection
  (if (Math|Random|RandomBoolwithWeight 0.5)
    (bind _isa (Utilities|FlowControl|FlipFlop)
      (:A
        _)
      (:B
        _))
    (Variables|Enemy|Conditions|SetStrafeRight _isa) ; Set if Enemy strafes to Left/Right
    (else
      (bind _isa_2 (Utilities|FlowControl|FlipFlop)
        (:A
          _)
        (:B
          _))
      (Variables|Enemy|Conditions|SetStrafeUp _isa_2) ; Set if Enemy strafes Up/Down
    ))
  (Utilities|Time|SetTimerbyEvent (delegate Custom|StrafeDirection) (Math|Random|RandomFloatinRange 2.5 5.0)))

(event Custom|TargetingAid
  (bind _spacefighter (Variables|Default|GetSpaceFighter))
  (bind _widgettargetlaser (Variables|Default|GetWidgetTargetLaser))
  (bind _returnvalue (Transformation|GetWorldLocation _spacefighter))
  (bind _outhit (Collision|LineTraceByChannel _returnvalue (+ _returnvalue (* (Transformation|GetVelocity) (/ (Transformation|GetDistanceTo (Variables|Enemy|References|GetPlayer%20Character%20REF)) 6e+04))) "TraceTypeQuery1" true 0 "ForOneFrame" true "(R=0.537255,G=0.007843,B=0.000000,A=0.749020)" "(R=0.095427,G=0.000000,B=1.000000,A=0.000000)" 1.0))
  (Development|SetHiddeninGame _widgettargetlaser false false)
  (Transformation|SetWorldLocation _widgettargetlaser (.TraceEnd (Collision|BreakHitResult _outhit)) false false)
  (Utilities|Time|SetTimerbyEvent (delegate Custom|TargetingAid) 0.01 true))

(event Custom|StopTargeting
  (Development|SetHiddeninGame (Variables|Default|GetWidgetTargetLaser) true false))