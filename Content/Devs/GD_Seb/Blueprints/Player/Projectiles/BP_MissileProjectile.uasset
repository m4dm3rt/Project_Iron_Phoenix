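; BP_MissileProjectile is a gravity-free player missile that damages asteroids and enemy swarm, sniper, bomber and drone actors.
; Sphere overlap casts through those types to apply missile damage, doubled on asteroids, with crosshair hitmarker and sound for enemies only.
; Hits spawn a small explosion and destroy the missile's components rather than the actor.
; HomingProjectile re-runs itself on a short delay, steering toward the closest recorded BP_EnemySwarm, without resetting ClosestDistance.
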(event OnComponentBeginOverlap(SphereCollision)
  (params (OverlappedComponent :type Primitive%20Component%20Object%20Reference) (OtherActor :type Actor%20Object%20Reference) (OtherComp :type Primitive%20Component%20Object%20Reference) (OtherBodyIndex :type Integer) (bFromSweep :type Boolean) (SweepResult :type Hit%20Result%20Structure%20%28by%20ref%29))
  (bind _returnvalue (Transformation|GetActorTransform))
  (bind _returnvalue_2 (Transformation|GetActorTransform))
  (bind _damage (Variables|Projectile|Settings|GetDamage))
  (bind _asbp_asteroid (Utilities|Casting|CastToBP_Asteroid OtherActor)
    (:then
      (Game|Damage|ApplyDamage _asbp_asteroid (* _damage 2.0) 0 0 "/Game/Devs/PRO_Mert/BluePrints/Player/Projectiles/DamageTypes/DT_Missile.DT_Missile_C")
      (Game|SpawnActorfromClass "/Game/Devs/DA_Leo/Leo_BluePrints/Leo_Enemies/BP_EnemyExplosion.BP_EnemyExplosion_C" (Math|Transform|MakeTransform (.location _returnvalue_2) (.rotation _returnvalue_2) "0.500000,0.500000,0.500000") "Undefined" "MultiplyWithRoot" 0 0)
      (Components|DestroyComponent (Variables|Default|GetProjectileMovement)))
    (:CastFailed
      (bind _asbp_enemy_swarm (Utilities|Casting|CastToBP_EnemySwarm OtherActor)
        (:then
          (Game|Damage|ApplyDamage _asbp_enemy_swarm _damage 0 0 "/Game/Devs/PRO_Mert/BluePrints/Player/Projectiles/DamageTypes/DT_Missile.DT_Missile_C"))
        (:CastFailed
          (bind _asbp_enemy_sniper (Utilities|Casting|CastToBP_EnemySniper OtherActor)
            (:then
              (Game|Damage|ApplyDamage _asbp_enemy_sniper _damage 0 0 "/Game/Devs/PRO_Mert/BluePrints/Player/Projectiles/DamageTypes/DT_Missile.DT_Missile_C"))
            (:CastFailed
              (bind _asbp_enemy_bomber (Utilities|Casting|CastToBP_EnemyBomber OtherActor)
                (:then
                  (Game|Damage|ApplyDamage _asbp_enemy_bomber _damage 0 0 "/Game/Devs/PRO_Mert/BluePrints/Player/Projectiles/DamageTypes/DT_Missile.DT_Missile_C"))
                (:CastFailed
                  (bind _asbp_enemy_drone (Utilities|Casting|CastToBP_EnemyDrone OtherActor))
                  (Game|Damage|ApplyDamage _asbp_enemy_drone _damage 0 0 "/Game/Devs/PRO_Mert/BluePrints/Player/Projectiles/DamageTypes/DT_Missile.DT_Missile_C")))))))
      (bind _foundwidgets (Widget|GetAllWidgetsOfClass "/Game/Devs/PRO_Mert/BluePrints/UI/HUD/PlayerCrosshair_WBP.PlayerCrosshair_WBP_C" false))
      (Default|Hitmarker (Utilities|Array|Get(acopy) _foundwidgets))
      (Audio|PlaySound2D "/Game/Devs/PRO_Mert/Sounds/SFX_Hitmarker.SFX_Hitmarker" 1.0 (Math|Random|RandomFloatinRange 0.9 1.1) 0.0 0 0 false)
      (Game|SpawnActorfromClass "/Game/Devs/DA_Leo/Leo_BluePrints/Leo_Enemies/BP_EnemyExplosion.BP_EnemyExplosion_C" (Math|Transform|MakeTransform (.location _returnvalue) (.rotation _returnvalue) "0.500000,0.500000,0.500000") "Undefined" "MultiplyWithRoot" 0 0)
      (Components|DestroyComponent (Variables|Default|GetProjectileMovement)))))

(event Custom|HomingProjectile
  ;[1 0.1979 0.1979] Homing Logic
  (Variables|/Script/Engine.ProjectileMovementComponent|SetbIsHomingProjectile (Variables|Default|GetProjectileMovement) true)
  (bind _outactors (Actor|GetAllActorsOfClass "/Game/Devs/PRO_Mert/BluePrints/Enemies/Actors/BP_EnemySwarm.BP_EnemySwarm_C"))
  (for _array_element _outactors
    (if (< (Math|Vector|VectorLength (- (Transformation|GetActorLocation _array_element) (Transformation|GetActorLocation))) (Variables|Projectile|Conditions|GetClosest%20Distance))
      (Variables|Projectile|Conditions|SetClosest%20Distance (Math|Vector|VectorLength (- (Transformation|GetActorLocation _array_element) (Transformation|GetActorLocation))))
      (Variables|Projectile|References|SetTarget _array_element)))
  (Variables|/Script/Engine.ProjectileMovementComponent|SetHomingTargetComponent (Variables|Default|GetProjectileMovement) (Variables|/Game/Devs/PRO_Mert/BluePrints/Enemies/Actors/BP_EnemySwarm.BP_EnemySwarm_C|GetSpaceFighter (Variables|Projectile|References|GetTarget)))
  (Utilities|FlowControl|Delay 0.02)
  (CallFunction|HomingProjectile))

(fn ConstructionScript
  (bind _projectilemovement (Variables|Default|GetProjectileMovement))
  (bind _output_get (Variables|/Script/Engine.ProjectileMovementComponent|SetInitialSpeed _projectilemovement (Variables|Projectile|Settings|GetSpeed)))
  (Variables|/Script/Engine.ProjectileMovementComponent|SetMaxSpeed _projectilemovement _output_get)
  (Variables|/Script/Engine.ProjectileMovementComponent|SetProjectileGravityScale _projectilemovement 0.0))