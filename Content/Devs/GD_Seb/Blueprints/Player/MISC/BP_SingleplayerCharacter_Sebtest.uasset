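; Test variant of the single-player character that opens the MainEditorSeb_W editor widget over a paused game.
; Shortly after the parent BeginPlay, or when debug key B is pressed, it pauses the game and creates a new widget in the viewport.
; It then shows the mouse cursor and switches input to UI-only, focused on the widget with the mouse locked in fullscreen.
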(event EventBeginPlay
  (bind _returnvalue (Game|GetPlayerController 0))
  (|CallParentFunction)
  (Utilities|FlowControl|Delay 0.1)
  (Game|SetGamePaused true)
  (bind _returnvalue_2 (UserInterface|CreateWidget "/Game/Devs/GD_Seb/Blueprints/Player/Editor/MainEditorSeb_W.MainEditorSeb_W_C"))
  (UserInterface|Viewport|AddtoViewport _returnvalue_2 0)
  (Variables|/Script/Engine.PlayerController|SetbShowMouseCursor _returnvalue true)
  (Input|SetInputModeUIOnly _returnvalue _returnvalue_2 "LockInFullscreen" false))

(event Collision|EventActorBeginOverlap
  (params (OtherActor :type Actor%20Object%20Reference)))

(event EventTick
  (params (DeltaSeconds :type Float%20%28single-precision%29))
  (|CallParentFunction DeltaSeconds) ; This node is disabled and will not be called.\nDrag off pins to build functionality.
)

(event Input|KeyboardEvents|DebugKeyB
  (params (Key :type Key%20Structure :default "None") (ActionValue :type Input%20Action%20Value%20Structure))
  (bind _returnvalue (Game|GetPlayerController 0))
  (:Pressed
    (Game|SetGamePaused true)
    (bind _returnvalue_2 (UserInterface|CreateWidget "/Game/Devs/GD_Seb/Blueprints/Player/Editor/MainEditorSeb_W.MainEditorSeb_W_C"))
    (UserInterface|Viewport|AddtoViewport _returnvalue_2 0)
    (Variables|/Script/Engine.PlayerController|SetbShowMouseCursor _returnvalue true)
    (Input|SetInputModeUIOnly _returnvalue _returnvalue_2 "LockInFullscreen" false)))

(fn ConstructionScript
  (|CallParentFunction))