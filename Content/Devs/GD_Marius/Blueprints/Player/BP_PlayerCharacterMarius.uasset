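; Player spaceship for a space shooter, handling flight, combat, camera, HUD and game menus.
; Tick turns input axes into physics force and torque, scaled down by excess cargo weight, with speed-driven engine audio and FOV.
; BPCPlayerStats backs shield, health, boost and XP, using Delay loops for regeneration and triggering slow-motion death.
; It switches ballistic/laser guns, passing projectile speed to a swarm enemy, flags enemies via overlap targeting, and includes debug keys.
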(event EventBeginPlay
  ;[1 0 0 0.25 20] Initial Events
  (|CGraphBeginPlay))

(event EventTick
  (params (DeltaSeconds :type Float%20%28single-precision%29))
  ;[1 0 0 0.25 20] Initial Events
  (|CGraphEventTick))

(event Input|KeyboardEvents|3
  (params (Key :type Key%20Structure))
  (:Pressed
    (Default|IncreaseXP (Variables|Default|GetBPC_PlayerStats) 25.0)))

(event Input|KeyboardEvents|1
  (params (Key :type Key%20Structure))
  (bind _bpc_playerstats (Variables|Default|GetBPC_PlayerStats))
  (:Pressed
    (Utilities|FlowControl|FlipFlop
      (:A
        (Development|PrintString "GODMODE")
        (bind _recovered (Default|RegenerateShield _bpc_playerstats 1e+05 :!label _label))
        (if _recovered
          (Utilities|FlowControl|Delay 0.2)
          (goto _label)))
      (:B
        (Development|PrintString "no godmode")
        (Default|RegenerateShield _bpc_playerstats 0.0)))))

(event Input|KeyboardEvents|2
  (params (Key :type Key%20Structure))
  (bind _bpc_playerstats (Variables|Default|GetBPC_PlayerStats))
  (:Pressed
    (bind _noshield (Default|DecreaseShield _bpc_playerstats 2e+01))
    (bind _isplayerdead (Default|DecreaseHealth _bpc_playerstats _noshield 2e+01))
    (if _isplayerdead
      (CallFunction|PlayerDies))))

(fn ConstructionScript
  (bind _2ndmovementmode (Variables|Player|Movement|Get2ndMovementMode))
  (bind _minimapregistry (Variables|Default|GetMinimapRegistry))
  (bind _returnvalue (Math|Float|SelectFloat 32.0 16.0 _2ndmovementmode))
  (Variables|/Game/OpenSpaceShooter/Blueprints/Components/MinimapRegistry.MinimapRegistry_C|SetIcon _minimapregistry (Variables|Player|References|GetMapIcon%20REF))
  (Variables|/Game/OpenSpaceShooter/Blueprints/Components/MinimapRegistry.MinimapRegistry_C|SetIconSizeOverride _minimapregistry (Math|Vector2D|MakeVector2D _returnvalue _returnvalue))
  (Variables|/Game/OpenSpaceShooter/Blueprints/Components/InventoryComponent.InventoryComponent_C|SetMaxWeight (Variables|Default|GetInventoryComponent) (Variables|Backend|Conditions|GetCargoInventory)))

(fn SetVelocity
  (params (NewVelocity :type Vector))
  (Physics|SetPhysicsLinearVelocity (Variables|Default|GetSpaceFighter) NewVelocity false "None"))

(fn GetWeapons
  (for _array_element (Actor|GetAllChildActors true)
    (bind _asship_weapon (Utilities|Casting|CastToShipWeapon _array_element))
    (Utilities|Array|Add (LocalVariables|GetTempArray) _asship_weapon))
  (return (LocalVariables|GetTempArray)))

(event Custom|Shield%20Regeneration
  (Utilities|FlowControl|Delay (Variables|Player|Combat|GetShieldRecovery%20Delay))
  (if (not (Variables|Backend|Conditions|GetPlayer%20Damaged)) :!label _label
    (bind _recovered (Default|RegenerateShield (Variables|Default|GetBPC_PlayerStats) 0.4))
    (if (not _recovered)
      (Utilities|FlowControl|Delay 0.002)
      (goto _label))))

(event Custom|GotHit
  (bind _bpc_playerstats (Variables|Default|GetBPC_PlayerStats))
  (bind _damage_received (Variables|Player|Combat|GetDamage%20Received))
  (bind _returnvalue (* _damage_received 1e+02))
  (Audio|PlaySound2D "/Game/Devs/GD_Alex/Sounds/ShootingSFX/HitEnemySound/Pew01.Pew01" 1.0 1.2 0.0 0 0 false) ; Hit SFX
  (Variables|Backend|Conditions|SetPlayer%20Damaged true)
  (Default|FadeDamage (Variables|Player|References|GetDamageHUD%20REF)) ; UI Feedback
  (bind _noshield (Default|DecreaseShield _bpc_playerstats _returnvalue))
  (bind _isplayerdead (Default|DecreaseHealth _bpc_playerstats _noshield _returnvalue))
  (if _isplayerdead ; Check if Player dies or not
    (CallFunction|PlayerDies)
    (else
      (Utilities|FlowControl|Delay 0.2)
      (Variables|Backend|Conditions|SetPlayer%20Damaged false)
      (CallFunction|ShieldRegeneration))))

(event Input|ActionEvents|InputActionSwitchCameras
  (params (Key :type Key%20Structure))
  (bind _reticlewidget (Variables|Default|GetReticleWidget))
  (bind _crosshairwidget (Variables|Default|GetCrosshairWidget))
  (bind _fpscamera (Variables|Default|GetFPSCamera))
  (bind _followcamera (Variables|Default|GetFollowCamera))
  (:Pressed
    (if (Variables|Backend|Conditions|GetFPS%20Mode)
      (Components|Activation|SetActive _followcamera true false)
      (Components|Activation|SetActive _fpscamera false false)
      (Variables|Backend|Conditions|SetFPS%20Mode false)
      (Transformation|SetRelativeTransform _crosshairwidget (Math|Transform|MakeTransform "5000.000000,0.000000,125.000000" "0.000000,180.000000,0.000000" "3.000000,3.000000,3.000000") false false)
      (Transformation|SetRelativeLocation _reticlewidget "0.000000,0.000000,125.000000" false false)
      (else
        (Components|Activation|SetActive _followcamera false false)
        (Components|Activation|SetActive _fpscamera true false)
        (Variables|Backend|Conditions|SetFPS%20Mode true)
        (Transformation|SetRelativeTransform _crosshairwidget (Math|Transform|MakeTransform "5000.000000,0.000000,0.000000" "0.000000,180.000000,0.000000" "3.000000,3.000000,3.000000") false false)
        (Transformation|SetRelativeLocation _reticlewidget "0, 0, 0" false false)))))

(event Custom|Update%20Maneuver
  (params (ThrustForward :type Float%20%28double-precision%29) (ThrustRight :type Float%20%28double-precision%29) (ThrustUp :type Float%20%28double-precision%29) (TurnRoll :type Float%20%28double-precision%29) (TurnPitch :type Float%20%28double-precision%29) (TurnYaw :type Float%20%28double-precision%29))
  (Variables|Player|Movement|SetAxis%20Thrust (Math|Vector|MakeVector ThrustForward ThrustRight ThrustUp))
  (Variables|Player|Movement|SetAxis%20Turn (Math|Vector|MakeVector TurnRoll TurnPitch TurnYaw)))

(event Input|AxisEvents|InputAxisMoveForward
  (params (AxisValue :type Float%20%28single-precision%29))
  (bind _returnvalue (Input|AxisValues|GetMoveUp))
  (bind _returnvalue_2 (Input|AxisValues|GetMoveRight))
  (bind _2ndmovementmode (Variables|Player|Movement|Get2ndMovementMode))
  (bind _boost (Variables|Player|Movement|GetBoost))
  (bind _output_get (Variables|Player|Movement|SetMoveForward%20Axis AxisValue))
  (Variables|Player|Movement|SetMoveRight%20Axis _returnvalue_2)
  (Variables|Player|Movement|SetMoveUp%20Axis _returnvalue)
  (CallFunction|UpdateManeuver (* _output_get _boost) (* (Math|Float|SelectFloat 0.0 _returnvalue_2 _2ndmovementmode) _boost) (* (Math|Float|SelectFloat 0.0 _returnvalue _2ndmovementmode) _boost) 0.0 (Math|Float|SelectFloat (Input|AxisValues|GetLookUp) 0.0 _2ndmovementmode) (Math|Float|SelectFloat (Input|AxisValues|GetMoveRight) 0.0 _2ndmovementmode)))

(event Input|AxisEvents|InputAxisWeaponChange
  (params (AxisValue :type Float%20%28single-precision%29))
  (if (== AxisValue 1.0)
    (if (Variables|Backend|Conditions|GetBallistic%20Gun)
      (Audio|PlaySound2D "/Game/SettingsMenu/Demo/SoundFX/PressedSound1.PressedSound1" 0.75 1.1 0.0 0 0 false) ; Gun Switch Audio
      (Variables|Backend|Conditions|SetLaser%20Gun true)
      (Variables|Backend|Conditions|SetBallistic%20Gun false)
      ;[1 1 1] Get Weapon References
      (bind _outactors (Actor|GetAllActorsOfClass "/Game/Devs/PRO_Mert/BluePrints/Player/Projectiles/LaserProjectile.LaserProjectile_C"))
      (Variables|Player|References|SetActiveGun (Variables|Player|References|GetGun2Class))
      (bind _outactors_2 (Actor|GetAllActorsOfClass "/Game/Devs/PRO_Mert/BluePrints/Enemies/Actors/BP_EnemyCharacterSwarm.BP_EnemyCharacterSwarm_C"))
      (Variables|/Game/Devs/PRO_Mert/BluePrints/Enemies/Actors/BP_EnemyCharacterSwarm.BP_EnemyCharacterSwarm_C|SetPlayerProjectileSpeed (Utilities|Array|Get(acopy) _outactors_2) (Variables|/Game/Devs/PRO_Mert/BluePrints/Player/Projectiles/LaserProjectile.LaserProjectile_C|GetMax%20Speed (Utilities|Array|Get(acopy) _outactors)))
      (elif (Variables|Backend|Conditions|GetLaser%20Gun)
        (Audio|PlaySound2D "/Game/SettingsMenu/Demo/SoundFX/PressedSound3.PressedSound3" 0.75 0.9 0.0 0 0 false) ; Gun Switch Audio
        (Variables|Backend|Conditions|SetBallistic%20Gun true)
        (Variables|Backend|Conditions|SetLaser%20Gun false)
        (bind _outactors_3 (Actor|GetAllActorsOfClass "/Game/Devs/PRO_Mert/BluePrints/Player/Projectiles/BallisticProjectile.BallisticProjectile_C"))
        (Variables|Player|References|SetActiveGun (Variables|Player|References|GetGun1Class))
        (bind _outactors_4 (Actor|GetAllActorsOfClass "/Game/Devs/PRO_Mert/BluePrints/Enemies/Actors/BP_EnemyCharacterSwarm.BP_EnemyCharacterSwarm_C"))
        (Variables|/Game/Devs/PRO_Mert/BluePrints/Enemies/Actors/BP_EnemyCharacterSwarm.BP_EnemyCharacterSwarm_C|SetPlayerProjectileSpeed (Utilities|Array|Get(acopy) _outactors_4) (Variables|/Game/Devs/PRO_Mert/BluePrints/Player/Projectiles/BallisticProjectile.BallisticProjectile_C|GetInitial%20Speed (Utilities|Array|Get(acopy) _outactors_3)))))))

(event Input|ActionEvents|InputActionInteract
  (params (Key :type Key%20Structure))
  (:Pressed
    (bind _array_element (Utilities|Array|ForEachLoopwithBreak (Collision|GetOverlappingActors "/Script/Engine.Actor" :!class /Script/Engine.Actor) :!label _label)
      (:LoopBody
        (if (Utilities|DoesObjectImplementInterface _array_element "/Game/Devs/PRO_Mert/BluePrints/Player/Interfaces/Interact.Interact_C")
          (Class|Interact|Interact(Message) _array_element)
          (goto _label Break))))))

(event Collision|EventHit
  (params (MyComp :type Primitive%20Component%20Object%20Reference) (Other :type Actor%20Object%20Reference) (OtherComp :type Primitive%20Component%20Object%20Reference) (bSelfMoved :type Boolean) (HitLocation :type Vector :default "0, 0, 0") (HitNormal :type Vector :default "0, 0, 0") (NormalImpulse :type Vector :default "0, 0, 0") (Hit :type Hit%20Result%20Structure%20%28by%20ref%29))
  (Utilities|FlowControl|Sequence
    (:then_0
      (Utilities|FlowControl|DoOnce false :!label _label
        (:Completed
          (Components|Activation|Activate (Variables|Default|GetP_Default) false) ; Call Hit VFX
          (bind _isplayerdead (Default|DecreaseHealth (Variables|Default|GetBPC_PlayerStats) true (Variables|Player|Combat|GetCollision%20Damage)))
          (if _isplayerdead
            (CallFunction|PlayerDies)))))
    (:then_1
      (Utilities|FlowControl|Delay 0.5)
      (goto _label Reset))))

(event Custom|StopBoost
  (bind _bpc_playerstats (Variables|Default|GetBPC_PlayerStats))
  (Variables|Backend|Conditions|SetBoosting false)
  (Variables|Player|Movement|SetBoost 1.0)
  (Utilities|FlowControl|Delay (Variables|Player|Movement|GetBoostRecovery%20Delay))
  (if (not (Variables|Backend|Conditions|GetBoosting)) :!label _label
    (if (not (== (Variables|/Game/Devs/PRO_Mert/BluePrints/Player/BPComponents/BPC_PlayerStats.BPC_PlayerStats_C|GetBoost _bpc_playerstats) (Variables|/Game/Devs/PRO_Mert/BluePrints/Player/BPComponents/BPC_PlayerStats.BPC_PlayerStats_C|GetMax%20Boost _bpc_playerstats)))
      (Default|RegenerateBoost _bpc_playerstats 1.0)
      (Utilities|FlowControl|Delay 0.05)
      (Utilities|FlowControl|Sequence
        (:then_0
          (goto _label))))))

(event Input|ActionEvents|InputActionBoost
  (params (Key :type Key%20Structure))
  (bind _bpc_playerstats (Variables|Default|GetBPC_PlayerStats))
  (:Pressed
    (if (> (Variables|/Game/Devs/PRO_Mert/BluePrints/Player/BPComponents/BPC_PlayerStats.BPC_PlayerStats_C|GetBoost (Variables|Default|GetBPC_PlayerStats)) 0.0)
      (Variables|Backend|Conditions|SetBoosting true)
      (Variables|Player|Movement|SetBoost (* (Variables|Player|Movement|GetBoost) (Variables|Player|Movement|GetBoost%20Velocity)))
      (bind _stamina_depleted (Default|DecreaseBoost _bpc_playerstats 1.0 :!label _label))
      (if _stamina_depleted
        (CallFunction|StopBoost)
        (elif (Variables|Backend|Conditions|GetBoosting)
          (if (not (== (Variables|/Game/Devs/PRO_Mert/BluePrints/Player/BPComponents/BPC_PlayerStats.BPC_PlayerStats_C|GetBoost _bpc_playerstats) (Variables|/Game/Devs/PRO_Mert/BluePrints/Player/BPComponents/BPC_PlayerStats.BPC_PlayerStats_C|GetMax%20Boost _bpc_playerstats)))
            (Utilities|FlowControl|Delay 0.05)
            (goto _label))))))
  (:Released
    (Variables|Backend|Conditions|SetBoosting false)
    (Variables|Player|Movement|SetBoost 1.0)
    (Utilities|FlowControl|Delay (Variables|Player|Movement|GetBoostRecovery%20Delay))
    (if (not (Variables|Backend|Conditions|GetBoosting)) :!label _label_2
      (if (not (== (Variables|/Game/Devs/PRO_Mert/BluePrints/Player/BPComponents/BPC_PlayerStats.BPC_PlayerStats_C|GetBoost _bpc_playerstats) (Variables|/Game/Devs/PRO_Mert/BluePrints/Player/BPComponents/BPC_PlayerStats.BPC_PlayerStats_C|GetMax%20Boost _bpc_playerstats)))
        (Default|RegenerateBoost _bpc_playerstats 1.0)
        (Utilities|FlowControl|Delay 0.05)
        (Utilities|FlowControl|Sequence
          (:then_0
            (goto _label_2)))))))

(event Custom|PlayerDies
  (bind _returnvalue (Game|GetPlayerController 0))
  (bind _spacefighter (Variables|Default|GetSpaceFighter))
  (Variables|Backend|Conditions|SetPlayer%20Death true)
  (Development|SetHiddeninGame _spacefighter true true)
  (Collision|SetCollisionEnabled _spacefighter "NoCollision")
  (Effects|SpawnEmitteratLocation "/Game/Realistic_Starter_VFX_Pack_Vol2/Particles/Explosion/P_Explosion_Big_A.P_Explosion_Big_A" (Transformation|GetActorLocation) "0, 0, 0" "2.500000,2.500000,2.500000") ; Call Explosion VFX
  (Audio|PlaySound2D "/Game/Devs/GD_Alex/Sounds/ShootingSFX/HitEnemySound/Pew01.Pew01" 1.5 1.2 0.0 0 0 false)
  (bind _returnvalue_2 (UserInterface|CreateWidget "/Game/Devs/PRO_Mert/BluePrints/Player/Widgets/PlayerDeath_W.PlayerDeath_W_C"))
  (UserInterface|Viewport|AddtoViewport _returnvalue_2 0)
  (bind _time (Timeline|Timeline PlayFromStart)
    (:Update
      (Utilities|Time|SetGlobalTimeDilation _time)
      (Input|DisableInput _returnvalue)
      (if (or (Game|Player|IsInputKeyDown _returnvalue "P") (Game|Player|IsInputKeyDown _returnvalue "Escape")) :!label _label
        (CallFunction|PauseGame)
        (else
          (Utilities|FlowControl|Delay 0.001)
          (goto _label))))))

(event Custom|PauseGame
  (bind _returnvalue (Game|GetPlayerController 0))
  (if (Variables|Backend|Conditions|GetPlayer%20Death)
    (Utilities|FlowControl|DoOnce false
      (:Completed
        (bind _returnvalue_2 (UserInterface|CreateWidget "/Game/SettingsMenu/Widgets/FinishedMenu_W.FinishedMenu_W_C"))
        (UserInterface|Viewport|AddtoViewport _returnvalue_2 0)
        (Input|SetInputModeUIOnly _returnvalue _returnvalue_2 "LockInFullscreen" false)))
    (else
      (bind _returnvalue_3 (UserInterface|CreateWidget "/Game/SettingsMenu/Widgets/PauseMenu_W.PauseMenu_W_C"))
      (UserInterface|Viewport|AddtoViewport _returnvalue_3 0)
      (Input|SetInputModeUIOnly _returnvalue _returnvalue_3 "LockInFullscreen" false)))
  (Variables|/Script/Engine.PlayerController|SetbShowMouseCursor _returnvalue true)
  (Game|SetGamePaused true))

(event Input|ActionEvents|InputActionPauseMenu
  (params (Key :type Key%20Structure))
  (:Pressed
    (CallFunction|PauseGame)))

(event Input|ActionEvents|InputActionShoot
  (params (Key :type Key%20Structure))
  (bind _gun1location (Variables|Default|GetGun1Location))
  (bind _activegun (Variables|Player|References|GetActiveGun))
  (:Pressed
    (Variables|Backend|Conditions|SetShooting true)
    ;[1 1 1] Get Projectile Stats & Shoot
    (if (not (Variables|Backend|Conditions|GetProjectile%20Shot))
      (Variables|Backend|Conditions|SetProjectile%20Shot true)
      (bind _outactors (Actor|GetAllActorsOfClass _activegun))
      (Game|SpawnActorfromClass _activegun (Math|Transform|MakeTransform (Transformation|GetWorldLocation _gun1location) (Transformation|GetWorldRotation _gun1location) (.scale (Transformation|GetActorTransform (Utilities|Array|Get(acopy) _outactors)))) "Undefined" "MultiplyWithRoot" 0 0 :!label _label)
      ;[1 1 1] Shooting Camera Shake
      (Camera|PlayWorldCameraShake "/Game/Devs/PRO_Mert/BluePrints/Player/CameraShakes/CS_Shooting.CS_Shooting_C" (Transformation|GetWorldLocation (Variables|Default|GetFollowCamera)) 0.0 1.0)
      (if (Variables|Backend|Conditions|GetBallistic%20Gun)
        (Audio|PlaySound2D "/Game/Devs/GD_Alex/Sounds/ShootingSFX_Pitch/SFX_Laser_Big.SFX_Laser_Big" 0.25 0.9 0.0 0 0 false) ; Shooting Audio
        (Utilities|FlowControl|Delay (Variables|Player|Combat|GetBallistic%20Cooldown)) ; Cooldown Time
        (if (Variables|Backend|Conditions|GetShooting) :!label _label_2
          (if (Variables|Backend|Conditions|GetProjectile%20Shot)
            (goto _label))
          (else
            ;[1 1 1] Stop Shooting - BugFix so triggering is not faster
            (Utilities|FlowControl|Delay 0.2)
            (Variables|Backend|Conditions|SetProjectile%20Shot false)))
        (elif (Variables|Backend|Conditions|GetLaser%20Gun)
          (Audio|PlaySound2D "/Game/Devs/GD_Alex/Sounds/ShootingSFX_Pitch/SFX_Kinetic_Small.SFX_Kinetic_Small" 0.25 1.0 0.0 0 0 false) ; Shooting Audio
          (Utilities|FlowControl|Delay (Variables|Player|Combat|GetLaser%20Cooldown)) ; Cooldown Time
          (goto _label_2)))))
  (:Released
    (Variables|Backend|Conditions|SetShooting false)))

(event Input|AxisEvents|InputAxisLookUp
  (params (AxisValue :type Float%20%28single-precision%29))
  (bind _returnvalue (Viewport|GetViewportSize))
  (bind _returnvalue_2 (Class|WidgetLayoutLibrary|GetViewportScale))
  (bind _returnvalue_3 (/ (.y _returnvalue) _returnvalue_2))
  (bind _returnvalue_4 (/ _returnvalue_3 2.0))
  (if (not (Game|IsGamePaused))
    (bind _returnvalue_5 (Class|WidgetLayoutLibrary|GetMousePositiononViewport))
    (Default|Pitch (Variables|Default|GetBP_EZDOF_Component) (/ (- (.y _returnvalue_5) _returnvalue_4) _returnvalue_4))))

(event Input|AxisEvents|InputAxisLookRight
  (params (AxisValue :type Float%20%28single-precision%29))
  (bind _returnvalue (Viewport|GetViewportSize))
  (bind _returnvalue_2 (Class|WidgetLayoutLibrary|GetViewportScale))
  (bind _returnvalue_3 (/ (.x _returnvalue) _returnvalue_2))
  (bind _returnvalue_4 (/ _returnvalue_3 2.0))
  (if (not (Game|IsGamePaused))
    (bind _returnvalue_5 (Class|WidgetLayoutLibrary|GetMousePositiononViewport))
    (Default|Yaw (Variables|Default|GetBP_EZDOF_Component) (/ (- (.x _returnvalue_5) _returnvalue_4) _returnvalue_4))))

(event Custom|Add%20XP
  (Default|IncreaseXP (Variables|Default|GetBPC_PlayerStats) (Variables|Backend|Conditions|GetReceived%20XP)))

(event OnComponentEndOverlap(TargetingMesh)
  (params (OverlappedComponent :type Primitive%20Component%20Object%20Reference) (OtherActor :type Actor%20Object%20Reference) (OtherComp :type Primitive%20Component%20Object%20Reference) (OtherBodyIndex :type Integer))
  (if (Variables|Backend|Conditions|GetTargeting)
    (Utilities|FlowControl|Sequence :!label _label
      (:then_0
        (Utilities|Casting|CastToBP_EnemyCharacterSwarm OtherActor))
      (:then_1
        (Utilities|Casting|CastToBP_EnemyCharacterSniper OtherActor)))
    (Variables|Backend|Conditions|SetTarget%20Found false)
    (Utilities|FlowControl|DoOnce false :!label _label_2
      (:Completed
        (CallFunction|TargetingEnemies)
        (Utilities|FlowControl|Delay 0.2)
        (goto _label_2 Reset)))
    (elif (Variables|Backend|Conditions|GetTarget%20Found)
      (goto _label))))

(event OnComponentBeginOverlap(TargetingMesh)
  (params (OverlappedComponent :type Primitive%20Component%20Object%20Reference) (OtherActor :type Actor%20Object%20Reference) (OtherComp :type Primitive%20Component%20Object%20Reference) (OtherBodyIndex :type Integer) (bFromSweep :type Boolean) (SweepResult :type Hit%20Result%20Structure%20%28by%20ref%29))
  (if (Variables|Backend|Conditions|GetTargeting) :!label _label
    (Utilities|FlowControl|Sequence
      (:then_0
        (bind _asbp_enemy_character_swarm (Utilities|Casting|CastToBP_EnemyCharacterSwarm OtherActor))
        (Default|TargetingAid _asbp_enemy_character_swarm))
      (:then_1
        (bind _asbp_enemy_character_sniper (Utilities|Casting|CastToBP_EnemyCharacterSniper OtherActor))
        (Default|TargetingAid _asbp_enemy_character_sniper)))
    (Variables|Backend|Conditions|SetTarget%20Found true)
    (else
      (Utilities|FlowControl|Delay 0.2)
      (goto _label))))

(event Custom|TargetingEnemies
  (Variables|Backend|Conditions|SetTargeting true)
  (if (Variables|Backend|Conditions|GetTarget%20Found) :!label _label
    (Audio|PlaySound2D "/Game/Devs/GD_Alex/Sounds/ShootingSFX/HitEnemySound/Pew01.Pew01" 1.0 2.0 0.0 0 0 false)
    (elif (Variables|Backend|Conditions|GetTargeting)
      (Audio|PlaySound2D "/Game/Devs/GD_Alex/Sounds/ShootingSFX/HitEnemySound/Pew01.Pew01" 0.5 1.0 0.0 0 0 false)
      (Utilities|FlowControl|Delay 0.1)
      (goto _label))))

(event Input|ActionEvents|InputActionTargetSystem
  (params (Key :type Key%20Structure))
  (:Pressed
    (if (Variables|Backend|Conditions|GetTargeting)
      (Variables|Backend|Conditions|SetTargeting false)
      (Variables|Backend|Conditions|SetTarget%20Found false)
      (else
        (Variables|Backend|Conditions|SetTargeting true)
        (if (Variables|Backend|Conditions|GetTarget%20Found) :!label _label
          (Audio|PlaySound2D "/Game/Devs/GD_Alex/Sounds/ShootingSFX/HitEnemySound/Pew01.Pew01" 1.0 2.0 0.0 0 0 false)
          (elif (Variables|Backend|Conditions|GetTargeting)
            (Audio|PlaySound2D "/Game/Devs/GD_Alex/Sounds/ShootingSFX/HitEnemySound/Pew01.Pew01" 0.5 1.0 0.0 0 0 false)
            (Utilities|FlowControl|Delay 0.1)
            (goto _label)))))))