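; BP_EnemyExplosion is a self-destroying enemy death effect that plays a big Niagara explosion and blasts apart a body geometry collection.
; On BeginPlay it picks the near or far explosion system by comparing distance to the first BP_SingleplayerCharacter (not the actual camera) against LODDistance.
; After a short delay it applies a radial impulse and activates the effect, later destroying the Niagara component, then the whole actor.
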(event Custom|Activate%20Explosion%20by%20Distance
  (bind _ns_bigexplosion (Variables|Default|GetNS_BigExplosion))
  ;[1 1 1] LOD
  (bind _distance (CallFunction|GetDistancetoCamera))
  (if (>= _distance (Variables|Default|GetLOD%20distance))
    (Class|NiagaraComponent|SetAsset _ns_bigexplosion "/Game/Devs/DA_Leo/Leo_VFX/Explosions/NS_FarBigExplosion.NS_FarBigExplosion" true)
    (else
      (Class|NiagaraComponent|SetAsset _ns_bigexplosion "/Game/Devs/DA_Leo/Leo_VFX/Explosions/NS_BigExplosion.NS_BigExplosion" true)))
  (CallFunction|PlayExplosion))

(event Custom|Play%20Explosion
  (bind _ns_bigexplosion (Variables|Default|GetNS_BigExplosion))
  ;[1 1 1] Explosion Animation
  (Utilities|FlowControl|Delay 0.2)
  (Physics|AddRadialImpulse (Variables|Default|GetGC_Body_Heavy) (Transformation|GetActorLocation) 2e+02 1e+04 "RIF_Constant" false)
  (Components|Activation|Activate _ns_bigexplosion false)
  (Utilities|FlowControl|Delay 7.0)
  (Components|DestroyComponent _ns_bigexplosion)
  (Utilities|FlowControl|Delay 2e+01)
  (Actor|DestroyActor))

(event EventBeginPlay
  (CallFunction|ActivateExplosionbyDistance))

(fn ConstructionScript)

(fn GetDistancetoCamera
  (bind _outactors (Actor|GetAllActorsOfClass "/Game/Devs/PRO_Mert/BluePrints/Player/MISC/BP_SingleplayerCharacter.BP_SingleplayerCharacter_C"))
  (return (Math|Vector|Distance(Vector) (Transformation|GetActorLocation) (Transformation|GetActorLocation (Utilities|Array|Get(acopy) _outactors)))))