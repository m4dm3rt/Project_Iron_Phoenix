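; Enemy explosion actor that plays a staged blast with debris physics, then destroys itself.
; Two staggered initial booms lead into a radial impulse on CGEnemyTest and the main Niagara explosion, followed by timed cleanup.
; BeginPlay runs this sequence automatically, duplicating PlayExplosion.
; ActivateExplosionbyDistance swaps the main effect between near and far variants by player distance, then calls PlayExplosion.
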(event Custom|Activate%20Explosion%20by%20Distance
  (params (Distance%20To%20Player :type Float%20%28double-precision%29))
  (bind _ns_bigexplosion (Variables|Default|GetNS_BigExplosion))
  ;[1 1 1] LOD
  (if (>= Distance%20To%20Player 5e+02)
    (Class|NiagaraComponent|SetAsset _ns_bigexplosion "/Game/Devs/DA_Leo/Leo_VFX/Explosions/NS_FarBigExplosion.NS_FarBigExplosion" true)
    (else
      (Class|NiagaraComponent|SetAsset _ns_bigexplosion "/Game/Devs/DA_Leo/Leo_VFX/Explosions/NS_BigExplosion.NS_BigExplosion" true)))
  (CallFunction|PlayExplosion))

(event Custom|Play%20Explosion
  (bind _ns_bigexplosion (Variables|Default|GetNS_BigExplosion))
  ;[1 1 1] Explosion Animation
  (Components|Activation|Activate (Variables|Default|GetInitialBoom) false)
  (Utilities|FlowControl|Delay 0.1)
  (Components|Activation|Activate (Variables|Default|GetInitialBoom1) false)
  (Utilities|FlowControl|Delay 0.2)
  (Physics|AddRadialImpulse (Variables|Default|GetCG_EnemyTest) (Transformation|GetActorLocation) 2e+02 5e+03 "RIF_Constant" false)
  (Components|Activation|Activate _ns_bigexplosion false)
  (Utilities|FlowControl|Delay 7.0)
  (Components|DestroyComponent _ns_bigexplosion)
  (Utilities|FlowControl|Delay 2e+01)
  (Actor|DestroyActor))

(event EventBeginPlay
  (bind _ns_bigexplosion (Variables|Default|GetNS_BigExplosion))
  (Components|Activation|Activate (Variables|Default|GetInitialBoom) false)
  (Utilities|FlowControl|Delay 0.1)
  (Components|Activation|Activate (Variables|Default|GetInitialBoom1) false)
  (Utilities|FlowControl|Delay 0.2)
  (Physics|AddRadialImpulse (Variables|Default|GetCG_EnemyTest) (Transformation|GetActorLocation) 2e+02 5e+03 "RIF_Constant" false)
  (Components|Activation|Activate _ns_bigexplosion false)
  (Utilities|FlowControl|Delay 7.0)
  (Components|DestroyComponent _ns_bigexplosion)
  (Utilities|FlowControl|Delay 2e+01)
  (Actor|DestroyActor))

(fn ConstructionScript)