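; BP_Skybox is a skybox actor that configures a cube mesh and its sun material in the construction script.
; It scales the mesh by a radius, then pushes sun brightness, disk size, direction and color into the materials.
; A valid linked directional light overrides sun direction, and optionally color.
; Star and nebula parameter setters exist but are disconnected, so they never run.
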(fn ConstructionScript
  (bind _sm_skybox_cube (Variables|Default|GetSM_Skybox_Cube))
  (Utilities|FlowControl|Sequence
    (:then_0
      (Transformation|SetRelativeScale3D (Variables|Default|GetSM_Skybox_Cube) (Math|Conversions|ToVector(Float) (Variables|Default|GetSphereRadius))))
    (:then_1
      (Rendering|Material|SetScalarParameterValueonMaterials _sm_skybox_cube "Sun Brightness" (Variables|Default|GetSunBrightness))
      (Rendering|Material|SetScalarParameterValueonMaterials _sm_skybox_cube "Sun Disk Size" (Variables|Default|GetSunDiskSize))
      (Rendering|Material|SetVectorParameterValueonMaterials _sm_skybox_cube "Sun Direction" (Math|Vector|GetForwardVector (Variables|Default|GetSunDirection)))
      (Rendering|Material|SetVectorParameterValueonMaterials _sm_skybox_cube "Sun Color" (Math|Conversions|ToVector(LinearColor) (Variables|Default|GetSunColor)))
      (bind _directionallight (Variables|Default|GetDirectionalLight)
        (:then
          (Rendering|Material|SetVectorParameterValueonMaterials _sm_skybox_cube "Sun Direction" (Transformation|GetActorForwardVector _directionallight))
          (if (Variables|Default|GetUseLightColor)
            (Rendering|Material|SetVectorParameterValueonMaterials _sm_skybox_cube "Sun Color" (Math|Conversions|ToVector(LinearColor) (Rendering|Components|Light|GetLightColor (Variables|/Script/Engine.Light|GetLightComponent _directionallight))))))
        (:else)))))