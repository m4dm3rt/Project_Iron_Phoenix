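; BP_LobbyPlatform is a multiplayer lobby platform that displays a character for the player controller assigned to it.
; SpawnPlayer stores the controller, destroys any existing character and spawns a BP_MPCharacter at the PlayerSpawn component's transform, ignoring collisions.
; ClearPlayer releases the controller and destroys the current character.
; The spawned character is not possessed here.
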(event Custom|SpawnPlayer
  (params (PC :type Player%20Controller%20Object%20Reference))
  (Variables|Default|SetPC PC)
  (Utilities|IsValid (Variables|Default|GetCurrentChar)
    (:Is%20Valid
      (Actor|DestroyActor (Variables|Default|GetCurrentChar)))
    (:Is%20Not%20Valid
      _))
  (bind _returnvalue (Game|SpawnActorfromClass "/Game/Devs/PRO_Mert/Multiplayer/InGame/Player/BP_MPCharacter.BP_MPCharacter_C" (Transformation|GetWorldTransform (Variables|Default|GetPlayerSpawn)) "AlwaysSpawn" "MultiplyWithRoot" 0 0))
  (Variables|Default|SetCurrentChar _returnvalue))

(event Custom|ClearPlayer
  (Variables|Default|SetPC 0)
  (Utilities|IsValid (Variables|Default|GetCurrentChar)
    (:Is%20Valid
      (Actor|DestroyActor (Variables|Default|GetCurrentChar))
      (Variables|Default|SetCurrentChar 0))))

(fn ConstructionScript)