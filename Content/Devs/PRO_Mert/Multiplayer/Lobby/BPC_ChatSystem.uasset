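; Player controller component that provides multiplayer text chat, filed with the lobby assets.
; On BeginPlay it creates the chat UI for the local controller only and caches its chatbox, which Enter focuses and the mouse wheel scrolls.
; SendChatMessageSrv relays a message by looping over the GameState PlayerArray and calling AddChatMessageClient on each controller's chat component, which appends it to that player's chatbox.
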(event Custom|SendChatMessage%20Srv
  (params (Message :type String))
  (for _array_element (Variables|/Script/Engine.GameStateBase|GetPlayerArray (Game|GetGameState))
    (CallFunction|AddChatMessageClient (Actor|GetComponentsByClass (Game|GetPlayerController _array_element) "BPC_ChatSystem_C") Message)))

(event Custom|AddChatMessage%20Client
  (params (Message :type String))
  (Default|AddChatMessage (Variables|Default|GetChatBox%20REF) Message))

(event EventBeginPlay
  (if (Pawn|IsLocalPlayerController (.AsPlayer%20Controller (Utilities|Casting|CastToPlayerController (Components|GetOwner))))
    (bind _returnvalue (UserInterface|CreateWidget "/Game/Devs/PRO_Mert/Multiplayer/Lobby/Widgets/WBP_ChatUi.WBP_ChatUi_C"))
    (bind _output_get (Variables|Default|SetChatUi%20REF _returnvalue))
    (UserInterface|Viewport|AddtoViewport _output_get 0)
    (Variables|Default|SetChatBox%20REF (Variables|/Game/Devs/PRO_Mert/Multiplayer/Lobby/Widgets/WBP_ChatUi.WBP_ChatUi_C|GetChatbox_W _output_get))))

(event Input|KeyboardEvents|Enter
  (params (Key :type Key%20Structure :default "None"))
  (:Pressed
    (Default|FocusChat (Variables|Default|GetChatBox%20REF))))

(event Input|MouseEvents|MouseWheelUp
  (params (Key :type Key%20Structure :default "None"))
  (:Pressed
    (Default|Scroll (Variables|Default|GetChatBox%20REF) true)))

(event Input|MouseEvents|MouseWheelDown
  (params (Key :type Key%20Structure :default "None"))
  (:Pressed
    (Default|Scroll (Variables|Default|GetChatBox%20REF) false)))