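; BP_LobbyCamera is the lobby camera that switches between a menu view and an editor view.
; On BeginPlay it creates and stores the Lobby_W widget, then copies the player's name into MainGameInstance.
; EditorMode and MenuMode set the input mode and play or reverse one timeline that blends spring arm length and camera FOV.
; A second timeline that would nudge the camera's relative location is never triggered.
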(event Custom|EditorMode
  ;[0.4179 0.6584 1] Editor HUD
  (Input|SetInputModeGameandUI (Game|GetPlayerController 0) 0 "LockInFullscreen" true false)
  (bind _smooth (Timeline|Timeline_0 Play)
    (:Update
      (Variables|/Script/Engine.SpringArmComponent|SetTargetArmLength (Variables|Default|GetSpringArm) (Math|Float|Lerp 0.0 1e+02 _smooth))
      (Camera|SetFieldOfView (Variables|Default|GetCamera) (Math|Float|Lerp 8e+01 6e+01 _smooth)))))

(event Custom|MenuMode
  ;[0.2941 0.3804 1] Menu HUD
  (Input|SetInputModeUIOnly (Game|GetPlayerController 0) 0 "LockInFullscreen" false)
  ;[0.4179 0.6584 1] Editor HUD
  (bind _smooth (Timeline|Timeline_0 Reverse)
    (:Update
      (Variables|/Script/Engine.SpringArmComponent|SetTargetArmLength (Variables|Default|GetSpringArm) (Math|Float|Lerp 0.0 1e+02 _smooth))
      (Camera|SetFieldOfView (Variables|Default|GetCamera) (Math|Float|Lerp 8e+01 6e+01 _smooth)))))

(event EventBeginPlay
  ;[0.2941 0.3804 1] Begin Play
  (Utilities|FlowControl|DoOnce false
    (:Completed
      (bind _returnvalue (UserInterface|CreateWidget "/Game/Devs/PRO_Mert/Multiplayer/Lobby/Widgets/Lobby_W.Lobby_W_C"))
      (Variables|Default|SetLobby%20W%20REF _returnvalue)
      (bind _asmain_game_instance (Utilities|Casting|CastToMainGameInstance (Game|GetGameInstance)))
      (Variables|/Game/Devs/PRO_Mert/BluePrints/Player/MISC/MainGameInstance.MainGameInstance_C|SetPlayerName _asmain_game_instance (Utilities|Text|ToText(String) (Class|AdvancedSessionsLibrary|GetPlayerName (Game|GetPlayerController 0)))))))

(fn ConstructionScript)