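; Multiplayer world border that warns a locally controlled player who leaves the play area and kills them if they stay out.
; Leaving SphereCollision reveals the border Sphere, and re-entering hides it.
; Exiting Sphere starts a countdown HUD, polled every 0.2 seconds until PlayerGone triggers PlayerDies on player 0's pawn.
; Re-entry fades and resets the HUD, with paired DoOnce gates preventing repeat triggers; disabled characters are ignored on exit.
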(event OnComponentBeginOverlap(Sphere)
  (params (OverlappedComponent :type Primitive%20Component%20Object%20Reference) (OtherActor :type Actor%20Object%20Reference) (OtherComp :type Primitive%20Component%20Object%20Reference) (OtherBodyIndex :type Integer) (bFromSweep :type Boolean) (SweepResult :type Hit%20Result%20Structure%20%28by%20ref%29))
  ;[1 1 1] Collision if Player is in Range
  (bind _asbp_multiplayer_character (Utilities|Casting|CastToBP_MultiplayerCharacter OtherActor))
  (if (Pawn|IsLocallyControlled _asbp_multiplayer_character)
    (Variables|Default|SetOutOfBounds false)
    (Default|FadeOut (Variables|Default|GetWorldBorder%20HUD%20REF))
    (Utilities|FlowControl|DoOnce false
      (:Completed
        (Utilities|FlowControl|Delay 0.5)
        (Widget|RemovefromParent (Variables|Default|GetWorldBorder%20HUD%20REF))
        (Default|ResetCountdown (Variables|Default|GetWorldBorder%20HUD%20REF))
        (Utilities|FlowControl|DoOnce false) ; enters at Reset
      ))))

(event OnComponentBeginOverlap(SphereCollision)
  (params (OverlappedComponent :type Primitive%20Component%20Object%20Reference) (OtherActor :type Actor%20Object%20Reference) (OtherComp :type Primitive%20Component%20Object%20Reference) (OtherBodyIndex :type Integer) (bFromSweep :type Boolean) (SweepResult :type Hit%20Result%20Structure%20%28by%20ref%29))
  ;[1 1 1] Show Border
  (bind _asbp_multiplayer_character (Utilities|Casting|CastToBP_MultiplayerCharacter OtherActor))
  (if (Pawn|IsLocallyControlled _asbp_multiplayer_character)
    (Development|SetHiddeninGame (Variables|Default|GetSphere) true false)))

(event OnComponentEndOverlap(SphereCollision)
  (params (OverlappedComponent :type Primitive%20Component%20Object%20Reference) (OtherActor :type Actor%20Object%20Reference) (OtherComp :type Primitive%20Component%20Object%20Reference) (OtherBodyIndex :type Integer))
  ;[1 1 1] Show Border
  (bind _asbp_multiplayer_character (Utilities|Casting|CastToBP_MultiplayerCharacter OtherActor))
  (if (Pawn|IsLocallyControlled _asbp_multiplayer_character)
    (if (not (Variables|/Game/Devs/PRO_Mert/Multiplayer/InGame/Player/BP_MultiplayerCharacter.BP_MultiplayerCharacter_C|GetisDisabled _asbp_multiplayer_character))
      (Development|SetHiddeninGame (Variables|Default|GetSphere) false false))))

(event OnComponentEndOverlap(Sphere)
  (params (OverlappedComponent :type Primitive%20Component%20Object%20Reference) (OtherActor :type Actor%20Object%20Reference) (OtherComp :type Primitive%20Component%20Object%20Reference) (OtherBodyIndex :type Integer))
  ;[1 1 1] Collision if Player is in Range
  (bind _asbp_multiplayer_character (Utilities|Casting|CastToBP_MultiplayerCharacter OtherActor))
  (if (Pawn|IsLocallyControlled _asbp_multiplayer_character)
    (if (not (Variables|/Game/Devs/PRO_Mert/Multiplayer/InGame/Player/BP_MultiplayerCharacter.BP_MultiplayerCharacter_C|GetisDisabled _asbp_multiplayer_character))
      (Variables|Default|SetOutOfBounds true)
      (Utilities|FlowControl|DoOnce false
        (:Completed
          (CallFunction|Timer)
          (bind _returnvalue (UserInterface|CreateWidget "/Game/Devs/PRO_Alex/Blueprints/Widgets/WorldBorder_HUD.WorldBorder_HUD_C"))
          (bind _output_get (Variables|Default|SetWorldBorder%20HUD%20REF _returnvalue))
          (UserInterface|Viewport|AddtoViewport _output_get 0)
          (Utilities|FlowControl|DoOnce false) ; enters at Reset
        )))))

(event Custom|Timer
  (bind _worldborder_hud_ref (Variables|Default|GetWorldBorder%20HUD%20REF))
  ;[1 1 1] Counting Timer
  (Default|CountingtoZero _worldborder_hud_ref)
  (if (Variables|/Game/Devs/PRO_Alex/Blueprints/Widgets/WorldBorder_HUD.WorldBorder_HUD_C|GetPlayerGone _worldborder_hud_ref) :!label _label
    (CallFunction|DestroyPlayer)
    (elif (Variables|Default|GetOutOfBounds)
      (Utilities|FlowControl|Delay 0.2)
      (goto _label))))

(event Custom|DestroyPlayer
  ;[1 1 1] Kill Player
  (bind _asbp_multiplayer_character (Utilities|Casting|CastToBP_MultiplayerCharacter (Game|Player|GetPlayerPawn 0)))
  (Default|PlayerDies _asbp_multiplayer_character))

(fn ConstructionScript)