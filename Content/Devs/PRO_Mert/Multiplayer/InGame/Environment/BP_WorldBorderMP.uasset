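; Multiplayer world border that gives a player leaving its collision sphere a HUD countdown, then kills them if it runs out.
; End overlap on the locally controlled, non-disabled character starts the countdown widget, and a delay loop polls it before calling PlayerDies.
; Re-entering fades out and resets the HUD, with paired DoOnce nodes re-arming each other.
; Swarm, sniper and bomber enemies only get their out-of-border flag toggled.
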(event OnComponentBeginOverlap(SphereCollision)
  (params (OverlappedComponent :type Primitive%20Component%20Object%20Reference) (OtherActor :type Actor%20Object%20Reference) (OtherComp :type Primitive%20Component%20Object%20Reference) (OtherBodyIndex :type Integer) (bFromSweep :type Boolean) (SweepResult :type Hit%20Result%20Structure%20%28by%20ref%29))
  ;[1 1 1] Collision if Player is in Range
  (Utilities|FlowControl|Sequence
    (:then_0
      _)
    (:then_1
      (bind _asbp_enemy_swarm_mp (Utilities|Casting|CastToBP_EnemySwarmMP OtherActor))
      (Variables|/Game/Devs/PRO_Mert/Multiplayer/InGame/Enemies/BP_EnemySwarmMP.BP_EnemySwarmMP_C|SetOutOufBorder _asbp_enemy_swarm_mp false))
    (:then_2
      (bind _asbp_enemy_sniper_mp (Utilities|Casting|CastToBP_EnemySniperMP OtherActor))
      (Variables|/Game/Devs/PRO_Mert/Multiplayer/InGame/Enemies/BP_EnemySniperMP.BP_EnemySniperMP_C|SetOutOufBorder _asbp_enemy_sniper_mp false))
    (:then_3
      (bind _asbp_enemy_bomber_mp (Utilities|Casting|CastToBP_EnemyBomberMP OtherActor))
      (Variables|/Game/Devs/PRO_Mert/Multiplayer/InGame/Enemies/BP_EnemyBomberMP.BP_EnemyBomberMP_C|SetOutOufBorder _asbp_enemy_bomber_mp false)))
  (bind _asbp_mpcharacter (Utilities|Casting|CastToBP_MPCharacter OtherActor))
  (if (Pawn|IsLocallyControlled _asbp_mpcharacter)
    (Variables|Default|SetOutOfBounds false)
    (Default|FadeOut (Variables|Default|GetWorldBorder%20HUD%20REF))
    (Utilities|FlowControl|DoOnce false
      (:Completed
        (Utilities|FlowControl|Delay 0.5)
        (Widget|RemovefromParent (Variables|Default|GetWorldBorder%20HUD%20REF))
        (Default|ResetCountdown (Variables|Default|GetWorldBorder%20HUD%20REF))
        (Utilities|FlowControl|DoOnce false) ; enters at Reset
      ))))

(event OnComponentEndOverlap(SphereCollision)
  (params (OverlappedComponent :type Primitive%20Component%20Object%20Reference) (OtherActor :type Actor%20Object%20Reference) (OtherComp :type Primitive%20Component%20Object%20Reference) (OtherBodyIndex :type Integer))
  ;[1 1 1] Collision if Player is in Range
  (Utilities|FlowControl|Sequence
    (:then_0
      _)
    (:then_1
      (bind _asbp_enemy_swarm_mp (Utilities|Casting|CastToBP_EnemySwarmMP OtherActor))
      (Variables|/Game/Devs/PRO_Mert/Multiplayer/InGame/Enemies/BP_EnemySwarmMP.BP_EnemySwarmMP_C|SetOutOufBorder _asbp_enemy_swarm_mp true))
    (:then_2
      (bind _asbp_enemy_sniper_mp (Utilities|Casting|CastToBP_EnemySniperMP OtherActor))
      (Variables|/Game/Devs/PRO_Mert/Multiplayer/InGame/Enemies/BP_EnemySniperMP.BP_EnemySniperMP_C|SetOutOufBorder _asbp_enemy_sniper_mp true))
    (:then_3
      (bind _asbp_enemy_bomber_mp (Utilities|Casting|CastToBP_EnemyBomberMP OtherActor))
      (Variables|/Game/Devs/PRO_Mert/Multiplayer/InGame/Enemies/BP_EnemyBomberMP.BP_EnemyBomberMP_C|SetOutOufBorder _asbp_enemy_bomber_mp true)))
  (bind _asbp_mpcharacter (Utilities|Casting|CastToBP_MPCharacter OtherActor))
  (if (Pawn|IsLocallyControlled _asbp_mpcharacter)
    (if (not (Variables|/Game/Devs/PRO_Mert/Multiplayer/InGame/MISC/BP_MPCharacter.BP_MPCharacter_C|GetisDisabled _asbp_mpcharacter))
      (Variables|Default|SetOutOfBounds true)
      (Utilities|FlowControl|DoOnce false
        (:Completed
          (CallFunction|Timer)
          (bind _returnvalue (UserInterface|CreateWidget "/Game/Devs/PRO_Alex/Blueprints/Widgets/WorldBorder_HUD.WorldBorder_HUD_C"))
          (bind _output_get (Variables|Default|SetWorldBorder%20HUD%20REF _returnvalue))
          (UserInterface|Viewport|AddtoViewport _output_get 0)
          (Utilities|FlowControl|DoOnce false) ; enters at Reset
        )))))

(event Custom|Timer
  (bind _worldborder_hud_ref (Variables|Default|GetWorldBorder%20HUD%20REF))
  ;[1 1 1] Counting Timer
  (Default|CountingtoZero _worldborder_hud_ref)
  (if (Variables|/Game/Devs/PRO_Alex/Blueprints/Widgets/WorldBorder_HUD.WorldBorder_HUD_C|GetPlayerGone _worldborder_hud_ref) :!label _label
    (CallFunction|DestroyPlayer)
    (elif (Variables|Default|GetOutOfBounds)
      (Utilities|FlowControl|Delay 0.2)
      (goto _label))))

(event Custom|DestroyPlayer
  ;[1 1 1] Kill Player
  (bind _asbp_mpcharacter (Utilities|Casting|CastToBP_MPCharacter (Game|Player|GetPlayerPawn 0)))
  (Default|PlayerDies _asbp_mpcharacter))

(fn ConstructionScript)