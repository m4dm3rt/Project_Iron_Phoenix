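; Multiplayer swarm enemy projectile that flies without gravity at a configurable speed, set on its movement component at construction.
; Capsule overlaps route through DamageSrv to DamageMC, a server-to-multicast pair by naming.
; Only multiplayer characters are affected: the projectile applies damage, spawns a scaled-up particle effect and destroys itself.
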(event OnComponentBeginOverlap(CapsuleCollision)
  (params (OverlappedComponent :type Primitive%20Component%20Object%20Reference) (OtherActor :type Actor%20Object%20Reference) (OtherComp :type Primitive%20Component%20Object%20Reference) (OtherBodyIndex :type Integer) (bFromSweep :type Boolean) (SweepResult :type Hit%20Result%20Structure%20%28by%20ref%29))
  (CallFunction|DamageSrv OtherActor))

(event Custom|Damage%20MC
  (params (Object :type Object%20Object%20Reference))
  (bind _asbp_multiplayer_character (Utilities|Casting|CastToBP_MultiplayerCharacter Object))
  (Game|Damage|ApplyDamage _asbp_multiplayer_character (Variables|Projectile|Settings|GetDamage) 0 0)
  (Effects|SpawnEmitteratLocation "/Game/Realistic_Starter_VFX_Pack_Vol2/Particles/Hit/P_Default.P_Default" (Transformation|GetActorLocation) "0, 0, 0" "15.000000,15.000000,15.000000")
  (Actor|DestroyActor))

(event Custom|Damage%20Srv
  (params (Object :type Object%20Object%20Reference))
  (CallFunction|DamageMC Object))

(fn ConstructionScript
  (bind _projectilemovement (Variables|Default|GetProjectileMovement))
  (bind _output_get (Variables|/Script/Engine.ProjectileMovementComponent|SetInitialSpeed _projectilemovement (Variables|Projectile|Settings|GetSpeed)))
  (Variables|/Script/Engine.ProjectileMovementComponent|SetMaxSpeed _projectilemovement _output_get)
  (Variables|/Script/Engine.ProjectileMovementComponent|SetProjectileGravityScale _projectilemovement 0.0))