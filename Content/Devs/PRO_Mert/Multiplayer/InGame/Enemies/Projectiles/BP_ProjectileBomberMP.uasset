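; Multiplayer enemy bomber projectile that flies straight without gravity and damages player characters and asteroids on overlap.
; Player hits route through DamageSrv to DamageMC, which applies damage, spawns an explosion and removes the mesh and indicator components.
; Asteroid hits apply half damage locally and remove the same components without the effect.
; Tick scales the widget indicator's image inversely with distance to the first player pawn.
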(event OnComponentBeginOverlap(ProjectileMesh)
  (params (OverlappedComponent :type Primitive%20Component%20Object%20Reference) (OtherActor :type Actor%20Object%20Reference) (OtherComp :type Primitive%20Component%20Object%20Reference) (OtherBodyIndex :type Integer) (bFromSweep :type Boolean) (SweepResult :type Hit%20Result%20Structure%20%28by%20ref%29))
  (CallFunction|DamageSrv OtherActor)
  (bind _asbp_asteroid (Utilities|Casting|CastToBP_Asteroid OtherActor))
  (Game|Damage|ApplyDamage _asbp_asteroid (/ (Variables|Projectile|Settings|GetDamage) 2.0) 0 0)
  (Components|DestroyComponent (Variables|Default|GetProjectileMesh)))

(event Custom|Damage%20MC
  (params (Object :type Object%20Object%20Reference))
  (bind _asbp_mpcharacter (Utilities|Casting|CastToBP_MPCharacter Object))
  (Game|Damage|ApplyDamage _asbp_mpcharacter (Variables|Projectile|Settings|GetDamage) 0 0)
  (Effects|SpawnEmitteratLocation "/Game/Realistic_Starter_VFX_Pack_Vol2/Particles/Destruction/P_Destruction_Metal.P_Destruction_Metal" (Transformation|GetActorLocation) "0, 0, 0" "100.000000,100.000000,100.000000")
  (Components|DestroyComponent (Variables|Default|GetProjectileMesh)))

(event Custom|Damage%20Srv
  (params (Object :type Object%20Object%20Reference))
  (CallFunction|DamageMC Object))

(event EventTick
  (params (DeltaSeconds :type Float%20%28single-precision%29))
  (bind _returnvalue (Game|Player|GetPlayerPawn 0))
  (bind _returnvalue_2 (Transformation|GetDistanceTo _returnvalue))
  (bind _returnvalue_3 (/ 1e+07 _returnvalue_2))
  (Class|Image|SetBrush (Variables|/Game/Devs/PRO_Mert/BluePrints/Enemies/Widgets/EnemyProjectile_W.EnemyProjectile_W_C|GetImage_MissileIndicator (.AsEnemy%20Projectile%20W (Utilities|Casting|CastToEnemyProjectile_W (UserInterface|GetWidget (Variables|Default|GetProjectileIndicator))))) (Utilities|Struct|MakeSlateBrush "Image" "NoTile" "NoMirror" (Utilities|Struct|MakeDeprecateSlateVector2D _returnvalue_3 _returnvalue_3) "(Left=0.000000,Top=0.000000,Right=0.000000,Bottom=0.000000)" "(SpecifiedColor=(R=1.000000,G=1.000000,B=1.000000,A=1.000000),ColorUseRule=UseColor_Specified)" "(CornerRadii=(X=0.000000,Y=0.000000,Z=0.000000,W=1.000000),Color=(SpecifiedColor=(R=0.000000,G=0.000000,B=0.000000,A=0.000000),ColorUseRule=UseColor_Specified),Width=0.000000,RoundingType=HalfHeightRadius,bUseBrushTransparency=False)" "/Game/Crosshairs/Sprites/Crosshairs/T_Triangle_Separated_Dot_Blue_Sprite1.T_Triangle_Separated_Dot_Blue_Sprite1")))

(fn ConstructionScript
  (bind _projectilemovement (Variables|Default|GetProjectileMovement))
  (bind _output_get (Variables|/Script/Engine.ProjectileMovementComponent|SetInitialSpeed _projectilemovement (Variables|Projectile|Settings|GetSpeed)))
  (Variables|/Script/Engine.ProjectileMovementComponent|SetMaxSpeed _projectilemovement _output_get)
  (Variables|/Script/Engine.ProjectileMovementComponent|SetProjectileGravityScale _projectilemovement 0.0))