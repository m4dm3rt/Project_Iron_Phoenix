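; Enemy spawner for multiplayer that spawns up to five waves of Swarm, Sniper and Bomber AI at six spawn points.
; In scripted mode, BeginPlay polls the kill counter to start each wave, whose six spawns are staggered by SpawnDelay.
; With Random set, looping timers drive spawns at one random point per call, adding a second timer after five kills.
; Waves after the first update the wave text on the first PlayerHUD_W found.
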(event Custom|SpawnWave5
  ;[1 1 1] Wave 5
  (|CG-SetWaveUI5) ; SetUi
  (|CG-SpawnWave5) ; SpawnEnemies
)

(event Custom|SpawnWave1
  ;[1 1 1] Wave1
  (|CG-SpawnWave1) ; SpawnEnemies
)

(event Custom|EnemyKillCounter
  ;[1 1 1] Enemy Killed counter
  (Variables|Conditions|SetEnemyKilled (+ (Variables|Conditions|GetEnemyKilled) 1.0))
  (Variables|Conditions|SetEnemyCount (- (Variables|Conditions|GetEnemyCount) 1.0)))

(event Custom|SpawnWave2
  ;[1 1 1] Wave 2
  (|CG-SetWaveUI2) ; SetUi
  (|CG-SpawnWave2) ; SpawnEnemies
)

(event Custom|SpawnWave3
  ;[1 1 1] Wave 3
  (|CG-SetWaveUI3) ; SetUi
  (|CG-SpawnWave3) ; SpawnEnemies
)

(event Custom|SpawnWave4
  ;[1 1 1] Wave 4
  (|CG-SetWaveUI4) ; SetUi
  (|CG-SpawnWave4) ; SpawnEnemies
)

(event EventBeginPlay
  ;[1 1 1] Begin Play
  (if (Variables|Settings|GetRandom?)
    ;[1 1 1] Random Spawn Caller
    (Utilities|Time|SetTimerbyEvent (EventDispatchers|CreateEvent :!event Custom|SpawnWave1) 3.0 true)
    (if (== (Variables|Conditions|GetEnemyKilled) 5.0) :!label _label
      (Utilities|Time|SetTimerbyEvent (EventDispatchers|CreateEvent :!event Custom|SpawnWave2) 3.0 true)
      (else
        (Utilities|FlowControl|Delay 5.0)
        (goto _label)))
    (else
      ;[1 1 1] Spawn Caller
      (Utilities|Time|SetTimerbyEvent (EventDispatchers|CreateEvent :!event Custom|SpawnWave1) (Variables|Settings|GetSpawnDelay))
      (if (== (Variables|Conditions|GetEnemyKilled) 6.0) :!label _label_2
        (Utilities|Time|SetTimerbyEvent (EventDispatchers|CreateEvent :!event Custom|SpawnWave2) (Variables|Settings|GetSpawnDelay))
        (if (== (Variables|Conditions|GetEnemyKilled) 12.0) :!label _label_3
          (Utilities|Time|SetTimerbyEvent (EventDispatchers|CreateEvent :!event Custom|SpawnWave3) (Variables|Settings|GetSpawnDelay))
          (if (== (Variables|Conditions|GetEnemyKilled) 18.0) :!label _label_4
            (Utilities|Time|SetTimerbyEvent (EventDispatchers|CreateEvent :!event Custom|SpawnWave4) (Variables|Settings|GetSpawnDelay))
            (if (== (Variables|Conditions|GetEnemyKilled) 24.0) :!label _label_5
              (Utilities|Time|SetTimerbyEvent (EventDispatchers|CreateEvent :!event Custom|SpawnWave5) (Variables|Settings|GetSpawnDelay))
              (else
                (Utilities|FlowControl|Delay 7.5)
                (goto _label_5)))
            (else
              (Utilities|FlowControl|Delay 7.5)
              (goto _label_4)))
          (else
            (Utilities|FlowControl|Delay 7.5)
            (goto _label_3)))
        (else
          (Utilities|FlowControl|Delay 7.5)
          (goto _label_2))))))

(fn ConstructionScript)