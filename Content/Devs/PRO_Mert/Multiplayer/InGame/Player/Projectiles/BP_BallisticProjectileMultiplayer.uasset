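; Multiplayer ballistic projectile that flies at constant speed without gravity and damages characters and asteroids.
; On BeginPlay it scales Damage by player 0's gun energy, up above the midpoint and down below, then enables hits after a short delay.
; Overlaps apply damage, spawn an impact emitter and destroy the projectile.
; Character hits also trigger player 0's crosshair hitmarker and sound, using player index 0 rather than the projectile's owner.
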(event OnComponentBeginOverlap(SphereCollision)
  (params (OverlappedComponent :type Primitive%20Component%20Object%20Reference) (OtherActor :type Actor%20Object%20Reference) (OtherComp :type Primitive%20Component%20Object%20Reference) (OtherBodyIndex :type Integer) (bFromSweep :type Boolean) (SweepResult :type Hit%20Result%20Structure%20%28by%20ref%29))
  (bind _damage (Variables|Projectile|Settings|GetDamage))
  (if (Variables|Projectile|Conditions|GetEnabledCollision)
    (bind _asbp_multiplayer_character (Utilities|Casting|CastToBP_MultiplayerCharacter OtherActor)
      (:then
        (Game|Damage|ApplyDamage _asbp_multiplayer_character _damage 0 0)
        (Effects|SpawnEmitteratLocation "/Game/Realistic_Starter_VFX_Pack_Vol2/Particles/Hit/P_Default.P_Default" (Transformation|GetActorLocation) "0, 0, 0" "10.000000,10.000000,10.000000")
        (bind _asbp_multiplayer_character_2 (Utilities|Casting|CastToBP_MultiplayerCharacter (Game|Player|GetPlayerPawn 0)))
        (Default|Hitmarker (.AsMultiplayer%20Crosshair%20W (Utilities|Casting|CastToMultiplayerCrosshair_W (UserInterface|GetWidget (Variables|/Game/Devs/PRO_Mert/Multiplayer/InGame/Player/BP_MultiplayerCharacter.BP_MultiplayerCharacter_C|GetCrosshairWidget _asbp_multiplayer_character_2)))))
        (Audio|PlaySound2D "/Game/Devs/PRO_Mert/Sounds/SFX_Hitmarker_v1.SFX_Hitmarker_v1" 1.0 (Math|Random|RandomFloatinRange 0.9 1.1) 0.0 0 0 false) ; Hit Audio
        (Actor|DestroyActor))
      (:CastFailed
        (bind _asbp_asteroid (Utilities|Casting|CastToBP_Asteroid OtherActor))
        (Game|Damage|ApplyDamage _asbp_asteroid _damage 0 0)
        (Effects|SpawnEmitteratLocation "/Game/Realistic_Starter_VFX_Pack_Vol2/Particles/Hit/P_Default.P_Default" (Transformation|GetActorLocation) "0, 0, 0" "20.000000,20.000000,20.000000")
        (Actor|DestroyActor)))))

(event EventBeginPlay
  (bind _asbp_multiplayer_character (Utilities|Casting|CastToBP_MultiplayerCharacter (Game|Player|GetPlayerPawn 0)))
  (if (> (Variables|/Game/Devs/PRO_Mert/Multiplayer/InGame/Player/BP_MultiplayerCharacter.BP_MultiplayerCharacter_C|GetEnergyGun _asbp_multiplayer_character) 5e+01)
    (Variables|Projectile|Settings|SetDamage (* (Variables|Projectile|Settings|GetDamage) (Variables|/Game/Devs/PRO_Mert/Multiplayer/InGame/Player/BP_MultiplayerCharacter.BP_MultiplayerCharacter_C|GetEnergyGunValue _asbp_multiplayer_character)))
    (elif (< (Variables|/Game/Devs/PRO_Mert/Multiplayer/InGame/Player/BP_MultiplayerCharacter.BP_MultiplayerCharacter_C|GetEnergyGun _asbp_multiplayer_character) 5e+01)
      (Variables|Projectile|Settings|SetDamage (/ (Variables|Projectile|Settings|GetDamage) (Variables|/Game/Devs/PRO_Mert/Multiplayer/InGame/Player/BP_MultiplayerCharacter.BP_MultiplayerCharacter_C|GetEnergyGunValue _asbp_multiplayer_character)))))
  (Utilities|FlowControl|Delay 0.15)
  (Variables|Projectile|Conditions|SetEnabledCollision true))

(fn ConstructionScript
  (bind _projectilemovement (Variables|Default|GetProjectileMovement))
  (bind _output_get (Variables|/Script/Engine.ProjectileMovementComponent|SetInitialSpeed _projectilemovement (Variables|Projectile|Settings|GetSpeed)))
  (Variables|/Script/Engine.ProjectileMovementComponent|SetMaxSpeed _projectilemovement _output_get)
  (Variables|/Script/Engine.ProjectileMovementComponent|SetProjectileGravityScale _projectilemovement 0.0))