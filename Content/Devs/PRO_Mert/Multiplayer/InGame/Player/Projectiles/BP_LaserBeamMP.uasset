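; Multiplayer laser beam projectile that fires a hitscan shot when spawned, with damage taken from MainGameInstance.
; BeginPlay sphere-traces along the Niagara beam, ignoring the instigator, and sets the beam's color and length.
; A cast chain applies damage to player characters and enemies, or double damage to asteroids and buoys, then plays impact VFX.
; Character and enemy hits add a hitmarker and sound, using the crosshair found on BP_SingleplayerCharacter.
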(event EventBeginPlay
  (bind _returnvalue (Transformation|GetActorLocation))
  (bind _ns_laser (Variables|Default|GetNS_Laser))
  (bind _asmain_game_instance (Utilities|Casting|CastToMainGameInstance (Game|GetGameInstance)))
  (Variables|Projectile|Settings|SetDamage (Variables|/Game/Devs/PRO_Mert/BluePrints/Player/MISC/MainGameInstance.MainGameInstance_C|GetLaserDamage _asmain_game_instance))
  (bind _outhit (Collision|SphereTraceByChannel _returnvalue (+ _returnvalue (* (Math|Vector|GetForwardVector (Variables|Default|GetNS_Laser)) (Variables|Projectile|Settings|GetWeapon%20Range))) 16.0 "TraceTypeQuery3" false (Utilities|Array|MakeArray (Variables|Actor|GetInstigator)) "None"))
  (Effects|Components|ParticleSystem|SetColorParameter _ns_laser "Beam Color" (Variables|Projectile|Settings|GetBeam%20Color))
  (Effects|Components|ParticleSystem|SetVectorParameter _ns_laser "Beam End" (Math|Vector|MakeVector (Variables|Projectile|Settings|GetWeapon%20Range) 0.0 0.0))
  (if (.bBlockingHit (Collision|BreakHitResult _outhit))
    (bind _asbp_mpcharacter (Utilities|Casting|CastToBP_MPCharacter (.HitActor (Collision|BreakHitResult _outhit)))
      (:then
        (Utilities|FlowControl|DoOnce false
          (:Completed
            (Game|Damage|ApplyDamage _asbp_mpcharacter (Variables|Projectile|Settings|GetDamage) 0 (Variables|Actor|GetInstigator) "/Game/Devs/PRO_Mert/BluePrints/Player/DamageTypes/DT_LaserBeam.DT_LaserBeam_C")
            (CallFunction|DestroyProjectileEnemy (.ImpactPoint (Collision|BreakHitResult _outhit)) :!label _label))))
      (:CastFailed
        (bind _asbp_enemy_swarm_mp (Utilities|Casting|CastToBP_EnemySwarmMP (.HitActor (Collision|BreakHitResult _outhit)))
          (:then
            (Utilities|FlowControl|DoOnce false
              (:Completed
                (Game|Damage|ApplyDamage _asbp_enemy_swarm_mp (Variables|Projectile|Settings|GetDamage) 0 (Variables|Actor|GetInstigator) "/Game/Devs/PRO_Mert/BluePrints/Player/DamageTypes/DT_LaserBeam.DT_LaserBeam_C")
                (goto _label))))
          (:CastFailed
            (bind _asbp_enemy_sniper_mp (Utilities|Casting|CastToBP_EnemySniperMP (.HitActor (Collision|BreakHitResult _outhit)))
              (:then
                (Utilities|FlowControl|DoOnce false
                  (:Completed
                    (Game|Damage|ApplyDamage _asbp_enemy_sniper_mp (Variables|Projectile|Settings|GetDamage) 0 (Variables|Actor|GetInstigator) "/Game/Devs/PRO_Mert/BluePrints/Player/DamageTypes/DT_LaserBeam.DT_LaserBeam_C")
                    (goto _label))))
              (:CastFailed
                (bind _asbp_enemy_bomber_mp (Utilities|Casting|CastToBP_EnemyBomberMP (.HitActor (Collision|BreakHitResult _outhit)))
                  (:then
                    (Utilities|FlowControl|DoOnce false
                      (:Completed
                        (Game|Damage|ApplyDamage _asbp_enemy_bomber_mp (Variables|Projectile|Settings|GetDamage) 0 (Variables|Actor|GetInstigator) "/Game/Devs/PRO_Mert/BluePrints/Player/DamageTypes/DT_LaserBeam.DT_LaserBeam_C")
                        (goto _label))))
                  (:CastFailed
                    (bind _asbp_enemy_drone_mp (Utilities|Casting|CastToBP_EnemyDroneMP (.HitActor (Collision|BreakHitResult _outhit)))
                      (:then
                        (Utilities|FlowControl|DoOnce false
                          (:Completed
                            (Game|Damage|ApplyDamage _asbp_enemy_drone_mp (Variables|Projectile|Settings|GetDamage) 0 (Variables|Actor|GetInstigator) "/Game/Devs/PRO_Mert/BluePrints/Player/DamageTypes/DT_LaserBeam.DT_LaserBeam_C")
                            (goto _label))))
                      (:CastFailed
                        (bind _asbp_asteroid (Utilities|Casting|CastToBP_Asteroid (.HitActor (Collision|BreakHitResult _outhit)))
                          (:then
                            (Utilities|FlowControl|DoOnce false
                              (:Completed
                                (Game|Damage|ApplyDamage _asbp_asteroid (* (Variables|Projectile|Settings|GetDamage) 2.0) 0 (Variables|Actor|GetInstigator) "/Game/Devs/PRO_Mert/BluePrints/Player/DamageTypes/DT_LaserBeam.DT_LaserBeam_C"))))
                          (:CastFailed
                            (bind _asbp_buoy (Utilities|Casting|CastToBP_Buoy (.HitActor (Collision|BreakHitResult _outhit))))
                            (Utilities|FlowControl|DoOnce false
                              (:Completed
                                (Game|Damage|ApplyDamage _asbp_buoy (* (Variables|Projectile|Settings|GetDamage) 2.0) 0 (Variables|Actor|GetInstigator) "/Game/Devs/PRO_Mert/BluePrints/Player/DamageTypes/DT_LaserBeam.DT_LaserBeam_C")))))
                        (CallFunction|DestroyProjectileWorld (.ImpactPoint (Collision|BreakHitResult _outhit)))))))))))))))

(fn ConstructionScript)

(fn DestroyProjectileWorld
  (params (NewLocation :type Vector))
  (bind _ns_hit_laserbattery (Variables|Default|GetNS_Hit_LaserBattery))
  (Transformation|SetWorldLocation _ns_hit_laserbattery NewLocation false false)
  (Components|Activation|Activate _ns_hit_laserbattery true))

(fn DestroyProjectileEnemy
  (params (NewLocation :type Vector))
  (bind _ns_hit_laserbattery (Variables|Default|GetNS_Hit_LaserBattery))
  (bind _returnvalue (Actor|GetActorOfClass "/Game/Devs/PRO_Mert/BluePrints/Player/MISC/BP_SingleplayerCharacter.BP_SingleplayerCharacter_C"))
  (Default|Hitmarker (Variables|/Game/Devs/PRO_Mert/BluePrints/Player/MISC/BP_SingleplayerCharacter.BP_SingleplayerCharacter_C|GetPlayerCrosshair%20REF _returnvalue))
  (Audio|PlaySound2D "/Game/Devs/PRO_Mert/Sounds/SFX_Hitmarker.SFX_Hitmarker" 1.0 (Math|Random|RandomFloatinRange 0.9 1.1) 0.0 0 0 false)
  (Transformation|SetWorldLocation _ns_hit_laserbattery NewLocation false false)
  (Components|Activation|Activate _ns_hit_laserbattery true))