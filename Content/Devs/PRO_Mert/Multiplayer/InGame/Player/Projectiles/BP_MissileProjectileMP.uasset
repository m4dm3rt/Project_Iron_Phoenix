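; Multiplayer missile projectile that damages characters other than its instigator, enemy ships, asteroids and buoys on sphere overlap, doubling damage to asteroids and buoys.
; Impacts trigger an explosion and destroy components; character and enemy hits also give local shooters a hitmarker.
; A gated Tick scales the indicator widget inversely with distance to the instigator.
; HomingProjectile polls target range to enable homing, but its only call here is unconnected.
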(event OnComponentBeginOverlap(Sphere)
  (params (OverlappedComponent :type Primitive%20Component%20Object%20Reference) (OtherActor :type Actor%20Object%20Reference) (OtherComp :type Primitive%20Component%20Object%20Reference) (OtherBodyIndex :type Integer) (bFromSweep :type Boolean) (SweepResult :type Hit%20Result%20Structure%20%28by%20ref%29))
  (bind _damage (Variables|Projectile|Settings|GetDamage))
  (bind _returnvalue (* _damage 2.0))
  (bind _asbp_mpcharacter (Utilities|Casting|CastToBP_MPCharacter (Utilities|SelectObject 0 OtherActor (== OtherActor (Variables|Actor|GetInstigator))))
    (:then
      (Utilities|FlowControl|DoOnce false
        (:Completed
          (Game|Damage|ApplyDamage _asbp_mpcharacter _damage 0 (Variables|Actor|GetInstigator) "/Game/Devs/PRO_Mert/Multiplayer/InGame/Player/DamageTypes/DT_MissileMP.DT_MissileMP_C")
          (CallFunction|DestroyProjectile :!label _label)
          (CallFunction|Deacticate))))
    (:CastFailed
      (bind _asbp_enemy_swarm_mp (Utilities|Casting|CastToBP_EnemySwarmMP OtherActor)
        (:then
          (Utilities|FlowControl|DoOnce false
            (:Completed
              (Game|Damage|ApplyDamage _asbp_enemy_swarm_mp _damage 0 (Variables|Actor|GetInstigator) "/Game/Devs/PRO_Mert/Multiplayer/InGame/Player/DamageTypes/DT_MissileMP.DT_MissileMP_C")
              (goto _label))))
        (:CastFailed
          (bind _asbp_enemy_sniper_mp (Utilities|Casting|CastToBP_EnemySniperMP OtherActor)
            (:then
              (Utilities|FlowControl|DoOnce false
                (:Completed
                  (Game|Damage|ApplyDamage _asbp_enemy_sniper_mp _damage 0 (Variables|Actor|GetInstigator) "/Game/Devs/PRO_Mert/Multiplayer/InGame/Player/DamageTypes/DT_MissileMP.DT_MissileMP_C")
                  (goto _label))))
            (:CastFailed
              (bind _asbp_enemy_bomber_mp (Utilities|Casting|CastToBP_EnemyBomberMP OtherActor)
                (:then
                  (Utilities|FlowControl|DoOnce false
                    (:Completed
                      (Game|Damage|ApplyDamage _asbp_enemy_bomber_mp _damage 0 (Variables|Actor|GetInstigator) "/Game/Devs/PRO_Mert/Multiplayer/InGame/Player/DamageTypes/DT_MissileMP.DT_MissileMP_C")
                      (goto _label))))
                (:CastFailed
                  (bind _asbp_asteroid (Utilities|Casting|CastToBP_Asteroid OtherActor)
                    (:then
                      (Utilities|FlowControl|DoOnce false
                        (:Completed
                          (Game|Damage|ApplyDamage _asbp_asteroid _returnvalue 0 (Variables|Actor|GetInstigator) "/Game/Devs/PRO_Mert/Multiplayer/InGame/Player/DamageTypes/DT_MissileMP.DT_MissileMP_C"))))
                    (:CastFailed
                      (bind _asbp_buoy (Utilities|Casting|CastToBP_Buoy OtherActor))
                      (Utilities|FlowControl|DoOnce false
                        (:Completed
                          (Game|Damage|ApplyDamage _asbp_buoy _returnvalue 0 (Variables|Actor|GetInstigator) "/Game/Devs/PRO_Mert/Multiplayer/InGame/Player/DamageTypes/DT_MissileMP.DT_MissileMP_C")))))
                  (Components|Activation|Activate (Variables|Default|GetNS_BigExplosion) true)
                  (Components|DestroyComponent (Variables|Default|GetProjectileMovement))
                  (CallFunction|Deacticate))))))))))

(event Custom|HomingProjectile
  (params (TargetEnemy :type Actor%20Object%20Reference))
  (bind _projectilemovement (Variables|Default|GetProjectileMovement))
  ;[1 0.1979 0.1979] Homing Logic
  (Utilities|IsValid TargetEnemy
    (:Is%20Valid
      (if (< (Math|Vector|VectorLength (- (Transformation|GetActorLocation TargetEnemy) (Transformation|GetActorLocation))) (Variables|Default|GetHomingRadius))
        (Variables|/Script/Engine.ProjectileMovementComponent|SetHomingTargetComponent _projectilemovement (Variables|/Script/Engine.Actor|GetRootComponent TargetEnemy))
        (Variables|/Script/Engine.ProjectileMovementComponent|SetbIsHomingProjectile _projectilemovement true))
      (Utilities|FlowControl|Delay 0.2)
      (CallFunction|HomingProjectile TargetEnemy))))

(event Custom|Deacticate
  (bind _missileindicator (Variables|Default|GetMissileIndicator))
  (bind _instigator (Variables|Actor|GetInstigator))
  (bind _returnvalue (Transformation|GetDistanceTo _instigator))
  (bind _returnvalue_2 (UserInterface|GetWidget _missileindicator))
  (bind _asmissile_mp_wbp (Utilities|Casting|CastToMissileMP_WBP _returnvalue_2))
  (bind _returnvalue_3 (/ 1e+07 _returnvalue))
  (bind _image_missileindicator (Variables|/Game/Devs/PRO_Mert/Multiplayer/InGame/HUD/WBP/MissileMP_WBP.MissileMP_WBP_C|GetImage_MissileIndicator _asmissile_mp_wbp))
  (Utilities|FlowControl|Gate true) ; enters at Close
)

(event Custom|Active
  (bind _missileindicator (Variables|Default|GetMissileIndicator))
  (bind _instigator (Variables|Actor|GetInstigator))
  (bind _returnvalue (Transformation|GetDistanceTo _instigator))
  (bind _returnvalue_2 (UserInterface|GetWidget _missileindicator))
  (bind _asmissile_mp_wbp (Utilities|Casting|CastToMissileMP_WBP _returnvalue_2))
  (bind _returnvalue_3 (/ 1e+07 _returnvalue))
  (bind _image_missileindicator (Variables|/Game/Devs/PRO_Mert/Multiplayer/InGame/HUD/WBP/MissileMP_WBP.MissileMP_WBP_C|GetImage_MissileIndicator _asmissile_mp_wbp))
  (Utilities|FlowControl|Gate true) ; enters at Open
)

(event EventBeginPlay
  (CallFunction|Active))

(event EventTick
  (params (DeltaSeconds :type Float%20%28single-precision%29))
  (bind _missileindicator (Variables|Default|GetMissileIndicator))
  (bind _instigator (Variables|Actor|GetInstigator))
  (bind _returnvalue (Transformation|GetDistanceTo _instigator))
  (bind _returnvalue_2 (UserInterface|GetWidget _missileindicator))
  (bind _asmissile_mp_wbp (Utilities|Casting|CastToMissileMP_WBP _returnvalue_2))
  (bind _returnvalue_3 (/ 1e+07 _returnvalue))
  (bind _image_missileindicator (Variables|/Game/Devs/PRO_Mert/Multiplayer/InGame/HUD/WBP/MissileMP_WBP.MissileMP_WBP_C|GetImage_MissileIndicator _asmissile_mp_wbp))
  (Utilities|FlowControl|Gate true
    (:Exit
      (Class|Image|SetBrush _image_missileindicator (Utilities|Struct|MakeSlateBrush "Image" "NoTile" "NoMirror" (Utilities|Struct|MakeDeprecateSlateVector2D _returnvalue_3 _returnvalue_3) "(Left=0.000000,Top=0.000000,Right=0.000000,Bottom=0.000000)" "(SpecifiedColor=(R=1.000000,G=1.000000,B=1.000000,A=1.000000),ColorUseRule=UseColor_Specified)" "(CornerRadii=(X=0.000000,Y=0.000000,Z=0.000000,W=1.000000),Color=(SpecifiedColor=(R=0.000000,G=0.000000,B=0.000000,A=0.000000),ColorUseRule=UseColor_Specified),Width=0.000000,RoundingType=HalfHeightRadius,bUseBrushTransparency=False)" (.resourceobject (Variables|/Script/UMG.Image|GetBrush _image_missileindicator)))))))

(fn ConstructionScript
  (bind _projectilemovement (Variables|Default|GetProjectileMovement))
  (bind _output_get (Variables|/Script/Engine.ProjectileMovementComponent|SetInitialSpeed _projectilemovement (Variables|Projectile|Settings|GetSpeed)))
  (Variables|/Script/Engine.ProjectileMovementComponent|SetMaxSpeed _projectilemovement _output_get))

(fn DestroyProjectile
  (bind _asbp_mpcharacter (Utilities|Casting|CastToBP_MPCharacter (Variables|Actor|GetInstigator)))
  (if (Pawn|IsLocallyControlled _asbp_mpcharacter)
    (Default|Hitmarker (.AsCrosshair%20MP%20W (Utilities|Casting|CastToCrosshairMP_W (UserInterface|GetWidget (Variables|/Game/Devs/PRO_Mert/Multiplayer/InGame/Player/BP_MPCharacter.BP_MPCharacter_C|GetCrosshairWidget _asbp_mpcharacter)))))
    (Audio|PlaySound2D "/Game/Devs/PRO_Mert/Sounds/SFX_Hitmarker.SFX_Hitmarker" 1.0 (Math|Random|RandomFloatinRange 0.9 1.1) 0.0 0 0 false))
  (Components|Activation|Activate (Variables|Default|GetNS_BigExplosion) true)
  (Components|DestroyComponent (Variables|Default|GetProjectileMovement)))