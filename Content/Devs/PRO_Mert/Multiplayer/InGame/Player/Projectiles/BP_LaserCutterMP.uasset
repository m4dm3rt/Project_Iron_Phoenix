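; Multiplayer laser cutter projectile that damages players, enemies, buoys and asteroid rings on sphere overlap.
; It reads damage from the game instance, ignores its instigator, and uses a cast chain to deal double point damage to buoys and asteroids.
; Character and enemy hits give the locally controlled shooter a hitmarker and sound.
; Every handled hit activates Niagara impact FX and destroys the mesh, movement and collision components, not the actor.
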(event OnComponentBeginOverlap(Sphere)
  (params (OverlappedComponent :type Primitive%20Component%20Object%20Reference) (OtherActor :type Actor%20Object%20Reference) (OtherComp :type Primitive%20Component%20Object%20Reference) (OtherBodyIndex :type Integer) (bFromSweep :type Boolean) (SweepResult :type Hit%20Result%20Structure%20%28by%20ref%29))
  (bind _returnvalue (Transformation|GetActorLocation))
  (bind _returnvalue_2 (Collision|MakeHitResult false false 0.0 0.0 "0, 0, 0" "0, 0, 0" "0,0,1" "0,0,1" 0 0))
  (bind _damage (Variables|Projectile|Settings|GetDamage))
  (bind _instigator (Variables|Actor|GetInstigator))
  (bind _returnvalue_3 (* _damage 2.0))
  (bind _asbp_mpcharacter (Utilities|Casting|CastToBP_MPCharacter (Utilities|SelectObject 0 OtherActor (== OtherActor (Variables|Actor|GetInstigator))))
    (:then
      (Utilities|FlowControl|DoOnce false
        (:Completed
          (Game|Damage|ApplyDamage _asbp_mpcharacter _damage 0 (Variables|Actor|GetInstigator) "/Game/Devs/PRO_Mert/BluePrints/Player/DamageTypes/DT_LaserCutter.DT_LaserCutter_C")
          (CallFunction|DestroyProjectileEnemy :!label _label))))
    (:CastFailed
      (bind _asbp_enemy_swarm_mp (Utilities|Casting|CastToBP_EnemySwarmMP OtherActor)
        (:then
          (Utilities|FlowControl|DoOnce false
            (:Completed
              (Game|Damage|ApplyDamage _asbp_enemy_swarm_mp _damage 0 (Variables|Actor|GetInstigator) "/Game/Devs/PRO_Mert/BluePrints/Player/DamageTypes/DT_LaserCutter.DT_LaserCutter_C")
              (goto _label))))
        (:CastFailed
          (bind _asbp_enemy_sniper_mp (Utilities|Casting|CastToBP_EnemySniperMP OtherActor)
            (:then
              (Utilities|FlowControl|DoOnce false
                (:Completed
                  (Game|Damage|ApplyDamage _asbp_enemy_sniper_mp _damage 0 (Variables|Actor|GetInstigator) "/Game/Devs/PRO_Mert/BluePrints/Player/DamageTypes/DT_LaserCutter.DT_LaserCutter_C")
                  (goto _label))))
            (:CastFailed
              (bind _asbp_enemy_bomber_mp (Utilities|Casting|CastToBP_EnemyBomberMP OtherActor)
                (:then
                  (Utilities|FlowControl|DoOnce false
                    (:Completed
                      (Game|Damage|ApplyDamage _asbp_enemy_bomber_mp _damage 0 (Variables|Actor|GetInstigator) "/Game/Devs/PRO_Mert/BluePrints/Player/DamageTypes/DT_LaserCutter.DT_LaserCutter_C")
                      (goto _label))))
                (:CastFailed
                  (bind _asbp_enemy_drone_mp (Utilities|Casting|CastToBP_EnemyDroneMP OtherActor)
                    (:then
                      (Utilities|FlowControl|DoOnce false
                        (:Completed
                          (Game|Damage|ApplyDamage _asbp_enemy_drone_mp _damage 0 (Variables|Actor|GetInstigator) "/Game/Devs/PRO_Mert/BluePrints/Player/DamageTypes/DT_LaserBeam.DT_LaserBeam_C")
                          (goto _label))))
                    (:CastFailed
                      (bind _asbp_buoy (Utilities|Casting|CastToBP_Buoy OtherActor)
                        (:then
                          (Utilities|FlowControl|DoOnce false
                            (:Completed
                              (Game|Damage|ApplyPointDamage _asbp_buoy _returnvalue_3 _returnvalue _returnvalue_2 0 _instigator "/Game/Devs/PRO_Mert/BluePrints/Player/DamageTypes/DT_LaserCutter.DT_LaserCutter_C"))))
                        (:CastFailed
                          (bind _asbp_single_asteroid_ring (Utilities|Casting|CastToBP_SingleAsteroidRing OtherActor)
                            (:then
                              (Utilities|FlowControl|DoOnce false
                                (:Completed
                                  (Game|Damage|ApplyPointDamage _asbp_single_asteroid_ring _returnvalue_3 _returnvalue _returnvalue_2 0 _instigator "/Game/Devs/PRO_Mert/BluePrints/Player/DamageTypes/DT_LaserCutter.DT_LaserCutter_C"))))
                            (:CastFailed
                              (bind _asbp_asteroid_ring (Utilities|Casting|CastToBP_AsteroidRing OtherActor))
                              (Utilities|FlowControl|DoOnce false
                                (:Completed
                                  (Game|Damage|ApplyPointDamage _asbp_asteroid_ring _returnvalue_3 _returnvalue _returnvalue_2 0 0 "/Game/Devs/PRO_Mert/BluePrints/Player/DamageTypes/DT_LaserCutter.DT_LaserCutter_C")))))))
                      (CallFunction|DestroyProjectileWorld))))))))))))

(event EventBeginPlay
  (bind _asmain_game_instance (Utilities|Casting|CastToMainGameInstance (Game|GetGameInstance)))
  (Variables|Projectile|Settings|SetDamage (Variables|/Game/Devs/PRO_Mert/BluePrints/Player/MISC/MainGameInstance.MainGameInstance_C|GetLaserDamage _asmain_game_instance)))

(fn ConstructionScript
  (bind _projectilemovement (Variables|Default|GetProjectileMovement))
  (bind _output_get (Variables|/Script/Engine.ProjectileMovementComponent|SetInitialSpeed _projectilemovement (Variables|Projectile|Settings|GetSpeed)))
  (Variables|/Script/Engine.ProjectileMovementComponent|SetMaxSpeed _projectilemovement _output_get))

(fn DestroyProjectileEnemy
  (bind _asbp_mpcharacter (Utilities|Casting|CastToBP_MPCharacter (Variables|Actor|GetInstigator)))
  (if (Pawn|IsLocallyControlled _asbp_mpcharacter)
    (Default|Hitmarker (.AsCrosshair%20MP%20W (Utilities|Casting|CastToCrosshairMP_W (UserInterface|GetWidget (Variables|/Game/Devs/PRO_Mert/Multiplayer/InGame/Player/BP_MPCharacter.BP_MPCharacter_C|GetCrosshairWidget _asbp_mpcharacter)))))
    (Audio|PlaySound2D "/Game/Devs/PRO_Mert/Sounds/SFX_Hitmarker.SFX_Hitmarker" 1.0 (Math|Random|RandomFloatinRange 0.9 11.0) 0.0 0 0 false))
  (Components|Activation|Activate (Variables|Default|GetNS_Hit_LaserCutter) true)
  (Components|DestroyComponent (Variables|Default|GetLaserMesh)))

(fn DestroyProjectileWorld
  (Components|Activation|Activate (Variables|Default|GetNS_Hit_LaserCutter) true)
  (Components|DestroyComponent (Variables|Default|GetLaserMesh)))