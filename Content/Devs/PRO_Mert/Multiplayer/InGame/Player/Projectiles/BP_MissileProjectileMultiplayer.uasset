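; Multiplayer missile projectile that damages player characters, swarm, sniper and bomber enemies, and asteroids on sphere overlap after a short arming delay.
; Non-asteroid hits show a hitmarker and play a sound for a locally controlled instigator; hits strip movement and visual components.
; Construction sets a gravity-free constant speed.
; A self-repeating HomingProjectile event, not called here, seeks the closest BP_EnemySwarm, not the multiplayer swarm class.
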(event OnComponentBeginOverlap(SphereCollision)
  (params (OverlappedComponent :type Primitive%20Component%20Object%20Reference) (OtherActor :type Actor%20Object%20Reference) (OtherComp :type Primitive%20Component%20Object%20Reference) (OtherBodyIndex :type Integer) (bFromSweep :type Boolean) (SweepResult :type Hit%20Result%20Structure%20%28by%20ref%29))
  (bind _damage (Variables|Projectile|Settings|GetDamage))
  (if (Variables|Projectile|Conditions|GetEnabledCollision)
    (bind _asbp_multiplayer_character (Utilities|Casting|CastToBP_MultiplayerCharacter OtherActor)
      (:then
        (Game|Damage|ApplyDamage _asbp_multiplayer_character _damage 0 0 "/Game/Devs/PRO_Mert/BluePrints/Player/Projectiles/DT_Missile.DT_Missile_C")
        (bind _asbp_multiplayer_character_2 (Utilities|Casting|CastToBP_MultiplayerCharacter (Variables|Actor|GetInstigator) :!label _label))
        (if (Pawn|IsLocallyControlled _asbp_multiplayer_character_2)
          (Default|Hitmarker (.AsMultiplayer%20Crosshair%20W (Utilities|Casting|CastToMultiplayerCrosshair_W (UserInterface|GetWidget (Variables|/Game/Devs/PRO_Mert/Multiplayer/InGame/Player/BP_MultiplayerCharacter.BP_MultiplayerCharacter_C|GetCrosshairWidget _asbp_multiplayer_character_2)))))
          (Audio|PlaySound2D "/Game/Devs/PRO_Mert/Sounds/SFX_Hitmarker.SFX_Hitmarker" 1.0 (Math|Random|RandomFloatinRange 0.9 1.1) 0.0 0 0 false) ; Hit Audio
        )
        (Components|DestroyComponent (Variables|Default|GetProjectileMovement)))
      (:CastFailed
        (bind _asbp_enemy_swarm_multiplayer (Utilities|Casting|CastToBP_EnemySwarmMultiplayer OtherActor)
          (:then
            (Game|Damage|ApplyDamage _asbp_enemy_swarm_multiplayer _damage 0 0 "/Game/Devs/PRO_Mert/BluePrints/Player/Projectiles/DT_Missile.DT_Missile_C")
            (goto _label))
          (:CastFailed
            (bind _asbp_enemy_sniper_multiplayer (Utilities|Casting|CastToBP_EnemySniperMultiplayer OtherActor)
              (:then
                (Game|Damage|ApplyDamage _asbp_enemy_sniper_multiplayer _damage 0 0 "/Game/Devs/PRO_Mert/BluePrints/Player/Projectiles/DT_Missile.DT_Missile_C")
                (goto _label))
              (:CastFailed
                (bind _asbp_enemy_bomber_multiplayer (Utilities|Casting|CastToBP_EnemyBomberMultiplayer OtherActor)
                  (:then
                    (Game|Damage|ApplyDamage _asbp_enemy_bomber_multiplayer _damage 0 0 "/Game/Devs/PRO_Mert/BluePrints/Player/Projectiles/DT_Missile.DT_Missile_C")
                    (goto _label))
                  (:CastFailed
                    (bind _asbp_asteroid_1 (Utilities|Casting|CastToBP_Asteroid1 OtherActor))
                    (Game|Damage|ApplyDamage _asbp_asteroid_1 _damage 0 0 "/Game/Devs/PRO_Mert/BluePrints/Player/Projectiles/DT_Missile.DT_Missile_C")
                    (Components|DestroyComponent (Variables|Default|GetProjectileMovement))))))))))))

(event Custom|HomingProjectile
  ;[1 0.1979 0.1979] Homing Logic
  (Variables|/Script/Engine.ProjectileMovementComponent|SetbIsHomingProjectile (Variables|Default|GetProjectileMovement) true)
  (bind _outactors (Actor|GetAllActorsOfClass "/Game/Devs/PRO_Mert/BluePrints/Enemies/Actors/BP_EnemySwarm.BP_EnemySwarm_C"))
  (for _array_element _outactors
    (if (< (Math|Vector|VectorLength (- (Transformation|GetActorLocation _array_element) (Transformation|GetActorLocation))) (Variables|Projectile|Conditions|GetClosest%20Distance))
      (Variables|Projectile|Conditions|SetClosest%20Distance (Math|Vector|VectorLength (- (Transformation|GetActorLocation _array_element) (Transformation|GetActorLocation))))
      (Variables|Projectile|References|SetTarget _array_element)))
  (Variables|/Script/Engine.ProjectileMovementComponent|SetHomingTargetComponent (Variables|Default|GetProjectileMovement) (Variables|/Game/Devs/PRO_Mert/BluePrints/Enemies/Actors/BP_EnemySwarm.BP_EnemySwarm_C|GetSpaceFighter (Variables|Projectile|References|GetTarget)))
  (Utilities|FlowControl|Delay 0.02)
  (CallFunction|HomingProjectile))

(event EventBeginPlay
  (Utilities|FlowControl|Delay 0.3)
  (Variables|Projectile|Conditions|SetEnabledCollision true))

(fn ConstructionScript
  (bind _projectilemovement (Variables|Default|GetProjectileMovement))
  (bind _output_get (Variables|/Script/Engine.ProjectileMovementComponent|SetInitialSpeed _projectilemovement (Variables|Projectile|Settings|GetSpeed)))
  (Variables|/Script/Engine.ProjectileMovementComponent|SetMaxSpeed _projectilemovement _output_get)
  (Variables|/Script/Engine.ProjectileMovementComponent|SetProjectileGravityScale _projectilemovement 0.0))