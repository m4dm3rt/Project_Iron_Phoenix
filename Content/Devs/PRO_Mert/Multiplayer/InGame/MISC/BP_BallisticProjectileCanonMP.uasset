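; Multiplayer ballistic cannon projectile that flies without gravity at a configurable speed and ignores its instigator when moving.
; On spawn it takes damage from player 0's Ballistic1Damage, not the instigator's; energy-gun scaling is never run.
; Sphere overlaps apply kinetic damage once to characters, swarm, sniper and bomber enemies, or doubled to asteroids, then destroy it.
; Non-asteroid hits trigger hitmarker widget and sound for a locally controlled instigator.
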(event OnComponentBeginOverlap(Sphere)
  (params (OverlappedComponent :type Primitive%20Component%20Object%20Reference) (OtherActor :type Actor%20Object%20Reference) (OtherComp :type Primitive%20Component%20Object%20Reference) (OtherBodyIndex :type Integer) (bFromSweep :type Boolean) (SweepResult :type Hit%20Result%20Structure%20%28by%20ref%29))
  (bind _damage (Variables|Projectile|Settings|GetDamage))
  (bind _asbp_mpcharacter (Utilities|Casting|CastToBP_MPCharacter OtherActor)
    (:then
      (Utilities|FlowControl|DoOnce false
        (:Completed
          (Game|Damage|ApplyDamage _asbp_mpcharacter _damage 0 0 "/Game/Devs/PRO_Mert/BluePrints/Player/Projectiles/DT_KineticCanon.DT_KineticCanon_C")
          (bind _asbp_mpcharacter_2 (Utilities|Casting|CastToBP_MPCharacter (Variables|Actor|GetInstigator) :!label _label))
          (if (Pawn|IsLocallyControlled _asbp_mpcharacter_2)
            (Default|Hitmarker (.AsCrosshair%20MP%20W (Utilities|Casting|CastToCrosshairMP_W (UserInterface|GetWidget (Variables|/Game/Devs/PRO_Mert/Multiplayer/InGame/MISC/BP_MPCharacter.BP_MPCharacter_C|GetCrosshairWidget _asbp_mpcharacter_2)))))
            (Audio|PlaySound2D "/Game/Devs/PRO_Mert/Sounds/SFX_Hitmarker.SFX_Hitmarker" 1.0 (Math|Random|RandomFloatinRange 0.9 11.0) 0.0 0 0 false))
          (Actor|DestroyActor))))
    (:CastFailed
      (bind _asbp_enemy_swarm_mp (Utilities|Casting|CastToBP_EnemySwarmMP OtherActor)
        (:then
          (Utilities|FlowControl|DoOnce false
            (:Completed
              (Game|Damage|ApplyDamage _asbp_enemy_swarm_mp _damage 0 0 "/Game/Devs/PRO_Mert/BluePrints/Player/Projectiles/DT_KineticCanon.DT_KineticCanon_C")
              (goto _label))))
        (:CastFailed
          (bind _asbp_enemy_sniper_mp (Utilities|Casting|CastToBP_EnemySniperMP OtherActor)
            (:then
              (Utilities|FlowControl|DoOnce false
                (:Completed
                  (Game|Damage|ApplyDamage _asbp_enemy_sniper_mp _damage 0 0 "/Game/Devs/PRO_Mert/BluePrints/Player/Projectiles/DT_KineticCanon.DT_KineticCanon_C")
                  (goto _label))))
            (:CastFailed
              (bind _asbp_enemy_bomber_mp (Utilities|Casting|CastToBP_EnemyBomberMP OtherActor)
                (:then
                  (Utilities|FlowControl|DoOnce false
                    (:Completed
                      (Game|Damage|ApplyDamage _asbp_enemy_bomber_mp _damage 0 0 "/Game/Devs/PRO_Mert/BluePrints/Player/Projectiles/DT_KineticCanon.DT_KineticCanon_C")
                      (goto _label))))
                (:CastFailed
                  (bind _asbp_asteroid (Utilities|Casting|CastToBP_Asteroid OtherActor))
                  (Utilities|FlowControl|DoOnce false
                    (:Completed
                      (Game|Damage|ApplyDamage _asbp_asteroid (* _damage 2.0) 0 0 "/Game/Devs/PRO_Mert/BluePrints/Player/Projectiles/DT_KineticCanon.DT_KineticCanon_C")
                      (Actor|DestroyActor))))))))))))

(event EventBeginPlay
  (Collision|IgnoreActorwhenMoving (Variables|Default|GetSphere) (Variables|Actor|GetInstigator) true)
  (bind _asbp_mpcharacter (Utilities|Casting|CastToBP_MPCharacter (Game|Player|GetPlayerPawn 0)))
  (Variables|Projectile|Settings|SetDamage (Variables|/Game/Devs/PRO_Mert/Multiplayer/InGame/MISC/BP_MPCharacter.BP_MPCharacter_C|GetBallistic1Damage _asbp_mpcharacter)))

(fn ConstructionScript
  (bind _projectilemovement (Variables|Default|GetProjectileMovement))
  (bind _output_get (Variables|/Script/Engine.ProjectileMovementComponent|SetInitialSpeed _projectilemovement (Variables|Projectile|Settings|GetSpeed)))
  (Variables|/Script/Engine.ProjectileMovementComponent|SetMaxSpeed _projectilemovement _output_get)
  (Variables|/Script/Engine.ProjectileMovementComponent|SetProjectileGravityScale _projectilemovement 0.0))