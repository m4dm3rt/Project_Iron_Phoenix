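; Multiplayer missile projectile that flies without gravity at a configurable speed and damages players, swarm, sniper and bomber enemies, or asteroids at double damage.
; Sphere overlaps apply missile damage, spawn a small explosion and destroy the missile's components, leaving the actor itself.
; Character and enemy hits show a hitmarker with sound for a locally controlled instigator.
; HomingProjectile, not called here, repeatedly retargets the nearest BP_EnemySwarm, not the MP variant.
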(event OnComponentBeginOverlap(Sphere)
  (params (OverlappedComponent :type Primitive%20Component%20Object%20Reference) (OtherActor :type Actor%20Object%20Reference) (OtherComp :type Primitive%20Component%20Object%20Reference) (OtherBodyIndex :type Integer) (bFromSweep :type Boolean) (SweepResult :type Hit%20Result%20Structure%20%28by%20ref%29))
  (bind _returnvalue (Transformation|GetActorTransform))
  (bind _returnvalue_2 (Transformation|GetActorTransform))
  (bind _damage (Variables|Projectile|Settings|GetDamage))
  (bind _asbp_mpcharacter (Utilities|Casting|CastToBP_MPCharacter OtherActor)
    (:then
      (Utilities|FlowControl|DoOnce false
        (:Completed
          (Game|Damage|ApplyDamage _asbp_mpcharacter _damage 0 0 "/Game/Devs/PRO_Mert/BluePrints/Player/Projectiles/DT_Missile.DT_Missile_C")
          (bind _asbp_mpcharacter_2 (Utilities|Casting|CastToBP_MPCharacter (Variables|Actor|GetInstigator) :!label _label))
          (if (Pawn|IsLocallyControlled _asbp_mpcharacter_2)
            (Default|Hitmarker (.AsCrosshair%20MP%20W (Utilities|Casting|CastToCrosshairMP_W (UserInterface|GetWidget (Variables|/Game/Devs/PRO_Mert/Multiplayer/InGame/MISC/BP_MPCharacter.BP_MPCharacter_C|GetCrosshairWidget _asbp_mpcharacter_2)))))
            (Audio|PlaySound2D "/Game/Devs/PRO_Mert/Sounds/SFX_Hitmarker.SFX_Hitmarker" 1.0 (Math|Random|RandomFloatinRange 0.9 11.0) 0.0 0 0 false))
          (Game|SpawnActorfromClass "/Game/Devs/DA_Leo/Leo_BluePrints/Leo_Enemies/BP_EnemyExplosion.BP_EnemyExplosion_C" (Math|Transform|MakeTransform (.location _returnvalue) (.rotation _returnvalue) "0.500000,0.500000,0.500000") "Undefined" "MultiplyWithRoot" 0 0)
          (Components|DestroyComponent (Variables|Default|GetProjectileMovement)))))
    (:CastFailed
      (bind _asbp_enemy_swarm_mp (Utilities|Casting|CastToBP_EnemySwarmMP OtherActor)
        (:then
          (Utilities|FlowControl|DoOnce false
            (:Completed
              (Game|Damage|ApplyDamage _asbp_enemy_swarm_mp _damage 0 0 "/Game/Devs/PRO_Mert/BluePrints/Player/Projectiles/DT_Missile.DT_Missile_C")
              (goto _label))))
        (:CastFailed
          (bind _asbp_enemy_sniper_mp (Utilities|Casting|CastToBP_EnemySniperMP OtherActor)
            (:then
              (Utilities|FlowControl|DoOnce false
                (:Completed
                  (Game|Damage|ApplyDamage _asbp_enemy_sniper_mp _damage 0 0 "/Game/Devs/PRO_Mert/BluePrints/Player/Projectiles/DT_Missile.DT_Missile_C")
                  (goto _label))))
            (:CastFailed
              (bind _asbp_enemy_bomber_mp (Utilities|Casting|CastToBP_EnemyBomberMP OtherActor)
                (:then
                  (Utilities|FlowControl|DoOnce false
                    (:Completed
                      (Game|Damage|ApplyDamage _asbp_enemy_bomber_mp _damage 0 0 "/Game/Devs/PRO_Mert/BluePrints/Player/Projectiles/DT_Missile.DT_Missile_C")
                      (goto _label))))
                (:CastFailed
                  (bind _asbp_asteroid (Utilities|Casting|CastToBP_Asteroid OtherActor))
                  (Utilities|FlowControl|DoOnce false
                    (:Completed
                      (Game|Damage|ApplyDamage _asbp_asteroid (* _damage 2.0) 0 0 "/Game/Devs/PRO_Mert/BluePrints/Player/Projectiles/DT_Missile.DT_Missile_C")
                      (Game|SpawnActorfromClass "/Game/Devs/DA_Leo/Leo_BluePrints/Leo_Enemies/BP_EnemyExplosion.BP_EnemyExplosion_C" (Math|Transform|MakeTransform (.location _returnvalue_2) (.rotation _returnvalue_2) "0.500000,0.500000,0.500000") "Undefined" "MultiplyWithRoot" 0 0)
                      (Components|DestroyComponent (Variables|Default|GetProjectileMovement)))))))))))))

(event Custom|HomingProjectile
  ;[1 0.1979 0.1979] Homing Logic
  (Variables|/Script/Engine.ProjectileMovementComponent|SetbIsHomingProjectile (Variables|Default|GetProjectileMovement) true)
  (bind _outactors (Actor|GetAllActorsOfClass "/Game/Devs/PRO_Mert/BluePrints/Enemies/Actors/BP_EnemySwarm.BP_EnemySwarm_C"))
  (for _array_element _outactors
    (if (< (Math|Vector|VectorLength (- (Transformation|GetActorLocation _array_element) (Transformation|GetActorLocation))) (Variables|Projectile|Conditions|GetClosest%20Distance))
      (Variables|Projectile|Conditions|SetClosest%20Distance (Math|Vector|VectorLength (- (Transformation|GetActorLocation _array_element) (Transformation|GetActorLocation))))
      (Variables|Projectile|References|SetTarget _array_element)))
  (Variables|/Script/Engine.ProjectileMovementComponent|SetHomingTargetComponent (Variables|Default|GetProjectileMovement) (Variables|/Game/Devs/PRO_Mert/BluePrints/Enemies/Actors/BP_EnemySwarm.BP_EnemySwarm_C|GetSpaceFighter (Variables|Projectile|References|GetTarget)))
  (Utilities|FlowControl|Delay 0.02)
  (CallFunction|HomingProjectile))

(event EventBeginPlay
  (Collision|IgnoreActorwhenMoving (Variables|Default|GetSphere) (Variables|Actor|GetInstigator) true))

(fn ConstructionScript
  (bind _projectilemovement (Variables|Default|GetProjectileMovement))
  (bind _output_get (Variables|/Script/Engine.ProjectileMovementComponent|SetInitialSpeed _projectilemovement (Variables|Projectile|Settings|GetSpeed)))
  (Variables|/Script/Engine.ProjectileMovementComponent|SetMaxSpeed _projectilemovement _output_get)
  (Variables|/Script/Engine.ProjectileMovementComponent|SetProjectileGravityScale _projectilemovement 0.0))