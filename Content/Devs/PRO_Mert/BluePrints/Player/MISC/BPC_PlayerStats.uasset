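; Player stats component that tracks health, shield, boost, XP and level for the single-player characters.
; BeginPlay reads the level from MainGameInstance and caches which of three character classes the player pawn is.
; Functions change each stat, cap regeneration at maximums and return depleted or full-shield flags.
; XP gains update the BP_SingleplayerCharacter HUD only; leveling resets XP, raises its threshold and saves the level to the game instance.
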(event EventBeginPlay
  (bind _returnvalue (Game|Player|GetPlayerPawn 0))
  (bind (_asbp_singleplayer_character_alex_j _bsuccess) (Utilities|Casting|CastToBP_SingleplayerCharacterAlexJ _returnvalue))
  (bind (_asbp_singleplayer_character _bsuccess_2) (Utilities|Casting|CastToBP_SingleplayerCharacter _returnvalue))
  (bind (_asbp_player_character_marius _bsuccess_3) (Utilities|Casting|CastToBP_SingleplayerCharacterMarius _returnvalue))
  (bind _asmain_game_instance (Utilities|Casting|CastToMainGameInstance (Game|GetGameInstance)))
  (Variables|Level&XP|SetLevel (Variables|/Game/Devs/PRO_Mert/BluePrints/Player/MISC/MainGameInstance.MainGameInstance_C|GetLevel _asmain_game_instance))
  (if _bsuccess_2
    (Variables|References|SetPlayer true)
    (Variables|References|SetPlayer%20REF _asbp_singleplayer_character)
    (elif _bsuccess
      (Variables|References|SetPlayer%20AlexJ true)
      (Variables|References|SetPlayer%20AlexJ%20REF _asbp_singleplayer_character_alex_j)
      (elif _bsuccess_3
        (Variables|References|SetPlayer%20Marius true)
        (Variables|References|SetPlayer%20Marius%20REF _asbp_player_character_marius)))))

(fn DecreaseHealth
  (params (NoShield :type Boolean) (Damage%20Received :type Float%20%28double-precision%29))
  (if NoShield
    (bind _output_get (Variables|Health|SetHealth (- (Variables|Health|GetHealth) Damage%20Received)))
    (if (<= (/ _output_get (Variables|Health|GetMax%20Health)) 0.0)
      (return true)
      (else
        (return false)))))

(fn RegenerateHealth
  (params (Health%20Increase :type Float%20%28double-precision%29))
  (bind _output_get (Variables|Health|SetHealth (+ (Variables|Health|GetHealth) Health%20Increase)))
  (if (> _output_get (Variables|Health|GetMax%20Health))
    (bind _output_get_2 (Variables|Health|SetHealth (Variables|Health|GetMax%20Health)))))

(fn IncreaseMaxHealth
  (params (Max%20Health%20Increase :type Float%20%28double-precision%29))
  (Variables|Health|SetMax%20Health (+ (Variables|Health|GetMax%20Health) Max%20Health%20Increase)))

(fn IncreaseXP
  (params (Add%20XP :type Float%20%28double-precision%29))
  (bind _returnvalue (Game|Player|GetPlayerPawn 0))
  (bind _asbp_singleplayer_character (Utilities|Casting|CastToBP_SingleplayerCharacter _returnvalue))
  (bind _playerhud_ref (Variables|/Game/Devs/PRO_Mert/BluePrints/Player/Actors/BP_SingleplayerCharacter.BP_SingleplayerCharacter_C|GetPlayerHUD%20REF _asbp_singleplayer_character))
  (bind _output_get (Variables|Level&XP|SetXP (+ (Variables|Level&XP|GetXP) Add%20XP)))
  (if (>= _output_get (Variables|Level&XP|GetMax%20XP))
    (Default|LevelUp _playerhud_ref)
    (Level&XP|IncreaseLevel)
    (else
      (Default|XPUp _playerhud_ref Add%20XP))))

(fn DecreaseShield
  (params (Damage%20Received :type Float%20%28double-precision%29))
  (bind _output_get (Variables|Shield|SetShield (- (Variables|Shield|GetShield) Damage%20Received)))
  (if (<= (/ _output_get (Variables|Shield|GetMax%20Shield)) 0.0)
    (return true)
    (else
      (return false))))

(fn RegenerateShield
  (params (Shield%20Recovery :type Float%20%28double-precision%29))
  (bind _max_shield (Variables|Shield|GetMax%20Shield))
  (bind _output_get (Variables|Shield|SetShield (+ (Variables|Shield|GetShield) Shield%20Recovery)))
  (if (> _output_get _max_shield)
    (bind _output_get_2 (Variables|Shield|SetShield (Variables|Shield|GetMax%20Shield))))
  (if (== _output_get_2 _max_shield)
    (return true)
    (else
      (return false))))

(fn IncreaseMaxShield
  (params (Max%20Shield%20Increase :type Float%20%28double-precision%29))
  (Variables|Shield|SetMax%20Shield (+ (Variables|Shield|GetMax%20Shield) Max%20Shield%20Increase)))

(fn DecreaseBoost
  (params (Boost%20Decrease :type Float%20%28double-precision%29))
  (bind _output_get (Variables|Boost|SetBoost (- (Variables|Boost|GetBoost) Boost%20Decrease)))
  (if (<= (/ _output_get (Variables|Boost|GetMax%20Boost)) 0.0)
    (return true)
    (else
      (return false))))

(fn RegenerateBoost
  (params (Boost%20Increase :type Float%20%28double-precision%29))
  (bind _output_get (Variables|Boost|SetBoost (+ (Variables|Boost|GetBoost) Boost%20Increase)))
  (if (> _output_get (Variables|Boost|GetMax%20Boost))
    (Variables|Boost|SetBoost (Variables|Boost|GetMax%20Boost))))

(fn IncreaseMaxBoost
  (params (Max%20Boost%20Increase :type Float%20%28double-precision%29))
  (Variables|Boost|SetMax%20Boost (+ (Variables|Boost|GetMax%20Boost) Max%20Boost%20Increase)))

(fn IncreaseLevel
  (bind _asmain_game_instance (Utilities|Casting|CastToMainGameInstance (Game|GetGameInstance)))
  (Variables|Level&XP|SetLevel (+ (Variables|/Game/Devs/PRO_Mert/BluePrints/Player/MISC/MainGameInstance.MainGameInstance_C|GetLevel _asmain_game_instance) 1.0))
  (Variables|Level&XP|SetMax%20XP (+ (Variables|Level&XP|GetMax%20XP) 5e+01))
  (Variables|Level&XP|SetXP 0.0)
  (bind _asmain_game_instance_2 (Utilities|Casting|CastToMainGameInstance (Game|GetGameInstance)))
  (Variables|/Game/Devs/PRO_Mert/BluePrints/Player/MISC/MainGameInstance.MainGameInstance_C|SetLevel _asmain_game_instance_2 (Variables|Level&XP|GetLevel)))