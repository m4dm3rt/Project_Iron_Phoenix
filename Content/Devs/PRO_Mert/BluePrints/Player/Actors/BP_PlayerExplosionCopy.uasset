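; BP_PlayerExplosionCopy is an explosion actor that plays a staged blast on BeginPlay and later destroys itself.
; It picks a near or far Niagara asset for the big explosion from its distance to the first BP_PlayerCharacter, despite the "camera" naming, and prints that distance.
; Delays sequence two initial booms, a radial impulse on the CGEnemyTest component with the main blast, then cleanup.
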(event Custom|Activate%20Explosion%20by%20Distance
  (bind _ns_bigexplosion (Variables|Default|GetNS_BigExplosion))
  ;[1 1 1] LOD
  (bind _distance (CallFunction|GetDistancetoCamera))
  (if (>= _distance (Variables|Default|GetLOD%20distance))
    (Class|NiagaraComponent|SetAsset _ns_bigexplosion "/Game/Devs/DA_Leo/Leo_VFX/Explosions/NS_FarBigExplosion.NS_FarBigExplosion" true)
    (else
      (Class|NiagaraComponent|SetAsset _ns_bigexplosion "/Game/Devs/DA_Leo/Leo_VFX/Explosions/NS_BigExplosion.NS_BigExplosion" true)))
  (CallFunction|PlayExplosion))

(event Custom|Play%20Explosion
  (bind _ns_bigexplosion (Variables|Default|GetNS_BigExplosion))
  ;[1 1 1] Explosion Animation
  (Components|Activation|Activate (Variables|Default|GetInitialBoom) false)
  (Utilities|FlowControl|Delay 0.1)
  (Components|Activation|Activate (Variables|Default|GetInitialBoom1) false)
  (Utilities|FlowControl|Delay 0.2)
  (Physics|AddRadialImpulse (Variables|Default|GetCG_EnemyTest) (Transformation|GetActorLocation) 2e+02 5e+03 "RIF_Constant" false)
  (Components|Activation|Activate _ns_bigexplosion false)
  (Utilities|FlowControl|Delay 7.0)
  (Components|DestroyComponent _ns_bigexplosion)
  (Utilities|FlowControl|Delay 2e+01)
  (Actor|DestroyActor))

(event EventBeginPlay
  (CallFunction|ActivateExplosionbyDistance))

(fn ConstructionScript)

(fn GetDistancetoCamera
  (bind _outactors (Actor|GetAllActorsOfClass "/Game/Devs/PRO_Mert/BluePrints/Player/Actors/BP_PlayerCharacter.BP_PlayerCharacter_C"))
  (Development|PrintString (Utilities|String|ToString(Float) (Math|Vector|Distance(Vector) (Transformation|GetActorLocation) (Transformation|GetActorLocation (Utilities|Array|Get(acopy) _outactors)))))
  (return (Math|Vector|Distance(Vector) (Transformation|GetActorLocation) (Transformation|GetActorLocation (Utilities|Array|Get(acopy) _outactors)))))