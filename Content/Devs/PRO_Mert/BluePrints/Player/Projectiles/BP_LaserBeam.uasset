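; Player laser beam projectile that fires one hitscan shot as soon as it spawns.
; BeginPlay reads damage from MainGameInstance, sphere-traces along the Niagara beam's forward vector and draws the beam at full weapon range, even on a hit.
; A cast chain applies double damage to asteroids and buoys, normal damage to four enemy types, then plays an impact effect.
; Energy-based damage scaling exists but is disconnected.
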(event EventBeginPlay
  (bind _returnvalue (Transformation|GetActorLocation))
  (bind _ns_hit_laserbattery (Variables|Default|GetNS_Hit_LaserBattery))
  (bind _ns_laser (Variables|Default|GetNS_Laser))
  (bind _asmain_game_instance (Utilities|Casting|CastToMainGameInstance (Game|GetGameInstance)))
  (Variables|Projectile|Settings|SetDamage (Variables|/Game/Devs/PRO_Mert/BluePrints/Player/MISC/MainGameInstance.MainGameInstance_C|GetLaserDamage _asmain_game_instance))
  (bind _outhit (Collision|SphereTraceByChannel _returnvalue (+ _returnvalue (* (Math|Vector|GetForwardVector (Variables|Default|GetNS_Laser)) (Variables|Projectile|Settings|GetWeapon%20Range))) 8.0 "TraceTypeQuery3" false 0 "None"))
  (Effects|Components|ParticleSystem|SetColorParameter _ns_laser "Beam Color" (Variables|Default|GetBeam%20Color))
  (Effects|Components|ParticleSystem|SetVectorParameter _ns_laser "Beam End" (Math|Vector|MakeVector (Variables|Projectile|Settings|GetWeapon%20Range) 0.0 0.0))
  (if (.bBlockingHit (Collision|BreakHitResult _outhit))
    (bind _asbp_single_asteroid_ring (Utilities|Casting|CastToBP_SingleAsteroidRing (.HitActor (Collision|BreakHitResult _outhit)))
      (:then
        (Game|Damage|ApplyDamage _asbp_single_asteroid_ring (* (Variables|Projectile|Settings|GetDamage) 2.0) 0 0 "/Game/Devs/PRO_Mert/BluePrints/Player/DamageTypes/DT_LaserBeam.DT_LaserBeam_C"))
      (:CastFailed
        (bind _asbp_asteroid (Utilities|Casting|CastToBP_Asteroid (.HitActor (Collision|BreakHitResult _outhit)))
          (:then
            (Game|Damage|ApplyDamage _asbp_asteroid (* (Variables|Projectile|Settings|GetDamage) 2.0) 0 0 "/Game/Devs/PRO_Mert/BluePrints/Player/DamageTypes/DT_LaserBeam.DT_LaserBeam_C"))
          (:CastFailed
            (bind _asbp_buoy (Utilities|Casting|CastToBP_Buoy (.HitActor (Collision|BreakHitResult _outhit)))
              (:then
                (Game|Damage|ApplyDamage _asbp_buoy (* (Variables|Projectile|Settings|GetDamage) 2.0) 0 0 "/Game/Devs/PRO_Mert/BluePrints/Player/DamageTypes/DT_LaserBeam.DT_LaserBeam_C"))
              (:CastFailed
                (bind _asbp_enemy_swarm (Utilities|Casting|CastToBP_EnemySwarm (.HitActor (Collision|BreakHitResult _outhit)))
                  (:then
                    (Game|Damage|ApplyDamage _asbp_enemy_swarm (Variables|Projectile|Settings|GetDamage) 0 0 "/Game/Devs/PRO_Mert/BluePrints/Player/DamageTypes/DT_LaserBeam.DT_LaserBeam_C"))
                  (:CastFailed
                    (bind _asbp_enemy_sniper (Utilities|Casting|CastToBP_EnemySniper (.HitActor (Collision|BreakHitResult _outhit)))
                      (:then
                        (Game|Damage|ApplyDamage _asbp_enemy_sniper (Variables|Projectile|Settings|GetDamage) 0 0 "/Game/Devs/PRO_Mert/BluePrints/Player/DamageTypes/DT_LaserBeam.DT_LaserBeam_C"))
                      (:CastFailed
                        (bind _asbp_enemy_bomber (Utilities|Casting|CastToBP_EnemyBomber (.HitActor (Collision|BreakHitResult _outhit)))
                          (:then
                            (Game|Damage|ApplyDamage _asbp_enemy_bomber (Variables|Projectile|Settings|GetDamage) 0 0 "/Game/Devs/PRO_Mert/BluePrints/Player/DamageTypes/DT_LaserBeam.DT_LaserBeam_C"))
                          (:CastFailed
                            (bind _asbp_enemy_drone (Utilities|Casting|CastToBP_EnemyDrone (.HitActor (Collision|BreakHitResult _outhit))))
                            (Game|Damage|ApplyDamage _asbp_enemy_drone (Variables|Projectile|Settings|GetDamage) 0 0 "/Game/Devs/PRO_Mert/BluePrints/Player/DamageTypes/DT_LaserBeam.DT_LaserBeam_C")))))))))))))
    (Transformation|SetWorldLocation _ns_hit_laserbattery (.ImpactPoint (Collision|BreakHitResult _outhit)) false false)
    (Components|Activation|Activate _ns_hit_laserbattery true)))

(fn ConstructionScript)