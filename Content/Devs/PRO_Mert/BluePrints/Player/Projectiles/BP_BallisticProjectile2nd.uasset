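; Player ballistic projectile, flying straight without gravity at a configurable speed, that damages asteroids, swarm, sniper and bomber enemies, and bomber projectiles.
; On BeginPlay it scales Damage up or down by the singleplayer character's energy gun setting.
; Each Tick it sphere-traces well ahead of itself instead of using collision events.
; A recognized hit applies damage, spawns an impact effect, triggers the crosshair hitmarker and sound, then destroys the projectile.
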(event EventTick
  (params (DeltaSeconds :type Float%20%28single-precision%29))
  (bind _projectilemesh (Variables|Default|GetProjectileMesh))
  (bind _damage (Variables|Projectile|Settings|GetDamage))
  (bind _returnvalue (Transformation|GetWorldLocation _projectilemesh))
  (bind (_outhit _returnvalue_2) (Collision|SphereTraceByChannel _returnvalue (+ _returnvalue (* (Math|Vector|GetForwardVector (Transformation|GetWorldRotation _projectilemesh)) 2e+03)) 5e+01 "TraceTypeQuery1" false 0 "None"))
  (if _returnvalue_2
    (bind _asbp_asteroid (Utilities|Casting|CastToBP_Asteroid (.HitActor (Collision|BreakHitResult _outhit)))
      (:then
        (Game|Damage|ApplyDamage _asbp_asteroid _damage 0 0))
      (:CastFailed
        (bind _asbp_enemy_swarm (Utilities|Casting|CastToBP_EnemySwarm (.HitActor (Collision|BreakHitResult _outhit)))
          (:then
            (Game|Damage|ApplyDamage _asbp_enemy_swarm _damage 0 0))
          (:CastFailed
            (bind _asbp_enemy_sniper (Utilities|Casting|CastToBP_EnemySniper (.HitActor (Collision|BreakHitResult _outhit)))
              (:then
                (Game|Damage|ApplyDamage _asbp_enemy_sniper _damage 0 0))
              (:CastFailed
                (bind _asbp_enemy_bomber (Utilities|Casting|CastToBP_EnemyBomber (.HitActor (Collision|BreakHitResult _outhit)))
                  (:then
                    (Game|Damage|ApplyDamage _asbp_enemy_bomber _damage 0 0))
                  (:CastFailed
                    (bind _asbp_projectile_bomber (Utilities|Casting|CastToBP_ProjectileBomber (.HitActor (Collision|BreakHitResult _outhit))))
                    (Game|Damage|ApplyDamage _asbp_projectile_bomber _damage 0 0)))))))))
    (Effects|SpawnEmitteratLocation "/Game/Realistic_Starter_VFX_Pack_Vol2/Particles/Hit/P_Default.P_Default" (.Location (Collision|BreakHitResult _outhit)) "0, 0, 0" "50.000000,50.000000,50.000000")
    (bind _foundwidgets (Widget|GetAllWidgetsOfClass "/Game/Devs/PRO_Mert/BluePrints/Player/Widgets/PlayerCrosshair_W.PlayerCrosshair_W_C" false))
    (Default|Hitmarker (Utilities|Array|Get(acopy) _foundwidgets))
    (Audio|PlaySound2D "/Game/Devs/GD_Alex/Sounds/Ambience/SFX_Collide.SFX_Collide" 0.5 1.0 0.0 0 0 false) ; Hit Audio
    (Actor|DestroyActor)))

(event EventBeginPlay
  (bind _returnvalue (Game|Player|GetPlayerPawn 0))
  (bind (_asbp_singleplayer_character _bsuccess) (Utilities|Casting|CastToBP_SingleplayerCharacter _returnvalue))
  (bind _energygun (Variables|/Game/Devs/PRO_Mert/BluePrints/Player/Actors/BP_SingleplayerCharacter.BP_SingleplayerCharacter_C|GetEnergyGun _asbp_singleplayer_character))
  (if _bsuccess
    (if (> _energygun 5e+01)
      (Variables|Projectile|Settings|SetDamage (* (Variables|Projectile|Settings|GetDamage) (Variables|/Game/Devs/PRO_Mert/BluePrints/Player/Actors/BP_SingleplayerCharacter.BP_SingleplayerCharacter_C|GetEnergyGunValue _asbp_singleplayer_character)))
      (elif (< _energygun 5e+01)
        (Variables|Projectile|Settings|SetDamage (/ (Variables|Projectile|Settings|GetDamage) (Variables|/Game/Devs/PRO_Mert/BluePrints/Player/Actors/BP_SingleplayerCharacter.BP_SingleplayerCharacter_C|GetEnergyGunValue _asbp_singleplayer_character)))))
    (elif (not (.bSuccess (Utilities|Casting|CastToBP_SingleplayerCharacterAlexJ _returnvalue)))
      (if (.bSuccess (Utilities|Casting|CastToBP_SingleplayerCharacterMarius _returnvalue))
        _))))

(fn ConstructionScript
  (bind _projectilemovement (Variables|Default|GetProjectileMovement))
  (bind _output_get (Variables|/Script/Engine.ProjectileMovementComponent|SetInitialSpeed _projectilemovement (Variables|Projectile|Settings|GetSpeed)))
  (Variables|/Script/Engine.ProjectileMovementComponent|SetMaxSpeed _projectilemovement _output_get)
  (Variables|/Script/Engine.ProjectileMovementComponent|SetProjectileGravityScale _projectilemovement 0.0))