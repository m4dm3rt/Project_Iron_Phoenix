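; BP_LaserProjectileSecond is a gravity-free laser projectile that damages asteroids, swarm enemies and sniper enemies on overlap, then destroys itself.
; Construction sets its constant speed, and a Hit event spawns an impact emitter.
; HomingProjectile re-runs itself on a short delay, scanning all BP_EnemySwarm actors for the closest and homing on its SpaceFighter component.
; ClosestDistance is not reset between scans, so the target changes only when a distance beats the stored minimum.
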(event OnComponentBeginOverlap(SphereCollision)
  (params (OverlappedComponent :type Primitive%20Component%20Object%20Reference) (OtherActor :type Actor%20Object%20Reference) (OtherComp :type Primitive%20Component%20Object%20Reference) (OtherBodyIndex :type Integer) (bFromSweep :type Boolean) (SweepResult :type Hit%20Result%20Structure%20%28by%20ref%29))
  (bind _damage (Variables|Projectile|Settings|GetDamage))
  ;[1 1 1] Damage
  (Utilities|FlowControl|Sequence
    (:then_0
      (bind _asbp_asteroid (Utilities|Casting|CastToBP_Asteroid OtherActor))
      (Game|Damage|ApplyDamage _asbp_asteroid _damage 0 0))
    (:then_1
      (bind _asbp_enemy_swarm (Utilities|Casting|CastToBP_EnemySwarm OtherActor))
      (Game|Damage|ApplyDamage _asbp_enemy_swarm _damage 0 0))
    (:then_2
      (bind _asbp_enemy_sniper (Utilities|Casting|CastToBP_EnemySniper OtherActor))
      (Game|Damage|ApplyDamage _asbp_enemy_sniper _damage 0 0)))
  (Actor|DestroyActor))

(event Custom|HomingProjectile
  ;[1 0.2969 0.2969] Homing Logic
  (Variables|/Script/Engine.ProjectileMovementComponent|SetbIsHomingProjectile (Variables|Default|GetProjectileMovement) true)
  (bind _outactors (Actor|GetAllActorsOfClass "/Game/Devs/PRO_Mert/BluePrints/Enemies/Actors/BP_EnemySwarm.BP_EnemySwarm_C"))
  (for _array_element _outactors
    (if (< (Math|Vector|VectorLength (- (Transformation|GetActorLocation _array_element) (Transformation|GetActorLocation))) (Variables|Projectile|Conditions|GetClosest%20Distance))
      (Variables|Projectile|Conditions|SetClosest%20Distance (Math|Vector|VectorLength (- (Transformation|GetActorLocation _array_element) (Transformation|GetActorLocation))))
      (Variables|Projectile|References|SetTarget _array_element)))
  (Variables|/Script/Engine.ProjectileMovementComponent|SetHomingTargetComponent (Variables|Default|GetProjectileMovement) (Variables|/Game/Devs/PRO_Mert/BluePrints/Enemies/Actors/BP_EnemySwarm.BP_EnemySwarm_C|GetSpaceFighter (Variables|Projectile|References|GetTarget)))
  (Utilities|FlowControl|Delay 0.02)
  (CallFunction|HomingProjectile))

(event Collision|EventHit
  (params (MyComp :type Primitive%20Component%20Object%20Reference) (Other :type Actor%20Object%20Reference) (OtherComp :type Primitive%20Component%20Object%20Reference) (bSelfMoved :type Boolean) (HitLocation :type Vector :default "0, 0, 0") (HitNormal :type Vector :default "0, 0, 0") (NormalImpulse :type Vector :default "0, 0, 0") (Hit :type Hit%20Result%20Structure%20%28by%20ref%29))
  ;[1 1 1] Play VFX
  (Effects|SpawnEmitteratLocation "/Game/Realistic_Starter_VFX_Pack_Vol2/Particles/Hit/P_Default.P_Default" HitLocation "0, 0, 0" "100.000000,100.000000,100.000000"))

(fn ConstructionScript
  (bind _projectilemovement (Variables|Default|GetProjectileMovement))
  (bind _output_get (Variables|/Script/Engine.ProjectileMovementComponent|SetInitialSpeed _projectilemovement (Variables|Projectile|Settings|GetSpeed)))
  (Variables|/Script/Engine.ProjectileMovementComponent|SetMaxSpeed _projectilemovement _output_get)
  (Variables|/Script/Engine.ProjectileMovementComponent|SetProjectileGravityScale _projectilemovement 0.0))