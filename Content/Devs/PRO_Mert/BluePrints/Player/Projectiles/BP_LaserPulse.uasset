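; BP_LaserPulse is a player laser shot that displays a Niagara beam along its forward direction over the weapon range.
; On BeginPlay it reads damage from MainGameInstance, runs a debug-drawn sphere trace along that line and sets the beam's color, end and shell scale.
; The trace result is unused and no damage is applied; the EnergyGun damage scaling is disconnected and never runs.
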(event EventBeginPlay
  (bind _returnvalue (Transformation|GetActorLocation))
  (bind _ns_laser (Variables|Default|GetNS_Laser))
  (bind _weapon_range (Variables|Default|GetWeapon%20Range))
  (bind _ns_laser_2 (Variables|Default|GetNS_Laser))
  (bind _returnvalue_2 (Math|Vector|GetForwardVector _ns_laser))
  (bind _returnvalue_3 (* _returnvalue_2 _weapon_range))
  (bind _asmain_game_instance (Utilities|Casting|CastToMainGameInstance (Game|GetGameInstance)))
  (Variables|Projectile|Settings|SetDamage (Variables|/Game/Devs/PRO_Mert/BluePrints/Player/MISC/MainGameInstance.MainGameInstance_C|GetLaserDamage _asmain_game_instance))
  (bind _outhit (Collision|SphereTraceByChannel _returnvalue (+ _returnvalue _returnvalue_3) 5e+01 "TraceTypeQuery1" false 0 "ForDuration"))
  (Effects|Components|ParticleSystem|SetColorParameter _ns_laser_2 "Beam Color" (Variables|Default|GetBeam%20Color))
  (Effects|Components|ParticleSystem|SetVectorParameter _ns_laser_2 "Beam End" _returnvalue_3)
  (Effects|Components|ParticleSystem|SetVectorParameter _ns_laser_2 "Beam Shell Scale" (Math|Vector|MakeVector (Math|Vector|VectorLength _returnvalue_3) 1e+01 1e+01)))

(fn ConstructionScript)