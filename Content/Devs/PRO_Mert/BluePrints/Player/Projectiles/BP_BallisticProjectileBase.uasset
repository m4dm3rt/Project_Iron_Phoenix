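; Base class for a player ballistic projectile that damages asteroids, swarm, sniper and bomber enemies, and bomber projectiles on overlap.
; Construction sets a straight, gravity-free flight at a configurable speed.
; BeginPlay scales damage up or down from BP_SingleplayerCharacter's gun energy setting; the other character variants get no adjustment.
; Hits spawn an effect and destroy the projectile; non-asteroid targets also trigger the crosshair hitmarker and a sound.
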(event OnComponentBeginOverlap(SphereCollision)
  (params (OverlappedComponent :type Primitive%20Component%20Object%20Reference) (OtherActor :type Actor%20Object%20Reference) (OtherComp :type Primitive%20Component%20Object%20Reference) (OtherBodyIndex :type Integer) (bFromSweep :type Boolean) (SweepResult :type Hit%20Result%20Structure%20%28by%20ref%29))
  (bind _damage (Variables|Projectile|Settings|GetDamage))
  (bind _asbp_asteroid (Utilities|Casting|CastToBP_Asteroid OtherActor)
    (:then
      (Game|Damage|ApplyDamage _asbp_asteroid _damage 0 0)
      (Effects|SpawnEmitteratLocation "/Game/Realistic_Starter_VFX_Pack_Vol2/Particles/Hit/P_Default.P_Default" (Transformation|GetActorLocation) "0, 0, 0" "20.000000,20.000000,20.000000")
      (Actor|DestroyActor))
    (:CastFailed
      (bind _asbp_enemy_swarm (Utilities|Casting|CastToBP_EnemySwarm OtherActor)
        (:then
          (Game|Damage|ApplyDamage _asbp_enemy_swarm _damage 0 0))
        (:CastFailed
          (bind _asbp_enemy_sniper (Utilities|Casting|CastToBP_EnemySniper OtherActor)
            (:then
              (Game|Damage|ApplyDamage _asbp_enemy_sniper _damage 0 0))
            (:CastFailed
              (bind _asbp_enemy_bomber (Utilities|Casting|CastToBP_EnemyBomber OtherActor)
                (:then
                  (Game|Damage|ApplyDamage _asbp_enemy_bomber _damage 0 0))
                (:CastFailed
                  (bind _asbp_projectile_bomber (Utilities|Casting|CastToBP_ProjectileBomber OtherActor))
                  (Game|Damage|ApplyDamage _asbp_projectile_bomber _damage 0 0)))))))
      (Effects|SpawnEmitteratLocation "/Game/Realistic_Starter_VFX_Pack_Vol2/Particles/Hit/P_Default.P_Default" (Transformation|GetActorLocation) "0, 0, 0" "10.000000,10.000000,10.000000")
      (bind _foundwidgets (Widget|GetAllWidgetsOfClass "/Game/Devs/PRO_Mert/BluePrints/Player/Widgets/PlayerCrosshair_W.PlayerCrosshair_W_C" false))
      (Default|Hitmarker (Utilities|Array|Get(acopy) _foundwidgets))
      (Audio|PlaySound2D "/Game/Devs/GD_Alex/Sounds/Ambience/SFX_Collide.SFX_Collide" 0.5 1.0 0.0 0 0 false) ; Hit Audio
      (Actor|DestroyActor))))

(event EventBeginPlay
  (bind _returnvalue (Game|Player|GetPlayerPawn 0))
  (bind (_asbp_singleplayer_character _bsuccess) (Utilities|Casting|CastToBP_SingleplayerCharacter _returnvalue))
  (bind _energygun (Variables|/Game/Devs/PRO_Mert/BluePrints/Player/Actors/BP_SingleplayerCharacter.BP_SingleplayerCharacter_C|GetEnergyGun _asbp_singleplayer_character))
  (if _bsuccess
    (if (> _energygun 5e+01)
      (Variables|Projectile|Settings|SetDamage (* (Variables|Projectile|Settings|GetDamage) (Variables|/Game/Devs/PRO_Mert/BluePrints/Player/Actors/BP_SingleplayerCharacter.BP_SingleplayerCharacter_C|GetEnergyGunValue _asbp_singleplayer_character)))
      (elif (< _energygun 5e+01)
        (Variables|Projectile|Settings|SetDamage (/ (Variables|Projectile|Settings|GetDamage) (Variables|/Game/Devs/PRO_Mert/BluePrints/Player/Actors/BP_SingleplayerCharacter.BP_SingleplayerCharacter_C|GetEnergyGunValue _asbp_singleplayer_character)))))
    (elif (not (.bSuccess (Utilities|Casting|CastToBP_SingleplayerCharacterAlexJ _returnvalue)))
      (if (.bSuccess (Utilities|Casting|CastToBP_SingleplayerCharacterMarius _returnvalue))
        _))))

(fn ConstructionScript
  (bind _projectilemovement (Variables|Default|GetProjectileMovement))
  (bind _output_get (Variables|/Script/Engine.ProjectileMovementComponent|SetInitialSpeed _projectilemovement (Variables|Projectile|Settings|GetSpeed)))
  (Variables|/Script/Engine.ProjectileMovementComponent|SetMaxSpeed _projectilemovement _output_get)
  (Variables|/Script/Engine.ProjectileMovementComponent|SetProjectileGravityScale _projectilemovement 0.0))