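; Player laser battery projectile that flies without gravity and takes its damage from the game instance.
; On capsule overlap it damages asteroids at double rate and destroys itself, or damages one of four enemy types at base rate.
; Enemy hits trigger the crosshair hitmarker, sound and Niagara effect, then remove movement, collision and mesh components without destroying the actor.
; A polling homing event exists, but its targeting trigger and the energy-based damage scaling are disconnected.
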(event OnComponentBeginOverlap(Capsule)
  (params (OverlappedComponent :type Primitive%20Component%20Object%20Reference) (OtherActor :type Actor%20Object%20Reference) (OtherComp :type Primitive%20Component%20Object%20Reference) (OtherBodyIndex :type Integer) (bFromSweep :type Boolean) (SweepResult :type Hit%20Result%20Structure%20%28by%20ref%29))
  (bind _damage (Variables|Projectile|Settings|GetDamage))
  (bind _asbp_asteroid (Utilities|Casting|CastToBP_Asteroid OtherActor)
    (:then
      (Game|Damage|ApplyDamage _asbp_asteroid (* _damage 2.0) 0 0 "/Game/Devs/PRO_Mert/BluePrints/Player/Projectiles/DT_LaserBattery.DT_LaserBattery_C")
      (Actor|DestroyActor))
    (:CastFailed
      (bind _asbp_enemy_swarm (Utilities|Casting|CastToBP_EnemySwarm OtherActor)
        (:then
          (Game|Damage|ApplyDamage _asbp_enemy_swarm _damage 0 0 "/Game/Devs/PRO_Mert/BluePrints/Player/Projectiles/DT_LaserBattery.DT_LaserBattery_C"))
        (:CastFailed
          (bind _asbp_enemy_sniper (Utilities|Casting|CastToBP_EnemySniper OtherActor)
            (:then
              (Game|Damage|ApplyDamage _asbp_enemy_sniper _damage 0 0 "/Game/Devs/PRO_Mert/BluePrints/Player/Projectiles/DT_LaserBattery.DT_LaserBattery_C"))
            (:CastFailed
              (bind _asbp_enemy_bomber (Utilities|Casting|CastToBP_EnemyBomber OtherActor)
                (:then
                  (Game|Damage|ApplyDamage _asbp_enemy_bomber _damage 0 0 "/Game/Devs/PRO_Mert/BluePrints/Player/Projectiles/DT_LaserBattery.DT_LaserBattery_C"))
                (:CastFailed
                  (bind _asbp_enemy_drone (Utilities|Casting|CastToBP_EnemyDrone OtherActor))
                  (Game|Damage|ApplyDamage _asbp_enemy_drone _damage 0 0 "/Game/Devs/PRO_Mert/BluePrints/Player/Projectiles/DT_LaserBattery.DT_LaserBattery_C")))))))
      (CallFunction|DestroyProjectile))))

(event Custom|HomingProjectile
  (params (Target :type Actor%20Object%20Reference))
  (bind _projectilemovement (Variables|Default|GetProjectileMovement))
  ;[1 0.1979 0.1979] Homing Logic
  (if (< (Math|Vector|VectorLength (- (Transformation|GetActorLocation Target) (Transformation|GetActorLocation))) (Variables|Projectile|Conditions|GetHomingRadius))
    (Variables|/Script/Engine.ProjectileMovementComponent|SetHomingTargetComponent _projectilemovement (Variables|/Script/Engine.Actor|GetRootComponent Target))
    (Variables|/Script/Engine.ProjectileMovementComponent|SetbIsHomingProjectile _projectilemovement true))
  (if (< (Math|Vector|VectorLength (- (Transformation|GetActorLocation Target) (Transformation|GetActorLocation))) (Variables|Projectile|Conditions|GetClosestDistance))
    (Game|Damage|ApplyDamage Target (Variables|Projectile|Settings|GetDamage) 0 0 "/Game/Devs/PRO_Mert/BluePrints/Player/Projectiles/DT_LaserBattery.DT_LaserBattery_C")
    (CallFunction|DestroyProjectile)
    (else
      (Utilities|FlowControl|Delay 0.2)
      (CallFunction|HomingProjectile Target))))

(event EventBeginPlay
  (bind _asmain_game_instance (Utilities|Casting|CastToMainGameInstance (Game|GetGameInstance)))
  (Variables|Projectile|Settings|SetDamage (Variables|/Game/Devs/PRO_Mert/BluePrints/Player/MISC/MainGameInstance.MainGameInstance_C|GetLaserDamage _asmain_game_instance)))

(fn ConstructionScript
  (bind _projectilemovement (Variables|Default|GetProjectileMovement))
  (bind _output_get (Variables|/Script/Engine.ProjectileMovementComponent|SetInitialSpeed _projectilemovement (Variables|Projectile|Settings|GetSpeed)))
  (Variables|/Script/Engine.ProjectileMovementComponent|SetMaxSpeed _projectilemovement _output_get)
  (Variables|/Script/Engine.ProjectileMovementComponent|SetProjectileGravityScale _projectilemovement 0.0)
  (Utilities|Casting|CastToMainGameInstance (Game|GetGameInstance)))

(fn DestroyProjectile
  (bind _foundwidgets (Widget|GetAllWidgetsOfClass "/Game/Devs/PRO_Mert/BluePrints/UI/HUD/PlayerCrosshair_WBP.PlayerCrosshair_WBP_C" false))
  (Default|Hitmarker (Utilities|Array|Get(acopy) _foundwidgets))
  (Audio|PlaySound2D "/Game/Devs/PRO_Mert/Sounds/SFX_Hitmarker.SFX_Hitmarker" 1.0 (Math|Random|RandomFloatinRange 0.9 1.1) 0.0 0 0 false)
  (Components|Activation|Activate (Variables|Default|GetNS_Hit_LaserBattery) true)
  (Components|DestroyComponent (Variables|Default|GetProjectileMovement)))