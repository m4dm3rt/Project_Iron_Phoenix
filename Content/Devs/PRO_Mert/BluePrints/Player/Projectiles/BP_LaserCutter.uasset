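; Player laser cutter projectile that damages asteroids, buoys and enemies on overlap, with base damage read from the game instance.
; A cast chain on the overlapped actor deals double damage to asteroids, asteroid rings and buoys, and normal damage to the four enemy types.
; Hits play an impact Niagara effect and remove the movement, mesh and collision components rather than the actor.
; Enemy hits also trigger the player's crosshair hitmarker and sound.
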(event OnComponentBeginOverlap(SphereCollision)
  (params (OverlappedComponent :type Primitive%20Component%20Object%20Reference) (OtherActor :type Actor%20Object%20Reference) (OtherComp :type Primitive%20Component%20Object%20Reference) (OtherBodyIndex :type Integer) (bFromSweep :type Boolean) (SweepResult :type Hit%20Result%20Structure%20%28by%20ref%29))
  (bind _returnvalue (Transformation|GetActorLocation))
  (bind _returnvalue_2 (Collision|MakeHitResult false false 0.0 0.0 "0, 0, 0" "0, 0, 0" "0,0,1" "0,0,1" 0 0))
  (bind _instigator (Variables|Actor|GetInstigator))
  (bind _damage (Variables|Projectile|Settings|GetDamage))
  (bind _returnvalue_3 (* _damage 2.0))
  (bind _asbp_asteroid_ring (Utilities|Casting|CastToBP_AsteroidRing OtherActor)
    (:then
      (Game|Damage|ApplyPointDamage _asbp_asteroid_ring _returnvalue_3 _returnvalue _returnvalue_2 0 _instigator "/Game/Devs/PRO_Mert/BluePrints/Player/DamageTypes/DT_LaserCutter.DT_LaserCutter_C")
      (CallFunction|DestroyProjectileWorld :!label _label))
    (:CastFailed
      (bind _asbp_single_asteroid_ring (Utilities|Casting|CastToBP_SingleAsteroidRing OtherActor)
        (:then
          (Game|Damage|ApplyDamage _asbp_single_asteroid_ring _returnvalue_3 0 _instigator "/Game/Devs/PRO_Mert/BluePrints/Player/DamageTypes/DT_LaserCutter.DT_LaserCutter_C")
          (goto _label))
        (:CastFailed
          (bind _asbp_asteroid (Utilities|Casting|CastToBP_Asteroid OtherActor)
            (:then
              (Game|Damage|ApplyDamage _asbp_asteroid _returnvalue_3 0 _instigator "/Game/Devs/PRO_Mert/BluePrints/Player/DamageTypes/DT_LaserCutter.DT_LaserCutter_C")
              (goto _label))
            (:CastFailed
              (bind _asbp_buoy (Utilities|Casting|CastToBP_Buoy OtherActor)
                (:then
                  (Game|Damage|ApplyPointDamage _asbp_buoy _returnvalue_3 _returnvalue _returnvalue_2 0 _instigator "/Game/Devs/PRO_Mert/BluePrints/Player/DamageTypes/DT_LaserCutter.DT_LaserCutter_C")
                  (goto _label))
                (:CastFailed
                  (bind _asbp_enemy_swarm (Utilities|Casting|CastToBP_EnemySwarm OtherActor)
                    (:then
                      (Game|Damage|ApplyDamage _asbp_enemy_swarm _damage 0 _instigator "/Game/Devs/PRO_Mert/BluePrints/Player/DamageTypes/DT_LaserCutter.DT_LaserCutter_C"))
                    (:CastFailed
                      (bind _asbp_enemy_sniper (Utilities|Casting|CastToBP_EnemySniper OtherActor)
                        (:then
                          (Game|Damage|ApplyDamage _asbp_enemy_sniper _damage 0 _instigator "/Game/Devs/PRO_Mert/BluePrints/Player/DamageTypes/DT_LaserCutter.DT_LaserCutter_C"))
                        (:CastFailed
                          (bind _asbp_enemy_bomber (Utilities|Casting|CastToBP_EnemyBomber OtherActor)
                            (:then
                              (Game|Damage|ApplyDamage _asbp_enemy_bomber _damage 0 _instigator "/Game/Devs/PRO_Mert/BluePrints/Player/DamageTypes/DT_LaserCutter.DT_LaserCutter_C"))
                            (:CastFailed
                              (bind _asbp_enemy_drone (Utilities|Casting|CastToBP_EnemyDrone OtherActor))
                              (Game|Damage|ApplyDamage _asbp_enemy_drone _damage 0 _instigator "/Game/Devs/PRO_Mert/BluePrints/Player/DamageTypes/DT_LaserCutter.DT_LaserCutter_C")))))))
                  (CallFunction|DestroyProjectileEnemy))))))))))

(event EventBeginPlay
  (bind _asmain_game_instance (Utilities|Casting|CastToMainGameInstance (Game|GetGameInstance)))
  (Variables|Projectile|Settings|SetDamage (Variables|/Game/Devs/PRO_Mert/BluePrints/Player/MISC/MainGameInstance.MainGameInstance_C|GetLaserDamage _asmain_game_instance)))

(fn ConstructionScript
  (bind _projectilemovement (Variables|Default|GetProjectileMovement))
  (bind _output_get (Variables|/Script/Engine.ProjectileMovementComponent|SetInitialSpeed _projectilemovement (Variables|Projectile|Settings|GetSpeed)))
  (Variables|/Script/Engine.ProjectileMovementComponent|SetMaxSpeed _projectilemovement _output_get))

(fn DestroyProjectileEnemy
  (bind _returnvalue (Actor|GetActorOfClass "/Game/Devs/PRO_Mert/BluePrints/Player/MISC/BP_SingleplayerCharacter.BP_SingleplayerCharacter_C"))
  (Default|Hitmarker (Variables|/Game/Devs/PRO_Mert/BluePrints/Player/MISC/BP_SingleplayerCharacter.BP_SingleplayerCharacter_C|GetPlayerCrosshair%20REF _returnvalue))
  (Audio|PlaySound2D "/Game/Devs/PRO_Mert/Sounds/SFX_Hitmarker.SFX_Hitmarker" 1.0 (Math|Random|RandomFloatinRange 0.9 1.1) 0.0 0 0 false)
  (Components|Activation|Activate (Variables|Default|GetNS_Hit_LaserCutter) true)
  (Components|DestroyComponent (Variables|Default|GetProjectileMovement)))

(fn DestroyProjectileWorld
  (Components|Activation|Activate (Variables|Default|GetNS_Hit_LaserCutter) true)
  (Components|DestroyComponent (Variables|Default|GetProjectileMovement)))