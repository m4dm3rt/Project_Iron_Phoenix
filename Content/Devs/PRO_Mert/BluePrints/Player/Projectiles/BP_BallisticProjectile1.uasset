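; BP_BallisticProjectile1 is a gravity-free, constant-speed player ballistic projectile for single-player.
; At BeginPlay it takes its damage from the player character, scaling it up or down by the EnergyGun setting.
; On overlap it damages asteroids, swarm, sniper and bomber enemies, or bomber projectiles, then destroys itself.
; All hits except asteroids use the ballistic damage type and trigger a crosshair hitmarker with a pitch-randomized sound.
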(event OnComponentBeginOverlap(SphereCollision)
  (params (OverlappedComponent :type Primitive%20Component%20Object%20Reference) (OtherActor :type Actor%20Object%20Reference) (OtherComp :type Primitive%20Component%20Object%20Reference) (OtherBodyIndex :type Integer) (bFromSweep :type Boolean) (SweepResult :type Hit%20Result%20Structure%20%28by%20ref%29))
  (bind _damage (Variables|Projectile|Settings|GetDamage))
  (bind _asbp_asteroid_1 (Utilities|Casting|CastToBP_Asteroid OtherActor)
    (:then
      (Game|Damage|ApplyDamage _asbp_asteroid_1 _damage 0 0)
      (Actor|DestroyActor))
    (:CastFailed
      (bind _asbp_enemy_swarm (Utilities|Casting|CastToBP_EnemySwarm OtherActor)
        (:then
          (Game|Damage|ApplyDamage _asbp_enemy_swarm _damage 0 0 "/Game/Devs/PRO_Mert/BluePrints/Player/Projectiles/DT_Ballistic.DT_Ballistic_C"))
        (:CastFailed
          (bind _asbp_enemy_sniper (Utilities|Casting|CastToBP_EnemySniper OtherActor)
            (:then
              (Game|Damage|ApplyDamage _asbp_enemy_sniper _damage 0 0 "/Game/Devs/PRO_Mert/BluePrints/Player/Projectiles/DT_Ballistic.DT_Ballistic_C"))
            (:CastFailed
              (bind _asbp_enemy_bomber (Utilities|Casting|CastToBP_EnemyBomber OtherActor)
                (:then
                  (Game|Damage|ApplyDamage _asbp_enemy_bomber _damage 0 0 "/Game/Devs/PRO_Mert/BluePrints/Player/Projectiles/DT_Ballistic.DT_Ballistic_C"))
                (:CastFailed
                  (bind _asbp_projectile_bomber (Utilities|Casting|CastToBP_ProjectileBomber OtherActor))
                  (Game|Damage|ApplyDamage _asbp_projectile_bomber _damage 0 0 "/Game/Devs/PRO_Mert/BluePrints/Player/Projectiles/DT_Ballistic.DT_Ballistic_C")))))))
      (bind _foundwidgets (Widget|GetAllWidgetsOfClass "/Game/Devs/PRO_Mert/BluePrints/Player/Widgets/PlayerCrosshair_W.PlayerCrosshair_W_C" false))
      (Default|Hitmarker (Utilities|Array|Get(acopy) _foundwidgets))
      (Audio|PlaySound2D "/Game/Devs/PRO_Mert/Sounds/SFX_Hitmarker.SFX_Hitmarker" 1.0 (Math|Random|RandomFloatinRange 0.9 1.1) 0.0 0 0 false) ; Hit Audio
      (Actor|DestroyActor))))

(event EventBeginPlay
  (bind _asbp_singleplayer_character (Utilities|Casting|CastToBP_SingleplayerCharacter (Game|Player|GetPlayerPawn 0)))
  (Variables|Projectile|Settings|SetDamage (Variables|/Game/Devs/PRO_Mert/BluePrints/Player/Actors/BP_SingleplayerCharacter.BP_SingleplayerCharacter_C|GetBallistic1Damage _asbp_singleplayer_character))
  (if (> (Variables|/Game/Devs/PRO_Mert/BluePrints/Player/Actors/BP_SingleplayerCharacter.BP_SingleplayerCharacter_C|GetEnergyGun _asbp_singleplayer_character) 5e+01)
    (Variables|Projectile|Settings|SetDamage (* (Variables|Projectile|Settings|GetDamage) (Variables|/Game/Devs/PRO_Mert/BluePrints/Player/Actors/BP_SingleplayerCharacter.BP_SingleplayerCharacter_C|GetEnergyGunValue _asbp_singleplayer_character)))
    (elif (< (Variables|/Game/Devs/PRO_Mert/BluePrints/Player/Actors/BP_SingleplayerCharacter.BP_SingleplayerCharacter_C|GetEnergyGun _asbp_singleplayer_character) 5e+01)
      (Variables|Projectile|Settings|SetDamage (/ (Variables|Projectile|Settings|GetDamage) (Variables|/Game/Devs/PRO_Mert/BluePrints/Player/Actors/BP_SingleplayerCharacter.BP_SingleplayerCharacter_C|GetEnergyGunValue _asbp_singleplayer_character))))))

(fn ConstructionScript
  (bind _projectilemovement (Variables|Default|GetProjectileMovement))
  (bind _output_get (Variables|/Script/Engine.ProjectileMovementComponent|SetInitialSpeed _projectilemovement (Variables|Projectile|Settings|GetSpeed)))
  (Variables|/Script/Engine.ProjectileMovementComponent|SetMaxSpeed _projectilemovement _output_get)
  (Variables|/Script/Engine.ProjectileMovementComponent|SetProjectileGravityScale _projectilemovement 0.0))