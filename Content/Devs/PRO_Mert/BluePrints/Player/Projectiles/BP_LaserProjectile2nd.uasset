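; Player laser projectile that damages asteroids, swarm enemies and sniper enemies, then spawns an impact emitter and destroys itself.
; Each tick detects hits with a 2000-unit sphere trace along the laser mesh's up vector.
; A self-repeating HomingProjectile event, not called within this graph, steers toward the closest swarm enemy found, without resetting the stored closest distance.
; The construction script sets a constant speed with no gravity.
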(event Custom|HomingProjectile
  ;[1 0.2969 0.2969] Homing Logic
  (Variables|/Script/Engine.ProjectileMovementComponent|SetbIsHomingProjectile (Variables|Default|GetProjectileMovement) true)
  (bind _outactors (Actor|GetAllActorsOfClass "/Game/Devs/PRO_Mert/BluePrints/Enemies/Actors/BP_EnemySwarm.BP_EnemySwarm_C"))
  (for _array_element _outactors
    (if (< (Math|Vector|VectorLength (- (Transformation|GetActorLocation _array_element) (Transformation|GetActorLocation))) (Variables|Projectile|Conditions|GetClosest%20Distance))
      (Variables|Projectile|Conditions|SetClosest%20Distance (Math|Vector|VectorLength (- (Transformation|GetActorLocation _array_element) (Transformation|GetActorLocation))))
      (Variables|Projectile|References|SetTarget _array_element)))
  (Variables|/Script/Engine.ProjectileMovementComponent|SetHomingTargetComponent (Variables|Default|GetProjectileMovement) (Variables|/Game/Devs/PRO_Mert/BluePrints/Enemies/Actors/BP_EnemySwarm.BP_EnemySwarm_C|GetSpaceFighter (Variables|Projectile|References|GetTarget)))
  (Utilities|FlowControl|Delay 0.02)
  (CallFunction|HomingProjectile))

(event EventTick
  (params (DeltaSeconds :type Float%20%28single-precision%29))
  (bind _damage (Variables|Projectile|Settings|GetDamage))
  (bind _lasermesh (Variables|Default|GetLaserMesh))
  (bind _returnvalue (Transformation|GetWorldLocation _lasermesh))
  (bind (_outhit _returnvalue_2) (Collision|SphereTraceByChannel _returnvalue (+ _returnvalue (* (Math|Vector|GetUpVector (Transformation|GetWorldRotation _lasermesh)) 2e+03)) 5e+01 "TraceTypeQuery1" false 0 "None"))
  (if _returnvalue_2
    (bind _asbp_asteroid (Utilities|Casting|CastToBP_Asteroid (.HitActor (Collision|BreakHitResult _outhit)))
      (:then
        (Game|Damage|ApplyDamage _asbp_asteroid _damage 0 0))
      (:CastFailed
        (bind _asbp_enemy_swarm (Utilities|Casting|CastToBP_EnemySwarm (.HitActor (Collision|BreakHitResult _outhit)))
          (:then
            (Game|Damage|ApplyDamage _asbp_enemy_swarm _damage 0 0))
          (:CastFailed
            (bind _asbp_enemy_sniper (Utilities|Casting|CastToBP_EnemySniper (.HitActor (Collision|BreakHitResult _outhit))))
            (Game|Damage|ApplyDamage _asbp_enemy_sniper _damage 0 0)))))
    (Effects|SpawnEmitteratLocation "/Game/Realistic_Starter_VFX_Pack_Vol2/Particles/Hit/P_Default.P_Default" (.Location (Collision|BreakHitResult _outhit)) "0, 0, 0" "50.000000,50.000000,50.000000")
    (Actor|DestroyActor)))

(fn ConstructionScript
  (bind _projectilemovement (Variables|Default|GetProjectileMovement))
  (bind _output_get (Variables|/Script/Engine.ProjectileMovementComponent|SetInitialSpeed _projectilemovement (Variables|Projectile|Settings|GetSpeed)))
  (Variables|/Script/Engine.ProjectileMovementComponent|SetMaxSpeed _projectilemovement _output_get)
  (Variables|/Script/Engine.ProjectileMovementComponent|SetProjectileGravityScale _projectilemovement 0.0))