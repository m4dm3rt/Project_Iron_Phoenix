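; Kinetic minigun projectile that flies without gravity at a set speed and damages asteroids and enemies on overlap.
; On BeginPlay it reads its damage from MainGameInstance.
; Sphere overlaps use a cast chain: asteroids take double damage, while swarm, sniper and bomber enemies take base damage and trigger the crosshair hitmarker with a pitch-varied sound.
; The projectile destroys itself after these hits; an EnergyGun damage-scaling branch is unconnected and never runs.
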(event OnComponentBeginOverlap(SphereCollision)
  (params (OverlappedComponent :type Primitive%20Component%20Object%20Reference) (OtherActor :type Actor%20Object%20Reference) (OtherComp :type Primitive%20Component%20Object%20Reference) (OtherBodyIndex :type Integer) (bFromSweep :type Boolean) (SweepResult :type Hit%20Result%20Structure%20%28by%20ref%29))
  (bind _damage (Variables|Projectile|Settings|GetDamage))
  (bind _asbp_asteroid (Utilities|Casting|CastToBP_Asteroid OtherActor)
    (:then
      (Game|Damage|ApplyDamage _asbp_asteroid (* _damage 2.0) 0 0 "/Game/Devs/PRO_Mert/BluePrints/Player/Projectiles/DT_KineticMinigun.DT_KineticMinigun_C")
      (Actor|DestroyActor))
    (:CastFailed
      (bind _asbp_enemy_swarm (Utilities|Casting|CastToBP_EnemySwarm OtherActor)
        (:then
          (Game|Damage|ApplyDamage _asbp_enemy_swarm _damage 0 0 "/Game/Devs/PRO_Mert/BluePrints/Player/Projectiles/DT_KineticMinigun.DT_KineticMinigun_C"))
        (:CastFailed
          (bind _asbp_enemy_sniper (Utilities|Casting|CastToBP_EnemySniper OtherActor)
            (:then
              (Game|Damage|ApplyDamage _asbp_enemy_sniper _damage 0 0 "/Game/Devs/PRO_Mert/BluePrints/Player/Projectiles/DT_KineticMinigun.DT_KineticMinigun_C"))
            (:CastFailed
              (bind _asbp_enemy_bomber (Utilities|Casting|CastToBP_EnemyBomber OtherActor))
              (Game|Damage|ApplyDamage _asbp_enemy_bomber _damage 0 0 "/Game/Devs/PRO_Mert/BluePrints/Player/Projectiles/DT_KineticMinigun.DT_KineticMinigun_C")))))
      (bind _foundwidgets (Widget|GetAllWidgetsOfClass "/Game/Devs/PRO_Mert/BluePrints/Player/Widgets/PlayerCrosshair_W.PlayerCrosshair_W_C" false))
      (Default|Hitmarker (Utilities|Array|Get(acopy) _foundwidgets))
      (Audio|PlaySound2D "/Game/Devs/PRO_Mert/Sounds/SFX_Hitmarker.SFX_Hitmarker" 1.0 (Math|Random|RandomFloatinRange 0.9 1.1) 0.0 0 0 false)
      (Actor|DestroyActor))))

(event EventBeginPlay
  (bind _asmain_game_instance (Utilities|Casting|CastToMainGameInstance (Game|GetGameInstance)))
  (Variables|Projectile|Settings|SetDamage (Variables|/Game/Devs/PRO_Mert/BluePrints/Player/MISC/MainGameInstance.MainGameInstance_C|GetKineticDamage _asmain_game_instance)))

(fn ConstructionScript
  (bind _projectilemovement (Variables|Default|GetProjectileMovement))
  (bind _output_get (Variables|/Script/Engine.ProjectileMovementComponent|SetInitialSpeed _projectilemovement (Variables|Projectile|Settings|GetSpeed)))
  (Variables|/Script/Engine.ProjectileMovementComponent|SetMaxSpeed _projectilemovement _output_get)
  (Variables|/Script/Engine.ProjectileMovementComponent|SetProjectileGravityScale _projectilemovement 0.0))