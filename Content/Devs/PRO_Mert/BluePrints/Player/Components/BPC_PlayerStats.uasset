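; Player stats component that holds health, shield and stamina, with functions to decrease, regenerate and raise the maximum of each.
; It caches the player character on BeginPlay and pushes health and shield ratios to its HUD bars, though DecreaseHealth and IncreaseMaxHealth write to the shield bar.
; Health drops only when NoShield is set, and decrease functions report depletion.
; Stamina has no HUD update, and GainXP is an empty stub.
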(event EventBeginPlay
  (bind _asbp_player_character (Utilities|Casting|CastToBP_PlayerCharacter (Game|Player|GetPlayerPawn 0)))
  (Variables|Default|SetPlayer%20REF _asbp_player_character))

(fn DecreaseHealth
  (params (NoShield :type Boolean) (Damage%20Received :type Float%20%28double-precision%29))
  (if NoShield
    (bind _output_get (Variables|Health|SetHealth (- (Variables|Health|GetHealth) Damage%20Received)))
    (Progress|SetPercent (Variables|/Game/Devs/PRO_Mert/BluePrints/Widgets/Player/PlayerHUD_W.PlayerHUD_W_C|GetProgressBar_Shield (Variables|/Game/Devs/PRO_Mert/BluePrints/Player/BP_PlayerCharacter.BP_PlayerCharacter_C|GetPlayerHUD%20REF (Variables|Default|GetPlayer%20REF))) (/ _output_get (Variables|Health|GetMax%20Health)))
    (if (<= _output_get 0.0)
      (return true)
      (else
        (return false)))))

(fn RegenerateHealth
  (params (Health%20Increase :type Float%20%28double-precision%29))
  (bind _output_get (Variables|Health|SetHealth (+ (Variables|Health|GetHealth) Health%20Increase)))
  (if (> _output_get (Variables|Health|GetMax%20Health))
    (bind _output_get_2 (Variables|Health|SetHealth (Variables|Health|GetMax%20Health))))
  (Progress|SetPercent (Variables|/Game/Devs/PRO_Mert/BluePrints/Widgets/Player/PlayerHUD_W.PlayerHUD_W_C|GetProgressBar_Health (Variables|/Game/Devs/PRO_Mert/BluePrints/Player/BP_PlayerCharacter.BP_PlayerCharacter_C|GetPlayerHUD%20REF (Variables|Default|GetPlayer%20REF))) (/ _output_get_2 (Variables|Health|GetMax%20Health))))

(fn IncreaseMaxHealth
  (params (Max%20Health%20Increase :type Float%20%28double-precision%29))
  (Variables|Health|SetMax%20Health (+ (Variables|Health|GetMax%20Health) Max%20Health%20Increase))
  (Progress|SetPercent (Variables|/Game/Devs/PRO_Mert/BluePrints/Widgets/Player/PlayerHUD_W.PlayerHUD_W_C|GetProgressBar_Shield (Variables|/Game/Devs/PRO_Mert/BluePrints/Player/BP_PlayerCharacter.BP_PlayerCharacter_C|GetPlayerHUD%20REF (Variables|Default|GetPlayer%20REF))) (/ (Variables|Health|GetHealth) (Variables|Health|GetMax%20Health))))

(fn GainXP)

(fn DecreaseShield
  (params (Damage%20Received :type Float%20%28double-precision%29))
  (bind _output_get (Variables|Shield|SetShield (- (Variables|Shield|GetShield) Damage%20Received)))
  (Progress|SetPercent (Variables|/Game/Devs/PRO_Mert/BluePrints/Widgets/Player/PlayerHUD_W.PlayerHUD_W_C|GetProgressBar_Shield (Variables|/Game/Devs/PRO_Mert/BluePrints/Player/BP_PlayerCharacter.BP_PlayerCharacter_C|GetPlayerHUD%20REF (Variables|Default|GetPlayer%20REF))) (/ _output_get (Variables|Shield|GetMax%20Shield)))
  (if (<= _output_get 0.0)
    (return true)
    (else
      (return false))))

(fn RegenerateShield
  (params (Shield%20Recovery :type Float%20%28double-precision%29))
  (bind _output_get (Variables|Shield|SetShield (+ (Variables|Shield|GetShield) Shield%20Recovery)))
  (if (> _output_get (Variables|Shield|GetMax%20Shield))
    (bind _output_get_2 (Variables|Shield|SetShield (Variables|Shield|GetMax%20Shield))))
  (Progress|SetPercent (Variables|/Game/Devs/PRO_Mert/BluePrints/Widgets/Player/PlayerHUD_W.PlayerHUD_W_C|GetProgressBar_Shield (Variables|/Game/Devs/PRO_Mert/BluePrints/Player/BP_PlayerCharacter.BP_PlayerCharacter_C|GetPlayerHUD%20REF (Variables|Default|GetPlayer%20REF))) (/ _output_get_2 (Variables|Shield|GetMax%20Shield)))
  (if (== (Variables|Shield|GetShield) (Variables|Shield|GetMax%20Shield))
    (return true)
    (else
      (return false))))

(fn IncreaseMaxShield
  (params (Max%20Shield%20Increase :type Float%20%28double-precision%29))
  (Variables|Shield|SetMax%20Shield (+ (Variables|Shield|GetMax%20Shield) Max%20Shield%20Increase))
  (Progress|SetPercent (Variables|/Game/Devs/PRO_Mert/BluePrints/Widgets/Player/PlayerHUD_W.PlayerHUD_W_C|GetProgressBar_Shield (Variables|/Game/Devs/PRO_Mert/BluePrints/Player/BP_PlayerCharacter.BP_PlayerCharacter_C|GetPlayerHUD%20REF (Variables|Default|GetPlayer%20REF))) (/ (Variables|Shield|GetShield) (Variables|Shield|GetMax%20Shield))))

(fn DecreaseStamina
  (params (Stamina%20Decrease :type Float%20%28double-precision%29))
  (bind _output_get (Variables|Stamina|SetStamina (- (Variables|Stamina|GetStamina) Stamina%20Decrease)))
  (if (<= _output_get 0.0)
    (return true)
    (else
      (return false))))

(fn RegenerateStamina
  (params (Stamina%20Increase :type Float%20%28double-precision%29))
  (bind _output_get (Variables|Stamina|SetStamina (+ (Variables|Stamina|GetStamina) Stamina%20Increase)))
  (if (> _output_get (Variables|Stamina|GetMax%20Stamina))
    (Variables|Stamina|SetStamina (Variables|Stamina|GetMax%20Stamina))))

(fn IncreaseMaxStamina
  (params (Max%20Stamina%20Increase :type Float%20%28double-precision%29))
  (Variables|Stamina|SetMax%20Stamina (+ (Variables|Stamina|GetMax%20Stamina) Max%20Stamina%20Increase)))