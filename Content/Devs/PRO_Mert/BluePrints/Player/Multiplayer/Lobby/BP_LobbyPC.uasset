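; Multiplayer lobby player controller that creates the local player's lobby UI and reports their lobby info to BP_LobbyGM.
; On BeginPlay, SetUp configures cursor, input mode and Lobby_W for the local controller, then lobby info is pushed to the game mode, including after a short delay.
; ReadyStatusServer toggles the ready flag and updates the game mode.
; OnStartGame shows the loading screen and disables input.
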(event Custom|OnStartGame
  (Default|ShowLoadingScreen (Variables|Default|GetLobbyW%20REF))
  (Input|DisableInput self))

(event Custom|ReadyStatus%20Server
  (bind _playerlobbyinfopc (Variables|Default|GetPlayerLobbyInfoPC))
  (Utilities|Struct|SetmembersinS_PlayerLobbyInfo _playerlobbyinfopc (not (.Ready (Utilities|Struct|BreakS_PlayerLobbyInfo _playerlobbyinfopc))))
  (bind _asbp_lobby_gm (Utilities|Casting|CastToBP_LobbyGM (Game|GetGameMode)))
  (Default|UpdatePlayerLobbyInfo _asbp_lobby_gm self))

(event Custom|TryUpdatingLobbyInfo
  (Utilities|FlowControl|Delay 0.1)
  (bind _asbp_lobby_gm (Utilities|Casting|CastToBP_LobbyGM (Game|GetGameMode)))
  (Default|UpdatePlayerLobbyInfo _asbp_lobby_gm self))

(event EventBeginPlay
  (CallFunction|SetUp)
  (Utilities|FlowControl|Delay 0.1)
  (bind _asbp_lobby_gm (Utilities|Casting|CastToBP_LobbyGM (Game|GetGameMode)))
  (Default|UpdatePlayerLobbyInfo _asbp_lobby_gm self))

(fn ConstructionScript)

(fn SetUp
  (if (Pawn|IsLocalPlayerController)
    (Variables|Default|SetbShowMouseCursor true)
    (bind _returnvalue (UserInterface|CreateWidget "/Game/Devs/PRO_Mert/BluePrints/UI/Menu/PlayerCursor_WBP.PlayerCursor_WBP_C"))
    (Class|PlayerController|SetMouseCursorWidget "Default" _returnvalue)
    (Input|SetInputModeGameandUI self 0 "DoNotLock" false false)
    (bind _returnvalue_2 (UserInterface|CreateWidget "/Game/Devs/PRO_Mert/BluePrints/Player/Multiplayer/Lobby/Lobby_W.Lobby_W_C"))
    (bind _output_get (Variables|Default|SetLobbyW%20REF _returnvalue_2))
    (UserInterface|Viewport|AddtoViewport _output_get 0)
    (bind _asbp_lobby_gm (Utilities|Casting|CastToBP_LobbyGM (Game|GetGameMode)))
    (Default|UpdatePlayerLobbyInfo _asbp_lobby_gm self)
    (CallFunction|TryUpdatingLobbyInfo)))