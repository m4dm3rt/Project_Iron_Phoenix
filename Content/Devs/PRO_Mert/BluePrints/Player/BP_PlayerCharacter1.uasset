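; Player-controlled space fighter pawn with physics flight, combat and HUD.
; Input sets thrust and turn axes, remapped by a capital-ship maneuver flag; Tick applies them as force and torque with angular damping, banking and auto-leveling.
; Tick also capsule-traces ahead to lock onto enemies.
; Other graphs handle two switchable repeat-fire guns, regenerating shield and boost, health and collision damage, strafe, roll, aim zoom and camera switching.
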(event Custom|Update%20Maneuver
  (params (ThrustForward :type Float%20%28double-precision%29) (ThrustRight :type Float%20%28double-precision%29) (ThrustUp :type Float%20%28double-precision%29) (TurnRoll :type Float%20%28double-precision%29) (TurnPitch :type Float%20%28double-precision%29) (TurnYaw :type Float%20%28double-precision%29))
  (Variables|Default|SetAxisThrust (Math|Vector|MakeVector ThrustForward ThrustRight ThrustUp))
  (Variables|Default|SetAxisTurn (Math|Vector|MakeVector TurnRoll TurnPitch TurnYaw)))

(event EventBeginPlay
  (|CGraphBeginPlay))

(event EventTick
  (params (DeltaSeconds :type Float%20%28single-precision%29))
  (bind _returnvalue (Transformation|GetActorRotation))
  (bind _returnvalue_2 (Input|AxisValues|GetMoveForward))
  (bind _capitalshipmaneuver (Variables|Default|GetCapitalShipManeuver))
  (bind _spacefighter (Variables|Default|GetSpaceFighter))
  (bind _axisthrust (Variables|Default|GetAxisThrust))
  (bind _axisthrust_2 (Variables|Default|GetAxisThrust))
  (bind _driverphsysics (Variables|Default|GetDriverPhsysics))
  (bind _driverphsysics_2 (Variables|Default|GetDriverPhsysics))
  (bind _returnvalue_3 (Transformation|GetWorldLocation _spacefighter))
  (bind (_roll _pitch _yaw) (Math|Rotator|BreakRotator _returnvalue))
  (Utilities|FlowControl|Sequence
    (:then_0
      (Utilities|FlowControl|Delay 0.001)
      (Class|PrimitiveComponent|AddTorqueinDegrees _driverphsysics (/ (Math|Vector|NegateVector (Physics|GetPhysicsAngularVelocityinDegrees _driverphsysics "None")) 0.5) "None" true)
      (bind _returnvalue_4 (Physics|GetPhysicsLinearVelocity _driverphsysics "None"))
      (Physics|SetPhysicsLinearVelocity _driverphsysics _returnvalue_4 false "None")
      (bind (_outhit _returnvalue_5) (Collision|CapsuleTraceByChannel _returnvalue_3 (+ _returnvalue_3 (* (Math|Vector|GetForwardVector (Transformation|GetActorRotation)) 2e+05)) (Variables|Player|Settings|Combat|GetTargetRadius) 0.0 "TraceTypeQuery1" false 0 "None"))
      (if _returnvalue_5
        (if (not (Variables|Player|Conditions|GetTargetLocked))
          (Utilities|Casting|CastToBP_EnemyCharacter1 (.HitActor (Collision|BreakHitResult _outhit)))
          (Utilities|FlowControl|Delay 1.0)
          (Utilities|Casting|CastToBP_EnemyCharacter1 (.HitActor (Collision|BreakHitResult _outhit)))
          (Variables|Player|Conditions|SetTargetLocked true)
          (Audio|PlaySound2D "/Game/Devs/GD_Alex/Sounds/ShootingSFX/HitEnemySound/PewCut.PewCut" 0.5 1.5 0.4 0 0 false)
          (goto _label Reset))
        (else
          (Utilities|FlowControl|DoOnce true :!label _label
            (:Completed
              (Utilities|FlowControl|Delay 2.0)
              (Variables|Player|Conditions|SetTargetLocked false)
              (Audio|PlaySound2D "/Game/Devs/GD_Alex/Sounds/ShootingSFX/HitEnemySound/PewCut.PewCut" 0.5 0.5 0.3 0 0 false))))))
    (:then_1
      ;[1 1 1] Turning effects
      (Transformation|AddActorLocalRotation (Math|Rotator|MakeRotator (* (+ (Math|Float|Clamp(Float) (.z (Variables|Default|GetAxisTurn)) -0.5 0.5) (.y _axisthrust_2)) 0.5) (Math|Float|SelectFloat (* (Math|Float|Clamp(Float) (.z _axisthrust_2) -0.1 0.1) (Math|Float|SelectFloat 1.0 _returnvalue_2 (== _returnvalue_2 0.0))) 0.0 _capitalshipmaneuver) 0.0) false false)
      (Transformation|SetActorRotation (Math|Rotator|Lerp(Rotator) _returnvalue (Math|Rotator|MakeRotator 0.0 (Math|Float|SelectFloat 0.0 _pitch _capitalshipmaneuver) _yaw) 0.02 true))
      ;[1 1 1] Apply forces and torque
      (Physics|AddForce _driverphsysics_2 (+ (* (Transformation|GetActorForwardVector) (* (.x _axisthrust) (Math|Float|SelectFloat 1.0 0.3 (> (.x _axisthrust) 0.0)))) (* (Math|Vector|Normalize (* (Transformation|GetActorRightVector) "1.000000,1.000000,0.000000")) (* (.y _axisthrust) 0.5)) (* "0.000000,0.000000,1.000000" (* (.z _axisthrust) 0.3))) "None" true)
      (Class|PrimitiveComponent|AddTorqueinDegrees _driverphsysics_2 (* (Math|Transform|TransformDirection (Transformation|GetActorTransform) (* (Math|Vector|ClampVectorSize (Variables|Default|GetAxisTurn) 0.0 (Math|Vector|VectorLength "1.000000,1.000000,1.000000")) (Variables|Default|GetTurnRate))) 2e+02) "None" true))))

(event Input|ActionEvents|InputActionInteract
  (params (Key :type Key%20Structure :default "None")))

(event Input|AxisEvents|InputAxisMoveForward
  (params (AxisValue :type Float%20%28single-precision%29))
  (bind _capitalshipmaneuver (Variables|Default|GetCapitalShipManeuver))
  (CallFunction|UpdateManeuver (* AxisValue 5e+02) (Math|Float|SelectFloat 0.0 (Input|AxisValues|GetMoveRight) _capitalshipmaneuver) (Math|Float|SelectFloat (Input|AxisValues|GetMoveUp) 0.0 _capitalshipmaneuver) (Math|Float|SelectFloat 0.0 (Input|AxisValues|GetRoll) _capitalshipmaneuver) (Math|Float|SelectFloat 0.0 (Input|AxisValues|GetLookUp) _capitalshipmaneuver) (Math|Float|SelectFloat (Input|AxisValues|GetMoveRight) (Input|AxisValues|GetLookRight) _capitalshipmaneuver)))

(fn ConstructionScript)

(fn SetVelocity
  (params (NewVelocity :type Vector))
  (Physics|SetPhysicsLinearVelocity (Variables|Default|GetDriverPhsysics) NewVelocity false "None"))

(event Input|ActionEvents|InputActionStrafeLeft
  (params (Key :type Key%20Structure :default "None"))
  (:Pressed
    (Variables|Player|Conditions|SetStrafingLeft true))
  (:Released
    (Variables|Player|Conditions|SetStrafingLeft false)))

(event Input|ActionEvents|InputActionStrafeRight
  (params (Key :type Key%20Structure :default "None"))
  (:Pressed
    (Variables|Player|Conditions|SetStrafingRight true))
  (:Released
    (Variables|Player|Conditions|SetStrafingRight false)))

(event Input|AxisEvents|InputAxisStrafe
  (params (AxisValue :type Float%20%28single-precision%29))
  (bind _strafevalue (Variables|Player|Conditions|GetStrafeValue))
  (Physics|SetPhysicsLinearVelocity (Variables|Default|GetDriverPhsysics) (Math|Vector|Lerp(Vector) "0, 0, 0" (* (* (* AxisValue (Variables|Player|Settings|Movement|GetGravityControl)) (Math|Vector|GetRightVector (Variables|Default|GetDriverPhsysics))) (Math|Float|Clamp(Float) (* (Variables|Player|Conditions|GetStrafeAmount) _strafevalue) 0.0 (Math|Conversions|ToFloat(Integer) (* _strafevalue 2)))) 0.01) true "None"))

(event Custom|ShieldRecovery
  (Utilities|FlowControl|Delay 4.0)
  (if (not (Variables|Player|Conditions|GetPlayerDamaged)) :!label _label
    (if (< (Variables|Player|Settings|GetShield) 1.0)
      (Utilities|FlowControl|Delay 0.002)
      (Variables|Player|Settings|SetShield (+ (Variables|Player|Settings|GetShield) 0.004))
      (goto _label))))

(event Custom|GotHit
  (Audio|PlaySound2D "/Game/Devs/GD_Alex/Sounds/ShootingSFX/HitEnemySound/Pew01.Pew01" 1.0 1.2 0.0 0 0 false)
  (Variables|Player|Conditions|SetPlayerDamaged true)
  (bind _output_get (Variables|Player|Settings|SetShield (- (Variables|Player|Settings|GetShield) (Variables|Player|Conditions|GetDamageReceived))))
  (if (< _output_get 0.001)
    (bind _output_get_2 (Variables|Player|Settings|SetHealth (- (Variables|Player|Settings|GetHealth) (Variables|Player|Conditions|GetDamageReceived))))
    (if (< _output_get_2 0.001)
      (Actor|DestroyActor)
      (else
        (Utilities|FlowControl|Delay 0.2)
        (Variables|Player|Conditions|SetPlayerDamaged false)
        (CallFunction|ShieldRecovery)))))

(event Input|ActionEvents|InputActionSwitchCameras
  (params (Key :type Key%20Structure :default "None"))
  (bind _spectatecamera (Variables|Default|GetSpectateCamera))
  (bind _followcamera (Variables|Default|GetFollowCamera))
  (bind _playerhud_ref (Variables|Player|References|GetPlayerHUD%20ref))
  (:Pressed
    (Utilities|FlowControl|FlipFlop
      (:A
        (Components|Activation|SetActive _followcamera false false)
        (Components|Activation|SetActive _spectatecamera true false)
        (Widget|RemovefromParent _playerhud_ref)
        (Variables|Player|Conditions|SetSpectating true))
      (:B
        (Components|Activation|SetActive _followcamera true false)
        (Components|Activation|SetActive _spectatecamera false false)
        (UserInterface|Viewport|AddtoViewport _playerhud_ref 0)
        (Variables|Player|Conditions|SetSpectating false)))))

(event Input|ActionEvents|InputActionRoll
  (params (Key :type Key%20Structure :default "None"))
  (:Pressed
    (Variables|Player|Conditions|SetRolling true))
  (:Released
    (Variables|Player|Conditions|SetRolling false)))

(event Input|AxisEvents|InputAxisRoll
  (params (AxisValue :type Float%20%28single-precision%29))
  (if (Variables|Player|Conditions|GetRolling)
    (Class|PrimitiveComponent|AddTorqueinDegrees (Variables|Default|GetDriverPhsysics) (Math|Vector|Lerp(Vector) "0, 0, 0" (* (Math|Vector|GetForwardVector (Variables|Default|GetDriverPhsysics)) (* AxisValue (Variables|Player|Settings|Movement|GetGravityControl))) (Variables|Player|Settings|Movement|GetRollVelocity)) "None" true)))

(event Input|ActionEvents|InputActionSwitchWeapons
  (params (Key :type Key%20Structure :default "None"))
  (:Pressed
    (if (not (Variables|Player|Conditions|GetShooting))
      (if (Variables|Player|Conditions|GetGun1)
        (Variables|Player|Conditions|SetGun2 true)
        (Variables|Player|Conditions|SetGun1 false)
        (Audio|PlaySound2D "/Game/Devs/GD_Alex/Sounds/ShootingSFX/HitEnemySound/PewCut.PewCut" 0.5 1.1 0.1 0 0 false)
        (elif (Variables|Player|Conditions|GetGun2)
          (Variables|Player|Conditions|SetGun2 false)
          (Variables|Player|Conditions|SetGun1 true)
          (Audio|PlaySound2D "/Game/Devs/GD_Alex/Sounds/ShootingSFX/HitEnemySound/PewCut.PewCut" 0.5 0.9 0.1 0 0 false))))))

(event Input|AxisEvents|InputAxisLookUp
  (params (AxisValue :type Float%20%28single-precision%29))
  (if (Variables|Default|GetCapitalShipManeuver)
    (Default|Pitch (Variables|Default|GetBP_EZDOF_Component) (* AxisValue 0.2))))

(event Input|AxisEvents|InputAxisLookRight
  (params (AxisValue :type Float%20%28single-precision%29))
  (if (Variables|Default|GetCapitalShipManeuver)
    (Default|Yaw (Variables|Default|GetBP_EZDOF_Component) (* AxisValue 0.2))))

(event Input|ActionEvents|InputActionRise
  (params (Key :type Key%20Structure))
  (:Pressed
    (Variables|Player|Conditions|SetRising true))
  (:Released
    (Variables|Player|Conditions|SetRising false)))

(event Input|ActionEvents|InputActionLower
  (params (Key :type Key%20Structure))
  (:Pressed
    (Variables|Player|Conditions|SetLowering true))
  (:Released
    (Variables|Player|Conditions|SetLowering false)))

(event Collision|EventHit
  (params (MyComp :type Primitive%20Component%20Object%20Reference) (Other :type Actor%20Object%20Reference) (OtherComp :type Primitive%20Component%20Object%20Reference) (bSelfMoved :type Boolean) (HitLocation :type Vector :default "0, 0, 0") (HitNormal :type Vector :default "0, 0, 0") (NormalImpulse :type Vector :default "0, 0, 0") (Hit :type Hit%20Result%20Structure%20%28by%20ref%29))
  (Utilities|FlowControl|Sequence
    (:then_0
      (Utilities|FlowControl|DoOnce false :!label _label
        (:Completed
          (Variables|Player|Conditions|SetThrottleAmount 0)
          (Components|Activation|Activate (Variables|Default|GetP_Default) false)
          (bind _output_get (Variables|Player|Settings|SetHealth (- (Variables|Player|Settings|GetHealth) (Variables|Player|Settings|Combat|GetCollisionDamage))))
          (if (< _output_get 0.001)
            (Actor|DestroyActor)))))
    (:then_1
      (Utilities|FlowControl|Delay 0.5)
      (goto _label Reset))))

(event Custom|BoostRecovery
  (Utilities|FlowControl|Delay 4.0)
  (if (not (Variables|Player|Conditions|GetBoosting))
    (Variables|Player|Conditions|SetBoostAmount 0)
    (if (not (Variables|Player|Conditions|GetBoosting)) :!label _label
      (if (< (Variables|Player|Settings|GetBoost) 1.0)
        (Utilities|FlowControl|Delay 0.002)
        (Variables|Player|Settings|SetBoost (+ (Variables|Player|Settings|GetBoost) 0.004))
        (goto _label)))))

(event Input|ActionEvents|InputActionBoost
  (params (Key :type Key%20Structure :default "None"))
  (:Pressed
    (Variables|Player|Conditions|SetBoosting true)
    (Development|SetHiddeninGame (Variables|Default|GetStaticMesh6) false false)
    (Utilities|FlowControl|Sequence
      (:then_0
        (bind _output_get (Variables|Player|Settings|SetBoost (- (Variables|Player|Settings|GetBoost) 0.01) :!label _label))
        (if (> _output_get 0.0)
          (if (Variables|Player|Conditions|GetBoosting)
            (Utilities|FlowControl|Sequence
              (:then_0
                (bind _result (Math|Integer|IncrementInt (Variables|Player|Conditions|GetBoostAmount))
                  (:%20%20
                    (bind _result_2 (Math|Integer|IncrementInt _result)
                      (:%20%20
                        (Variables|Player|Conditions|SetBoostAmount _result_2)
                        (Utilities|FlowControl|Delay 0.02)
                        (goto _label))))))
              (:then_1
                (Utilities|FlowControl|DoOnce false :!label _label_2
                  (:Completed
                    (Audio|PlaySound2D "/Game/Devs/GD_Alex/Sounds/ShootingSFX/HitEnemySound/PewCut.PewCut" 0.5 1.0 0.0 0 0 false)))))
            (else
              (Utilities|FlowControl|DoOnce false :!label _label_3
                (:Completed
                  (Audio|PlaySound2D "/Game/Devs/GD_Alex/Sounds/ShootingSFX/HitEnemySound/PewCut.PewCut" 0.5 0.6 0.0 0 0 false)
                  (CallFunction|BoostRecovery)
                  (goto _label_2 Reset)))))
          (else
            (goto _label_3))))
      (:then_1
        (goto _label_3 Reset))))
  (:Released
    (Variables|Player|Conditions|SetBoosting false)
    (Development|SetHiddeninGame (Variables|Default|GetStaticMesh5) true false)
    (goto _label_3)))

(event Input|ActionEvents|InputActionShoot
  (params (Key :type Key%20Structure :default "None"))
  (bind _gun1location (Variables|Default|GetGun1Location))
  (bind _gun2location (Variables|Default|GetGun2Location))
  (bind _gun1class (Variables|Player|References|GetGun1Class))
  (bind _gun2class (Variables|Player|References|GetGun2Class))
  (:Pressed
    (Variables|Player|Conditions|SetShooting true)
    (if (Variables|Player|Conditions|GetGun1)
      (bind _outactors (Actor|GetAllActorsOfClass _gun1class))
      (Game|SpawnActorfromClass _gun1class (Math|Transform|MakeTransform (Transformation|GetWorldLocation _gun1location) (Transformation|GetWorldRotation _gun1location) (.scale (Transformation|GetActorTransform (Utilities|Array|Get(acopy) _outactors)))) "Undefined" "MultiplyWithRoot" 0 0 :!label _label)
      (Audio|PlaySound2D "/Game/Devs/GD_Alex/Sounds/ShootingSFX/Laser/LaserShoot2.LaserShoot2" 0.25 0.9 0.0 0 0 false)
      (Utilities|FlowControl|Delay (Variables|Player|Settings|Combat|GetProjectile%201%20Cooldown))
      (if (Variables|Player|Conditions|GetShooting)
        (goto _label))
      (elif (Variables|Player|Conditions|GetGun2)
        (bind _outactors_2 (Actor|GetAllActorsOfClass _gun2class))
        (Game|SpawnActorfromClass _gun2class (Math|Transform|MakeTransform (Transformation|GetWorldLocation _gun2location) (Transformation|GetWorldRotation _gun2location) (.scale (Transformation|GetActorTransform (Utilities|Array|Get(acopy) _outactors_2)))) "Undefined" "MultiplyWithRoot" 0 0 :!label _label_2)
        (Audio|PlaySound2D "/Game/Devs/GD_Alex/Sounds/ShootingSFX/Laser/LaserShoot.LaserShoot" 0.5 1.0 0.0 0 0 false)
        (Utilities|FlowControl|Delay (Variables|Player|Settings|Combat|GetProjectile%202%20Cooldown))
        (if (Variables|Player|Conditions|GetShooting)
          (goto _label_2)))))
  (:Released
    (Variables|Player|Conditions|SetShooting false)))

(event Input|ActionEvents|InputActionThrottleUp
  (params (Key :type Key%20Structure :default "None"))
  (:Released
    (Variables|Player|Conditions|SetThrottleUp false)))

(event Input|ActionEvents|InputActionThrottleDown
  (params (Key :type Key%20Structure :default "None"))
  (:Released
    (Variables|Player|Conditions|SetThrottleDown false)))

(event Input|ActionEvents|InputActionAim
  (params (Key :type Key%20Structure :default "None"))
  (bind _crosshair (Variables|Default|GetCrosshair))
  (bind _crosshairaim (Variables|Default|GetCrosshairAim))
  (bind _followcamera (Variables|Default|GetFollowCamera))
  (:Pressed
    (bind _newtrack_0 (Timeline|Timeline PlayFromStart)
      (:Update
        (Camera|SetFieldOfView _followcamera (Math|Float|Lerp 9e+01 6e+01 _newtrack_0))
        (Development|SetHiddeninGame _crosshair true false)
        (Development|SetHiddeninGame _crosshairaim false false))))
  (:Released
    (bind _newtrack_0_2 (Timeline|Timeline_0 PlayFromStart)
      (:Update
        (Camera|SetFieldOfView _followcamera (Math|Float|Lerp 6e+01 9e+01 _newtrack_0_2))
        (Development|SetHiddeninGame _crosshair false false)
        (Development|SetHiddeninGame _crosshairaim true false)))))

(event Input|AxisEvents|InputAxisCameraDistance
  (params (AxisValue :type Float%20%28single-precision%29))
  (bind _cameraspringarm (Variables|Default|GetCameraSpringArm))
  (if (< (Variables|/Script/Engine.SpringArmComponent|GetTargetArmLength _cameraspringarm) 1e+03)
    (if (> (Variables|/Script/Engine.SpringArmComponent|GetTargetArmLength _cameraspringarm) 4e+02)
      (Variables|/Script/Engine.SpringArmComponent|SetTargetArmLength _cameraspringarm (+ (* AxisValue 1e+01) (Variables|/Script/Engine.SpringArmComponent|GetTargetArmLength _cameraspringarm)))
      (else
        (Variables|/Script/Engine.SpringArmComponent|SetTargetArmLength _cameraspringarm 401.0)))
    (else
      (Variables|/Script/Engine.SpringArmComponent|SetTargetArmLength _cameraspringarm 999.0))))