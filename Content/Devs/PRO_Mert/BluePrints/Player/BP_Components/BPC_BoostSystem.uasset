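; BPC_BoostSystem is a component that manages a boost resource through current and maximum values.
; On BeginPlay it caches the player pawn as a BP_SingleplayerCharacter reference, which its boost functions do not use.
; DecreaseBoost subtracts without clamping and returns true once the boost ratio reaches zero or below.
; RegenerateBoost adds boost capped at the maximum, and IncreaseMaxBoost raises that maximum without refilling current boost.
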(event EventBeginPlay
  (bind _asbp_singleplayer_character (Utilities|Casting|CastToBP_SingleplayerCharacter (Game|Player|GetPlayerPawn 0)))
  (Variables|Default|SetPlayer%20REF _asbp_singleplayer_character))

(fn DecreaseBoost
  (params (Boost%20Decrease :type Float%20%28double-precision%29))
  (bind _output_get (Variables|Default|SetCurrentBoost (- (Variables|Default|GetCurrentBoost) Boost%20Decrease)))
  (if (<= (/ _output_get (Variables|Default|GetMaxBoost)) 0.0)
    (return true)
    (else
      (return false))))

(fn RegenerateBoost
  (params (Boost%20Increase :type Float%20%28double-precision%29))
  (bind _output_get (Variables|Default|SetCurrentBoost (+ (Variables|Default|GetCurrentBoost) Boost%20Increase)))
  (if (> _output_get (Variables|Default|GetMaxBoost))
    (Variables|Default|SetCurrentBoost (Variables|Default|GetMaxBoost))))

(fn IncreaseMaxBoost
  (params (Max%20Boost%20Increase :type Float%20%28double-precision%29))
  (Variables|Default|SetMaxBoost (+ (Variables|Default|GetMaxBoost) Max%20Boost%20Increase)))