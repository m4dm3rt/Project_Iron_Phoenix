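; Player progression component that tracks XP and level for the singleplayer character.
; IncreaseXP adds to current, general and progressed totals, mirrors them to MainGameInstance, and triggers IncreaseLevel at the threshold or shows XP gain on the HUD.
; IncreaseLevel resets XP without carryover, raises the next threshold linearly, and plays camera shake and sound.
; Both functions save to the same slot through newly created save objects, each filling only some fields.
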(event EventBeginPlay
  (bind _asbp_singleplayer_character (Utilities|Casting|CastToBP_SingleplayerCharacter (Game|Player|GetPlayerPawn 0)))
  (Variables|Backend|SetPlayer%20REF _asbp_singleplayer_character))

(fn IncreaseXP
  (params (Add%20XP :type Float%20%28double-precision%29))
  (bind _player_ref (Variables|Backend|GetPlayer%20REF))
  (bind _playerhud_ref (Variables|/Game/Devs/PRO_Mert/BluePrints/Player/MISC/BP_SingleplayerCharacter.BP_SingleplayerCharacter_C|GetPlayerHUD%20REF _player_ref))
  (bind _output_get (Variables|Backend|SetCurrentXP (+ (Variables|Backend|GetCurrentXP) Add%20XP)))
  (bind _output_get_2 (Variables|Backend|SetGeneralXP (+ (Variables|Backend|GetGeneralXP) Add%20XP)))
  (bind _asmain_game_instance (Utilities|Casting|CastToMainGameInstance (Game|GetGameInstance)))
  (Utilities|FlowControl|Sequence
    (:then_0
      (bind _output_get_3 (Variables|/Game/Devs/PRO_Mert/BluePrints/Player/MISC/MainGameInstance.MainGameInstance_C|SetXP _asmain_game_instance _output_get))
      (Variables|/Game/Devs/PRO_Mert/BluePrints/Player/MISC/MainGameInstance.MainGameInstance_C|SetGeneralXP _asmain_game_instance _output_get_2)
      (bind _returnvalue (SaveGame|CreateSaveGameObject "/Game/Devs/PRO_Alex/Blueprints/EditorPlayer/SaveConfig.SaveConfig_C"))
      (Variables|/Game/Devs/PRO_Alex/Blueprints/EditorPlayer/SaveConfig.SaveConfig_C|SetXP _returnvalue _output_get_3)
      (Variables|/Game/Devs/PRO_Alex/Blueprints/EditorPlayer/SaveConfig.SaveConfig_C|SetGeneralXP _returnvalue _output_get_2)
      (SaveGame|SaveGametoSlot _returnvalue (Variables|Backend|GetPlayerLevelSaveGame))
      (if (>= _output_get_3 (Variables|Backend|GetMaxXP))
        (Default|LevelUp _playerhud_ref)
        (CallFunction|IncreaseLevel)
        (else
          (Default|XPUp _playerhud_ref Add%20XP)
          (Default|Save _playerhud_ref))))
    (:then_1
      (bind _output_get_4 (Variables|Backend|SetProgressed%20XP (+ (Variables|Backend|GetProgressed%20XP) Add%20XP)))
      (Variables|/Game/Devs/PRO_Mert/BluePrints/Player/MISC/MainGameInstance.MainGameInstance_C|SetXP_Progressed _asmain_game_instance _output_get_4))))

(fn IncreaseLevel
  (bind _asmain_game_instance (Utilities|Casting|CastToMainGameInstance (Game|GetGameInstance)))
  (bind _output_get (Variables|Backend|SetCurrentLevel (+ (Variables|/Game/Devs/PRO_Mert/BluePrints/Player/MISC/MainGameInstance.MainGameInstance_C|GetLevel _asmain_game_instance) 1.0)))
  (bind _output_get_2 (Variables|/Game/Devs/PRO_Mert/BluePrints/Player/MISC/MainGameInstance.MainGameInstance_C|SetLevel _asmain_game_instance _output_get))
  (bind _returnvalue (SaveGame|CreateSaveGameObject "/Game/Devs/PRO_Alex/Blueprints/EditorPlayer/SaveConfig.SaveConfig_C"))
  (Variables|/Game/Devs/PRO_Alex/Blueprints/EditorPlayer/SaveConfig.SaveConfig_C|SetLevel _returnvalue _output_get_2)
  (bind _output_get_3 (Variables|/Game/Devs/PRO_Mert/BluePrints/Player/MISC/MainGameInstance.MainGameInstance_C|SetXP _asmain_game_instance 0.0))
  (Variables|/Game/Devs/PRO_Alex/Blueprints/EditorPlayer/SaveConfig.SaveConfig_C|SetXP _returnvalue _output_get_3)
  (SaveGame|SaveGametoSlot _returnvalue (Variables|Backend|GetPlayerLevelSaveGame))
  (Default|Save (Variables|/Game/Devs/PRO_Mert/BluePrints/Player/MISC/BP_SingleplayerCharacter.BP_SingleplayerCharacter_C|GetPlayerHUD%20REF (Variables|Backend|GetPlayer%20REF)))
  (Camera|PlayWorldCameraShake "/Game/Devs/PRO_Mert/BluePrints/Player/CameraShakes/CS_LevelUp.CS_LevelUp_C" (Transformation|GetWorldLocation (Variables|/Game/Devs/PRO_Mert/BluePrints/Player/MISC/BP_SingleplayerCharacter.BP_SingleplayerCharacter_C|GetMainCamera (Variables|Backend|GetPlayer%20REF))) 0.0 1e+02)
  (Class|FMODBlueprintStatics|PlayEvent2D "/Game/FMOD/Events/Meta/SFX_055_Statistic_CountUp.SFX_055_Statistic_CountUp")
  (Variables|Backend|SetCurrentXP 0.0)
  (Variables|Backend|SetMaxXP (+ (Variables|Backend|GetMaxXP) 5e+02)))