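; Player health component that tracks health and shield for the single-player ship and handles its death.
; Functions damage, regenerate and raise both pools, returning depleted or full flags, with health damage applying only when shieldless.
; Health hits blink HUD and reticle elements, adding smoke and a global damage parameter at half health.
; A one-shot death event disables collision, explodes the ship, saves the death count, then shows the end screen and pauses.
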(event EventBeginPlay
  (bind _asbp_singleplayer_character (Utilities|Casting|CastToBP_SingleplayerCharacter (Game|Player|GetPlayerPawn 0)))
  (Variables|References|SetPlayer%20REF _asbp_singleplayer_character))

(fn DecreaseHealth
  (params (NoShield :type Boolean) (Damage%20Received :type Float%20%28double-precision%29))
  (bind _maxhealth (Variables|Health|GetMaxHealth))
  (bind _player_ref (Variables|References|GetPlayer%20REF))
  (if NoShield
    (Default|BlinkShield (Variables|/Game/Devs/PRO_Mert/BluePrints/Player/MISC/BP_SingleplayerCharacter.BP_SingleplayerCharacter_C|GetPlayerReticle%20REF (Variables|References|GetPlayer%20REF)))
    (bind _output_get (Variables|Health|SetCurrentHealth (Math|Float|Clamp(Float) (- (Variables|Health|GetCurrentHealth) Damage%20Received) 0.0 _maxhealth)))
    (if (<= (/ _output_get _maxhealth) 0.0)
      (return true)
      (elif (<= (/ _output_get _maxhealth) 0.5)
        (Components|Activation|Activate (Variables|/Game/Devs/PRO_Mert/BluePrints/Player/MISC/BP_SingleplayerCharacter.BP_SingleplayerCharacter_C|GetNS_Smoke _player_ref) false)
        (Default|BlinkHealth (Variables|/Game/Devs/PRO_Mert/BluePrints/Player/MISC/BP_SingleplayerCharacter.BP_SingleplayerCharacter_C|GetPlayerReticle%20REF _player_ref))
        (Default|BlinkHealth (Variables|/Game/Devs/PRO_Mert/BluePrints/Player/MISC/BP_SingleplayerCharacter.BP_SingleplayerCharacter_C|GetPlayerHUD%20REF _player_ref))
        (Class|FMODBlueprintStatics|SetGlobalParameterbyName "damage_level" 1.0)
        (else
          (return false))))))

(fn RegenerateHealth
  (params (Health%20Increase :type Float%20%28double-precision%29))
  (bind _maxhealth (Variables|Health|GetMaxHealth))
  (bind _output_get (Variables|Health|SetCurrentHealth (+ (Variables|Health|GetCurrentHealth) Health%20Increase)))
  (if (> _output_get _maxhealth)
    (bind _output_get_2 (Variables|Health|SetCurrentHealth (Variables|Health|GetMaxHealth))))
  (if (>= _output_get_2 _maxhealth)
    (return true)
    (else
      (return false))))

(fn IncreaseMaxHealth
  (params (Max%20Health%20Increase :type Float%20%28double-precision%29))
  (Variables|Health|SetMaxHealth (+ (Variables|Health|GetMaxHealth) Max%20Health%20Increase)))

(fn DecreaseShield
  (params (Damage%20Received :type Float%20%28double-precision%29))
  (bind _maxshield (Variables|Shield|GetMaxShield))
  (if (<= (/ (Variables|Shield|GetCurrentShield) _maxshield) 0.0)
    (return true)
    (else
      (Variables|Shield|SetCurrentShield (Math|Float|Clamp(Float) (- (Variables|Shield|GetCurrentShield) Damage%20Received) 0.0 _maxshield))
      (return false))))

(fn RegenerateShield
  (params (Shield%20Recovery :type Float%20%28double-precision%29))
  (bind _maxshield (Variables|Shield|GetMaxShield))
  (bind _output_get (Variables|Shield|SetCurrentShield (+ (Variables|Shield|GetCurrentShield) Shield%20Recovery)))
  (if (> _output_get _maxshield)
    (bind _output_get_2 (Variables|Shield|SetCurrentShield (Variables|Shield|GetMaxShield))))
  (if (== _output_get_2 _maxshield)
    (return true)
    (else
      (return false))))

(fn IncreaseMaxShield
  (params (Max%20Shield%20Increase :type Float%20%28double-precision%29))
  (Variables|Shield|SetMaxShield (+ (Variables|Shield|GetMaxShield) Max%20Shield%20Increase)))

(event Custom|PlayerDeath
  (bind _returnvalue (Game|GetPlayerController 0))
  (bind _player_ref (Variables|References|GetPlayer%20REF))
  (bind _player_ref_2 (Variables|References|GetPlayer%20REF))
  (Utilities|FlowControl|DoOnce false
    (:Completed
      (Default|StopShooting _player_ref)
      (Variables|Health|SetisDead true)
      (Utilities|FlowControl|Sequence
        (:then_0
          (Components|Activation|Activate (Variables|/Game/Devs/PRO_Mert/BluePrints/Player/MISC/BP_SingleplayerCharacter.BP_SingleplayerCharacter_C|GetNS_PlayerExplosion _player_ref) false)
          (Collision|SetCollisionEnabled (Variables|/Script/Project_Iron_Phoenix.SingleplayerPawn|GetCapsuleComponent (Variables|References|GetPlayer%20REF)) "NoCollision")
          (Class|FMODBlueprintStatics|SetGlobalParameterbyName "combat_status" 2.0)
          (Class|FMODBlueprintStatics|SetGlobalParameterbyName "lockon_status" 2.0)
          (bind _asmain_game_instance (Utilities|Casting|CastToMainGameInstance (Game|GetGameInstance)))
          (bind _output_get (Variables|/Game/Devs/PRO_Mert/BluePrints/Player/MISC/MainGameInstance.MainGameInstance_C|SetDeathCount _asmain_game_instance (+ (Variables|/Game/Devs/PRO_Mert/BluePrints/Player/MISC/MainGameInstance.MainGameInstance_C|GetDeathCount _asmain_game_instance) 1.0)))
          (bind _returnvalue_2 (SaveGame|CreateSaveGameObject "/Game/Devs/PRO_Alex/Blueprints/EditorPlayer/SaveConfig.SaveConfig_C"))
          (Variables|/Game/Devs/PRO_Alex/Blueprints/EditorPlayer/SaveConfig.SaveConfig_C|SetDeathCount _returnvalue_2 _output_get)
          (SaveGame|SaveGametoSlot _returnvalue_2 (Variables|References|GetPlayerLevel%20SaveGame)))
        (:then_1
          (Utilities|FlowControl|Delay 2.0)
          (Development|SetHiddeninGame (Variables|/Game/Devs/PRO_Mert/BluePrints/Player/MISC/BP_SingleplayerCharacter.BP_SingleplayerCharacter_C|GetEditorShip _player_ref_2) true false)
          (Widget|RemovefromParent (Variables|/Game/Devs/PRO_Mert/BluePrints/Player/MISC/BP_SingleplayerCharacter.BP_SingleplayerCharacter_C|GetPlayerHUD%20REF _player_ref_2))
          (bind _returnvalue_3 (UserInterface|CreateWidget "/Game/Devs/PRO_Mert/BluePrints/UI/Menu/EndScreen_W.EndScreen_W_C"))
          (UserInterface|Viewport|AddtoViewport _returnvalue_3 0)
          (Input|SetInputModeUIOnly _returnvalue _returnvalue_3 "DoNotLock" false)
          (Variables|/Script/Engine.PlayerController|SetbShowMouseCursor _returnvalue true)
          (Utilities|FlowControl|Delay 2.0)
          (Components|DestroyComponent (Variables|/Game/Devs/PRO_Mert/BluePrints/Player/MISC/BP_SingleplayerCharacter.BP_SingleplayerCharacter_C|GetMainCamera (Variables|References|GetPlayer%20REF)))
          (Game|SetGamePaused true)
          (bind _returnvalue_4 (Actor|GetActorOfClass "/Game/Devs/PRO_Alex/Blueprints/EditorPlayer/EditorPlayer.EditorPlayer_C"))
          (Default|PlayVoicelineSound _returnvalue_4 "/Game/Devs/GD_Seb/Voicelines/Death/Death_Cue.Death_Cue"))))))