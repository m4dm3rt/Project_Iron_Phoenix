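; Machine gun projectile that flies without gravity at a configurable speed and damages asteroids and enemy ships.
; On sphere overlap it writes its damage into the hit AsteroidMert or BP_EnemyCharacter, calls GotHit and destroys itself.
; A self-repeating homing event targets the nearest enemy's SpaceFighter, but its visible trigger is disconnected and BeginPlay's target-lock check leads nowhere.
; The Hit event spawns a scaled-up particle effect at the impact location.
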(event OnComponentBeginOverlap(SphereCollision)
  (params (OverlappedComponent :type Primitive%20Component%20Object%20Reference) (OtherActor :type Actor%20Object%20Reference) (OtherComp :type Primitive%20Component%20Object%20Reference) (OtherBodyIndex :type Integer) (bFromSweep :type Boolean) (SweepResult :type Hit%20Result%20Structure%20%28by%20ref%29))
  (bind _damage (Variables|Projectile|Settings|GetDamage))
  (Utilities|FlowControl|Sequence
    (:then_0
      (bind _asasteroid_mert (Utilities|Casting|CastToAsteroidMert OtherActor))
      (Variables|/Game/Devs/PRO_Mert/BluePrints/Environment/AsteroidMert.AsteroidMert_C|SetDamage%20Received _asasteroid_mert _damage)
      (Default|GotHit _asasteroid_mert))
    (:then_1
      (bind _asbp_enemy_character (Utilities|Casting|CastToBP_EnemyCharacter OtherActor))
      (Variables|/Game/Devs/PRO_Mert/BluePrints/Enemies/BP_EnemyCharacter.BP_EnemyCharacter_C|SetDamage%20Received _asbp_enemy_character _damage)
      (Default|GotHit _asbp_enemy_character)))
  (Actor|DestroyActor))

(event Custom|HomingProjectile
  (bind _projectilemovement (Variables|Default|GetProjectileMovement))
  (Variables|/Script/Engine.ProjectileMovementComponent|SetbIsHomingProjectile _projectilemovement true)
  (bind _outactors (Actor|GetAllActorsOfClass "/Game/Devs/PRO_Mert/BluePrints/Enemies/BP_EnemyCharacter.BP_EnemyCharacter_C"))
  (for _array_element _outactors
    (if (< (Math|Vector|VectorLength (- (Transformation|GetActorLocation _array_element) (Transformation|GetActorLocation))) (Variables|Projectile|Conditions|GetClosest%20Distance))
      (Variables|Projectile|Conditions|SetClosest%20Distance (Math|Vector|VectorLength (- (Transformation|GetActorLocation _array_element) (Transformation|GetActorLocation))))
      (Variables|Projectile|References|SetTarget _array_element)))
  (Variables|/Script/Engine.ProjectileMovementComponent|SetHomingTargetComponent _projectilemovement (Variables|/Game/Devs/PRO_Mert/BluePrints/Enemies/BP_EnemyCharacter.BP_EnemyCharacter_C|GetSpaceFighter (Variables|Projectile|References|GetTarget)))
  (Utilities|FlowControl|Delay 0.02)
  (CallFunction|HomingProjectile))

(event EventBeginPlay
  (bind _asbp_player_character (Utilities|Casting|CastToBP_PlayerCharacter (Game|Player|GetPlayerPawn 0)))
  (if (Variables|/Game/Devs/PRO_Mert/BluePrints/Player/BP_PlayerCharacter.BP_PlayerCharacter_C|GetTargetLocked _asbp_player_character)
    _))

(event Collision|EventHit
  (params (MyComp :type Primitive%20Component%20Object%20Reference) (Other :type Actor%20Object%20Reference) (OtherComp :type Primitive%20Component%20Object%20Reference) (bSelfMoved :type Boolean) (HitLocation :type Vector :default "0, 0, 0") (HitNormal :type Vector :default "0, 0, 0") (NormalImpulse :type Vector :default "0, 0, 0") (Hit :type Hit%20Result%20Structure%20%28by%20ref%29))
  (Effects|SpawnEmitteratLocation "/Game/Realistic_Starter_VFX_Pack_Vol2/Particles/Hit/P_Default.P_Default" HitLocation "0, 0, 0" "100.000000,100.000000,100.000000"))

(fn ConstructionScript
  (bind _projectilemovement (Variables|Default|GetProjectileMovement))
  (bind _speed (Variables|Projectile|Settings|GetSpeed))
  (bind _output_get (Variables|/Script/Engine.ProjectileMovementComponent|SetInitialSpeed _projectilemovement _speed))
  (Variables|/Script/Engine.ProjectileMovementComponent|SetMaxSpeed _projectilemovement _output_get)
  (Variables|/Script/Engine.ProjectileMovementComponent|SetProjectileGravityScale _projectilemovement 0.0)
  (Variables|/Script/Engine.ProjectileMovementComponent|SetHomingAccelerationMagnitude _projectilemovement _speed))