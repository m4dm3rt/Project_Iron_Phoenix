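; Enemy space fighter Character that hunts the player, shoots, and takes damage.
; Sensing cone overlaps set CanSeePlayer, making Tick turn it toward the player, fire on random delays, and approach or strafe on timer-flipped axes; otherwise it drifts randomly.
; Tick also updates health and distance widgets and places an in-range aim marker projected from velocity.
; GotHit triggers effects and the HUD hitmarker, and on death increments the EnemySpawner's kill count.
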(event EventBeginPlay
  (bind _returnvalue (Transformation|GetActorRotation))
  (bind _outactors (Actor|GetAllActorsOfClass (Variables|Enemy|References|GetPlayer%20REF)))
  (Variables|Enemy|References|SetPlayer%20Character%20REF (Utilities|Array|Get(acopy) _outactors))
  (CallFunction|StrafeDirection)
  (Transformation|SetActorRotation (Math|Rotator|MakeRotator (.roll _returnvalue) (.pitch _returnvalue) (- (.yaw _returnvalue) 9e+01))))

(event EventTick
  (params (DeltaSeconds :type Float%20%28single-precision%29))
  (|CGraphEventTick))

(fn ConstructionScript
  (bind _vision_cone_height (Variables|Enemy|Settings|Sensing|GetVision%20Cone%20Height))
  (bind _charactermovement (Variables|Character|GetCharacterMovement))
  (Variables|/Script/Engine.CharacterMovementComponent|SetMaxFlySpeed _charactermovement (Variables|Enemy|Settings|Movement|GetAcceleration))
  (Variables|/Script/Engine.CharacterMovementComponent|SetBrakingDecelerationFlying _charactermovement (Variables|Enemy|Settings|Movement|GetDecelaration))
  (Transformation|SetRelativeTransform (Variables|Default|GetSensingCone) (Math|Transform|MakeTransform "0.000000,10000.000000,0.000000" "90.000000,-90.000000,180.000000" (Math|Vector|MakeVector _vision_cone_height _vision_cone_height (Variables|Enemy|Settings|Sensing|GetVision%20Cone%20Lenght))) false false))

(event Custom|ShootProjectile
  (bind _enemygunclass_ref (Variables|Enemy|References|GetEnemyGunClass%20REF))
  (bind _gun1location (Variables|Default|GetGun1Location))
  (if (Variables|Enemy|Conditions|GetCanSeePlayer)
    (Utilities|FlowControl|Delay (Math|Random|RandomFloatinRange (Variables|Enemy|Settings|Combat|GetShot%20Cooldown%20Min) (Variables|Enemy|Settings|Combat|GetShot%20Cooldown%20Max)))
    (bind _outactors (Actor|GetAllActorsOfClass _enemygunclass_ref))
    (Game|SpawnActorfromClass _enemygunclass_ref (Math|Transform|MakeTransform (Transformation|GetWorldLocation _gun1location) (Transformation|GetWorldRotation _gun1location) (.scale (Transformation|GetActorTransform (Utilities|Array|Get(acopy) _outactors)))) "Undefined" "MultiplyWithRoot" 0 0)
    (Audio|PlaySoundatLocation "/Game/Devs/GD_Alex/Sounds/ShootingSFX/Laser/LaserShoot.LaserShoot" (Transformation|GetActorLocation) "0, 0, 0" 0.1 1.0 0.0 0 0 0 0)))

(event OnComponentBeginOverlap(SensingCone)
  (params (OverlappedComponent :type Primitive%20Component%20Object%20Reference) (OtherActor :type Actor%20Object%20Reference) (OtherComp :type Primitive%20Component%20Object%20Reference) (OtherBodyIndex :type Integer) (bFromSweep :type Boolean) (SweepResult :type Hit%20Result%20Structure%20%28by%20ref%29))
  (Variables|Enemy|References|SetPlayer%20REF (Utilities|GetClass OtherActor))
  (Variables|Enemy|Conditions|SetCanSeePlayer true))

(event OnComponentEndOverlap(SensingCone)
  (params (OverlappedComponent :type Primitive%20Component%20Object%20Reference) (OtherActor :type Actor%20Object%20Reference) (OtherComp :type Primitive%20Component%20Object%20Reference) (OtherBodyIndex :type Integer))
  (Variables|Enemy|References|SetPlayer%20REF (Utilities|GetClass OtherActor))
  (Variables|Enemy|Conditions|SetCanSeePlayer false))

(event Custom|GotHit
  (bind _returnvalue (Transformation|GetActorTransform))
  (bind _returnvalue_2 (Transformation|GetActorTransform))
  (Variables|Enemy|Settings|General|SetHealth (- (Variables|Enemy|Settings|General|GetHealth) (Variables|Enemy|Conditions|GetDamage%20Received)))
  (Effects|SpawnEmitteratLocation "/Game/Realistic_Starter_VFX_Pack_Vol2/Particles/Hit/P_Asphalt.P_Asphalt" (.location _returnvalue_2) (.rotation _returnvalue_2) "25.000000,25.000000,25.000000")
  (Audio|PlaySound2D "/Game/Devs/GD_Alex/Sounds/ShootingSFX/HitEnemySound/Pew01.Pew01" 1.0 1.0 0.0 0 0 false)
  (Variables|Enemy|Conditions|SetEnemy%20Got%20Hit true)
  (bind _foundwidgets (Widget|GetAllWidgetsOfClass "/Game/Devs/PRO_Mert/BluePrints/Widgets/PlayerCrosshairMovingHUD.PlayerCrosshairMovingHUD_C" false))
  (Default|Hitmarker (Utilities|Array|Get(acopy) _foundwidgets))
  (Utilities|FlowControl|Sequence
    (:then_0
      (if (< (Variables|Enemy|Settings|General|GetHealth) 0.001)
        (Actor|DestroyActor)
        (Effects|SpawnEmitteratLocation "/Game/Realistic_Starter_VFX_Pack_Vol2/Particles/Explosion/P_Explosion_Big_A.P_Explosion_Big_A" (.location _returnvalue) (.rotation _returnvalue) "3.000000,3.000000,3.000000")
        (bind _outactors (Actor|GetAllActorsOfClass "/Game/Devs/PRO_Alex/Blueprints/Enemy-Spawner/EnemySpawner.EnemySpawner_C"))
        (Variables|/Game/Devs/PRO_Alex/Blueprints/Enemy-Spawner/EnemySpawner.EnemySpawner_C|SetEnemyKilled (Utilities|Array|Get(acopy) _outactors) (+ (Variables|/Game/Devs/PRO_Alex/Blueprints/Enemy-Spawner/EnemySpawner.EnemySpawner_C|GetEnemyKilled (Utilities|Array|Get(acopy) _outactors)) 1.0))))
    (:then_1
      (Utilities|FlowControl|Delay 0.3)
      (Variables|Enemy|Conditions|SetEnemy%20Got%20Hit false))))

(event Custom|StrafeDirection
  (Utilities|FlowControl|FlipFlop
    (:A
      (bind _isa (Utilities|FlowControl|FlipFlop)
        (:A
          _)
        (:B
          _))
      (Variables|Enemy|Conditions|SetStrafeRight _isa))
    (:B
      (bind _isa_2 (Utilities|FlowControl|FlipFlop)
        (:A
          _)
        (:B
          _))
      (Variables|Enemy|Conditions|SetStrafeUp _isa_2)))
  (Utilities|Time|SetTimerbyEvent (delegate Custom|StrafeDirection) (Math|Random|RandomFloatinRange 2.0 5.0)))