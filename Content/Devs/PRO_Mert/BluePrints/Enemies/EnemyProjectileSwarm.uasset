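; Enemy swarm projectile that damages the player character on contact.
; The construction script sets the projectile movement's initial and max speed from a Speed variable and turns gravity off for straight flight.
; When the collision sphere overlaps the player, it writes Damage into the player's DamageReceived, calls GotHit and destroys itself.
; Overlaps with any other actor are ignored.
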(event OnComponentBeginOverlap(SphereCollision)
  (params (OverlappedComponent :type Primitive%20Component%20Object%20Reference) (OtherActor :type Actor%20Object%20Reference) (OtherComp :type Primitive%20Component%20Object%20Reference) (OtherBodyIndex :type Integer) (bFromSweep :type Boolean) (SweepResult :type Hit%20Result%20Structure%20%28by%20ref%29))
  (bind _asbp_player_character (Utilities|Casting|CastToBP_PlayerCharacter OtherActor))
  (Variables|/Game/Devs/PRO_Mert/BluePrints/Player/BP_PlayerCharacter.BP_PlayerCharacter_C|SetDamage%20Received _asbp_player_character (Variables|Projectile|Settings|GetDamage))
  (Default|GotHit _asbp_player_character)
  (Actor|DestroyActor))

(fn ConstructionScript
  (bind _projectilemovement (Variables|Default|GetProjectileMovement))
  (bind _output_get (Variables|/Script/Engine.ProjectileMovementComponent|SetInitialSpeed _projectilemovement (Variables|Projectile|Settings|GetSpeed)))
  (Variables|/Script/Engine.ProjectileMovementComponent|SetMaxSpeed _projectilemovement _output_get)
  (Variables|/Script/Engine.ProjectileMovementComponent|SetProjectileGravityScale _projectilemovement 0.0))