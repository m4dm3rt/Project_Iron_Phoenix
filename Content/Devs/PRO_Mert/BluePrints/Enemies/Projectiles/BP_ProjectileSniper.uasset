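; BP_ProjectileSniper is an enemy sniper projectile that flies without gravity at a speed set from its Speed variable in the construction script.
; Each tick it resizes its EnemyProjectile_W indicator image inversely to its distance from the player, so the marker grows as it nears.
; On capsule overlap it damages the singleplayer character with an explosion emitter, or applies point damage to an asteroid ring, then destroys itself.
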(event OnComponentBeginOverlap(CapsuleCollision)
  (params (OverlappedComponent :type Primitive%20Component%20Object%20Reference) (OtherActor :type Actor%20Object%20Reference) (OtherComp :type Primitive%20Component%20Object%20Reference) (OtherBodyIndex :type Integer) (bFromSweep :type Boolean) (SweepResult :type Hit%20Result%20Structure%20%28by%20ref%29))
  (bind _asbp_singleplayer_character (Utilities|Casting|CastToBP_SingleplayerCharacter OtherActor)
    (:then
      (Game|Damage|ApplyDamage _asbp_singleplayer_character (Variables|Projectile|Settings|GetDamage) 0 0)
      (Effects|SpawnEmitteratLocation "/Game/Realistic_Starter_VFX_Pack_Vol2/Particles/Hit/P_Default.P_Default" (Transformation|GetActorLocation) "0, 0, 0" "25.000000,25.000000,25.000000")
      (Actor|DestroyActor))
    (:CastFailed
      (bind _asbp_single_asteroid_ring (Utilities|Casting|CastToBP_SingleAsteroidRing OtherActor))
      (Game|Damage|ApplyPointDamage _asbp_single_asteroid_ring (Variables|Projectile|Settings|GetDamage) (Transformation|GetActorLocation) (Collision|MakeHitResult false false 0.0 0.0 "0, 0, 0" "0, 0, 0" "0,0,1" "0,0,1" 0 0))
      (Actor|DestroyActor))))

(event EventTick
  (params (DeltaSeconds :type Float%20%28single-precision%29))
  (bind _returnvalue (Game|Player|GetPlayerPawn 0))
  (bind _projectileindicator (Variables|Default|GetProjectileIndicator))
  (bind _returnvalue_2 (Transformation|GetDistanceTo _returnvalue))
  (bind _returnvalue_3 (UserInterface|GetWidget _projectileindicator))
  (bind _asenemy_projectile_w (Utilities|Casting|CastToEnemyProjectile_W _returnvalue_3))
  (bind _returnvalue_4 (/ 1e+07 _returnvalue_2))
  (bind _image_missileindicator (Variables|/Game/Devs/PRO_Mert/BluePrints/Enemies/Widgets/EnemyProjectile_W.EnemyProjectile_W_C|GetImage_MissileIndicator _asenemy_projectile_w))
  (Class|Image|SetBrush _image_missileindicator (Utilities|Struct|MakeSlateBrush "Image" "NoTile" "NoMirror" (Utilities|Struct|MakeDeprecateSlateVector2D _returnvalue_4 _returnvalue_4) "(Left=0.000000,Top=0.000000,Right=0.000000,Bottom=0.000000)" "(SpecifiedColor=(R=1.000000,G=1.000000,B=1.000000,A=1.000000),ColorUseRule=UseColor_Specified)" "(CornerRadii=(X=0.000000,Y=0.000000,Z=0.000000,W=1.000000),Color=(SpecifiedColor=(R=0.000000,G=0.000000,B=0.000000,A=0.000000),ColorUseRule=UseColor_Specified),Width=0.000000,RoundingType=HalfHeightRadius,bUseBrushTransparency=False)" (.resourceobject (Variables|/Script/UMG.Image|GetBrush _image_missileindicator)))))

(fn ConstructionScript
  (bind _projectilemovement (Variables|Default|GetProjectileMovement))
  (bind _output_get (Variables|/Script/Engine.ProjectileMovementComponent|SetInitialSpeed _projectilemovement (Variables|Projectile|Settings|GetSpeed)))
  (Variables|/Script/Engine.ProjectileMovementComponent|SetMaxSpeed _projectilemovement _output_get)
  (Variables|/Script/Engine.ProjectileMovementComponent|SetProjectileGravityScale _projectilemovement 0.0))