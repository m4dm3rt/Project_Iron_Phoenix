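; Projectile for an enemy drone that damages the singleplayer character or asteroids it overlaps.
; The construction script drives ProjectileMovement from the Speed variable and disables gravity for straight flight.
; On sphere overlap it deals full Damage to the character with an emitter effect, or half to an asteroid without one, then destroys itself.
; Overlaps with any other actor are ignored.
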(event OnComponentBeginOverlap(SphereCollision)
  (params (OverlappedComponent :type Primitive%20Component%20Object%20Reference) (OtherActor :type Actor%20Object%20Reference) (OtherComp :type Primitive%20Component%20Object%20Reference) (OtherBodyIndex :type Integer) (bFromSweep :type Boolean) (SweepResult :type Hit%20Result%20Structure%20%28by%20ref%29))
  (bind _asbp_singleplayer_character (Utilities|Casting|CastToBP_SingleplayerCharacter OtherActor)
    (:then
      (Game|Damage|ApplyDamage _asbp_singleplayer_character (Variables|Projectile|Settings|GetDamage) 0 0)
      (Effects|SpawnEmitteratLocation "/Game/Realistic_Starter_VFX_Pack_Vol2/Particles/Hit/P_Default.P_Default" (Transformation|GetActorLocation) "0, 0, 0" "15.000000,15.000000,15.000000")
      (Actor|DestroyActor))
    (:CastFailed
      (bind _asbp_asteroid (Utilities|Casting|CastToBP_Asteroid OtherActor))
      (Game|Damage|ApplyDamage _asbp_asteroid (/ (Variables|Projectile|Settings|GetDamage) 2.0) 0 0)
      (Actor|DestroyActor))))

(fn ConstructionScript
  (bind _projectilemovement (Variables|Default|GetProjectileMovement))
  (bind _output_get (Variables|/Script/Engine.ProjectileMovementComponent|SetInitialSpeed _projectilemovement (Variables|Projectile|Settings|GetSpeed)))
  (Variables|/Script/Engine.ProjectileMovementComponent|SetMaxSpeed _projectilemovement _output_get)
  (Variables|/Script/Engine.ProjectileMovementComponent|SetProjectileGravityScale _projectilemovement 0.0))