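; BP_Center is a spherical arena boundary that tracks whether enemies are inside or outside its volume.
; Sphere begin overlap clears each enemy's OutOufBorder flag, and end overlap sets it.
; Both events use a Sequence of per-class casts covering Swarm, Sniper and Bomber enemies, their MP variants, and Drone.
; The actor only writes the flag, leaving any reaction to the enemy Blueprints.
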(event OnComponentBeginOverlap(Sphere)
  (params (OverlappedComponent :type Primitive%20Component%20Object%20Reference) (OtherActor :type Actor%20Object%20Reference) (OtherComp :type Primitive%20Component%20Object%20Reference) (OtherBodyIndex :type Integer) (bFromSweep :type Boolean) (SweepResult :type Hit%20Result%20Structure%20%28by%20ref%29))
  (Utilities|FlowControl|Sequence
    (:then_0
      (bind _asbp_enemy_swarm (Utilities|Casting|CastToBP_EnemySwarm OtherActor))
      (Variables|/Game/Devs/PRO_Mert/BluePrints/Enemies/Actors/BP_EnemySwarm.BP_EnemySwarm_C|SetOutOufBorder _asbp_enemy_swarm false))
    (:then_1
      (bind _asbp_enemy_sniper (Utilities|Casting|CastToBP_EnemySniper OtherActor))
      (Variables|/Game/Devs/PRO_Mert/BluePrints/Enemies/Actors/BP_EnemySniper.BP_EnemySniper_C|SetOutOufBorder _asbp_enemy_sniper false))
    (:then_2
      (bind _asbp_enemy_bomber (Utilities|Casting|CastToBP_EnemyBomber OtherActor))
      (Variables|/Game/Devs/PRO_Mert/BluePrints/Enemies/Actors/BP_EnemyBomber.BP_EnemyBomber_C|SetOutOufBorder _asbp_enemy_bomber false))
    (:then_3
      (bind _asbp_enemy_drone (Utilities|Casting|CastToBP_EnemyDrone OtherActor))
      (Variables|/Game/Devs/PRO_Mert/BluePrints/Enemies/Actors/BP_EnemyDrone.BP_EnemyDrone_C|SetOutOufBorder _asbp_enemy_drone false))
    (:then_4
      (bind _asbp_enemy_swarm_mp (Utilities|Casting|CastToBP_EnemySwarmMP OtherActor))
      (Variables|/Game/Devs/PRO_Mert/Multiplayer/InGame/Enemies/BP_EnemySwarmMP.BP_EnemySwarmMP_C|SetOutOufBorder _asbp_enemy_swarm_mp false))
    (:then_5
      (bind _asbp_enemy_sniper_mp (Utilities|Casting|CastToBP_EnemySniperMP OtherActor))
      (Variables|/Game/Devs/PRO_Mert/Multiplayer/InGame/Enemies/BP_EnemySniperMP.BP_EnemySniperMP_C|SetOutOufBorder _asbp_enemy_sniper_mp false))
    (:then_6
      (bind _asbp_enemy_bomber_mp (Utilities|Casting|CastToBP_EnemyBomberMP OtherActor))
      (Variables|/Game/Devs/PRO_Mert/Multiplayer/InGame/Enemies/BP_EnemyBomberMP.BP_EnemyBomberMP_C|SetOutOufBorder _asbp_enemy_bomber_mp false))))

(event OnComponentEndOverlap(Sphere)
  (params (OverlappedComponent :type Primitive%20Component%20Object%20Reference) (OtherActor :type Actor%20Object%20Reference) (OtherComp :type Primitive%20Component%20Object%20Reference) (OtherBodyIndex :type Integer))
  (Utilities|FlowControl|Sequence
    (:then_0
      (bind _asbp_enemy_swarm (Utilities|Casting|CastToBP_EnemySwarm OtherActor))
      (Variables|/Game/Devs/PRO_Mert/BluePrints/Enemies/Actors/BP_EnemySwarm.BP_EnemySwarm_C|SetOutOufBorder _asbp_enemy_swarm true))
    (:then_1
      (bind _asbp_enemy_sniper (Utilities|Casting|CastToBP_EnemySniper OtherActor))
      (Variables|/Game/Devs/PRO_Mert/BluePrints/Enemies/Actors/BP_EnemySniper.BP_EnemySniper_C|SetOutOufBorder _asbp_enemy_sniper true))
    (:then_2
      (bind _asbp_enemy_bomber (Utilities|Casting|CastToBP_EnemyBomber OtherActor))
      (Variables|/Game/Devs/PRO_Mert/BluePrints/Enemies/Actors/BP_EnemyBomber.BP_EnemyBomber_C|SetOutOufBorder _asbp_enemy_bomber true))
    (:then_3
      (bind _asbp_enemy_drone (Utilities|Casting|CastToBP_EnemyDrone OtherActor))
      (Variables|/Game/Devs/PRO_Mert/BluePrints/Enemies/Actors/BP_EnemyDrone.BP_EnemyDrone_C|SetOutOufBorder _asbp_enemy_drone true))
    (:then_4
      (bind _asbp_enemy_swarm_mp (Utilities|Casting|CastToBP_EnemySwarmMP OtherActor))
      (Variables|/Game/Devs/PRO_Mert/Multiplayer/InGame/Enemies/BP_EnemySwarmMP.BP_EnemySwarmMP_C|SetOutOufBorder _asbp_enemy_swarm_mp true))
    (:then_5
      (bind _asbp_enemy_sniper_mp (Utilities|Casting|CastToBP_EnemySniperMP OtherActor))
      (Variables|/Game/Devs/PRO_Mert/Multiplayer/InGame/Enemies/BP_EnemySniperMP.BP_EnemySniperMP_C|SetOutOufBorder _asbp_enemy_sniper_mp true))
    (:then_6
      (bind _asbp_enemy_bomber_mp (Utilities|Casting|CastToBP_EnemyBomberMP OtherActor))
      (Variables|/Game/Devs/PRO_Mert/Multiplayer/InGame/Enemies/BP_EnemyBomberMP.BP_EnemyBomberMP_C|SetOutOufBorder _asbp_enemy_bomber_mp true))))

(fn ConstructionScript)