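; BP_EnemiesBorder is a border actor with a sphere collision that tracks whether swarm, sniper and bomber enemies are outside its area.
; On begin overlap, a Sequence of casts clears the OutOufBorder flag on the matching enemy type.
; On end overlap, only BP_EnemySwarm gets the flag set to true; sniper and bomber enemies have it set to false again, so exiting never flags them.
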(event OnComponentBeginOverlap(SphereCollision)
  (params (OverlappedComponent :type Primitive%20Component%20Object%20Reference) (OtherActor :type Actor%20Object%20Reference) (OtherComp :type Primitive%20Component%20Object%20Reference) (OtherBodyIndex :type Integer) (bFromSweep :type Boolean) (SweepResult :type Hit%20Result%20Structure%20%28by%20ref%29))
  ;[1 1 1] Collision if Player is in Range
  (Utilities|FlowControl|Sequence
    (:then_0
      (bind _asbp_enemy_swarm (Utilities|Casting|CastToBP_EnemySwarm OtherActor))
      (Variables|/Game/Devs/PRO_Mert/BluePrints/Enemies/Actors/BP_EnemySwarm.BP_EnemySwarm_C|SetOutOufBorder _asbp_enemy_swarm false))
    (:then_1
      (bind _asbp_enemy_sniper (Utilities|Casting|CastToBP_EnemySniper OtherActor))
      (Variables|/Game/Devs/PRO_Mert/BluePrints/Enemies/Actors/BP_EnemySniper.BP_EnemySniper_C|SetOutOufBorder _asbp_enemy_sniper false))
    (:then_2
      (bind _asbp_enemy_bomber (Utilities|Casting|CastToBP_EnemyBomber OtherActor))
      (Variables|/Game/Devs/PRO_Mert/BluePrints/Enemies/Actors/BP_EnemyBomber.BP_EnemyBomber_C|SetOutOufBorder _asbp_enemy_bomber false))))

(event OnComponentEndOverlap(SphereCollision)
  (params (OverlappedComponent :type Primitive%20Component%20Object%20Reference) (OtherActor :type Actor%20Object%20Reference) (OtherComp :type Primitive%20Component%20Object%20Reference) (OtherBodyIndex :type Integer))
  ;[1 1 1] Collision if Player is in Range
  (Utilities|FlowControl|Sequence
    (:then_0
      (bind _asbp_enemy_swarm (Utilities|Casting|CastToBP_EnemySwarm OtherActor))
      (Variables|/Game/Devs/PRO_Mert/BluePrints/Enemies/Actors/BP_EnemySwarm.BP_EnemySwarm_C|SetOutOufBorder _asbp_enemy_swarm true))
    (:then_1
      (bind _asbp_enemy_sniper (Utilities|Casting|CastToBP_EnemySniper OtherActor))
      (Variables|/Game/Devs/PRO_Mert/BluePrints/Enemies/Actors/BP_EnemySniper.BP_EnemySniper_C|SetOutOufBorder _asbp_enemy_sniper false))
    (:then_2
      (bind _asbp_enemy_bomber (Utilities|Casting|CastToBP_EnemyBomber OtherActor))
      (Variables|/Game/Devs/PRO_Mert/BluePrints/Enemies/Actors/BP_EnemyBomber.BP_EnemyBomber_C|SetOutOufBorder _asbp_enemy_bomber false))))

(fn ConstructionScript)