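; Flying sniper enemy ship that homes in on the player, then fires on random cooldowns and strafes on randomly timed direction changes within attack range.
; Hits drain a regenerating shield before health, scaled by the player's gun type and shown on widget bars.
; Death notifies the wave spawner, awards XP and spawns an explosion.
; TargetingAid places an aim marker along its velocity, casting to three player character classes.
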(event EventBeginPlay
  ;[1 0 0 0.25 20] Initial Events
  (|CGraphBeginPlay))

(event EventTick
  (params (DeltaSeconds :type Float%20%28single-precision%29))
  ;[1 0 0 0.25 20] Initial Events
  (|CGraphEventTick))

(fn ConstructionScript
  (bind _charactermovement (Variables|Character|GetCharacterMovement))
  (Variables|/Script/Engine.CharacterMovementComponent|SetMaxFlySpeed _charactermovement (Variables|Enemy|Settings|Movement|GetAcceleration))
  (Variables|/Script/Engine.CharacterMovementComponent|SetBrakingDecelerationFlying _charactermovement (Variables|Enemy|Settings|Movement|GetDecelaration)))

(event Custom|ShootProjectile
  (bind _enemygunclass_ref (Variables|Enemy|References|GetEnemyGunClass%20REF))
  (if true
    ;[1 1 1] Get & Shoot Projectile
    (Utilities|FlowControl|Delay (Math|Random|RandomFloatinRange (Variables|Enemy|Settings|Combat|GetShot%20Cooldown%20Min) (Variables|Enemy|Settings|Combat|GetShot%20Cooldown%20Max))) ; Cooldown Time
    (bind _outactors (Actor|GetAllActorsOfClass _enemygunclass_ref))
    (Game|SpawnActorfromClass _enemygunclass_ref (Math|Transform|MakeTransform (Transformation|GetActorLocation) (Transformation|GetActorRotation) (.scale (Transformation|GetActorTransform (Utilities|Array|Get(acopy) _outactors)))) "Undefined" "MultiplyWithRoot" 0 0)
    (Audio|PlaySoundatLocation "/Game/Devs/GD_Alex/Sounds/ShootingSFX/Laser/LaserShoot.LaserShoot" (Transformation|GetActorLocation) "0, 0, 0" 0.1 1.0 0.0 0 0 0 0) ; Shooting Audio
  ))

(event Custom|RoamToPlayer
  (bind _returnvalue (Transformation|GetActorLocation))
  (bind _player_character_ref (Variables|Enemy|References|GetPlayer%20Character%20REF))
  (bind _returnvalue_2 (Transformation|GetActorLocation _player_character_ref))
  (bind _returnvalue_3 (Math|Rotator|FindLookatRotation _returnvalue _returnvalue_2))
  (if (not (< (Transformation|GetDistanceTo _player_character_ref) (Variables|Enemy|Settings|Combat|GetSeePlayer%20Distance))) :!label _label
    (Transformation|SetActorRotation (Math|Interpolation|RInterpTo (Transformation|GetActorRotation) _returnvalue_3 (Utilities|Time|GetWorldDeltaSeconds) 0.0))
    (Pawn|Input|AddMovementInput (Math|Rotator|GetRotationXVector _returnvalue_3) 1.0 false)
    (Utilities|FlowControl|Delay 0.002)
    (goto _label)))

(event Custom|ShieldRecovery
  ;[1 1 1] Shield Regeneration
  (Utilities|FlowControl|Delay (Variables|Enemy|Settings|Combat|GetShield%20Regen%20Time))
  (if (Variables|Enemy|Conditions|GetShield%20Regenerated) :!label _label
    (Variables|Enemy|Conditions|SetShield%20Regenerated true :!label _label_2)
    (else
      (CallFunction|ShieldVisual)
      (if (not (Variables|Enemy|Conditions|GetEnemy%20Damaged))
        (if (< (Variables|Enemy|Settings|General|GetShield) 1.0)
          (Utilities|FlowControl|Delay 0.002)
          (Variables|Enemy|Settings|General|SetShield (+ (Variables|Enemy|Settings|General|GetShield) (Variables|Enemy|Settings|Combat|GetShield%20Regen%20Value)))
          (goto _label)
          (else
            (goto _label_2)))))))

(event Custom|GotHit
  (bind _returnvalue (Game|Player|GetPlayerPawn 0))
  (bind _returnvalue_2 (Game|Player|GetPlayerPawn 0))
  (bind _returnvalue_3 (Transformation|GetActorTransform))
  (bind _damage_received (Variables|Enemy|Conditions|GetDamage%20Received))
  (bind _damage_received_2 (Variables|Enemy|Conditions|GetDamage%20Received))
  (Effects|SpawnEmitteratLocation "/Game/StarterContent/Particles/P_Explosion.P_Explosion" (.location _returnvalue_3) (.rotation _returnvalue_3) "20.000000,20.000000,20.000000") ; Call Hit VFX
  ;[1 1 1] Hitmark
  (Audio|PlaySound2D "/Game/Devs/GD_Alex/Sounds/Ambience/SFX_Collide.SFX_Collide" 0.5 1.0 0.0 0 0 false) ; Hit Audio
  (bind _foundwidgets (Widget|GetAllWidgetsOfClass "/Game/Devs/PRO_Mert/BluePrints/Player/Widgets/PlayerCrosshair_W.PlayerCrosshair_W_C" false))
  (Default|Hitmarker (Utilities|Array|Get(acopy) _foundwidgets))
  (Variables|Enemy|Conditions|SetEnemy%20Damaged true)
  (bind _output_get (Variables|Enemy|Settings|General|SetShield (- (Variables|Enemy|Settings|General|GetShield) (Math|Float|SelectFloat (* (Variables|Enemy|Settings|Combat|GetLaser%20Damage%20Multiplier) _damage_received) _damage_received (Math|Boolean|ORBoolean (Variables|/Game/Devs/PRO_Mert/BluePrints/Player/Actors/BP_PlayerCharacter.BP_PlayerCharacter_C|GetLaser%20Gun (.AsBP%20Player%20Character (Utilities|Casting|CastToBP_PlayerCharacter _returnvalue_2))) (Variables|/Game/Devs/GD_Marius/Blueprints/Player/BP_PlayerCharacterMarius.BP_PlayerCharacterMarius_C|GetLaser%20Gun (.AsBP%20Player%20Character%20Marius (Utilities|Casting|CastToBP_PlayerCharacterMarius _returnvalue_2))) (Variables|/Game/Devs/GD_Alex/BluePrints/Player/BP_PlayerCharacterAlexJ.BP_PlayerCharacterAlexJ_C|GetLaser%20Gun (.AsBP%20Player%20Character%20Alex%20J (Utilities|Casting|CastToBP_PlayerCharacterAlexJ _returnvalue_2)))))))) ; Decrease Shield
  (CallFunction|ShieldVisual)
  (Utilities|FlowControl|Sequence
    (:then_0
      (|CGraphShow/HideShield))
    (:then_1
      (if (< _output_get 0.001) ; Check if Shield is active
        (bind _output_get_2 (Variables|Enemy|Settings|General|SetHealth (- (Variables|Enemy|Settings|General|GetHealth) (Math|Float|SelectFloat (* (Variables|Enemy|Settings|Combat|GetBallistic%20Damage%20Multiplier) _damage_received_2) _damage_received_2 (Math|Boolean|ORBoolean (Variables|/Game/Devs/PRO_Mert/BluePrints/Player/Actors/BP_PlayerCharacter.BP_PlayerCharacter_C|GetBallistic%20Gun (.AsBP%20Player%20Character (Utilities|Casting|CastToBP_PlayerCharacter _returnvalue))) (Variables|/Game/Devs/GD_Marius/Blueprints/Player/BP_PlayerCharacterMarius.BP_PlayerCharacterMarius_C|GetBallistic%20Gun (.AsBP%20Player%20Character%20Marius (Utilities|Casting|CastToBP_PlayerCharacterMarius _returnvalue))) (Variables|/Game/Devs/GD_Alex/BluePrints/Player/BP_PlayerCharacterAlexJ.BP_PlayerCharacterAlexJ_C|GetBallistic%20Gun (.AsBP%20Player%20Character%20Alex%20J (Utilities|Casting|CastToBP_PlayerCharacterAlexJ _returnvalue)))))))) ; Decrease Health
        (if (< _output_get_2 0.001)
          (CallFunction|EnemyDeath)
          (else
            (Utilities|FlowControl|Delay 0.2 :!label _label)
            (Variables|Enemy|Conditions|SetEnemy%20Damaged false)
            (CallFunction|ShieldRecovery)))
        (else
          (goto _label))))))

(event Custom|EnemyDeath
  (bind _returnvalue (Game|Player|GetPlayerPawn 0))
  (bind _xp_reward (Variables|Enemy|Settings|General|GetXP%20Reward))
  (bind (_asbp_player_character _bsuccess) (Utilities|Casting|CastToBP_PlayerCharacter _returnvalue))
  (bind (_asbp_player_character_marius _bsuccess_2) (Utilities|Casting|CastToBP_PlayerCharacterMarius _returnvalue))
  (bind (_asbp_player_character_alex_j _bsuccess_3) (Utilities|Casting|CastToBP_PlayerCharacterAlexJ _returnvalue))
  ;[1 1 1] WaveSpawner count
  (bind _outactors (Actor|GetAllActorsOfClass "/Game/Devs/PRO_Alex/Blueprints/Enemy-Spawner/EnemySpawner.EnemySpawner_C"))
  (Default|EnemyCounter (Utilities|Array|Get(acopy) _outactors))
  ;[1 1 1] Give Player Points according to Reward
  (if _bsuccess
    (Variables|/Game/Devs/PRO_Mert/BluePrints/Player/Actors/BP_PlayerCharacter.BP_PlayerCharacter_C|SetReceived%20XP _asbp_player_character _xp_reward)
    ;[1 1 1] Player Points Count
    (Default|AddPoints _asbp_player_character)
    ;[1 1 1] Death
    (Actor|DestroyActor :!label _label)
    (Game|SpawnActorfromClass "/Game/Devs/PRO_Mert/BluePrints/Enemies/Actors/BP_EnemySniperExplosionCopy.BP_EnemySniperExplosionCopy_C" (Math|Transform|MakeTransform (Transformation|GetActorLocation) (Transformation|GetActorRotation) "1.000000,1.000000,1.000000") "Undefined" "MultiplyWithRoot" 0 0)
    (elif _bsuccess_2
      (Variables|/Game/Devs/GD_Marius/Blueprints/Player/BP_PlayerCharacterMarius.BP_PlayerCharacterMarius_C|SetReceived%20XP _asbp_player_character_marius _xp_reward)
      (Default|AddPoints _asbp_player_character_marius)
      (goto _label)
      (elif _bsuccess_3
        (Variables|/Game/Devs/GD_Alex/BluePrints/Player/BP_PlayerCharacterAlexJ.BP_PlayerCharacterAlexJ_C|SetReceived%20XP _asbp_player_character_alex_j _xp_reward)
        (Default|AddPoints _asbp_player_character_alex_j)
        (goto _label)))))

(event Custom|ShieldVisual
  (bind _hitsphere (Variables|Default|GetHitSphere))
  (if (< (Variables|Enemy|Settings|General|GetShield) 0.01)
    (Development|SetHiddeninGame _hitsphere true false)
    (else
      (Development|SetHiddeninGame _hitsphere false false))))

(event Custom|StrafeDirection
  (Utilities|FlowControl|FlipFlop
    (:A
      (bind _isa (Utilities|FlowControl|FlipFlop)
        (:A
          _)
        (:B
          _))
      (Variables|Enemy|Conditions|SetStrafeRight _isa) ; Set if Enemy strafes to Left/Right
    )
    (:B
      (bind _isa_2 (Utilities|FlowControl|FlipFlop)
        (:A
          _)
        (:B
          _))
      (Variables|Enemy|Conditions|SetStrafeUp _isa_2) ; Set if Enemy strafes Up/Down
    ))
  (Utilities|Time|SetTimerbyEvent (delegate Custom|StrafeDirection) (Math|Random|RandomFloatinRange 2.0 5.0)))

(event Custom|TargetingAid
  (bind _returnvalue (Game|Player|GetPlayerPawn 0))
  (bind _returnvalue_2 (Transformation|GetVelocity))
  (bind _widgetaimtarget (Variables|Default|GetWidgetAimTarget))
  (bind _spacefighter (Variables|Default|GetSpaceFighter))
  (bind _player_character_ref (Variables|Enemy|References|GetPlayer%20Character%20REF))
  (bind _returnvalue_3 (Transformation|GetDistanceTo _player_character_ref))
  (bind _returnvalue_4 (Transformation|GetWorldLocation _spacefighter))
  (bind (_asbp_player_character _bsuccess) (Utilities|Casting|CastToBP_PlayerCharacter _returnvalue))
  (bind (_asbp_player_character_marius _bsuccess_2) (Utilities|Casting|CastToBP_PlayerCharacterMarius _returnvalue))
  (bind (_asbp_player_character_alex_j _bsuccess_3) (Utilities|Casting|CastToBP_PlayerCharacterAlexJ _returnvalue))
  (if _bsuccess
    (if (Variables|/Game/Devs/PRO_Mert/BluePrints/Player/Actors/BP_PlayerCharacter.BP_PlayerCharacter_C|GetTargeting _asbp_player_character)
      (if (< (Transformation|GetDistanceTo (Variables|Enemy|References|GetPlayer%20Character%20REF)) (Variables|Enemy|Settings|Combat|GetTargetAimDistance)) :!label _label
        (bind _outactors (Actor|GetAllActorsOfClass "/Game/Devs/PRO_Mert/BluePrints/Enemies/Actors/BP_EnemyCharacterSwarm.BP_EnemyCharacterSwarm_C"))
        (bind _outhit (Collision|LineTraceByChannel _returnvalue_4 (+ _returnvalue_4 (* _returnvalue_2 (/ (Math|Vector|VectorLength _returnvalue_2) (/ _returnvalue_3 (* (/ _returnvalue_3 2e+05) 7.5))))) "TraceTypeQuery1" true _outactors "ForOneFrame" true "(R=0.377410,G=0.401042,B=0.383318,A=1.000000)" "(R=0.095427,G=0.000000,B=1.000000,A=1.000000)" 1.0))
        (Development|SetHiddeninGame _widgetaimtarget false false)
        (Transformation|SetWorldLocation _widgetaimtarget (Math|Vector|VectorGetAbs (.TraceEnd (Collision|BreakHitResult _outhit))) false false)
        (Utilities|FlowControl|Delay 0.01)
        (CallFunction|TargetingAid)
        (else
          (Development|SetHiddeninGame (Variables|Default|GetWidgetAimTarget) true false :!label _label_2)))
      (else
        (goto _label_2)))
    (elif _bsuccess_2
      (if (Variables|/Game/Devs/GD_Marius/Blueprints/Player/BP_PlayerCharacterMarius.BP_PlayerCharacterMarius_C|GetTargeting _asbp_player_character_marius)
        (goto _label)
        (else
          (goto _label_2)))
      (elif _bsuccess_3
        (if (Variables|/Game/Devs/GD_Alex/BluePrints/Player/BP_PlayerCharacterAlexJ.BP_PlayerCharacterAlexJ_C|GetTargeting _asbp_player_character_alex_j)
          (goto _label)
          (else
            (goto _label_2)))))))