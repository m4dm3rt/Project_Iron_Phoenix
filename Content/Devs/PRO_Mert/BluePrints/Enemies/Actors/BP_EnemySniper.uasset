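; Flying sniper enemy fighter that hunts the player, firing after random cooldowns once in range.
; Each tick it aims ahead using player velocity and distance, then approaches, timer-strafes within attack range, or steers to BP_Center when out of border.
; Shield and health functions scale damage by type, triggering a predicted-position targeting marker.
; Damage also drives HUD bars and delayed shield regeneration; death awards XP and notifies the spawner.
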(event EventBeginPlay
  ;[1 0 0 0.25 40] Initial Events
  (|CG-BeginPlay))

(event EventTick
  (params (DeltaSeconds :type Float%20%28single-precision%29))
  ;[1 0 0 0.25 40] Initial Events
  (|CG-EventTick))

(fn ConstructionScript
  (bind _hitbox_scale (Variables|Enemy|Settings|Combat|GetHitbox%20Scale))
  (bind _charactermovement (Variables|Character|GetCharacterMovement))
  (Variables|/Script/Engine.CharacterMovementComponent|SetMaxFlySpeed _charactermovement (Variables|Enemy|Settings|Movement|GetAcceleration))
  (Variables|/Script/Engine.CharacterMovementComponent|SetBrakingDecelerationFlying _charactermovement (Variables|Enemy|Settings|Movement|GetDecelaration))
  (Transformation|SetRelativeScale3D (Variables|Default|GetHitSphere) (Math|Vector|MakeVector _hitbox_scale _hitbox_scale _hitbox_scale)))

(fn ReceiveShieldDamage
  (params (DamageReceived :type Float%20%28double-precision%29) (DamageType :type String))
  (bind _damage_received (Variables|Enemy|Conditions|GetDamage%20Received))
  (Variables|Enemy|Conditions|SetDamaged true)
  (Variables|Enemy|Conditions|SetShield%20Regenerated false)
  (CallFunction|TargetingAid)
  (if (Utilities|Enum|Equal(Enum) DamageType "Missile")
    (Variables|Enemy|Settings|General|SetShield (Math|Float|Clamp(Float) (- (Variables|Enemy|Settings|General|GetShield) (Variables|Enemy|Conditions|GetDamage%20Received)) 0.0 (Variables|Enemy|Settings|General|GetShield))) ; Decrease Shield
    (bind _output_get (Variables|Enemy|Conditions|SetMissile%20Damage (Math|Float|Absolute(Float) (- (Variables|Enemy|Settings|General|GetShield) (Variables|Enemy|Conditions|GetDamage%20Received)))))
    (else
      (Variables|Enemy|Settings|General|SetShield (Math|Float|Clamp(Float) (- (Variables|Enemy|Settings|General|GetShield) (* (Math|Float|SelectFloat (* (Variables|Enemy|Settings|Combat|GetLaser%20Damage%20Multiplier) _damage_received) _damage_received (Utilities|Enum|Equal(Enum) DamageType "Laser")) 1.2)) 0.0 (Variables|Enemy|Settings|General|GetShield))) ; Decrease Shield
    ))
  (return (Variables|Enemy|Settings|General|GetShield) _output_get))

(fn ReceiveHealthDamage
  (params (DamageReceived :type Float%20%28double-precision%29) (DamageType :type String))
  (bind _damage_received (Variables|Enemy|Conditions|GetDamage%20Received))
  (Variables|Enemy|Conditions|SetDamaged true)
  (CallFunction|TargetingAid)
  (if (Utilities|Enum|Equal(Enum) DamageType "Missile")
    (Variables|Enemy|Settings|General|SetHealth (- (Variables|Enemy|Settings|General|GetHealth) (* (Variables|Enemy|Conditions|GetDamage%20Received) 2.0))) ; Decrease Health
    (else
      (Variables|Enemy|Settings|General|SetHealth (- (Variables|Enemy|Settings|General|GetHealth) (* (Math|Float|SelectFloat (* (Variables|Enemy|Settings|Combat|GetKinetic%20Damage%20Multiplier) _damage_received) _damage_received (Utilities|Enum|Equal(Enum) DamageType "Kinetic")) 1.5))) ; Decrease Health
    ))
  (return (Variables|Enemy|Settings|General|GetHealth)))

(event Custom|SetShieldHealthW
  (bind _player_character_ref (Variables|Enemy|References|GetPlayer%20Character%20REF))
  (bind _playerhud_ref (Variables|/Game/Devs/PRO_Mert/BluePrints/Player/MISC/BP_SingleplayerCharacter.BP_SingleplayerCharacter_C|GetPlayerHUD%20REF _player_character_ref))
  (Progress|SetPercent (Variables|/Game/Devs/PRO_Mert/BluePrints/UI/HUD/PlayerHUD_W.PlayerHUD_W_C|GetEnemy_ShieldBar _playerhud_ref) (/ (Variables|Enemy|Settings|General|GetShield) 1e+02))
  (Progress|SetPercent (Variables|/Game/Devs/PRO_Mert/BluePrints/UI/HUD/PlayerHUD_W.PlayerHUD_W_C|GetEnemy_HealthBar _playerhud_ref) (/ (Variables|Enemy|Settings|General|GetHealth) 1e+02))
  (Variables|/Game/Devs/PRO_Mert/BluePrints/UI/HUD/PlayerHUD_W.PlayerHUD_W_C|SetEnemySniperHealth _playerhud_ref true)
  (Variables|/Game/Devs/PRO_Mert/BluePrints/UI/HUD/PlayerHUD_W.PlayerHUD_W_C|SetEnemyREF _playerhud_ref (Utilities|GetDisplayName self))
  (if (Variables|Enemy|Conditions|GetShield%20Regenerated) :!label _label
    (Variables|/Game/Devs/PRO_Mert/BluePrints/UI/HUD/PlayerHUD_W.PlayerHUD_W_C|SetEnemySniperHealth _playerhud_ref false)
    (else
      (Utilities|FlowControl|Delay 0.2)
      (goto _label))))

(event Custom|HideHealthReticle
  (Variables|/Game/Devs/PRO_Mert/BluePrints/UI/HUD/PlayerHUD_W.PlayerHUD_W_C|SetEnemySniperHealth (Variables|/Game/Devs/PRO_Mert/BluePrints/Player/MISC/BP_SingleplayerCharacter.BP_SingleplayerCharacter_C|GetPlayerHUD%20REF (Variables|Enemy|References|GetPlayer%20Character%20REF)) false))

(event Custom|ShootProjectile
  ;[1 1 1] Shoot Projectile
  (Utilities|FlowControl|Delay (Math|Random|RandomFloatinRange (Variables|Enemy|Settings|Combat|GetShot%20Cooldown%20Min) (Variables|Enemy|Settings|Combat|GetShot%20Cooldown%20Max))) ; Cooldown Time
  (Class|EnemyAI|SpawnProjectile (Variables|Enemy|References|GetEnemyGunClass%20REF)))

(event Custom|ShieldRecovery
  ;[1 1 1] Shield Regeneration
  (if (Variables|Enemy|Conditions|GetShield%20Regenerated) :!label _label
    (Variables|Enemy|Conditions|SetShield%20Regenerated true :!label _label_2)
    (if (not (< (Variables|Enemy|Settings|General|GetHealth) 1e+02))
      (Default|StopHighlight (Variables|/Game/Devs/PRO_Mert/BluePrints/Enemies/MISC/BP_IndicatorComponent.BP_IndicatorComponent_C|GetEnemyIndicator_W%20REF (Variables|Default|GetBP_IndicatorComponent)))
      (CallFunction|StopTargeting))
    (else
      (Utilities|FlowControl|Sequence
        (:then_0
          (if (not (Variables|Enemy|Conditions|GetDamaged))
            (if (< (Variables|Enemy|Settings|General|GetShield) 1e+02)
              (Utilities|FlowControl|Delay 0.002)
              (Variables|Enemy|Settings|General|SetShield (+ (Variables|Enemy|Settings|General|GetShield) (Variables|Enemy|Settings|Combat|GetShield%20Regen%20Value)))
              (goto _label)
              (else
                (goto _label_2)))))
        (:then_1
          (if (Utilities|Enum|Equal(Enum) (Variables|/Game/Devs/PRO_Mert/BluePrints/UI/HUD/PlayerHUD_W.PlayerHUD_W_C|GetEnemyREF (Variables|/Game/Devs/PRO_Mert/BluePrints/Player/MISC/BP_SingleplayerCharacter.BP_SingleplayerCharacter_C|GetPlayerHUD%20REF (Variables|Enemy|References|GetPlayer%20Character%20REF))) (Utilities|GetDisplayName self)) ; Check if HUD Health is this Enemy
            (CallFunction|SetShieldHealthW)))))))

(event Custom|EnemyDeath
  (bind _player_character_ref (Variables|Enemy|References|GetPlayer%20Character%20REF))
  (Utilities|FlowControl|DoOnce false
    (:Completed
      ;[1 1 1] WaveSpawner count
      (bind _returnvalue (Actor|GetActorOfClass "/Game/Devs/PRO_Alex/Blueprints/World/EnemySpawner.EnemySpawner_C"))
      (Default|EnemyKillCounter _returnvalue)
      ;[1 1 1] Give Player Points according to Reward
      (Default|AddXP _player_character_ref (Variables|Enemy|Settings|General|GetXP%20Reward))
      ;[1 1 1] Death
      (Default|DestroySFX _player_character_ref)
      (Game|SpawnActorfromClass "/Game/Devs/DA_Leo/Leo_BluePrints/Leo_Enemies/BP_EnemyExplosion.BP_EnemyExplosion_C" (Transformation|GetActorTransform) "Undefined" "MultiplyWithRoot" 0 0)
      (Utilities|FlowControl|Delay 0.2)
      (Actor|DestroyActor))))

(event Game|Damage|EventAnyDamage
  (params (Damage :type Float%20%28single-precision%29) (DamageType :type Damage%20Type%20Object%20Reference) (InstigatedBy :type Controller%20Object%20Reference) (DamageCauser :type Actor%20Object%20Reference))
  (bind _output_get (Variables|Enemy|Conditions|SetDamage%20Received Damage))
  (bind _output_get_2 (Variables|Enemy|References|SetDamageType DamageType))
  (bind (_damageout _damagetype) (Class|BaseDamage|ProccessDamage(Message) _output_get_2 _output_get))
  (bind _health (CallFunction|ReceiveHealthDamage _damageout _damagetype))
  (Default|HighlightEnemy (Variables|/Game/Devs/PRO_Mert/BluePrints/Enemies/MISC/BP_IndicatorComponent.BP_IndicatorComponent_C|GetEnemyIndicator_W%20REF (Variables|Default|GetBP_IndicatorComponent)))
  (if (<= _health 0.0)
    (CallFunction|EnemyDeath)
    (CallFunction|HideHealthReticle)
    (else
      (CallFunction|SetShieldHealthW)
      (Utilities|Time|SetTimerbyEvent (EventDispatchers|CreateEvent :!event Custom|ShieldRecovery) (Variables|Enemy|Settings|Combat|GetShield%20Regen%20Delay))
      (Utilities|FlowControl|Delay 0.2)
      (Variables|Enemy|Conditions|SetDamaged false))))

(event Custom|StrafeDirection
  (if (Math|Random|RandomBoolwithWeight 0.5)
    (bind _isa (Utilities|FlowControl|FlipFlop)
      (:A
        _)
      (:B
        _))
    (Variables|Enemy|Conditions|SetStrafeRight _isa) ; Set if Enemy strafes to Left/Right
    (else
      (bind _isa_2 (Utilities|FlowControl|FlipFlop)
        (:A
          _)
        (:B
          _))
      (Variables|Enemy|Conditions|SetStrafeUp _isa_2) ; Set if Enemy strafes Up/Down
    ))
  (Utilities|Time|SetTimerbyEvent (delegate Custom|StrafeDirection) (Math|Random|RandomFloatinRange (Variables|Enemy|Settings|Combat|GetCombatStrafeMinDirChange) (Variables|Enemy|Settings|Combat|GetCombatStrafeMaxDirChange))))

(event Custom|TargetingAid
  (bind _player_character_ref (Variables|Enemy|References|GetPlayer%20Character%20REF))
  (bind _spacefighter (Variables|Default|GetSpaceFighter))
  (bind _returnvalue (Transformation|GetWorldLocation _spacefighter))
  (if (and (Variables|/Game/Devs/PRO_Mert/BluePrints/Player/MISC/BP_SingleplayerCharacter.BP_SingleplayerCharacter_C|GetLaserBeam _player_character_ref) (Variables|/Script/Project_Iron_Phoenix.SingleplayerPawn|GetLaserGun _player_character_ref))
    (bind _outhit (Collision|LineTraceByChannel _returnvalue _returnvalue "TraceTypeQuery1" true 0 "ForOneFrame" true "(R=0.537255,G=0.007843,B=0.000000,A=0.749020)" "(R=0.095427,G=0.000000,B=1.000000,A=0.000000)" 1.0))
    (Development|SetHiddeninGame (Variables|Default|GetWidgetTargetBallistic) false false)
    (Transformation|SetWorldLocation (Variables|Default|GetSphereCollisionTarget) (.TraceEnd (Collision|BreakHitResult _outhit)) false false)
    (else
      (bind _outhit_2 (Collision|LineTraceByChannel _returnvalue (+ _returnvalue (* (Transformation|GetVelocity) (/ (Transformation|GetDistanceTo _player_character_ref) 6e+04))) "TraceTypeQuery1" true 0 "ForOneFrame" true "(R=0.537255,G=0.007843,B=0.000000,A=0.749020)" "(R=0.095427,G=0.000000,B=1.000000,A=0.000000)" 1.0))
      (Development|SetHiddeninGame (Variables|Default|GetWidgetTargetBallistic) false false)
      (Transformation|SetWorldLocation (Variables|Default|GetSphereCollisionTarget) (.TraceEnd (Collision|BreakHitResult _outhit_2)) false false)))
  (Utilities|Time|SetTimerbyEvent (delegate Custom|TargetingAid) 0.01 true))

(event Custom|StopTargeting
  (Development|SetHiddeninGame (Variables|Default|GetWidgetTargetBallistic) true false))