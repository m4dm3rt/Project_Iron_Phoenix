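; Flying sniper enemy for multiplayer that hunts player pawn 0 with velocity-led aim.
; Tick closes distance, fires on randomized delays when in range, and strafes on a randomly re-rolled axis within attack distance.
; Damage drains a regenerating shield, then health, using weapon-type multipliers and updating the player's HUD bars.
; Death notifies the wave spawner and spawns an explosion; item drop and targeting-aid logic are disconnected.
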(event EventBeginPlay
  ;[1 0 0 0.25 40] Initial Events
  (|CG-BeginPlay))

(event EventTick
  (params (DeltaSeconds :type Float%20%28single-precision%29))
  ;[1 0 0 0.25 40] Initial Events
  (|CG-EventTick))

(fn ConstructionScript
  (bind _hitbox_scale (Variables|Enemy|Settings|Combat|GetHitbox%20Scale))
  (bind _charactermovement (Variables|Character|GetCharacterMovement))
  (Variables|/Script/Engine.CharacterMovementComponent|SetMaxFlySpeed _charactermovement (Variables|Enemy|Settings|Movement|GetAcceleration))
  (Variables|/Script/Engine.CharacterMovementComponent|SetBrakingDecelerationFlying _charactermovement (Variables|Enemy|Settings|Movement|GetDecelaration))
  (Transformation|SetRelativeScale3D (Variables|Default|GetHitSphere) (Math|Vector|MakeVector _hitbox_scale _hitbox_scale _hitbox_scale)))

(event Custom|SetShieldHealthW
  (bind _returnvalue (Game|Player|GetPlayerPawn 0))
  (bind _asbp_multiplayer_character (Utilities|Casting|CastToBP_MultiplayerCharacter _returnvalue))
  (bind _multiplayerhud_ref (Variables|/Game/Devs/PRO_Mert/BluePrints/Multiplayer/InGame/Player/BP_MultiplayerCharacter.BP_MultiplayerCharacter_C|GetMultiplayerHUD%20REF _asbp_multiplayer_character))
  (Progress|SetPercent (Variables|/Game/Devs/PRO_Mert/BluePrints/Multiplayer/InGame/Widgets/MultiplayerHUD_W.MultiplayerHUD_W_C|GetEnemy_ShieldBar _multiplayerhud_ref) (/ (Variables|Enemy|Settings|General|GetShield) 1e+02))
  (Progress|SetPercent (Variables|/Game/Devs/PRO_Mert/BluePrints/Multiplayer/InGame/Widgets/MultiplayerHUD_W.MultiplayerHUD_W_C|GetEnemy_HealthBar _multiplayerhud_ref) (/ (Variables|Enemy|Settings|General|GetHealth) 1e+02))
  (Variables|/Game/Devs/PRO_Mert/BluePrints/Multiplayer/InGame/Widgets/MultiplayerHUD_W.MultiplayerHUD_W_C|SetEnemySniperHealth _multiplayerhud_ref true)
  (Variables|/Game/Devs/PRO_Mert/BluePrints/Multiplayer/InGame/Widgets/MultiplayerHUD_W.MultiplayerHUD_W_C|SetEnemy%20REF _multiplayerhud_ref (Utilities|GetDisplayName self))
  (if (Variables|Enemy|Conditions|GetShield%20Regenerated) :!label _label
    (Variables|/Game/Devs/PRO_Mert/BluePrints/Multiplayer/InGame/Widgets/MultiplayerHUD_W.MultiplayerHUD_W_C|SetEnemySniperHealth _multiplayerhud_ref false)
    (else
      (Utilities|FlowControl|Delay 0.2)
      (goto _label))))

(event Custom|HideHealthReticle
  (Variables|/Game/Devs/PRO_Mert/BluePrints/Multiplayer/InGame/Widgets/MultiplayerHUD_W.MultiplayerHUD_W_C|SetEnemySniperHealth (Variables|/Game/Devs/PRO_Mert/BluePrints/Multiplayer/InGame/Player/BP_MultiplayerCharacter.BP_MultiplayerCharacter_C|GetMultiplayerHUD%20REF (.AsBP%20Multiplayer%20Character (Utilities|Casting|CastToBP_MultiplayerCharacter (Game|Player|GetPlayerPawn 0)))) false))

(event Custom|ShootProjectile
  (bind _returnvalue (Transformation|GetActorTransform))
  (bind _enemygunclass_ref (Variables|Enemy|References|GetEnemyGunClass%20REF))
  ;[1 1 1] Get & Shoot Projectile
  (Utilities|FlowControl|Delay (Math|Random|RandomFloatinRange (Variables|Enemy|Settings|Combat|GetShot%20Cooldown%20Min) (Variables|Enemy|Settings|Combat|GetShot%20Cooldown%20Max))) ; Cooldown Time
  (bind _outactors (Actor|GetAllActorsOfClass _enemygunclass_ref))
  (Game|SpawnActorfromClass _enemygunclass_ref (Math|Transform|MakeTransform (.location _returnvalue) (.rotation _returnvalue) (.scale (Transformation|GetActorTransform (Utilities|Array|Get(acopy) _outactors)))) "Undefined" "MultiplyWithRoot" 0 0)
  (Audio|PlaySoundatLocation "/Game/Devs/GD_Alex/Sounds/ShootingSFX/Laser/LaserShoot.LaserShoot" (Transformation|GetActorLocation) "0, 0, 0" 0.1 1.0 0.0 0 0 0 0) ; Shooting Audio
)

(event Custom|ShieldRecovery
  ;[1 1 1] Shield Regeneration
  (if (Variables|Enemy|Conditions|GetShield%20Regenerated) :!label _label
    (Variables|Enemy|Conditions|SetShield%20Regenerated true :!label _label_2)
    (Default|HideRed (Variables|/Game/Devs/PRO_Mert/BluePrints/Enemies/MISC/BP_IndicatorComponent.BP_IndicatorComponent_C|GetEnemyIndicator_W%20REF (Variables|Default|GetBP_IndicatorComponent)))
    (else
      (CallFunction|ShieldVisual)
      (Utilities|FlowControl|Sequence
        (:then_0
          (if (< (Variables|Enemy|Settings|General|GetShield) 1e+02)
            (Utilities|FlowControl|Delay 0.002)
            (Variables|Enemy|Settings|General|SetShield (+ (Variables|Enemy|Settings|General|GetShield) (Variables|Enemy|Settings|Combat|GetShield%20Regen%20Value)))
            (goto _label)
            (else
              (goto _label_2))))
        (:then_1
          (if (Utilities|Enum|Equal(Enum) (Variables|/Game/Devs/PRO_Mert/BluePrints/Multiplayer/InGame/Widgets/MultiplayerHUD_W.MultiplayerHUD_W_C|GetEnemy%20REF (Variables|/Game/Devs/PRO_Mert/BluePrints/Multiplayer/InGame/Player/BP_MultiplayerCharacter.BP_MultiplayerCharacter_C|GetMultiplayerHUD%20REF (.AsBP%20Multiplayer%20Character (Utilities|Casting|CastToBP_MultiplayerCharacter (Game|Player|GetPlayerPawn 0))))) (Utilities|GetDisplayName self)) ; Check if HUD Health is this Enemy
            (CallFunction|SetShieldHealthW)))))))

(event Custom|EnemyDeath
  ;[1 1 1] WaveSpawner count
  (bind _outactors (Actor|GetAllActorsOfClass "/Game/Devs/PRO_Mert/BluePrints/Multiplayer/InGame/Enemies/BP_EnemySpawnerMultiplayer.BP_EnemySpawnerMultiplayer_C"))
  (Default|EnemyKillCounter (Utilities|Array|Get(acopy) _outactors))
  ;[1 1 1] Death
  (Actor|DestroyActor)
  (Game|SpawnActorfromClass "/Game/Devs/PRO_Mert/BluePrints/Enemies/Actors/BP_EnemySwarmExplosion.BP_EnemySwarmExplosion_C" (Transformation|GetActorTransform) "Undefined" "MultiplyWithRoot" 0 0))

(event Custom|ShieldVisual
  (bind _hitsphere (Variables|Default|GetHitSphere))
  (if (< (Variables|Enemy|Settings|General|GetShield) 0.01)
    (Development|SetHiddeninGame _hitsphere true false)
    (else
      (Development|SetHiddeninGame _hitsphere false false))))

(event Game|Damage|EventAnyDamage
  (params (Damage :type Float%20%28single-precision%29) (DamageType :type Damage%20Type%20Object%20Reference) (InstigatedBy :type Controller%20Object%20Reference) (DamageCauser :type Actor%20Object%20Reference))
  (Variables|Enemy|Conditions|SetDamage%20Received Damage)
  (Variables|Enemy|Conditions|SetShield%20Regenerated false)
  (bind _output_get (Variables|Enemy|Settings|General|SetShield (- (Variables|Enemy|Settings|General|GetShield) (Math|Float|SelectFloat (* (Variables|Enemy|Settings|Combat|GetLaser%20Damage%20Multiplier) (Variables|Enemy|Conditions|GetDamage%20Received)) (Variables|Enemy|Conditions|GetDamage%20Received) (Variables|/Game/Devs/PRO_Mert/BluePrints/Multiplayer/InGame/Player/BP_MultiplayerCharacter.BP_MultiplayerCharacter_C|GetLaserGun (.AsBP%20Multiplayer%20Character (Utilities|Casting|CastToBP_MultiplayerCharacter (Game|Player|GetPlayerPawn 0)))))))) ; Decrease Shield
  (CallFunction|ShieldVisual)
  (Default|ShowRed (Variables|/Game/Devs/PRO_Mert/BluePrints/Enemies/MISC/BP_IndicatorComponent.BP_IndicatorComponent_C|GetEnemyIndicator_W%20REF (Variables|Default|GetBP_IndicatorComponent)))
  (if (<= _output_get 0.0) ; Check if Shield is active
    (bind _output_get_2 (Variables|Enemy|Settings|General|SetHealth (- (Variables|Enemy|Settings|General|GetHealth) (Math|Float|SelectFloat (* (Variables|Enemy|Settings|Combat|GetBallistic%20Damage%20Multiplier) (Variables|Enemy|Conditions|GetDamage%20Received)) (Variables|Enemy|Conditions|GetDamage%20Received) (Variables|/Game/Devs/PRO_Mert/BluePrints/Multiplayer/InGame/Player/BP_MultiplayerCharacter.BP_MultiplayerCharacter_C|GetBallisticGun (.AsBP%20Multiplayer%20Character (Utilities|Casting|CastToBP_MultiplayerCharacter (Game|Player|GetPlayerPawn 0)))))))) ; Decrease Health
    (if (<= _output_get_2 0.0)
      (CallFunction|EnemyDeath)
      (CallFunction|HideHealthReticle)
      (else
        (CallFunction|SetShieldHealthW :!label _label)
        (Utilities|Time|SetTimerbyEvent (EventDispatchers|CreateEvent :!event Custom|ShieldRecovery) (Variables|Enemy|Settings|Combat|GetShield%20Regen%20Delay))))
    (else
      (goto _label))))

(event Custom|StrafeDirection
  (if (Math|Random|RandomBoolwithWeight 0.5)
    (bind _isa (Utilities|FlowControl|FlipFlop)
      (:A
        _)
      (:B
        _))
    (Variables|Enemy|Conditions|SetStrafeRight _isa) ; Set if Enemy strafes to Left/Right
    (else
      (bind _isa_2 (Utilities|FlowControl|FlipFlop)
        (:A
          _)
        (:B
          _))
      (Variables|Enemy|Conditions|SetStrafeUp _isa_2) ; Set if Enemy strafes Up/Down
    ))
  (Utilities|Time|SetTimerbyEvent (delegate Custom|StrafeDirection) (Math|Random|RandomFloatinRange 3.0 6.0)))

(event Custom|TargetingAid)