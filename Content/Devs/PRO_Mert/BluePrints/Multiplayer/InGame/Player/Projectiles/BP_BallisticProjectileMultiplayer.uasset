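; Multiplayer ballistic projectile that flies straight at a configurable speed with gravity disabled in the construction script.
; Each tick it sphere-traces well ahead along its forward vector rather than relying on collision events.
; A cast chain damages asteroids, swarm and sniper enemies, and player characters, who take double damage.
; Those hits share one path that spawns an emitter, triggers the crosshair hitmarker, plays a sound and destroys the projectile.
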(event EventTick
  (params (DeltaSeconds :type Float%20%28single-precision%29))
  (bind _damage (Variables|Projectile|Settings|GetDamage))
  (bind _sphere (Variables|Default|GetSphere))
  (bind _returnvalue (Transformation|GetWorldLocation _sphere))
  (bind (_outhit _returnvalue_2) (Collision|SphereTraceByChannel _returnvalue (+ _returnvalue (* (Math|Vector|GetForwardVector (Transformation|GetWorldRotation _sphere)) 2e+03)) 1e+02 "TraceTypeQuery1" false 0 "None"))
  (if _returnvalue_2
    (bind _asbp_asteroid (Utilities|Casting|CastToBP_Asteroid (.HitActor (Collision|BreakHitResult _outhit)))
      (:then
        (Game|Damage|ApplyDamage _asbp_asteroid _damage 0 0))
      (:CastFailed
        (bind _asbp_enemy_swarm_multiplayer (Utilities|Casting|CastToBP_EnemySwarmMultiplayer (.HitActor (Collision|BreakHitResult _outhit)))
          (:then
            (Game|Damage|ApplyDamage _asbp_enemy_swarm_multiplayer _damage 0 0))
          (:CastFailed
            (bind _asbp_enemy_sniper_multiplayer (Utilities|Casting|CastToBP_EnemySniperMultiplayer (.HitActor (Collision|BreakHitResult _outhit)))
              (:then
                (Game|Damage|ApplyDamage _asbp_enemy_sniper_multiplayer _damage 0 0))
              (:CastFailed
                (bind _asbp_multiplayer_character (Utilities|Casting|CastToBP_MultiplayerCharacter (.HitActor (Collision|BreakHitResult _outhit))))
                (Game|Damage|ApplyDamage _asbp_multiplayer_character (* _damage 2.0) 0 0)))))))
    (Effects|SpawnEmitteratLocation "/Game/Realistic_Starter_VFX_Pack_Vol2/Particles/Hit/P_Default.P_Default" (.Location (Collision|BreakHitResult _outhit)) "0, 0, 0" "50.000000,50.000000,50.000000")
    (bind _foundwidgets (Widget|GetAllWidgetsOfClass "/Game/Devs/PRO_Mert/BluePrints/Multiplayer/InGame/Widgets/MultiplayerCrosshair_W.MultiplayerCrosshair_W_C" false))
    (Default|Hitmarker (Utilities|Array|Get(acopy) _foundwidgets))
    (Audio|PlaySound2D "/Game/Devs/GD_Alex/Sounds/Ambience/SFX_Collide.SFX_Collide" 0.5 1.0 0.0 0 0 false) ; Hit Audio
    (Actor|DestroyActor)))

(fn ConstructionScript
  (bind _projectilemovement (Variables|Default|GetProjectileMovement))
  (bind _output_get (Variables|/Script/Engine.ProjectileMovementComponent|SetInitialSpeed _projectilemovement (Variables|Projectile|Settings|GetSpeed)))
  (Variables|/Script/Engine.ProjectileMovementComponent|SetMaxSpeed _projectilemovement _output_get)
  (Variables|/Script/Engine.ProjectileMovementComponent|SetProjectileGravityScale _projectilemovement 0.0))