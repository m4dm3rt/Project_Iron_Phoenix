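; Multiplayer missile projectile that damages asteroids, swarm and sniper enemies, and player characters.
; Construction sets a constant speed without gravity; each Tick sphere-traces ahead along the mesh's up vector, applies damage on a matching hit, spawns an explosion and destroys its components, not the actor.
; HomingProjectile, not called within this graph, re-runs every 0.02 seconds to home on the nearest BP_EnemySwarm, rather than the multiplayer enemy classes.
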(event Custom|HomingProjectile
  ;[1 0.1979 0.1979] Homing Logic
  (Variables|/Script/Engine.ProjectileMovementComponent|SetbIsHomingProjectile (Variables|Default|GetProjectileMovement) true)
  (bind _outactors (Actor|GetAllActorsOfClass "/Game/Devs/PRO_Mert/BluePrints/Enemies/Actors/BP_EnemySwarm.BP_EnemySwarm_C"))
  (for _array_element _outactors
    (if (< (Math|Vector|VectorLength (- (Transformation|GetActorLocation _array_element) (Transformation|GetActorLocation))) (Variables|Projectile|Conditions|GetClosest%20Distance))
      (Variables|Projectile|Conditions|SetClosest%20Distance (Math|Vector|VectorLength (- (Transformation|GetActorLocation _array_element) (Transformation|GetActorLocation))))
      (Variables|Projectile|References|SetTarget _array_element)))
  (Variables|/Script/Engine.ProjectileMovementComponent|SetHomingTargetComponent (Variables|Default|GetProjectileMovement) (Variables|/Game/Devs/PRO_Mert/BluePrints/Enemies/Actors/BP_EnemySwarm.BP_EnemySwarm_C|GetSpaceFighter (Variables|Projectile|References|GetTarget)))
  (Utilities|FlowControl|Delay 0.02)
  (CallFunction|HomingProjectile))

(event EventTick
  (params (DeltaSeconds :type Float%20%28single-precision%29))
  (bind _damage (Variables|Projectile|Settings|GetDamage))
  (bind _staticmesh (Variables|Default|GetStaticMesh))
  (bind _returnvalue (Transformation|GetWorldLocation _staticmesh))
  (bind (_outhit _returnvalue_2) (Collision|SphereTraceByChannel _returnvalue (+ _returnvalue (* (Math|Vector|GetUpVector (Transformation|GetWorldRotation _staticmesh)) 2e+03)) 1e+02 "TraceTypeQuery1" false 0 "None"))
  (if _returnvalue_2
    (bind _asbp_asteroid (Utilities|Casting|CastToBP_Asteroid (.HitActor (Collision|BreakHitResult _outhit)))
      (:then
        (Game|Damage|ApplyDamage _asbp_asteroid _damage 0 0))
      (:CastFailed
        (bind _asbp_enemy_swarm_multiplayer (Utilities|Casting|CastToBP_EnemySwarmMultiplayer (.HitActor (Collision|BreakHitResult _outhit)))
          (:then
            (Game|Damage|ApplyDamage _asbp_enemy_swarm_multiplayer _damage 0 0))
          (:CastFailed
            (bind _asbp_enemy_sniper_multiplayer (Utilities|Casting|CastToBP_EnemySniperMultiplayer (.HitActor (Collision|BreakHitResult _outhit)))
              (:then
                (Game|Damage|ApplyDamage _asbp_enemy_sniper_multiplayer _damage 0 0))
              (:CastFailed
                (bind _asbp_multiplayer_character (Utilities|Casting|CastToBP_MultiplayerCharacter (.HitActor (Collision|BreakHitResult _outhit))))
                (Game|Damage|ApplyDamage _asbp_multiplayer_character _damage 0 0)))))))
    (Effects|SpawnEmitteratLocation "/Game/Realistic_Starter_VFX_Pack_Vol2/Particles/Explosion/P_Explosion_Smoke.P_Explosion_Smoke" (.Location (Collision|BreakHitResult _outhit)) "0, 0, 0" "25.000000,25.000000,25.000000")
    (Components|DestroyComponent (Variables|Default|GetMissileIndicator))))

(fn ConstructionScript
  (bind _projectilemovement (Variables|Default|GetProjectileMovement))
  (bind _output_get (Variables|/Script/Engine.ProjectileMovementComponent|SetInitialSpeed _projectilemovement (Variables|Projectile|Settings|GetSpeed)))
  (Variables|/Script/Engine.ProjectileMovementComponent|SetMaxSpeed _projectilemovement _output_get)
  (Variables|/Script/Engine.ProjectileMovementComponent|SetProjectileGravityScale _projectilemovement 0.0))