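; Asteroid actor that scatters in a huge random volume and, if destructible, explodes when damage depletes its health.
; BeginPlay enables collision and visibility through separate random picks from ten meshes, then randomly relocates the meshes and explosion effect.
; Death passes through DestroySrv to DestroyMC, which fires Niagara and destroys the meshes.
; It then grants XP to player zero's singleplayer character, with multiplayer sound chained behind that cast.
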(event Custom|Destroy%20MC
  (Components|Activation|Activate (Variables|Default|GetNS_AsteroidExplosion) false)
  (Components|DestroyComponent (Variables|Default|GetAsteroidMesh5))
  ;[1 1 1] Give Player Points according to Reward
  (bind _asbp_singleplayer_character (Utilities|Casting|CastToBP_SingleplayerCharacter (Game|Player|GetPlayerPawn 0)))
  (Variables|/Game/Devs/PRO_Mert/BluePrints/Player/MISC/BP_SingleplayerCharacter.BP_SingleplayerCharacter_C|SetReceivedXP _asbp_singleplayer_character (Variables|Asteroid|Settings|GetXP%20Reward))
  ;[1 1 1] Player Points Count
  (Default|AddXP _asbp_singleplayer_character)
  (Default|DestroySFX _asbp_singleplayer_character)
  (bind _asbp_mpcharacter (Utilities|Casting|CastToBP_MPCharacter (Game|Player|GetPlayerPawn 0)))
  (Default|DestroySFX _asbp_mpcharacter))

(event Custom|Destroy%20Srv
  (CallFunction|DestroyMC))

(event Game|Damage|EventAnyDamage
  (params (Damage :type Float%20%28single-precision%29) (DamageType :type Damage%20Type%20Object%20Reference) (InstigatedBy :type Controller%20Object%20Reference) (DamageCauser :type Actor%20Object%20Reference))
  (Variables|Asteroid|Conditions|SetDamage%20Received Damage)
  (if (Variables|Asteroid|Settings|GetDestructible)
    (bind _output_get (Variables|Asteroid|Settings|SetHealth (- (Variables|Asteroid|Settings|GetHealth) (Variables|Asteroid|Conditions|GetDamage%20Received))))
    (if (< _output_get 0.001)
      (CallFunction|DestroySrv))))

(event EventBeginPlay
  (bind _asteroidmesh6 (Variables|Default|GetAsteroidMesh6))
  (bind _asteroidmesh1 (Variables|Default|GetAsteroidMesh1))
  (bind _asteroidmesh2 (Variables|Default|GetAsteroidMesh2))
  (bind _asteroidmesh3 (Variables|Default|GetAsteroidMesh3))
  (bind _asteroidmesh4 (Variables|Default|GetAsteroidMesh4))
  (bind _asteroidmesh (Variables|Default|GetAsteroidMesh))
  (bind _asteroidmesh7 (Variables|Default|GetAsteroidMesh7))
  (bind _asteroidmesh5 (Variables|Default|GetAsteroidMesh5))
  (bind _asteroidmesh8 (Variables|Default|GetAsteroidMesh8))
  (bind _asteroidmesh9 (Variables|Default|GetAsteroidMesh9))
  (bind _array (Utilities|Array|MakeArray _asteroidmesh _asteroidmesh1 _asteroidmesh2 _asteroidmesh3 _asteroidmesh4 _asteroidmesh5 _asteroidmesh6 _asteroidmesh7 _asteroidmesh8 _asteroidmesh9))
  (bind _outitem (Utilities|Array|Random _array))
  (Collision|SetCollisionEnabled _outitem "QueryAndPhysics")
  (Rendering|SetVisibility _outitem true false)
  (Transformation|SetWorldLocation _asteroidmesh (Math|Vector|MakeVector (Math|Random|RandomFloatinRange -5e+05 5e+05) (Math|Random|RandomFloatinRange -5e+05 5e+05) (Math|Random|RandomFloatinRange -5e+05 5e+05)) false false))

(fn ConstructionScript)