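; Asteroid ring actor that scatters instanced meshes around a distortable ring and turns them into individual, damageable asteroid actors.
; The construction script builds one instanced component per mesh type, placing asteroids from a random stream using cumulative spawn rates.
; Point damage swaps the hit instance for a BP_SingleAsteroidRing and forwards the damage, or SpawnAllOnStart converts every instance at BeginPlay.
; Tick is enabled only with nonzero revolving or orbiting rates.
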(event Game|Damage|EventPointDamage
  (params (Damage :type Float%20%28single-precision%29) (DamageType :type Damage%20Type%20Object%20Reference) (HitLocation :type Vector :default "0, 0, 0") (HitNormal :type Vector :default "0, 0, 0") (HitComponent :type Primitive%20Component%20Object%20Reference) (BoneName :type Name :default "None") (ShotFromDirection :type Vector :default "0, 0, 0") (InstigatedBy :type Controller%20Object%20Reference) (DamageCauser :type Actor%20Object%20Reference) (HitInfo :type Hit%20Result%20Structure%20%28by%20ref%29))
  (bind _asteroid (CallFunction|SpawnAsteroid HitComponent (.HitItem (Collision|BreakHitResult HitInfo))))
  (Game|Damage|ApplyPointDamage _asteroid Damage ShotFromDirection HitInfo InstigatedBy DamageCauser (Utilities|GetClass DamageType)))

(event EventBeginPlay
  (bind _instancedmeshes (Variables|Default|GetInstancedMeshes))
  (Actor|Tick|SetActorTickEnabled (or (!= (Variables|Default|GetRevolvingRate) 0.0) (!= (Variables|Default|GetOrbitingRate) 0.0)))
  (if (Variables|Default|GetSpawnAllOnStart)
    (for _array_element _instancedmeshes
      (for _index (range 0 (- (Components|InstancedStaticMesh|GetInstanceCount _array_element) 1))
        (Game|SpawnActorfromClass "/Game/Devs/PRO_Mert/BluePrints/Environment/BP_SingleAsteroidRing.BP_SingleAsteroidRing_C" (.OutInstanceTransform (Components|InstancedStaticMesh|GetInstanceTransform _array_element _index true)) "AdjustIfPossibleButAlwaysSpawn" "OverrideRootScale" 0 0.05 "0.000000,0.000000,0.000000" (Variables|/Script/Engine.StaticMeshComponent|GetStaticMesh _array_element) (Variables|Actor|GetInstigator)))
      (Components|InstancedStaticMesh|ClearInstances _array_element))
    (Components|InstancedStaticMesh|ClearInstances _array_element)
    (else
      (Collision|SetCollisionEnabled _instancedmeshes "QueryAndPhysics"))))

(fn ConstructionScript
  (bind _randomseed (Variables|Default|GetRandomSeed))
  (bind _accumulatedspawnrates (LocalVariables|GetAccumulatedSpawnRates))
  (Utilities|Array|Clear (Variables|Default|GetInstancedMeshes))
  (for (_array_element _array_index) (Variables|Default|GetMesh)
    (bind _returnvalue (AddComponent|AddInstancedStaticMeshComponent false))
    (Components|StaticMesh|SetStaticMesh _returnvalue (.Mesh (Utilities|Struct|BreakS_MeshSpawn _array_element)))
    (Collision|SetCollisionEnabled _returnvalue "QueryAndPhysics")
    (Collision|SetCollisionObjectType _returnvalue "ECC_Destructible")
    (Utilities|Array|SetArrayElem (LocalVariables|GetAccumulatedSpawnRates) _array_index (+ (.SpawnRate (Utilities|Struct|BreakS_MeshSpawn _array_element)) (Math|Float|SelectFloat 0.0 (Utilities|Array|Get(acopy) (LocalVariables|GetAccumulatedSpawnRates) (- _array_index 1)) (== _array_index 0))) true)
    ;[1 1 1] To avoid random component order
    (Utilities|Array|Add (Variables|Default|GetInstancedMeshes) _returnvalue))
  (for _index (range 1 (Variables|Default|GetNumAsteroids))
    (bind _array_index_2 (Utilities|Array|ForEachLoopwithBreak (Variables|Default|GetMesh) :!label _label)
      (:LoopBody
        (if (< (Math|Random|RandomFloatinRangefromStream (Variables|Default|GetRandomSeed) 0.0 (Utilities|Array|Get(acopy) _accumulatedspawnrates (Utilities|Array|LastIndex _accumulatedspawnrates))) (Utilities|Array|Get(acopy) (LocalVariables|GetAccumulatedSpawnRates) _array_index_2))
          (Components|InstancedStaticMesh|AddInstance (Utilities|Array|Get(acopy) (Variables|Default|GetInstancedMeshes) _array_index_2) (Math|Transform|MakeTransform (+ (* (Math|Vector|RotateVectorAroundAxis (Math|Vector|MakeVector (Variables|Default|GetRingRadius) 0.0 0.0) (Math|Random|RandomFloatinRangefromStream _randomseed (Variables|Default|GetRingStart) (Variables|Default|GetRingEnd)) "0, 0,1.000000") (Math|Vector|MakeVector (+ (Variables|Default|GetRingDistortion) 1.0) 1.0 0.0)) (* (* (Math|Random|RandomUnitVectorfromStream _randomseed) (* (Math|Float|Power (Math|Random|RandomFloatfromStream _randomseed) (Variables|Default|GetSphereCenteredness)) (Variables|Default|GetSphereRadius))) (Variables|Default|GetSphereDistortion))) (Math|Random|RandomRotator true) (Math|Conversions|ToVector(Float) (Math|Random|RandomFloatinRangefromStream (Variables|Default|GetRandomSeed) (Variables|Default|GetAsteroidSizeMin) (Variables|Default|GetAsteroidSizeMax)))) false)
          (goto _label Break))))))

(fn AsteroidTransformation
  (params (Index%20From%20Width%20Loop :type Integer) (Number%20of%20Instance%20by%20Width :type Integer) (Index%20from%20Lenght%20Loop :type Integer) (Number%20of%20Instances%20By%20Lenght :type Integer))
  (bind _returnvalue (Math|Vector|MakeVector 0.0 0.0 1.0))
  (bind _returnvalue_2 (Math|Conversions|ToFloat(Integer) Number%20of%20Instances%20By%20Lenght))
  (bind _returnvalue_3 (Math|Conversions|ToFloat(Integer) Index%20from%20Lenght%20Loop))
  (bind _returnvalue_4 (Math|Conversions|ToFloat(Integer) Index%20From%20Width%20Loop))
  (bind _returnvalue_5 (Math|Conversions|ToFloat(Integer) Number%20of%20Instance%20by%20Width))
  (bind _returnvalue_6 (Math|Float|MakeLiteralFloat 3.6e+02))
  (bind _transformrandom (Variables|Transform|GetTransformRandom))
  (bind _randomizeposition (Variables|Transform|GetRandomizePosition))
  (bind _randomizezaxisposition (Variables|Transform|GetRandomizeZAxisPosition))
  (bind _ringwidth (Variables|Instances|GetRingWidth))
  (bind _ringwidth_2 (Variables|Instances|GetRingWidth))
  (bind _ringradius (Variables|Default|GetRingRadius))
  (bind _returnvalue_7 (Math|Random|RandomFloatfromStream _transformrandom))
  (bind _returnvalue_8 (Math|Random|RandomUnitVectorfromStream _transformrandom))
  (bind _returnvalue_9 (/ _returnvalue_4 _returnvalue_5))
  (bind _returnvalue_10 (/ _returnvalue_3 _returnvalue_2))
  (bind _returnvalue_11 (* _returnvalue_8 _randomizeposition))
  (bind _returnvalue_12 (* _returnvalue_10 _returnvalue_6))
  (bind _returnvalue_13 (- _returnvalue_7 0.5))
  (bind _returnvalue_14 (- _returnvalue_9 0.5))
  (bind _returnvalue_15 (* _returnvalue_13 _randomizezaxisposition _ringwidth))
  (bind _returnvalue_16 (* _returnvalue_14 _ringwidth_2))
  (bind _returnvalue_17 (+ _ringradius _returnvalue_16))
  (bind _returnvalue_18 (+ _returnvalue_15 _returnvalue_11))
  (bind _returnvalue_19 (Math|Vector|MakeVector 0.0 _returnvalue_17 0.0))
  (bind _returnvalue_20 (+ _returnvalue_18 _returnvalue_19))
  (bind _returnvalue_21 (Math|Vector|RotateVectorAroundAxis _returnvalue_20 _returnvalue_12 _returnvalue))
  (return _returnvalue_21 (Math|Rotator|Lerp(Rotator) (Class|KismetMathLibrary|MakeRotfromYZ (Math|Vector|CrossProduct _returnvalue _returnvalue_21) _returnvalue) (Class|KismetMathLibrary|RandomRotatorfromStream (Variables|Transform|GetTransformRandom) true) (Variables|Transform|GetRandomizeRotation) true)))

(fn SpawnAsteroid
  (params (HitComponent :type Primitive%20Component%20Object%20Reference) (ReplaceInstance :type Integer))
  (bind _asinstanced_static_mesh_component (Utilities|Casting|CastToInstancedStaticMeshComponent HitComponent))
  (bind _returnvalue (Game|SpawnActorfromClass "/Game/Devs/PRO_Mert/BluePrints/Environment/BP_SingleAsteroidRing.BP_SingleAsteroidRing_C" (.OutInstanceTransform (Components|InstancedStaticMesh|GetInstanceTransform _asinstanced_static_mesh_component ReplaceInstance true)) "AdjustIfPossibleButAlwaysSpawn" "OverrideRootScale" 0 0.05 "0.000000,0.000000,0.000000" (Variables|/Script/Engine.StaticMeshComponent|GetStaticMesh _asinstanced_static_mesh_component) (Variables|Actor|GetInstigator)))
  (Class|InstancedStaticMeshComponent|RemoveInstance _asinstanced_static_mesh_component ReplaceInstance)
  (return _returnvalue))