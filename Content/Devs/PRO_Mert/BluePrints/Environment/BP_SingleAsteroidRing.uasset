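; An asteroid actor, with its mesh set in the construction script, that can be shot and destroyed for an XP reward.
; Point damage lowers Health when Destructible is set; at zero, DestroySrv relays to DestroyMC, passing the shot direction as explosion location.
; DestroyMC fires two Niagara explosions, destroys only the mesh component, then calls AddXP and DestroySFX on player 0's singleplayer character.
; The multiplayer character's DestroySFX sits behind that singleplayer cast.
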(event Custom|Destroy%20MC
  (params (ExplosionLocation :type Vector))
  (bind _ns_bigexplosion (Variables|Default|GetNS_BigExplosion))
  (Transformation|SetWorldLocation _ns_bigexplosion ExplosionLocation false false)
  (Components|Activation|Activate _ns_bigexplosion false)
  (Components|DestroyComponent (Variables|Default|GetAsteroidMesh))
  ;[1 1 1] Give Player Points according to Reward
  (bind _asbp_singleplayer_character (Utilities|Casting|CastToBP_SingleplayerCharacter (Game|Player|GetPlayerPawn 0)))
  (Default|AddXP _asbp_singleplayer_character (Variables|Asteroid|Settings|GetXP%20Reward))
  (Default|DestroySFX _asbp_singleplayer_character)
  (bind _asbp_mpcharacter (Utilities|Casting|CastToBP_MPCharacter (Game|Player|GetPlayerPawn 0)))
  (Default|DestroySFX _asbp_mpcharacter))

(event Custom|Destroy%20Srv
  (params (ExplosionLocation :type Vector))
  (CallFunction|DestroyMC ExplosionLocation))

(event Game|Damage|EventPointDamage
  (params (Damage :type Float%20%28single-precision%29) (DamageType :type Damage%20Type%20Object%20Reference) (HitLocation :type Vector :default "0, 0, 0") (HitNormal :type Vector :default "0, 0, 0") (HitComponent :type Primitive%20Component%20Object%20Reference) (BoneName :type Name :default "None") (ShotFromDirection :type Vector :default "0, 0, 0") (InstigatedBy :type Controller%20Object%20Reference) (DamageCauser :type Actor%20Object%20Reference) (HitInfo :type Hit%20Result%20Structure%20%28by%20ref%29))
  (Variables|Asteroid|Conditions|SetDamage%20Received Damage)
  (if (Variables|Asteroid|Settings|GetDestructible)
    (bind _output_get (Variables|Asteroid|Settings|SetHealth (- (Variables|Asteroid|Settings|GetHealth) (Variables|Asteroid|Conditions|GetDamage%20Received))))
    (if (<= _output_get 0.0)
      (CallFunction|DestroySrv ShotFromDirection))))

(fn ConstructionScript
  (Components|StaticMesh|SetStaticMesh (Variables|Default|GetAsteroidMesh) (Variables|Default|GetMesh)))