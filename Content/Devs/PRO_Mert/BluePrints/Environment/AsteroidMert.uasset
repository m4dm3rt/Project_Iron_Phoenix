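; Asteroid actor that rotates in place, takes damage and awards the player points when destroyed.
; BeginPlay points the RotatingMovement component at the asteroid mesh and applies the configured rotation speed.
; GotHit subtracts the received damage from health and spawns an impact effect.
; At depleted health it spawns an explosion, destroys itself, then passes its XP reward to BP_PlayerCharacter and calls AddPoints.
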(event Custom|GotHit
  (bind _returnvalue (Transformation|GetActorTransform))
  (bind _returnvalue_2 (Transformation|GetActorTransform))
  (Variables|Asteroid|Settings|SetHealth (- (Variables|Asteroid|Settings|GetHealth) (Variables|Asteroid|Conditions|GetDamage%20Received)))
  (Effects|SpawnEmitteratLocation "/Game/Realistic_Starter_VFX_Pack_Vol2/Particles/Hit/P_Asphalt.P_Asphalt" (.location _returnvalue_2) (.rotation _returnvalue_2) "150.000000,150.000000,150.000000")
  (if (< (Variables|Asteroid|Settings|GetHealth) 0.001)
    (Effects|SpawnEmitteratLocation "/Game/Realistic_Starter_VFX_Pack_Vol2/Particles/Explosion/P_Explosion_Side.P_Explosion_Side" (.location _returnvalue) (.rotation _returnvalue) "100.000000,100.000000,100.000000")
    (Actor|DestroyActor)
    ;[1 1 1] Give Player Points according to Reward
    (bind _asbp_player_character (Utilities|Casting|CastToBP_PlayerCharacter (Game|Player|GetPlayerPawn 0)))
    (Variables|/Game/Devs/PRO_Mert/BluePrints/Player/BP_PlayerCharacter.BP_PlayerCharacter_C|SetReceived%20XP _asbp_player_character (Variables|Asteroid|Settings|GetXPReward))
    ;[1 1 1] Player Points Count
    (Default|AddPoints _asbp_player_character)))

(event EventBeginPlay
  (bind _rotatingmovement (Variables|Default|GetRotatingMovement))
  (Components|Movement|SetUpdatedComponent _rotatingmovement (Variables|Default|GetAsteroidMesh))
  (Variables|/Script/Engine.RotatingMovementComponent|SetRotationRate _rotatingmovement (Variables|Asteroid|Conditions|GetRotate%20Speed)))

(fn ConstructionScript)