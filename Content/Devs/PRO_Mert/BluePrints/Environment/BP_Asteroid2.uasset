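; BP_Asteroid2 is a spinning asteroid that can be set as destructible and awards XP when destroyed.
; Tick rotates the mesh on all three axes by DeltaSeconds plus Rotation, added rather than multiplied.
; When destructible, damage drains Health at double strength until depleted, then spawns a large explosion and destroys the actor.
; It then passes XPReward to player 0 through a cast chain over three single-player character classes.
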(event Game|Damage|EventAnyDamage
  (params (Damage :type Float%20%28single-precision%29) (DamageType :type Damage%20Type%20Object%20Reference) (InstigatedBy :type Controller%20Object%20Reference) (DamageCauser :type Actor%20Object%20Reference))
  (bind _returnvalue (Transformation|GetActorTransform))
  (bind _returnvalue_2 (Game|Player|GetPlayerPawn 0))
  (bind _xp_reward (Variables|Asteroid|Settings|GetXP%20Reward))
  (bind (_asbp_singleplayer_character_alex_j _bsuccess) (Utilities|Casting|CastToBP_SingleplayerCharacterAlexJ _returnvalue_2))
  (bind (_asbp_singleplayer_character _bsuccess_2) (Utilities|Casting|CastToBP_SingleplayerCharacter _returnvalue_2))
  (bind (_asbp_singleplayer_character_marius _bsuccess_3) (Utilities|Casting|CastToBP_SingleplayerCharacterMarius _returnvalue_2))
  (Variables|Asteroid|Conditions|SetDamage%20Received Damage)
  (if (Variables|Asteroid|Settings|GetDestructible)
    (bind _output_get (Variables|Asteroid|Settings|SetHealth (- (Variables|Asteroid|Settings|GetHealth) (* (Variables|Asteroid|Conditions|GetDamage%20Received) 2.0))))
    (if (< _output_get 0.001)
      (Effects|SpawnEmitteratLocation "/Game/Realistic_Starter_VFX_Pack_Vol2/Particles/Explosion/P_Explosion_Side.P_Explosion_Side" (.location _returnvalue) (.rotation _returnvalue) "100.000000,100.000000,100.000000")
      (Actor|DestroyActor)
      ;[1 1 1] Give Player Points according to Reward
      (if _bsuccess_2
        (Variables|/Game/Devs/PRO_Mert/BluePrints/Player/Actors/BP_SingleplayerCharacter.BP_SingleplayerCharacter_C|SetReceivedXP _asbp_singleplayer_character _xp_reward)
        ;[1 1 1] Player Points Count
        (Default|AddXP _asbp_singleplayer_character)
        (elif _bsuccess
          (Variables|/Game/Devs/GD_Alex/BluePrints/Player/BP_SingleplayerCharacterAlexJ.BP_SingleplayerCharacterAlexJ_C|SetReceivedXP _asbp_singleplayer_character_alex_j _xp_reward)
          (Default|AddXP _asbp_singleplayer_character_alex_j)
          (elif _bsuccess_3
            (Variables|/Game/Devs/GD_Marius/Blueprints/Player/BP_SingleplayerCharacterMarius.BP_SingleplayerCharacterMarius_C|SetReceivedXP _asbp_singleplayer_character_marius _xp_reward)
            (Default|AddXP _asbp_singleplayer_character_marius)))))))

(event EventTick
  (params (DeltaSeconds :type Float%20%28single-precision%29))
  (bind _rotation (Variables|Asteroid|Conditions|GetRotation))
  (bind _returnvalue (+ DeltaSeconds _rotation))
  (Transformation|AddLocalRotation (Variables|Default|GetAsteroidMesh) (Math|Rotator|MakeRotator _returnvalue _returnvalue _returnvalue) false false))

(fn ConstructionScript)