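; BP_Buoy is a destructible buoy whose destruction starts the enemy waves in single-player and multiplayer.
; Incoming damage is doubled, drains shield, then health, and updates both widget bars through Srv/MC event pairs.
; At zero health it explodes, removes its mesh and bars, then branches on player class to start the HUD timer and spawner wave.
; The single-player branch also ends the tutorial and clears two tutorial swarms.
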(event Custom|Destroy%20MC
  (bind _returnvalue (Game|Player|GetPlayerPawn 0))
  (Components|Activation|Activate (Variables|Default|GetNS_BigExplosion) true)
  (Components|DestroyComponent (Variables|Default|GetMesh))
  (bind _asbp_singleplayer_character (Utilities|Casting|CastToBP_SingleplayerCharacter _returnvalue)
    (:then
      (Default|DestroySFX _asbp_singleplayer_character)
      (Default|Timer (Variables|/Game/Devs/PRO_Mert/BluePrints/Player/MISC/BP_SingleplayerCharacter.BP_SingleplayerCharacter_C|GetPlayerHUD%20REF _asbp_singleplayer_character))
      (Default|FadeOut (Variables|/Game/Devs/PRO_Mert/BluePrints/Player/MISC/BP_SingleplayerCharacter.BP_SingleplayerCharacter_C|GetPlayerStartW%20REF _asbp_singleplayer_character))
      (Default|TutorialEnd (Variables|/Game/Devs/PRO_Mert/BluePrints/Player/MISC/BP_SingleplayerCharacter.BP_SingleplayerCharacter_C|GetTutorialW%20REF _asbp_singleplayer_character))
      (bind _outactors (Actor|GetAllActorsOfClass "/Game/Devs/PRO_Mert/BluePrints/Enemies/Actors/BP_EnemySwarm_Tutorial.BP_EnemySwarm_Tutorial_C"))
      (Actor|DestroyActor (Utilities|Array|Get(acopy) _outactors))
      (bind _returnvalue_2 (Actor|GetActorOfClass "/Game/Devs/PRO_Alex/Blueprints/World/EnemySpawner.EnemySpawner_C"))
      (Variables|/Game/Devs/PRO_Alex/Blueprints/World/EnemySpawner.EnemySpawner_C|SetEnemyCount _returnvalue_2 0.0)
      (bind _returnvalue_3 (Actor|GetActorOfClass "/Game/Devs/PRO_Alex/Blueprints/World/EnemySpawner.EnemySpawner_C"))
      (Default|WaveStart _returnvalue_3))
    (:CastFailed
      (bind _asbp_mpcharacter (Utilities|Casting|CastToBP_MPCharacter _returnvalue))
      (Default|DestroySFX _asbp_mpcharacter)
      (Default|Timer (Variables|/Game/Devs/PRO_Mert/Multiplayer/InGame/Player/BP_MPCharacter.BP_MPCharacter_C|GetMultiplayerHUD%20REF _asbp_mpcharacter))
      (bind _returnvalue_4 (Actor|GetActorOfClass "/Game/Devs/PRO_Mert/Multiplayer/InGame/Enemies/BP_EnemySpawnerMP.BP_EnemySpawnerMP_C"))
      (Default|WaveStart _returnvalue_4))))

(event Custom|Destroy%20Srv
  (CallFunction|DestroyMC))

(event Custom|UpdateHealth%20MC
  (Progress|SetPercent (Variables|/Game/Devs/PRO_Mert/Multiplayer/InGame/HUD/WBP/EnemyShieldMP_WBP.EnemyShieldMP_WBP_C|GetShieldBar (.AsEnemy%20Shield%20MP%20WBP (Utilities|Casting|CastToEnemyShieldMP_WBP (UserInterface|GetWidget (Variables|Default|GetWidgetShield))))) (/ (Variables|Default|GetShield) 1e+02))
  (Progress|SetPercent (Variables|/Game/Devs/PRO_Mert/Multiplayer/InGame/HUD/WBP/EnemyHealthMP_WBP.EnemyHealthMP_WBP_C|GetHealthBar (.AsEnemy%20Health%20MP%20WBP (Utilities|Casting|CastToEnemyHealthMP_WBP (UserInterface|GetWidget (Variables|Default|GetWidgetHealth))))) (/ (Variables|Default|GetHealth) 1e+02)))

(event Custom|UpdateHealth%20Srv
  (CallFunction|UpdateHealthMC))

(event Game|Damage|EventAnyDamage
  (params (Damage :type Float%20%28single-precision%29) (DamageType :type Damage%20Type%20Object%20Reference) (InstigatedBy :type Controller%20Object%20Reference) (DamageCauser :type Actor%20Object%20Reference))
  (Variables|Default|SetDamage%20Received (* Damage 2.0))
  (bind _output_get (Variables|Default|SetShield (- (Variables|Default|GetShield) (Variables|Default|GetDamage%20Received)))) ; Decrease Shield
  (if (<= _output_get 0.0) ; Check if Shield is active
    (bind _output_get_2 (Variables|Default|SetHealth (- (Variables|Default|GetHealth) (Variables|Default|GetDamage%20Received))))
    (if (<= _output_get_2 0.0)
      (CallFunction|DestroySrv)
      (else
        (CallFunction|UpdateHealthSrv :!label _label)))
    (else
      (goto _label))))

(fn ConstructionScript)