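; Test Blueprint for a player-flown pawn with six-axis movement, mouse steering, shooting state and a pause menu.
; Axis inputs feed movement variables and roll, while Tick calls ApplyImpulseToCapsule and applies local roll.
; Cursor offset from viewport center drives capsule yaw and pitch, scaled by saved mouse settings and halved while targeting.
; Pausing opens the menu and sets the FMOD lock-on parameter; resuming clears firing, restores lock-on audio and reloads settings.
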(event EventBeginPlay
  (Variables|Default|SetcanLook true))

(event EventTick
  (params (DeltaSeconds :type Float%20%28single-precision%29))
  (Class|SingleplayerPawn|ApplyImpulsetoCapsule)
  (Transformation|AddActorLocalRotation (Math|Rotator|MakeRotator (* (Variables|Default|GetRollVelocity) (.x (Variables|Default|GetAxisTurn))) 0.0 0.0) false false))

(event Input|AxisEvents|InputAxisMoveRight/Left
  (params (AxisValue :type Float%20%28single-precision%29))
  (Variables|Default|SetMoveRightAxis AxisValue))

(event Input|AxisEvents|InputAxisMoveUp/Down
  (params (AxisValue :type Float%20%28single-precision%29))
  (Variables|Default|SetMoveUpAxis AxisValue))

(event Input|AxisEvents|InputAxisRollRight/Left
  (params (AxisValue :type Float%20%28single-precision%29))
  (Variables|Default|SetAxisTurn (Math|Vector|MakeVector AxisValue (Input|AxisValues|GetLookUp/Down) (Input|AxisValues|GetLookRight/Left))))

(event Input|AxisEvents|InputAxisMoveForward/Backward
  (params (AxisValue :type Float%20%28single-precision%29))
  (Variables|Default|SetMoveForwardAxis AxisValue))

(event Input|MouseEvents|LeftMouseButton
  (params (Key :type Key%20Structure :default "None"))
  (:Pressed
    (Class|SingleplayerPawn|SpawnActor)))

(fn ConstructionScript)

(event Custom|PauseGame
  (bind _returnvalue (Game|GetPlayerController 0))
  ;[1 1 1] Set Widget
  (bind _returnvalue_2 (UserInterface|CreateWidget "/Game/Devs/PRO_Mert/BluePrints/UI/Menu/PauseMenu_W.PauseMenu_W_C"))
  (UserInterface|Viewport|AddtoViewport _returnvalue_2 0)
  (Input|SetInputModeUIOnly _returnvalue _returnvalue_2 "LockInFullscreen" false)
  ;[1 1 1] Set Pause
  (Variables|/Script/Engine.PlayerController|SetbShowMouseCursor _returnvalue true)
  (Class|FMODBlueprintStatics|SetGlobalParameterbyName "lockon_status" 1.0)
  (Game|SetGamePaused true))

(event Custom|ResumeGame
  (Variables|Default|SetShootingLaser false)
  (Variables|Default|SetShootingKinetic false)
  (if (Variables|Default|GetisTargeting)
    (AddComponent|AddFMODAudioComponent false)
    (Class|FMODBlueprintStatics|SetGlobalParameterbyName "lockon_status" 0.0))
  (bind _returnvalue (SaveGame|DoesSaveGameExist "Settings"))
  (if _returnvalue
    (bind _returnvalue_2 (SaveGame|LoadGamefromSlot "Settings"))
    (bind _assettings_save (Utilities|Casting|CastToSettingsSave _returnvalue_2))
    (Variables|Default|SetSettings (Variables|/Game/Devs/PRO_Mert/BluePrints/UI/Menu/Settings/SettingsSave.SettingsSave_C|GetSettings _assettings_save))))

(event Input|ActionEvents|InputActionPauseMenu
  (params (Key :type Key%20Structure))
  ;[1 1 1] Input
  (:Pressed
    (CallFunction|PauseGame)))

(event Input|AxisEvents|InputAxisLookUp/Down
  (params (AxisValue :type Float%20%28single-precision%29))
  (bind _returnvalue (Viewport|GetViewportSize))
  (bind _returnvalue_2 (Class|WidgetLayoutLibrary|GetViewportScale))
  (bind _settings (Variables|Default|GetSettings))
  (bind _turnrate (Variables|Default|GetTurnRate))
  (bind _mousespeedy (Utilities|Struct|BreakSettingsStructure _settings))
  (bind _returnvalue_3 (/ (.y _returnvalue) _returnvalue_2))
  (bind _returnvalue_4 (/ _returnvalue_3 2.0))
  (bind _returnvalue_5 (* _turnrate _mousespeedy))
  (if (Variables|Default|GetcanLook)
    (if (not (Variables|Default|GetFreeLook))
      (if (not (Variables|Default|GetisDead))
        (if (not (Game|IsGamePaused))
          (bind _returnvalue_6 (Class|WidgetLayoutLibrary|GetMousePositiononViewport))
          (Class|SingleplayerPawn|AddCapsulePitchInput (Math|Float|SelectFloat (* (Math|Float|SelectFloat (* _returnvalue_5 (/ (- (.y _returnvalue_6) _returnvalue_4) _returnvalue_4) 0.5) (* (/ (- (.y _returnvalue_6) _returnvalue_4) _returnvalue_4) _returnvalue_5) (Variables|Default|GetisTargeting)) -1.0) (Math|Float|SelectFloat (* _returnvalue_5 (/ (- (.y _returnvalue_6) _returnvalue_4) _returnvalue_4) 0.5) (* (/ (- (.y _returnvalue_6) _returnvalue_4) _returnvalue_4) _returnvalue_5) (Variables|Default|GetisTargeting)) (Utilities|Struct|BreakSettingsStructure (Variables|Default|GetSettings)))))))))

(event Input|AxisEvents|InputAxisLookRight/left
  (params (AxisValue :type Float%20%28single-precision%29))
  (bind _returnvalue (Viewport|GetViewportSize))
  (bind _returnvalue_2 (Class|WidgetLayoutLibrary|GetViewportScale))
  (bind _turnrate (Variables|Default|GetTurnRate))
  (bind _settings (Variables|Default|GetSettings))
  (bind _mousespeedx (Utilities|Struct|BreakSettingsStructure _settings))
  (bind _returnvalue_3 (/ (.x _returnvalue) _returnvalue_2))
  (bind _returnvalue_4 (* _turnrate _mousespeedx))
  (bind _returnvalue_5 (/ _returnvalue_3 2.0))
  (if (Variables|Default|GetcanLook)
    (if (not (Variables|Default|GetFreeLook))
      (if (not (Variables|Default|GetisDead))
        (if (not (Game|IsGamePaused))
          (bind _returnvalue_6 (Class|WidgetLayoutLibrary|GetMousePositiononViewport))
          (Class|SingleplayerPawn|AddCapsuleYawInput (Math|Float|SelectFloat (* _returnvalue_4 (/ (- (.x _returnvalue_6) _returnvalue_5) _returnvalue_5) 0.5) (* (/ (- (.x _returnvalue_6) _returnvalue_5) _returnvalue_5) _returnvalue_4) (Variables|Default|GetisTargeting))))))))