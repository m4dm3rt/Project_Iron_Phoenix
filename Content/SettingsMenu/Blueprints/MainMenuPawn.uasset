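; Main menu pawn that brings up the menu screen and applies stored display settings when play begins.
; BeginPlay creates the MainMenu_W widget, shows the mouse cursor and switches input to UI only.
; It then calls GetSettings and, on success, applies gamma and an FPS cap looked up from an index array through console commands.
; A timeline for subtle camera drift exists but is never triggered.
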(event EventBeginPlay
  (bind _returnvalue (Game|GetPlayerController 0))
  (bind _returnvalue_2 (UserInterface|CreateWidget "/Game/SettingsMenu/Widgets/MainMenu_W.MainMenu_W_C"))
  (bind _output_get (Variables|Default|SetMainMenuWidgetRef _returnvalue_2))
  (UserInterface|Viewport|AddtoViewport _output_get 0)
  (Variables|/Script/Engine.PlayerController|SetbShowMouseCursor _returnvalue true)
  (Input|SetInputModeUIOnly _returnvalue 0 "DoNotLock" false)
  (bind (_settings _success_) (CallFunction|GetSettings))
  (if _success_
    (Development|ExecuteConsoleCommand (Utilities|String|Append "gamma " (Utilities|String|ToString(Float) (.Gamma (Utilities|Struct|BreakSettingsStructure _settings)))) (Game|GetPlayerController 0))
    (Development|ExecuteConsoleCommand (Utilities|String|Append "t.MaxFPS " (Utilities|String|ToString(Integer) (Utilities|Array|Get(acopy) (Variables|Default|GetFPSLimitIndexArray) (.FpsLimit (Utilities|Struct|BreakSettingsStructure _settings))))) 0)))

(fn ConstructionScript)