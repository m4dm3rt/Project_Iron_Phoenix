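; Ship-mounted turret weapon actor, configured from a data table row that sets its meshes, muzzle offset, ammo class and firing stats.
; OpenFire and CeaseFire toggle Tick-driven gates that spawn projectiles on cooldown or refill ammo after a delay.
; Emptying a clip triggers overheat, blocking fire until ammo reaches a threshold; zero clip size means endless ammo.
; SetNewWeapon swaps weapons, restoring runtime state from a comma-separated string built by GetCustomDataString.
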(event Custom|Open%20Fire
  (bind _returnvalue (Actor|GetParentActor))
  (bind _weapondata (Variables|Internal|GetWeaponData))
  (bind _arrow (Variables|Default|GetArrow))
  (bind (_firingsound _ammoclass _cooldown) (Utilities|Struct|BreakS_WeaponData _weapondata))
  (bind _returnvalue_2 (Transformation|GetWorldLocation _arrow))
  (bind _aspawn (Utilities|Casting|CastToPawn _returnvalue))
  (if (not (Variables|Internal|GetIsOverheat))
    (CallFunction|StopReloading)
    (Utilities|FlowControl|Gate true) ; enters at Open
  ))

(event Custom|Start%20Reloading
  (bind _weapondata (Variables|Internal|GetWeaponData))
  (bind (_clipsize _reloadrate _overheatthreshold) (Utilities|Struct|BreakS_WeaponData _weapondata))
  (Utilities|FlowControl|Gate false) ; enters at Open
)

(event Custom|Stop%20Reloading
  (bind _weapondata (Variables|Internal|GetWeaponData))
  (bind (_clipsize _reloadrate _overheatthreshold) (Utilities|Struct|BreakS_WeaponData _weapondata))
  (Variables|Internal|SetReloadProgress 0.0)
  (Variables|Internal|SetReloadDelayProgress 0.0)
  (Utilities|FlowControl|Gate false) ; enters at Close
)

(event Custom|Point%20Turret%20To
  (params (TargetLocation :type Vector) (Alpha :type Float%20%28double-precision%29))
  (Variables|Internal|SetTargetLocation TargetLocation)
  (Transformation|SetWorldRotation (Variables|Default|GetTurret) (Math|Rotator|Lerp(Rotator) (Transformation|GetWorldRotation (Variables|Default|GetTurret)) (Math|Rotator|MakeRotfromXZ (- TargetLocation (Transformation|GetWorldLocation (Variables|Default|GetTurret))) (Transformation|GetActorUpVector)) Alpha true) false false))

(event Custom|Cease%20Fire
  (bind _returnvalue (Actor|GetParentActor))
  (bind _weapondata (Variables|Internal|GetWeaponData))
  (bind _arrow (Variables|Default|GetArrow))
  (bind (_firingsound _ammoclass _cooldown) (Utilities|Struct|BreakS_WeaponData _weapondata))
  (bind _returnvalue_2 (Transformation|GetWorldLocation _arrow))
  (bind _aspawn (Utilities|Casting|CastToPawn _returnvalue))
  (CallFunction|StartReloading)
  (Utilities|FlowControl|Gate true) ; enters at Close
)

(event EventBeginPlay
  (Variables|Internal|SetCurrentAmmo (Utilities|Struct|BreakS_WeaponData (Variables|Internal|GetWeaponData))))

(event Collision|EventActorBeginOverlap
  (params (OtherActor :type Actor%20Object%20Reference)))

(event EventTick
  (params (DeltaSeconds :type Float%20%28single-precision%29))
  (bind _returnvalue (Actor|GetParentActor))
  (bind _weapondata (Variables|Internal|GetWeaponData))
  (bind _weapondata_2 (Variables|Internal|GetWeaponData))
  (bind _arrow (Variables|Default|GetArrow))
  (bind (_firingsound _ammoclass _cooldown) (Utilities|Struct|BreakS_WeaponData _weapondata))
  (bind (_clipsize _reloadrate _overheatthreshold) (Utilities|Struct|BreakS_WeaponData _weapondata_2))
  (bind _returnvalue_2 (Transformation|GetWorldLocation _arrow))
  (bind _aspawn (Utilities|Casting|CastToPawn _returnvalue))
  (Utilities|FlowControl|Sequence
    (:then_0
      (Variables|Internal|SetCooldownProgress (- (Variables|Internal|GetCooldownProgress) DeltaSeconds))
      (if (and (<= (Variables|Internal|GetCooldownProgress) 0.0) (or (> (Variables|Internal|GetCurrentAmmo) 0) (<= (Utilities|Struct|BreakS_WeaponData (Variables|Internal|GetWeaponData)) 0)))
        (Utilities|FlowControl|Gate true
          (:Exit
            (Game|SpawnActorfromClass _ammoclass (Math|Transform|MakeTransform _returnvalue_2 (Math|Rotator|FindLookatRotation _returnvalue_2 (Variables|Internal|GetTargetLocation))) "Undefined" "SelectDefaultAtRuntime" _aspawn _aspawn)
            (Audio|PlaySoundatLocation _firingsound (Transformation|GetActorLocation) "0, 0, 0" 1.0 1.0 0.0 0 0 0 0)
            (Variables|Internal|SetCooldownProgress _cooldown)
            (if (> (Utilities|Struct|BreakS_WeaponData (Variables|Internal|GetWeaponData)) 0)
              (bind _result (Math|Integer|DecrementInt (Variables|Internal|GetCurrentAmmo))
                (:%20%20
                  (bind _output_get (Variables|Internal|SetIsOverheat (<= _result 0)))
                  (if _output_get
                    (CallFunction|CeaseFire)))))))))
    (:then_1
      (Utilities|FlowControl|Gate false
        (:Exit
          (bind _output_get_2 (Variables|Internal|SetReloadDelayProgress (+ (Variables|Internal|GetReloadDelayProgress) (Utilities|Time|GetWorldDeltaSeconds))))
          (if (>= _output_get_2 (Utilities|Struct|BreakS_WeaponData (Variables|Internal|GetWeaponData)))
            (bind _output_get_3 (Variables|Internal|SetReloadProgress (+ (Variables|Internal|GetReloadProgress) (Utilities|Time|GetWorldDeltaSeconds))))
            (if (Math|Boolean|ANDBoolean (>= _output_get_3 (/ 1.0 _reloadrate)) (< (Variables|Internal|GetCurrentAmmo) _clipsize) (> _reloadrate 0.0))
              (Variables|Internal|SetReloadProgress 0.0)
              (bind _result_2 (Math|Integer|IncrementInt (Variables|Internal|GetCurrentAmmo))
                (:%20%20
                  (if (>= _result_2 _overheatthreshold)
                    (Variables|Internal|SetIsOverheat false)))))))))))

(fn ConstructionScript
  (CallFunction|SetNewWeapon (Variables|Default|GetWeaponClass)))

(fn SetNewWeapon
  (params (WeaponClass :type Data%20Table%20Row%20Handle%20Structure) (CustomData :type String))
  (bind (_currentammo _cooldownprogress _reloadprogress _reloaddelayprogress _isoverheat) (CallFunction|ParseCustomDataString CustomData))
  (Actor|Tick|SetActorTickEnabled (Utilities|Name|NotEqual(Name) (.RowName (Utilities|Struct|BreakDataTableRowHandle WeaponClass)) "Empty"))
  (bind _output_get (Variables|Default|SetWeaponClass WeaponClass))
  (bind _returnvalue (Utilities|GetDataTableRow (.DataTable (Utilities|Struct|BreakDataTableRowHandle _output_get)) (.RowName (Utilities|Struct|BreakDataTableRowHandle _output_get)))
    (:then
      (bind _output_get_2 (Variables|Internal|SetWeaponData _returnvalue))
      (Components|StaticMesh|SetStaticMesh (Variables|Default|GetMount) (.MountMesh (Utilities|Struct|BreakS_WeaponData _output_get_2)))
      (Components|StaticMesh|SetStaticMesh (Variables|Default|GetTurret) (.TurretMesh (Utilities|Struct|BreakS_WeaponData _output_get_2)))
      (Transformation|SetRelativeLocation (Variables|Default|GetArrow) (.MuzzleOffset (Utilities|Struct|BreakS_WeaponData _output_get_2)) false false)
      (Variables|Internal|SetCurrentAmmo _currentammo)
      (Variables|Internal|SetCooldownProgress _cooldownprogress)
      (Variables|Internal|SetReloadProgress _reloadprogress)
      (Variables|Internal|SetReloadDelayProgress _reloaddelayprogress)
      (Variables|Internal|SetIsOverheat _isoverheat)
      (Default|CallWeaponChanged))))

(fn GetCustomDataString
  (return (Utilities|String|JoinStringArray (Utilities|Array|MakeArray (Utilities|String|ToString(Integer) (Variables|Internal|GetCurrentAmmo)) (Utilities|String|ToString(Float) (Variables|Internal|GetCooldownProgress)) (Utilities|String|ToString(Float) (Variables|Internal|GetReloadProgress)) (Utilities|String|ToString(Float) (Variables|Internal|GetReloadDelayProgress)) (Utilities|String|ToString(Boolean) (Variables|Internal|GetIsOverheat))) ",")))

(fn ParseCustomDataString
  (params (DataString :type String))
  (bind _returnvalue (Utilities|String|ParseIntoArray DataString ","))
  (if (> (Utilities|String|Len DataString) 0)
    (return (Math|Conversions|ToInteger(Byte) (Utilities|Array|Get(acopy) _returnvalue)) (Math|Conversions|ToFloat(Integer) (Utilities|Array|Get(acopy) _returnvalue 1)) (Math|Conversions|ToFloat(Integer) (Utilities|Array|Get(acopy) _returnvalue 2)) (Math|Conversions|ToFloat(Integer) (Utilities|Array|Get(acopy) _returnvalue 3)) (Utilities|Enum|Equal(Enum) (Utilities|Array|Get(acopy) _returnvalue 4) "true"))
    (else
      (return (Utilities|Struct|BreakS_WeaponData (Variables|Internal|GetWeaponData)) 0.0 0.0 0.0 false))))