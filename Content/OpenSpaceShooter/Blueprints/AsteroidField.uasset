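; Asteroid field actor that procedurally scatters weighted mesh variants in a distortable ring or sphere for the space shooter.
; The construction script builds instanced mesh components using a random stream.
; Tick orbits and spins instances when rates are nonzero.
; BeginPlay optionally converts all instances to Asteroid actors; otherwise point damage, including from Pawn collisions, lazily swaps the struck instance for an actor, forwarding damage and impulse.
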(event EventBeginPlay
  (bind _instancedmeshes (Variables|Default|GetInstancedMeshes))
  (Actor|Tick|SetActorTickEnabled (or (!= (Variables|Default|GetRevolvingRate) 0.0) (!= (Variables|Default|GetOrbitingRate) 0.0)))
  (if (Variables|Default|GetSpawnAllOnStart)
    (for _array_element _instancedmeshes
      (for _index (range 0 (- (Components|InstancedStaticMesh|GetInstanceCount _array_element) 1))
        (Game|SpawnActorfromClass "/Game/OpenSpaceShooter/Blueprints/Asteroid.Asteroid_C" (.OutInstanceTransform (Components|InstancedStaticMesh|GetInstanceTransform _array_element _index true)) "Undefined" "OverrideRootScale" 0 (Variables|/Script/Engine.StaticMeshComponent|GetStaticMesh _array_element) 0))
      (Components|InstancedStaticMesh|ClearInstances _array_element))
    (else
      (Collision|SetCollisionEnabled _instancedmeshes "QueryAndPhysics"))))

(event Collision|EventActorBeginOverlap
  (params (OtherActor :type Actor%20Object%20Reference)))

(event Collision|EventHit
  (params (MyComp :type Primitive%20Component%20Object%20Reference) (Other :type Actor%20Object%20Reference) (OtherComp :type Primitive%20Component%20Object%20Reference) (bSelfMoved :type Boolean) (HitLocation :type Vector :default "0, 0, 0") (HitNormal :type Vector :default "0, 0, 0") (NormalImpulse :type Vector :default "0, 0, 0") (Hit :type Hit%20Result%20Structure%20%28by%20ref%29))
  (bind _returnvalue (Transformation|GetActorLocation Other))
  (Utilities|Casting|CastToPawn Other :!pinned true) ; To prevent traffic jam
  (bind _outhit (Collision|LineTraceByChannel _returnvalue (Math|Vector|Lerp(Vector) _returnvalue HitLocation 2.0) "TraceTypeQuery1" false (Utilities|Array|MakeArray Other) "None" false))
  (Game|Damage|ApplyPointDamage self (Math|Float|MapRangeClamped (Math|Vector|VectorLength (Transformation|GetVelocity Other)) 0.0 5e+04 0.1 1.0) HitNormal _outhit 0 Other))

(event EventTick
  (params (DeltaSeconds :type Float%20%28single-precision%29))
  (for _array_element (Variables|Default|GetInstancedMeshes)
    (for _index (range 0 (- (Components|InstancedStaticMesh|GetInstanceCount _array_element) 1))
      (Components|InstancedStaticMesh|UpdateInstanceTransform _array_element _index (Math|Transform|MakeTransform (Math|Vector|ClampVectorSize (Math|Vector|RotateVectorAroundAxis (.location (.OutInstanceTransform (Components|InstancedStaticMesh|GetInstanceTransform _array_element _index false))) (* (/ (Variables|Default|GetOrbitingRate) (Math|Float|Power (/ (Math|Vector|VectorLength (.location (.OutInstanceTransform (Components|InstancedStaticMesh|GetInstanceTransform _array_element _index false)))) (+ (Variables|Default|GetRingRadius) (Variables|Default|GetSphereRadius))) (Variables|Default|GetOrbitingRatePower))) (Utilities|Time|GetWorldDeltaSeconds)) "0,0.000000,1.000000") 0.0 (Math|Vector|VectorLength (.location (.OutInstanceTransform (Components|InstancedStaticMesh|GetInstanceTransform _array_element _index false))))) (Math|Rotator|CombineRotators (.rotation (.OutInstanceTransform (Components|InstancedStaticMesh|GetInstanceTransform _array_element _index false))) (* (Math|Rotator|MakeRotator (Math|Trig|Sin(Radians) (* (Math|Vector|GetMaxElement (.scale (.OutInstanceTransform (Components|InstancedStaticMesh|GetInstanceTransform _array_element _index false)))) 23.0)) (Math|Trig|Sin(Radians) (* (Math|Vector|GetMaxElement (.scale (.OutInstanceTransform (Components|InstancedStaticMesh|GetInstanceTransform _array_element _index false)))) 53.0)) (Math|Trig|Sin(Radians) (* (Math|Vector|GetMaxElement (.scale (.OutInstanceTransform (Components|InstancedStaticMesh|GetInstanceTransform _array_element _index false)))) 37.0))) (Variables|Default|GetRevolvingRate))) (.scale (.OutInstanceTransform (Components|InstancedStaticMesh|GetInstanceTransform _array_element _index false)))) false false false))
    (Components|InstancedStaticMesh|UpdateInstanceTransform _array_element 0 (.OutInstanceTransform (Components|InstancedStaticMesh|GetInstanceTransform _array_element 0 false)) false true false)))

(event Game|Damage|EventPointDamage
  (params (Damage :type Float%20%28single-precision%29) (DamageType :type Damage%20Type%20Object%20Reference) (HitLocation :type Vector :default "0, 0, 0") (HitNormal :type Vector :default "0, 0, 0") (HitComponent :type Primitive%20Component%20Object%20Reference) (BoneName :type Name :default "None") (ShotFromDirection :type Vector :default "0, 0, 0") (InstigatedBy :type Controller%20Object%20Reference) (DamageCauser :type Actor%20Object%20Reference) (HitInfo :type Hit%20Result%20Structure%20%28by%20ref%29))
  (bind _asteroid (CallFunction|SpawnAsteroid HitComponent (.HitItem (Collision|BreakHitResult HitInfo))))
  (Game|Damage|ApplyPointDamage _asteroid Damage ShotFromDirection HitInfo InstigatedBy DamageCauser (Utilities|GetClass DamageType))
  (Physics|AddImpulseatLocation (Variables|/Game/OpenSpaceShooter/Blueprints/Asteroid.Asteroid_C|GetStaticMesh _asteroid) (* ShotFromDirection (* (Physics|GetMass (Variables|/Game/OpenSpaceShooter/Blueprints/Asteroid.Asteroid_C|GetStaticMesh _asteroid)) (Math|Float|MapRangeClamped (Math|Vector|VectorLength (Transformation|GetVelocity DamageCauser)) 0.0 1e+04 5e+02 2e+03))) HitLocation "None" :!pinned true) ; Pass impact to real asteroid
)

(fn ConstructionScript
  (bind _randomseed (Variables|Default|GetRandomSeed))
  (bind _textrender (Variables|Default|GetTextRender))
  (bind _accumulatedspawnrates (LocalVariables|GetAccumulatedSpawnRates))
  ;[1 1 1] Since 4.23 recompile does not properly resets arrays
  (Utilities|Array|Clear (Variables|Default|GetInstancedMeshes))
  (Rendering|Components|TextRender|SetWorldSize _textrender (* (+ (Variables|Default|GetRingRadius) (Variables|Default|GetSphereRadius)) 0.1))
  (Rendering|SetVisibility _textrender (> (Variables|Default|GetNumAsteroids) 1000) false)
  (for (_array_element _array_index) (Variables|Default|GetMeshes)
    (bind _returnvalue (AddComponent|AddInstancedStaticMeshComponent false))
    (Components|StaticMesh|SetStaticMesh _returnvalue (.Mesh (Utilities|Struct|BreakS_MeshSpawnRate _array_element)))
    (Collision|SetCollisionEnabled _returnvalue "NoCollision")
    (Utilities|Array|SetArrayElem (LocalVariables|GetAccumulatedSpawnRates) _array_index (+ (.SpawnRate (Utilities|Struct|BreakS_MeshSpawnRate _array_element)) (Math|Float|SelectFloat 0.0 (Utilities|Array|Get(acopy) (LocalVariables|GetAccumulatedSpawnRates) (- _array_index 1)) (== _array_index 0))) true)
    ;[1 1 1] To avoid random component order
    (Utilities|Array|Add (Variables|Default|GetInstancedMeshes) _returnvalue))
  (for _index (range 1 (Variables|Default|GetNumAsteroids))
    (bind _array_index_2 (Utilities|Array|ForEachLoopwithBreak (Variables|Default|GetMeshes) :!label _label)
      (:LoopBody
        (if (< (Math|Random|RandomFloatinRangefromStream (Variables|Default|GetRandomSeed) 0.0 (Utilities|Array|Get(acopy) _accumulatedspawnrates (Utilities|Array|LastIndex _accumulatedspawnrates))) (Utilities|Array|Get(acopy) (LocalVariables|GetAccumulatedSpawnRates) _array_index_2))
          (Components|InstancedStaticMesh|AddInstance (Utilities|Array|Get(acopy) (Variables|Default|GetInstancedMeshes) _array_index_2) (Math|Transform|MakeTransform (+ (* (Math|Vector|RotateVectorAroundAxis (Math|Vector|MakeVector (Variables|Default|GetRingRadius) 0.0 0.0) (Math|Random|RandomFloatinRangefromStream _randomseed (Variables|Default|GetRingStart) (Variables|Default|GetRingEnd)) "0, 0,1.000000") (Math|Vector|MakeVector (+ (Variables|Default|GetRingDistortion) 1.0) 1.0 0.0)) (* (* (Math|Random|RandomUnitVectorfromStream _randomseed) (* (Math|Float|Power (Math|Random|RandomFloatfromStream _randomseed) (Variables|Default|GetSphereCenteredness)) (Variables|Default|GetSphereRadius))) (Variables|Default|GetSphereDistortion))) (Math|Random|RandomRotator true) (Math|Conversions|ToVector(Float) (Math|Random|RandomFloatinRangefromStream (Variables|Default|GetRandomSeed) (Variables|Default|GetAsteroidSizeMin) (Variables|Default|GetAsteroidSizeMax)))) false)
          (goto _label Break))))))

(fn SpawnAsteroid
  (params (HitComponent :type Primitive%20Component%20Object%20Reference) (ReplaceInstance :type Integer))
  (bind _asinstanced_static_mesh_component (Utilities|Casting|CastToInstancedStaticMeshComponent HitComponent))
  (bind _returnvalue (Game|SpawnActorfromClass "/Game/OpenSpaceShooter/Blueprints/Asteroid.Asteroid_C" (.OutInstanceTransform (Components|InstancedStaticMesh|GetInstanceTransform _asinstanced_static_mesh_component ReplaceInstance true)) "Undefined" "OverrideRootScale" 0 (Variables|/Script/Engine.StaticMeshComponent|GetStaticMesh _asinstanced_static_mesh_component) 0))
  (Class|InstancedStaticMeshComponent|RemoveInstance _asinstanced_static_mesh_component ReplaceInstance)
  (return _returnvalue))