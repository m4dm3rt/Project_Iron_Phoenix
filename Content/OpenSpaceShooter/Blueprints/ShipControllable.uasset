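; Player-controllable ship pawn that extends ship base logic with flight input, camera, turret aiming, dual-trigger firing and boarding from another pawn.
; Movement axes feed UpdateManeuver, remapped for capital ships, while mouse offset from screen center drives pitch and yaw.
; Tick fakes camera lag, scales dust with speed and aims turrets at InputSender's trace.
; Possession toggles controls; boarding possesses the ship and transfers inventory.
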(event HandleInput(InputReceiver)
  (params (Sender :type Input%20Sender%20Object%20Reference) (Input :type String))
  (bind _returnvalue (Components|GetOwner Sender))
  (bind _self self)
  (bind _aspawn (Utilities|Casting|CastToPawn _returnvalue))
  (Pawn|Possess (Pawn|GetController _aspawn) _self)
  (Default|TakeAllfrom (Actor|GetComponentbyClass _self "/Game/OpenSpaceShooter/Blueprints/Components/InventoryComponent.InventoryComponent_C") (Actor|GetComponentbyClass _aspawn "/Game/OpenSpaceShooter/Blueprints/Components/InventoryComponent.InventoryComponent_C"))
  (Audio|PlaySound2D "/Game/OpenSpaceShooter/Audio/Airlock_Cue.Airlock_Cue" 1.0 1.0 0.0 0 0))

(event Custom|Temp%20Disable%20Camera%20Lag
  (bind _springarm (Variables|Default|GetSpringArm))
  (Variables|/Script/Engine.SpringArmComponent|SetbEnableCameraRotationLag _springarm false)
  (Utilities|FlowControl|Delay 0.05)
  (Variables|/Script/Engine.SpringArmComponent|SetbEnableCameraRotationLag _springarm true))

(event EventBeginPlay
  (|CallParentFunction)
  (bind _returnvalue (UserInterface|CreateWidget "/Game/OpenSpaceShooter/Widgets/WBP_MasterWidget.WBP_MasterWidget_C"))
  (UserInterface|Viewport|AddtoViewport _returnvalue 0))

(event Collision|EventActorBeginOverlap
  (params (OtherActor :type Actor%20Object%20Reference))
  (|CallParentFunction OtherActor) ; This node is disabled and will not be called.\nDrag off pins to build functionality.
)

(event EventTick
  (params (DeltaSeconds :type Float%20%28single-precision%29))
  (bind _springarm (Variables|Default|GetSpringArm))
  (bind _inputsender (Variables|Default|GetInputSender))
  (bind _springarm_2 (Variables|Default|GetSpringArm))
  (bind _hitresult (Variables|/Game/OpenSpaceShooter/Blueprints/Components/InputSender.InputSender_C|GetHitResult _inputsender))
  (bind (_bblockinghit _binitialoverlap _time _distance _location _impactpoint _normal _impactnormal _physmat _hitactor _hitcomponent _hitbonename _bonename _hititem _elementindex _faceindex _tracestart _traceend) (Collision|BreakHitResult _hitresult))
  (|CallParentFunction DeltaSeconds)
  ;[1 1 1] Because Native Cam Lag Jitters
  (Transformation|SetRelativeLocation _springarm_2 (Math|Vector|Lerp(Vector) (Variables|/Script/Engine.SceneComponent|GetRelativeLocation _springarm_2) (Math|Transform|InverseTransformDirection (Transformation|GetActorTransform) (* (Transformation|GetVelocity) -0.03)) 0.1) false false)
  (Effects|Components|ParticleSystem|SetFloatParameter (Variables|Default|GetP_Ambient_Dust) "Spawn Rate" (Math|Float|MapRangeClamped (Math|Vector|VectorLength (Transformation|GetVelocity)) 0.0 (Variables|Default|GetMaxSpeed) 5.0 2e+01))
  ;[1 1 1] Compensate turning effects in ShipBase
  (Transformation|AddLocalRotation _springarm (Math|Rotator|MakeRotator (* (+ (Math|Float|Clamp(Float) (.z (Variables|Default|GetAxisTurn)) -0.5 0.5) (.y (Variables|Default|GetAxisThrust))) -0.5) 0.0 0.0) false false)
  (Transformation|SetRelativeRotation _springarm (Math|Rotator|Lerp(Rotator) (Variables|/Script/Engine.SceneComponent|GetRelativeRotation _springarm) "0, 0, 0" 0.02 true) false false)
  (for _array_element (CallFunction|GetWeapons)
    (Default|PointTurretto _array_element (Math|Vector|SelectVector (Math|Vector|SelectVector _impactpoint _traceend (and _bblockinghit (CallFunction|NotTraceBlocker _hitcomponent))) (+ (Transformation|GetActorLocation) (* (Transformation|GetActorForwardVector) (Variables|/Game/OpenSpaceShooter/Blueprints/Components/InputSender.InputSender_C|GetTraceDistance _inputsender))) (Variables|/Game/OpenSpaceShooter/Blueprints/Components/InputSender.InputSender_C|GetActivated _inputsender)) 0.1)))

(event EventPossessed
  (params (NewController :type Controller%20Object%20Reference))
  (bind _bsuccess (Utilities|Casting|CastToPlayerController NewController))
  (Components|Activation|SetActive (Variables|Default|GetP_Ambient_Dust) _bsuccess false)
  (CallFunction|SetControlsEnabled _bsuccess))

(event EventUnpossessed
  (params (OldController :type Controller%20Object%20Reference))
  (Components|Activation|Deactivate (Variables|Default|GetP_Ambient_Dust))
  (CallFunction|SetControlsEnabled false)
  (Utilities|FlowControl|Delay 0.02) ; For unknown reason, input still comes in on unpossess.
  (CallFunction|UpdateManeuver 0.0 0.0 0.0 0.0 0.0 0.0))

(event Input|ActionEvents|InputActionInteract
  (params (Key :type Key%20Structure :default "None"))
  (:Pressed
    (Default|SendInput (Variables|Default|GetInputSender) "Interact")))

(event Input|AxisEvents|InputAxisMoveForward
  (params (AxisValue :type Float%20%28single-precision%29))
  (bind _capitalshipmaneuver (Variables|Default|GetCapitalShipManeuver))
  (CallFunction|UpdateManeuver AxisValue (Math|Float|SelectFloat 0.0 (Input|AxisValues|GetMoveRight) _capitalshipmaneuver) (Math|Float|SelectFloat (Input|AxisValues|GetMoveUp) 0.0 _capitalshipmaneuver) 0.0 (Math|Float|SelectFloat 0.0 (Input|AxisValues|GetLookUp) _capitalshipmaneuver) (Math|Float|SelectFloat (Input|AxisValues|GetMoveRight) 0.0 _capitalshipmaneuver)))

(event Input|AxisEvents|InputAxisLookUp
  (params (AxisValue :type Float%20%28single-precision%29))
  (bind _returnvalue (Viewport|GetViewportSize))
  (bind _returnvalue_2 (Class|WidgetLayoutLibrary|GetViewportScale))
  (bind _returnvalue_3 (/ (.y _returnvalue) _returnvalue_2))
  (bind _returnvalue_4 (/ _returnvalue_3 2.0))
  (if (not (Game|IsGamePaused))
    (bind _returnvalue_5 (Class|WidgetLayoutLibrary|GetMousePositiononViewport))
    (Default|Pitch (Variables|Default|GetBP_EZDOF_Component) (/ (- (.y _returnvalue_5) _returnvalue_4) _returnvalue_4))))

(event Input|AxisEvents|InputAxisLookRight
  (params (AxisValue :type Float%20%28single-precision%29))
  (bind _returnvalue (Viewport|GetViewportSize))
  (bind _returnvalue_2 (Class|WidgetLayoutLibrary|GetViewportScale))
  (bind _returnvalue_3 (/ (.x _returnvalue) _returnvalue_2))
  (bind _returnvalue_4 (/ _returnvalue_3 2.0))
  (if (not (Game|IsGamePaused))
    (bind _returnvalue_5 (Class|WidgetLayoutLibrary|GetMousePositiononViewport))
    (Default|Yaw (Variables|Default|GetBP_EZDOF_Component) (/ (- (.x _returnvalue_5) _returnvalue_4) _returnvalue_4))))

(event Input|MouseEvents|LeftMouseButton
  (params (Key :type Key%20Structure :default "None"))
  (:Pressed
    (CallFunction|OpenFire "NewEnumerator0"))
  (:Released
    (CallFunction|CeaseFire "NewEnumerator0")))

(event Input|KeyboardEvents|Q
  (params (Key :type Key%20Structure :default "None"))
  (:Pressed
    (Variables|/Game/OpenSpaceShooter/Blueprints/Components/InputSender.InputSender_C|SetLockedTargetActor (Variables|Default|GetInputSender) 0)))

(event Input|MouseEvents|RightMouseButton
  (params (Key :type Key%20Structure :default "None"))
  (:Pressed
    (CallFunction|OpenFire "NewEnumerator1"))
  (:Released
    (CallFunction|CeaseFire "NewEnumerator1")))

(fn ConstructionScript
  (bind _springarm (Variables|Default|GetSpringArm))
  (bind _hull (Variables|Default|GetHull))
  (bind _sphereradius (Collision|GetComponentBounds _hull))
  (bind _returnvalue (* _sphereradius 3.0))
  (|CallParentFunction)
  (Variables|/Script/Engine.SpringArmComponent|SetbUsePawnControlRotation _springarm (Variables|Default|GetCapitalShipManeuver))
  (Variables|/Script/Engine.SpringArmComponent|SetSocketOffset _springarm (Math|Vector|MakeVector 0.0 0.0 _sphereradius))
  (Variables|/Script/Engine.SpringArmComponent|SetTargetArmLength _springarm _returnvalue)
  (Variables|/Game/OpenSpaceShooter/Blueprints/Components/InputSender.InputSender_C|SetMinDistance (Variables|Default|GetInputSender) (+ _returnvalue 5e+02)))

(fn SetControlsEnabled
  (params (NewValue :type Boolean))
  (Variables|/Game/OpenSpaceShooter/Blueprints/Components/InputSender.InputSender_C|SetActivated (Variables|Default|GetInputSender) NewValue)
  (if NewValue
    (Input|EnableInput 0)
    (else
      (Input|DisableInput 0)
      (Default|CeaseFire (CallFunction|GetWeapons)))))

(fn NotTraceBlocker
  (params (Comp :type Primitive%20Component%20Object%20Reference))
  (if (Utilities|IsValid Comp)
    (return (Utilities|Enum|Equal(Enum) (Collision|GetCollisionResponsetoChannel Comp "ECC_WorldStatic") "ECR_Block"))
    (else
      (return false))))