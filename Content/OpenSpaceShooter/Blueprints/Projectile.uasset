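; Projectile actor for the space shooter, configured from exposed mesh, speed, lifetime and hit radius, optionally inheriting the instigator's velocity on spawn.
; When a homing target is set, Tick lerps velocity toward it at the homing rate.
; The trigger's first overlap with a blocking, non-instigator object deals point damage, pushes physics bodies (more gently for ships), plays impact effects and destroys the projectile.
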(event OnComponentBeginOverlap(Trigger)
  (params (OverlappedComponent :type Primitive%20Component%20Object%20Reference) (OtherActor :type Actor%20Object%20Reference) (OtherComp :type Primitive%20Component%20Object%20Reference) (OtherBodyIndex :type Integer) (bFromSweep :type Boolean) (SweepResult :type Hit%20Result%20Structure%20%28by%20ref%29))
  (bind _returnvalue (Transformation|GetActorLocation))
  (bind (_bblockinghit _binitialoverlap _time _distance _location _impactpoint) (Collision|BreakHitResult SweepResult))
  (bind _returnvalue_2 (== _distance 0.0))
  (bind _returnvalue_3 (Math|Vector|SelectVector _returnvalue _impactpoint _returnvalue_2))
  (if (and (Utilities|Enum|Equal(Enum) (Collision|GetCollisionResponsetoChannel OtherComp "ECC_WorldDynamic") "ECR_Block") (!= OtherActor (Variables|Actor|GetInstigator)))
    (Utilities|FlowControl|DoOnce false
      (:Completed
        (if (Physics|IsSimulatingPhysics OtherComp "None")
          (Physics|AddImpulseatLocation OtherComp (* (Transformation|GetActorForwardVector) (* (Physics|GetMass OtherComp) (Math|Float|SelectFloat 2e+01 1e+03 (.bSuccess (Utilities|Casting|CastToShipBase OtherActor))))) _returnvalue_3 "None"))
        (Game|Damage|ApplyPointDamage OtherActor (Variables|Default|GetDamage) (Transformation|GetActorForwardVector) SweepResult (Game|GetInstigatorController) self)
        (Effects|SpawnEmitteratLocation (Variables|Default|GetHitEffect) _returnvalue_3 (Math|Random|RandomRotator true) (Math|Conversions|ToVector(Float) (* (.SphereRadius (Collision|GetComponentBounds (Variables|Default|GetProjectileMesh))) 0.02)))
        (Audio|PlaySoundatLocation (Variables|Default|GetHitSound) _returnvalue_3 "0, 0, 0" 1.0 1.0 0.0 0 0 0 0)
        (CallFunction|HandleDeath)))))

(event Custom|Handle%20Death
  (Actor|DestroyActor))

(event EventBeginPlay
  (Audio|PlaySoundatLocation (Variables|Default|GetFiringSound) (Transformation|GetActorLocation) "0, 0, 0" 1.0 1.0 0.0 0 0 0 0)
  (if (Variables|Default|GetInheriteVelocity)
    (bind _instigator (Variables|Actor|GetInstigator)
      (:then
        (Variables|/Script/Engine.MovementComponent|SetVelocity (Variables|Default|GetProjectileMovement) (+ (Transformation|GetVelocity _instigator) (Transformation|GetVelocity))))
      (:else))))

(event EventTick
  (params (DeltaSeconds :type Float%20%28single-precision%29))
  (bind _projectilemovement (Variables|Default|GetProjectileMovement))
  (bind _homingtargetcomponent (Variables|/Script/Engine.ProjectileMovementComponent|GetHomingTargetComponent _projectilemovement)
    (:then
      (Variables|/Script/Engine.MovementComponent|SetVelocity _projectilemovement (Math|Vector|Lerp(Vector) (Variables|/Script/Engine.MovementComponent|GetVelocity _projectilemovement) (* (Math|Vector|Normalize (- (Transformation|GetWorldLocation _homingtargetcomponent) (Transformation|GetActorLocation))) (Variables|/Script/Engine.ProjectileMovementComponent|GetInitialSpeed _projectilemovement)) (Variables|Default|GetHomingRate))))
    (:else)))

(fn ConstructionScript
  (bind _projectilemovement (Variables|Default|GetProjectileMovement))
  (Components|StaticMesh|SetStaticMesh (Variables|Default|GetProjectileMesh) (Variables|Default|GetMesh))
  (Variables|/Script/Engine.ProjectileMovementComponent|SetInitialSpeed _projectilemovement (Variables|Default|GetInitialSpeed))
  (Variables|/Script/Engine.ProjectileMovementComponent|SetMaxSpeed _projectilemovement (Variables|Default|GetMaxSpeed))
  (Actor|SetLifeSpan (Variables|Default|GetLifetime))
  (Components|Sphere|SetSphereRadius (Variables|Default|GetTrigger) (Variables|Default|GetHitRadius) false))