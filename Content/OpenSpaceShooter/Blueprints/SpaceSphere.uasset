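; SpaceSphere is a space backdrop sphere with a material-driven sun, stars and nebula.
; Its construction script scales the sphere by a radius and pushes sun, star density and brightness, and nebula desaturation settings into its materials.
; A valid DirectionalLight overrides the sun direction and optionally its color, while UpdateSun resets on each construction run.
; The event graph contains no active logic.
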(event EventBeginPlay)

(event Collision|EventActorBeginOverlap
  (params (OtherActor :type Actor%20Object%20Reference)))

(event EventTick
  (params (DeltaSeconds :type Float%20%28single-precision%29)))

(fn ConstructionScript
  (bind _sphere (Variables|Default|GetSphere))
  (bind _sphere_2 (Variables|Default|GetSphere))
  (Utilities|FlowControl|Sequence
    (:then_0
      (Transformation|SetRelativeScale3D (Variables|Default|GetSphere) (Math|Conversions|ToVector(Float) (Variables|SpaceSphere|GetSphereRadius))))
    (:then_1
      (Variables|Sun|SetUpdateSun false)
      (Rendering|Material|SetScalarParameterValueonMaterials _sphere_2 "Sun Brightness" (Variables|Sun|GetSunBrightness))
      (Rendering|Material|SetScalarParameterValueonMaterials _sphere_2 "Sun Disk Size" (Variables|Sun|GetSunDiskSize))
      (Rendering|Material|SetVectorParameterValueonMaterials _sphere_2 "Sun Direction" (Math|Vector|GetForwardVector (Variables|Sun|GetSunDirection)))
      (Rendering|Material|SetVectorParameterValueonMaterials _sphere_2 "Sun Color" (Math|Conversions|ToVector(LinearColor) (Variables|Sun|GetSunColor)))
      (bind _directionallight (Variables|Sun|GetDirectionalLight)
        (:then
          (Rendering|Material|SetVectorParameterValueonMaterials _sphere_2 "Sun Direction" (Transformation|GetActorForwardVector _directionallight))
          (if (Variables|Sun|GetUseLightColor)
            (Rendering|Material|SetVectorParameterValueonMaterials _sphere_2 "Sun Color" (Math|Conversions|ToVector(LinearColor) (Rendering|Components|Light|GetLightColor (Variables|/Script/Engine.Light|GetLightComponent _directionallight))))))
        (:else)))
    (:then_2
      (Rendering|Material|SetScalarParameterValueonMaterials _sphere "Star Density" (Variables|StarField|GetStarDensity))
      (Rendering|Material|SetScalarParameterValueonMaterials _sphere "Star Brightness" (Variables|StarField|GetStarBrightness)))
    (:then_3
      (Rendering|Material|SetScalarParameterValueonMaterials (Variables|Default|GetSphere) "Nebula Desaturation" (Variables|Nabula|GetNabulaDesaturation)))))