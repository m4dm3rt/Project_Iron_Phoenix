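; ShipBase is a physics-driven spaceship base with flight, grouped weapons, shields, health and cargo, configured in its construction script.
; UpdateManeuver stores thrust and turn axes that Tick turns into hull force and torque, with cosmetic banking, auto-leveling, overweight slowdown and speed-based engine audio.
; OpenFire and CeaseFire drive child-actor ShipWeapons matching a group.
; On death it explodes, scatters its cargo as launched DropItems and destroys itself.
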(event OnDeath(HealthComponent)
  (params (Instigator :type Controller%20Object%20Reference) (Causer :type Actor%20Object%20Reference))
  (bind _returnvalue (Transformation|GetActorLocation))
  (bind _returnvalue_2 (Math|Random|RandomUnitVector))
  (Effects|SpawnEmitteratLocation "/Game/OpenSpaceShooter/Particles/P_Explosion.P_Explosion" _returnvalue "0, 0, 0" (Math|Conversions|ToVector(Float) (* (.SphereRadius (Collision|GetComponentBounds (Variables|Default|GetHull))) 0.02)))
  (Audio|PlaySoundatLocation "/Game/OpenSpaceShooter/Audio/Explosion_Cue.Explosion_Cue" _returnvalue "0, 0, 0" 2e+01 1.0 0.0 0 0 0 0)
  (while (> (Default|GetCurrentWeight (Variables|Default|GetInventoryComponent)) 0.0)
    (bind _returnvalue_3 (Game|SpawnActorfromClass "/Game/OpenSpaceShooter/Blueprints/DropItem.DropItem_C" (Math|Conversions|ToTransform(Vector) (+ (Transformation|GetActorLocation) (* _returnvalue_2 5e+02))) "Undefined" "OverrideRootScale" 0 (* _returnvalue_2 2e+03) 0))
    (Default|TakeItemfrom (Variables|/Game/OpenSpaceShooter/Blueprints/DropItem.DropItem_C|GetInventoryComponent _returnvalue_3) (Variables|Default|GetInventoryComponent)))
  (Actor|DestroyActor))

(event Custom|Open%20Fire
  (params (WeaponGroup :type E_WeaponGroup%20Enum :default "NewEnumerator0"))
  (for _array_element (CallFunction|GetWeapons)
    (if (Utilities|Enum|Equal(Enum) WeaponGroup (Variables|/Game/OpenSpaceShooter/Blueprints/ShipWeapon.ShipWeapon_C|GetGroup _array_element))
      (Default|OpenFire _array_element))))

(event Custom|Cease%20Fire
  (params (WeaponGroup :type E_WeaponGroup%20Enum :default "NewEnumerator0"))
  (for _array_element (CallFunction|GetWeapons)
    (if (Utilities|Enum|Equal(Enum) WeaponGroup (Variables|/Game/OpenSpaceShooter/Blueprints/ShipWeapon.ShipWeapon_C|GetGroup _array_element))
      (Default|CeaseFire _array_element))))

(event Custom|Update%20Maneuver
  (params (ThrustForward :type Float%20%28double-precision%29) (ThrustRight :type Float%20%28double-precision%29) (ThrustUp :type Float%20%28double-precision%29) (TurnRoll :type Float%20%28double-precision%29) (TurnPitch :type Float%20%28double-precision%29) (TurnYaw :type Float%20%28double-precision%29))
  (Variables|Ship|Maneuver|SetAxisThrust (Math|Vector|MakeVector ThrustForward ThrustRight ThrustUp))
  (Variables|Ship|Maneuver|SetAxisTurn (Math|Vector|MakeVector TurnRoll TurnPitch TurnYaw)))

(event EventTick
  (params (DeltaSeconds :type Float%20%28single-precision%29))
  (bind _returnvalue (Transformation|GetVelocity))
  (bind _returnvalue_2 (Transformation|GetActorRotation))
  (bind _returnvalue_3 (Input|AxisValues|GetMoveForward))
  (bind _capitalshipmaneuver (Variables|Ship|Maneuver|GetCapitalShipManeuver))
  (bind _maxspeed (Variables|Ship|Maneuver|GetMaxSpeed))
  (bind _hull (Variables|Default|GetHull))
  (bind _enginesound (Variables|Default|GetEngineSound))
  (bind _axisthrust (Variables|Ship|Maneuver|GetAxisThrust))
  (bind _axisthrust_2 (Variables|Ship|Maneuver|GetAxisThrust))
  (bind _enginesound_2 (Variables|Default|GetEngineSound))
  (bind _inventorycomponent (Variables|Default|GetInventoryComponent))
  (bind _returnvalue_4 (Math|Vector|VectorLength _returnvalue))
  (bind (_roll _pitch _yaw) (Math|Rotator|BreakRotator _returnvalue_2))
  ;[1 1 1] Update engine sound volume and pitch
  (Audio|Components|Audio|SetVolumeMultiplier _enginesound (Math|Float|Lerp (Variables|/Script/Engine.AudioComponent|GetVolumeMultiplier _enginesound_2) (Math|Float|MapRangeClamped _returnvalue_4 0.0 (/ _maxspeed 2.0) 0.0 1.0) 0.05) :!class /Script/Engine.AudioComponent)
  (Audio|Components|Audio|SetPitchMultiplier _enginesound (Math|Float|Lerp (Variables|/Script/Engine.AudioComponent|GetPitchMultiplier _enginesound_2) (Math|Float|MapRangeClamped _returnvalue_4 0.0 _maxspeed 0.4 1.0) 0.05))
  (if (Physics|IsSimulatingPhysics (Variables|Default|GetHull) "None")
    ;[1 1 1] Turning effects.
    (Transformation|AddActorLocalRotation (Math|Rotator|MakeRotator (* (+ (Math|Float|Clamp(Float) (.z (Variables|Ship|Maneuver|GetAxisTurn)) -0.5 0.5) (.y _axisthrust_2)) 0.5) (Math|Float|SelectFloat (* (Math|Float|Clamp(Float) (.z _axisthrust_2) -0.1 0.1) (Math|Float|SelectFloat 1.0 _returnvalue_3 (== _returnvalue_3 0.0))) 0.0 _capitalshipmaneuver) 0.0) false false)
    (Transformation|SetActorRotation (Math|Rotator|Lerp(Rotator) _returnvalue_2 (Math|Rotator|MakeRotator 0.0 (Math|Float|SelectFloat 0.0 _pitch _capitalshipmaneuver) _yaw) 0.02 true))
    ;[1 1 1] Apply forces and torque
    (Physics|AddForce _hull (* (+ (* (Transformation|GetActorForwardVector) (* (.x _axisthrust) (Math|Float|SelectFloat 1.0 0.3 (> (.x _axisthrust) 0.0)))) (* (Math|Vector|Normalize (* (Transformation|GetActorRightVector) "1.000000,1.000000,0.000000")) (* (.y _axisthrust) 0.5)) (* "0.000000,0.000000,1.000000" (* (.z _axisthrust) 0.3))) (* (Variables|Ship|Maneuver|GetMaxSpeed) (Math|Float|MapRangeClamped (/ (Default|GetCurrentWeight _inventorycomponent) (Variables|/Game/OpenSpaceShooter/Blueprints/Components/InventoryComponent.InventoryComponent_C|GetMaxWeight _inventorycomponent)) 1.0 1.5 1.0 0.1))) "None" true)
    (Class|PrimitiveComponent|AddTorqueinDegrees _hull (* (Math|Transform|TransformDirection (Transformation|GetActorTransform) (* (Math|Vector|ClampVectorSize (Variables|Ship|Maneuver|GetAxisTurn) 0.0 (Math|Vector|VectorLength "1.000000,1.000000,1.000000")) (Variables|Ship|Maneuver|GetTurnRate))) 2e+02) "None" true)))

(fn ConstructionScript
  (bind _capitalshipmaneuver (Variables|Ship|Maneuver|GetCapitalShipManeuver))
  (bind _minimapregistry (Variables|Default|GetMinimapRegistry))
  (bind _returnvalue (Math|Float|SelectFloat 32.0 16.0 _capitalshipmaneuver))
  (Variables|/Game/OpenSpaceShooter/Blueprints/Components/InputReceiver.InputReceiver_C|SetName (Variables|Default|GetInputReceiver) (Variables|Ship|Hull|GetName))
  (Components|StaticMesh|SetStaticMesh (Variables|Default|GetHull) (Variables|Ship|Hull|GetMesh))
  (Variables|/Game/OpenSpaceShooter/Blueprints/Components/MinimapRegistry.MinimapRegistry_C|SetIcon _minimapregistry (Variables|Ship|Hull|GetMapIcon))
  (Variables|/Game/OpenSpaceShooter/Blueprints/Components/MinimapRegistry.MinimapRegistry_C|SetIconSizeOverride _minimapregistry (Math|Vector2D|MakeVector2D _returnvalue _returnvalue))
  (Variables|/Game/OpenSpaceShooter/Blueprints/Components/HealthComponent.HealthComponent_C|SetMaxHealth (Variables|Default|GetHealthComponent) (Variables|Ship|Hull|GetMaxHealth))
  (Default|SetNewShield (Variables|Default|GetShieldComponent) (Variables|Ship|Equipments|GetShieldClass))
  (Variables|/Game/OpenSpaceShooter/Blueprints/Components/InventoryComponent.InventoryComponent_C|SetMaxWeight (Variables|Default|GetInventoryComponent) (Variables|Default|GetCargoSpace)))

(fn SetVelocity
  (params (NewVelocity :type Vector))
  (Physics|SetPhysicsLinearVelocity (Variables|Default|GetHull) NewVelocity false "None"))

(fn GetWeapons
  (for _array_element (Actor|GetAllChildActors true)
    (bind _asship_weapon (Utilities|Casting|CastToShipWeapon _array_element))
    (Utilities|Array|Add (LocalVariables|GetTempArray) _asship_weapon))
  (return (LocalVariables|GetTempArray)))