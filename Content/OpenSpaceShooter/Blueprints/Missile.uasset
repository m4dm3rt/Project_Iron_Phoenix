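; Homing missile projectile for the space shooter that ignites shortly after spawning and seeks its instigator's locked target.
; After a short delay, a gated ignition sets the homing target from the instigator's InputSender and starts the rocket trail and sound.
; HandleDeath, also triggered when Lifetime expires, closes the gate, unregisters from the minimap, and disables collision, mesh, movement and effects.
; The actor is destroyed only when the trail particles finish.
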(event OnSystemFinished(P_RocketTrail)
  (params (PSystem :type Particle%20System%20Component%20Object%20Reference))
  (Actor|DestroyActor))

(event Custom|Shut%20Engine
  (Utilities|FlowControl|Gate false) ; enters at Close
)

(event EventBeginPlay
  (|CallParentFunction)
  (Utilities|FlowControl|Sequence
    (:then_0
      (Utilities|FlowControl|Delay 0.3)
      (Utilities|FlowControl|Gate false
        (:Exit
          (Variables|/Script/Engine.ProjectileMovementComponent|SetHomingTargetComponent (Variables|Default|GetProjectileMovement) (CallFunction|GetHomingTarget))
          (Components|Activation|Activate (Variables|Default|GetP_RocketTrail) false)
          (Audio|Components|Audio|FadeIn (Variables|Default|GetBlasterSound) 0.2 1.0 0.0 "Linear" :!class /Script/Engine.AudioComponent))))
    (:then_1
      (Utilities|FlowControl|Delay (Variables|Default|GetLifetime))
      (CallFunction|HandleDeath))))

(event Collision|EventActorBeginOverlap
  (params (OtherActor :type Actor%20Object%20Reference)))

(event EventTick
  (params (DeltaSeconds :type Float%20%28single-precision%29))
  (|CallParentFunction DeltaSeconds))

(event EventHandleDeath
  (CallFunction|ShutEngine)
  (Default|Unregister (Variables|Default|GetMinimapRegistry))
  (Collision|SetActorEnableCollision false)
  (Rendering|SetVisibility (Variables|Default|GetProjectileMesh) false false)
  (Components|Activation|Deactivate (Variables|Default|GetP_RocketTrail))
  (Audio|Components|Audio|Stop (Variables|Default|GetBlasterSound)))

(fn ConstructionScript
  (|CallParentFunction)
  (Actor|SetLifeSpan 0.0))

(fn GetHomingTarget
  (bind _returnvalue (Game|GetInstigator))
  (bind _returnvalue_2 (Actor|GetComponentbyClass _returnvalue "/Game/OpenSpaceShooter/Blueprints/Components/InputSender.InputSender_C"))
  (bind _lockedtargetactor (Variables|/Game/OpenSpaceShooter/Blueprints/Components/InputSender.InputSender_C|GetLockedTargetActor _returnvalue_2))
  (Utilities|IsValid _returnvalue
    (:Is%20Valid
      (Utilities|IsValid _returnvalue_2
        (:Is%20Valid
          (Utilities|IsValid _lockedtargetactor
            (:Is%20Valid
              (return (Variables|/Script/Engine.Actor|GetRootComponent _lockedtargetactor)))
            (:Is%20Not%20Valid
              _)))
        (:Is%20Not%20Valid
          _)))
    (:Is%20Not%20Valid
      _))
  (return 0))