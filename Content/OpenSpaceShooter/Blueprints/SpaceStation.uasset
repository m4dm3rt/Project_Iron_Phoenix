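; Space station that ships dock at and undock from, triggered through its input receiver.
; Docking disables player controls, then a timeline eases the ship toward the nearest of four points spaced 90 degrees apart, which slide inward as it plays.
; When docking finishes, the master widget opens the station panel.
; Undocking rotates the ship 180 degrees, drives it forward on a sine-eased timeline, then restores controls.
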(event HandleInput(InputReceiver)
  (params (Sender :type Input%20Sender%20Object%20Reference) (Input :type String))
  (bind _asship_base (Utilities|Casting|CastToShipBase (Components|GetOwner Sender)))
  (CallFunction|Dock _asship_base))

(event Custom|Dock
  (params (Passenger :type Ship%20Base%20Object%20Reference))
  (bind _returnvalue (Transformation|GetActorLocation))
  (bind _returnvalue_2 (Transformation|GetActorLocation Passenger))
  (bind _dock_line (Variables|Default|GetDock%20Line))
  (bind _returnvalue_3 (Components|Timeline|GetPlaybackPosition _dock_line))
  (bind _returnvalue_4 (Math|Float|Lerp 3.2e+04 2e+04 _returnvalue_3))
  (bind _returnvalue_5 (Math|Vector|MakeVector _returnvalue_4 0.0 -1.3e+03))
  (bind _returnvalue_6 (Math|Vector|RotateVectorAroundAxis _returnvalue_5 9e+01 "0, 0,1.000000"))
  (bind _returnvalue_7 (+ _returnvalue _returnvalue_5))
  (bind _returnvalue_8 (Math|Vector|RotateVectorAroundAxis _returnvalue_6 9e+01 "0, 0,1.000000"))
  (bind _returnvalue_9 (+ _returnvalue _returnvalue_6))
  (bind _returnvalue_10 (Math|Vector|RotateVectorAroundAxis _returnvalue_8 9e+01 "0, 0,1.000000"))
  (bind _returnvalue_11 (+ _returnvalue _returnvalue_8))
  (bind _returnvalue_12 (+ _returnvalue _returnvalue_10))
  (bind _array (Utilities|Array|MakeArray _returnvalue_7 _returnvalue_9 _returnvalue_11 _returnvalue_12))
  (bind _closest (CallFunction|FindClosestLocation _returnvalue_2 _array))
  (bind _asship_controllable (Utilities|Casting|CastToShipControllable Passenger)
    (:then
      (Default|SetControlsEnabled _asship_controllable false))
    (:CastFailed
      _))
  (Components|Timeline|SetPlayRate (Variables|Default|GetDock%20Line) 0.2)
  (bind _output (Timeline|Dock%20Line PlayFromStart)
    (:Update
      (Pawn|SetControlRotation (Pawn|GetController Passenger) (Math|Rotator|Lerp(Rotator) (Pawn|GetControlRotation Passenger :!class /Script/Engine.Pawn) (Transformation|GetActorRotation Passenger) 0.05 true))
      (Transformation|SetActorTransform Passenger (Math|Transform|Lerp(Transform) (Transformation|GetActorTransform Passenger) (Math|Transform|MakeTransform _closest (Math|Rotator|FindLookatRotation _returnvalue_2 _closest)) (Math|Float|Clamp(Float) (Math|Float|Power _output 3.0) 0.0 0.05)))
      (Default|UpdateManeuver Passenger 0.0 0.0 0.0 0.0 0.0 0.0))
    (:Finished
      (CallFunction|DockFinished Passenger))))

(event Custom|Dock%20Finished
  (params (Passenger :type Ship%20Base%20Object%20Reference))
  (bind _foundwidgets (Widget|GetAllWidgetsOfClass "/Game/OpenSpaceShooter/Widgets/WBP_MasterWidget.WBP_MasterWidget_C" true))
  (Utilities|IsValid (Utilities|Array|Get(acopy) _foundwidgets)
    (:Is%20Valid
      (Default|OpenSpaceStationPanel (Utilities|Array|Get(acopy) _foundwidgets) self Passenger))))

(event Custom|Undock
  (params (Passenger :type Ship%20Base%20Object%20Reference))
  (bind _asship_controllable (Utilities|Casting|CastToShipControllable Passenger)
    (:then
      (Default|TempDisableCameraLag _asship_controllable))
    (:CastFailed
      _))
  (Transformation|AddActorLocalRotation Passenger "0,180.000000, 0" false false)
  (Components|Timeline|SetPlayRate (Variables|Default|GetUndock%20Line) 0.5)
  (bind _output (Timeline|Undock%20Line PlayFromStart)
    (:Update
      (Pawn|SetControlRotation (Pawn|GetController Passenger) (Transformation|GetActorRotation Passenger))
      (Default|SetVelocity Passenger (* (Transformation|GetActorForwardVector Passenger) (* (Variables|/Game/OpenSpaceShooter/Blueprints/ShipBase.ShipBase_C|GetMaxSpeed Passenger) (Math|Trig|Sin(Degrees) (* _output 9e+01)) 0.4))))
    (:Finished
      (CallFunction|UndockFinished Passenger))))

(event Custom|Undock%20Finished
  (params (Passenger :type Ship%20Base%20Object%20Reference))
  (bind _asship_controllable (Utilities|Casting|CastToShipControllable Passenger))
  (Default|SetControlsEnabled _asship_controllable true))

(event EventBeginPlay
  (|CallParentFunction) ; This node is disabled and will not be called.\nDrag off pins to build functionality.
)

(event Collision|EventActorBeginOverlap
  (params (OtherActor :type Actor%20Object%20Reference))
  (|CallParentFunction OtherActor) ; This node is disabled and will not be called.\nDrag off pins to build functionality.
)

(event EventTick
  (params (DeltaSeconds :type Float%20%28single-precision%29))
  (|CallParentFunction DeltaSeconds) ; This node is disabled and will not be called.\nDrag off pins to build functionality.
)

(fn ConstructionScript
  (|CallParentFunction))