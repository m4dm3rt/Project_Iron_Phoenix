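; Actor component that tracks the health of its owner in the space shooter and signals death.
; On BeginPlay it fills health to maximum, binds to the owner's any-damage event and looks up an optional ShieldComponent.
; Damage passes through the shield when one exists, and the amount it returns is subtracted from health.
; At zero, health is clamped and OnDeath fires with the instigator and causer, with no guard against repeat calls.
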(event Custom|Handle%20Damage
  (params (DamagedActor :type Actor%20Object%20Reference) (Damage :type Float%20%28single-precision%29) (DamageType :type Damage%20Type%20Object%20Reference) (InstigatedBy :type Controller%20Object%20Reference) (DamageCauser :type Actor%20Object%20Reference))
  (bind _shield (Variables|Default|GetShield))
  (bind _returnvalue (Utilities|IsValid _shield))
  (if _returnvalue
    (bind _overkill (Default|ApplyDamage _shield Damage)))
  (bind _output_get (Variables|Internal|SetCurrentHealth (- (Variables|Internal|GetCurrentHealth) (Math|Float|SelectFloat _overkill Damage _returnvalue))))
  (if (<= _output_get 0.0)
    (Variables|Internal|SetCurrentHealth 0.0)
    (Default|CallOnDeath InstigatedBy DamageCauser)))

(event EventBeginPlay
  (bind _returnvalue (Components|GetOwner))
  (Variables|Internal|SetCurrentHealth (Variables|Default|GetMaxHealth))
  (EventDispatchers|AssignOnTakeAnyDamage _returnvalue (delegate Custom|Handle%20Damage))
  (Variables|Default|SetShield (Actor|GetComponentbyClass _returnvalue "/Game/OpenSpaceShooter/Blueprints/Components/ShieldComponent.ShieldComponent_C")))

(event EventTick
  (params (DeltaSeconds :type Float%20%28single-precision%29)))