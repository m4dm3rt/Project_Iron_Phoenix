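; MinimapRegistry is a component that registers itself with the WBP_Minimap widget so it can be tracked on the minimap.
; On BeginPlay it finds the first minimap widget and passes itself to RegisterObject, retrying a few times after a short delay if none exists yet.
; On EndPlay it looks up the widget again and unregisters itself.
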(event Custom|Register
  (bind _foundwidgets (Widget|GetAllWidgetsOfClass "/Game/OpenSpaceShooter/Widgets/WBP_Minimap.WBP_Minimap_C" false))
  (Utilities|IsValid (Utilities|Array|Get(acopy) _foundwidgets)
    (:Is%20Valid
      (Default|RegisterObject (Utilities|Array|Get(acopy) _foundwidgets) self))
    (:Is%20Not%20Valid
      (Utilities|FlowControl|DoN 3 ; try more times if the map is not yet instantiated
        (:Exit
          (Utilities|FlowControl|Delay 0.01)
          (CallFunction|Register))))))

(event Custom|Unregister
  (bind _foundwidgets (Widget|GetAllWidgetsOfClass "/Game/OpenSpaceShooter/Widgets/WBP_Minimap.WBP_Minimap_C" false))
  (Utilities|IsValid (Utilities|Array|Get(acopy) _foundwidgets)
    (:Is%20Valid
      (Default|UnregisterObject (Utilities|Array|Get(acopy) _foundwidgets) self))))

(event EventBeginPlay
  (CallFunction|Register))

(event EventTick
  (params (DeltaSeconds :type Float%20%28single-precision%29)))

(event EventEndPlay
  (params (EndPlayReason :type EEndPlayReason%20Enum :default "Destroyed"))
  (CallFunction|Unregister))