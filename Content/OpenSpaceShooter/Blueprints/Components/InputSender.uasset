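; Component that lets a player target, lock onto and send input to actors carrying an InputReceiver component.
; While activated, Tick sphere-traces from the player camera, caches the hit actor and its receiver, and accumulates lock time on a steady target until it calls OnLocked.
; SendInput forwards input to the current receiver when in range.
; Receivers define input, scan and lock ranges: zero means unlimited, and negative lock range means unlockable.
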(event Custom|Send%20Input
  (params (Input :type String))
  (if (CallFunction|IsTargetinInputRange)
    (Default|CallHandleInput (Variables|Default|GetInputReceiver) self Input)))

(event EventBeginPlay)

(event EventTick
  (params (DeltaSeconds :type Float%20%28single-precision%29))
  (bind _returnvalue (Game|GetPlayerCameraManager 0))
  (bind _returnvalue_2 (Camera|GetCameraLocation _returnvalue))
  (bind _returnvalue_3 (Camera|GetCameraRotation _returnvalue))
  (bind _returnvalue_4 (Math|Vector|GetForwardVector _returnvalue_3))
  (if (Variables|Default|GetActivated)
    (bind _outhit (Collision|SphereTraceByChannel (+ _returnvalue_2 (* _returnvalue_4 (Variables|Default|GetMinDistance))) (+ _returnvalue_2 (* _returnvalue_4 (Variables|Default|GetTraceDistance))) (Variables|Default|GetTraceRadius) "TraceTypeQuery1" false 0 "None"))
    (Variables|Default|SetHitResult _outhit)
    (Utilities|FlowControl|Sequence
      (:then_0
        (if (Math|Boolean|ANDBoolean (== (Variables|Default|GetTargetActor) (.HitActor (Collision|BreakHitResult _outhit))) (!= (Variables|Default|GetLockedTargetActor) (.HitActor (Collision|BreakHitResult _outhit))) (CallFunction|IsTargetinLockRange))
          (bind _output_get (Variables|Internal|SetLockProgress (+ (Variables|Internal|GetLockProgress) (Utilities|Time|GetWorldDeltaSeconds))))
          (if (>= _output_get (Variables|Default|GetLockTime))
            (Default|CallOnLocked (Actor|GetComponentbyClass (Variables|Default|GetTargetActor) "/Game/OpenSpaceShooter/Blueprints/Components/InputReceiver.InputReceiver_C") self)
            ;[1 1 1] keep old target if new target is destroyed on locked (pickup, etc.)
            (Utilities|IsValid (Variables|Default|GetTargetActor)
              (:Is%20Valid
                (Variables|Default|SetLockedTargetActor (Variables|Default|GetTargetActor)))
              (:Is%20Not%20Valid
                _))
            (Variables|Internal|SetLockProgress 0.0 :!label _label))
          (else
            (goto _label))))
      (:then_1
        (bind _output_get_2 (Variables|Default|SetTargetActor (.HitActor (Collision|BreakHitResult _outhit))))
        (Utilities|IsValid _output_get_2
          (:Is%20Valid
            (Variables|Default|SetInputReceiver (Actor|GetComponentbyClass (.HitActor (Collision|BreakHitResult _outhit)) "/Game/OpenSpaceShooter/Blueprints/Components/InputReceiver.InputReceiver_C")))
          (:Is%20Not%20Valid
            (Variables|Default|SetInputReceiver 0)))))
    (else
      (Variables|Default|SetHitResult "")
      (Variables|Default|SetTargetActor 0)
      (Variables|Default|SetLockedTargetActor 0)
      (Variables|Default|SetInputReceiver 0)
      (Variables|Internal|SetLockProgress 0.0))))

(fn IsTargetinInputRange
  (bind _hitresult (Variables|Default|GetHitResult))
  (bind (_bblockinghit _binitialoverlap _time _distance) (Collision|BreakHitResult _hitresult))
  (bind _inputreceiver (Variables|Default|GetInputReceiver)
    (:then
      (return (or (>= (Variables|/Game/OpenSpaceShooter/Blueprints/Components/InputReceiver.InputReceiver_C|GetInputRange _inputreceiver) (Math|Float|SelectFloat _distance (Variables|Default|GetTraceDistance) _bblockinghit)) (<= (Variables|/Game/OpenSpaceShooter/Blueprints/Components/InputReceiver.InputReceiver_C|GetInputRange _inputreceiver) 0.0))))
    (:else
      (return false))))

(fn IsTargetinScanRange
  (bind _hitresult (Variables|Default|GetHitResult))
  (bind (_bblockinghit _binitialoverlap _time _distance) (Collision|BreakHitResult _hitresult))
  (bind _inputreceiver (Variables|Default|GetInputReceiver)
    (:then
      (return (or (>= (Variables|/Game/OpenSpaceShooter/Blueprints/Components/InputReceiver.InputReceiver_C|GetScanRange _inputreceiver) (Math|Float|SelectFloat _distance (Variables|Default|GetTraceDistance) _bblockinghit)) (<= (Variables|/Game/OpenSpaceShooter/Blueprints/Components/InputReceiver.InputReceiver_C|GetScanRange _inputreceiver) 0.0))))
    (:else
      (return false))))

(fn IsTargetinLockRange
  (bind _hitresult (Variables|Default|GetHitResult))
  (bind (_bblockinghit _binitialoverlap _time _distance) (Collision|BreakHitResult _hitresult))
  (bind _inputreceiver (Variables|Default|GetInputReceiver)
    (:then
      (return (or (>= (Variables|/Game/OpenSpaceShooter/Blueprints/Components/InputReceiver.InputReceiver_C|GetLockRange _inputreceiver) (Math|Float|SelectFloat _distance (Variables|Default|GetTraceDistance) _bblockinghit)) (== (Variables|/Game/OpenSpaceShooter/Blueprints/Components/InputReceiver.InputReceiver_C|GetLockRange _inputreceiver) 0.0))))
    (:else
      (return false))))