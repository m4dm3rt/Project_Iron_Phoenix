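; Actor component that gives its owner a regenerating shield, configured from a data table row chosen by the shield class.
; ApplyDamage drains the shield, resets the regen delay and returns overkill damage, while Tick refills it once the delay has passed.
; SetNewShield swaps shield stats and signals the change.
; Current charge and delay progress serialize to a comma-separated string, which SetNewShield can restore, defaulting to full charge when empty.
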(event EventBeginPlay
  (CallFunction|SetNewShield (Variables|Default|GetShieldClass)))

(event EventTick
  (params (DeltaSeconds :type Float%20%28single-precision%29))
  (Variables|Internal|SetRegenDelayProgress (+ (Variables|Internal|GetRegenDelayProgress) DeltaSeconds))
  (if (>= (Variables|Internal|GetRegenDelayProgress) (Variables|Internal|GetRegenDelay))
    (Variables|Internal|SetCurrentShield (Math|Float|Clamp(Float) (+ (Variables|Internal|GetCurrentShield) (* DeltaSeconds (Variables|Internal|GetRegenRate))) 0.0 (Variables|Internal|GetMaxShield)))))

(fn ApplyDamage
  (params (Damage :type Float%20%28double-precision%29))
  (Variables|Internal|SetRegenDelayProgress 0.0)
  (LocalVariables|SetTempOverkill (Math|Float|SelectFloat 0.0 (Math|Float|Absolute(Float) (- (Variables|Internal|GetCurrentShield) Damage)) (>= (- (Variables|Internal|GetCurrentShield) Damage) 0.0)))
  (Variables|Internal|SetCurrentShield (Math|Float|Clamp(Float) (- (Variables|Internal|GetCurrentShield) Damage) 0.0 (Variables|Internal|GetMaxShield)))
  (return (LocalVariables|GetTempOverkill)))

(fn SetNewShield
  (params (NewShieldClass :type Data%20Table%20Row%20Handle%20Structure) (CustomData :type String))
  (bind (_currentshield _regendelayprogress) (CallFunction|ParseCustomDataString CustomData))
  (bind _output_get (Variables|Default|SetShieldClass NewShieldClass))
  (bind _returnvalue (Utilities|GetDataTableRow (.DataTable (Utilities|Struct|BreakDataTableRowHandle _output_get)) (.RowName (Utilities|Struct|BreakDataTableRowHandle _output_get)))
    (:then
      (bind _output_get_2 (Variables|Internal|SetShieldData _returnvalue))
      (Variables|Internal|SetMaxShield (.MaxShield (Utilities|Struct|BreakS_ShieldData _output_get_2)))
      (Variables|Internal|SetCurrentShield _currentshield)
      (Variables|Internal|SetRegenRate (.ShieldRegenRate (Utilities|Struct|BreakS_ShieldData _output_get_2)))
      (Variables|Internal|SetRegenDelay (.ShieldRegenDelay (Utilities|Struct|BreakS_ShieldData _output_get_2)))
      (Variables|Internal|SetRegenDelayProgress _regendelayprogress)
      (Default|CallShieldChanged))))

(fn GetCustomDataString
  (return (Utilities|String|JoinStringArray (Utilities|Array|MakeArray (Utilities|String|ToString(Float) (Variables|Internal|GetCurrentShield)) (Utilities|String|ToString(Float) (Variables|Internal|GetRegenDelayProgress))) ",")))

(fn ParseCustomDataString
  (params (DataString :type String))
  (bind _returnvalue (Utilities|String|ParseIntoArray DataString ","))
  (if (> (Utilities|String|Len DataString) 0)
    (return (Math|Conversions|ToFloat(Integer) (Utilities|Array|Get(acopy) _returnvalue)) (Math|Conversions|ToFloat(Integer) (Utilities|Array|Get(acopy) _returnvalue 1)))
    (else
      (return (Variables|Internal|GetMaxShield) 0.0))))