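; Inventory component for the space shooter that holds item stacks as data table row references with count and custom data.
; Create, take, split, merge, swap and destroy functions edit the Contents array and signal changes through CallContentsChanged.
; Transfers and merges share FillSlot, which fills matching stacks up to MaxStack (zero means unlimited), while transfers append new slots for leftovers.
; Item details and total weight come from data table lookups.
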(event EventBeginPlay)

(event EventTick
  (params (DeltaSeconds :type Float%20%28single-precision%29)))

(fn TakeAllfrom
  (params (OtherInventory :type Inventory%20Component%20Object%20Reference))
  (while (> (Utilities|Array|Length (Variables|InventoryComponent_C|GetContents OtherInventory)) 0)
    (Inventory|Operation|TakeItemfrom OtherInventory)))

(fn GetCurrentWeight
  (for _array_element (Variables|Default|GetContents)
    (LocalVariables|SetTempWeight (+ (.SlotWeight (Inventory|Info|GetItemDetails _array_element)) (LocalVariables|GetTempWeight))))
  (return (LocalVariables|GetTempWeight)))

(fn TakeItemfrom
  (params (OtherInventory :type Inventory%20Component%20Object%20Reference) (OtherSlot :type Integer) (NumGiven :type Integer))
  (bind _contents (Variables|InventoryComponent_C|GetContents OtherInventory))
  (bind _output (Utilities|Array|Get(acopy) _contents OtherSlot))
  (bind (_item _count _customdata) (Utilities|Struct|BreakS_InventoryItem _output))
  (LocalVariables|SetNumLeft (Math|Integer|SelectInt NumGiven (Utilities|Struct|BreakS_InventoryItem (Utilities|Array|Get(acopy) (Variables|InventoryComponent_C|GetContents OtherInventory) OtherSlot)) (> NumGiven 0)))
  (for _index (range 0 (Utilities|Array|LastIndex (Variables|Default|GetContents))) :!label _label
    (bind _numleft (Inventory|HelperFunction|FillSlot _index OtherInventory OtherSlot (LocalVariables|GetNumLeft)))
    (bind _output_get (LocalVariables|SetNumLeft _numleft))
    (if (<= _output_get 0)
      (Default|CallContentsChanged OtherInventory)
      (Default|CallContentsChanged)
      (return)))
  (Utilities|Array|Add (Variables|Default|GetContents) (Utilities|Struct|MakeS_InventoryItem _item 0 _customdata)) ; execution of this line indicates there are still items left
  (goto _label))

(fn GetItemDetails
  (params (Item :type S%20Inventory%20Item%20Structure%20%28by%20ref%29))
  (bind (_item _count) (Utilities|Struct|BreakS_InventoryItem Item))
  (bind (_datatable _rowname) (Utilities|Struct|BreakDataTableRowHandle _item))
  (bind _returnvalue (Utilities|GetDataTableRow _datatable _rowname)
    (:then
      (return _returnvalue (* _count (Utilities|Struct|BreakS_ItemDetails _returnvalue))))))

(fn SameItem
  (params (A :type S%20Inventory%20Item%20Structure) (B :type S%20Inventory%20Item%20Structure))
  (bind _item (Utilities|Struct|BreakS_InventoryItem A))
  (bind _item_2 (Utilities|Struct|BreakS_InventoryItem B))
  (bind (_datatable _rowname) (Utilities|Struct|BreakDataTableRowHandle _item))
  (bind (_datatable_2 _rowname_2) (Utilities|Struct|BreakDataTableRowHandle _item_2))
  (return (and (== _datatable _datatable_2) (Utilities|Name|Equal(Name) _rowname _rowname_2))))

(fn CreateItem
  (params (NewItem :type S%20Inventory%20Item%20Structure))
  (bind (_item _count _customdata) (Utilities|Struct|BreakS_InventoryItem NewItem))
  (bind _details (Inventory|Info|GetItemDetails NewItem))
  (bind _maxstack (Utilities|Struct|BreakS_ItemDetails _details))
  (bind _returnvalue (== _maxstack 0))
  (bind _returnvalue_2 (Math|Integer|SelectInt _count _maxstack _returnvalue))
  (bind _returnvalue_3 (Math|Integer|%(Integer) _count _returnvalue_2))
  (for _index (range 0 (- (/ _count _returnvalue_2) 1))
    (Utilities|Array|Add (Variables|Default|GetContents) (Utilities|Struct|MakeS_InventoryItem _item _returnvalue_2 _customdata)) ; No same item found.
  )
  (if (> _returnvalue_3 0)
    (Utilities|Array|Add (Variables|Default|GetContents) (Utilities|Struct|MakeS_InventoryItem _item _returnvalue_3 _customdata)) ; No same item found.
  )
  (Default|CallContentsChanged)
  (return))

(fn SwapItems
  (params (Slot1 :type Integer) (Slot2 :type Integer))
  (Utilities|Array|Swap (Variables|Default|GetContents) Slot1 Slot2)
  (Default|CallContentsChanged))

(fn SplitItem
  (params (Slot :type Integer))
  (bind _contents (Variables|Default|GetContents))
  (bind _output (Utilities|Array|Get(acopy) _contents Slot))
  (bind (_item _count _customdata) (Utilities|Struct|BreakS_InventoryItem _output))
  (bind _returnvalue (/ _count 2))
  (if (> _returnvalue 0)
    (Utilities|Array|Add _contents (Utilities|Struct|MakeS_InventoryItem _item _returnvalue _customdata)))
  (Utilities|Struct|SetmembersinS_InventoryItem _output (+ _returnvalue (Math|Integer|%(Integer) _count 2)))
  (Default|CallContentsChanged))

(fn MergeItems
  (params (FromSlot :type Integer) (ToSlot :type Integer))
  (Inventory|HelperFunction|FillSlot ToSlot self FromSlot (Utilities|Struct|BreakS_InventoryItem (Utilities|Array|Get(acopy) (Variables|Default|GetContents) FromSlot)))
  (Default|CallContentsChanged))

(fn DestroyItem
  (params (DestroySlot :type Integer) (DestroyCount :type Integer))
  (bind _contents (Variables|Default|GetContents))
  (bind _output (Utilities|Array|Get(acopy) _contents DestroySlot))
  (bind _count (Utilities|Struct|BreakS_InventoryItem _output))
  (if (and (> DestroyCount 0) (< DestroyCount _count))
    (Utilities|Struct|SetmembersinS_InventoryItem _output (- _count DestroyCount))
    (else
      (Utilities|Array|RemoveIndex _contents DestroySlot)))
  (Default|CallContentsChanged))

(fn FillSlot
  (params (SelfSlot :type Integer) (OtherInventory :type Inventory%20Component%20Object%20Reference) (OtherSlot :type Integer) (NumGiven :type Integer))
  (bind _contents (Variables|Default|GetContents))
  (bind _contents_2 (Variables|Default|GetContents))
  (bind _output (Utilities|Array|Get(acopy) _contents SelfSlot))
  (bind _output_2 (Utilities|Array|Get(acopy) _contents_2 SelfSlot))
  (bind _contents_3 (Variables|InventoryComponent_C|GetContents OtherInventory))
  (bind _details (Inventory|Info|GetItemDetails _output))
  (bind _output_3 (Utilities|Array|Get(acopy) _contents_3 OtherSlot))
  (bind _maxstack (Utilities|Struct|BreakS_ItemDetails _details))
  (if (and (== SelfSlot OtherSlot) (== OtherInventory self))
    (return 0)
    (else
      (if (not (Inventory|Info|SameItem (Utilities|Array|Get(acopy) (Variables|InventoryComponent_C|GetContents OtherInventory) OtherSlot) (Utilities|Array|Get(acopy) (Variables|Default|GetContents) SelfSlot)))
        _
        (else
          (LocalVariables|SetNumTaken (Math|Integer|SelectInt NumGiven (Math|Integer|Min(Integer) NumGiven (- _maxstack (.Count (Utilities|Struct|BreakS_InventoryItem _output)))) (== _maxstack 0)))
          (Utilities|Struct|SetmembersinS_InventoryItem _output_2 (+ (Utilities|Struct|BreakS_InventoryItem _output_2) (LocalVariables|GetNumTaken)))
          (if (> (- (Utilities|Struct|BreakS_InventoryItem _output_3) (LocalVariables|GetNumTaken)) 0)
            (Utilities|Struct|SetmembersinS_InventoryItem _output_3 (- (Utilities|Struct|BreakS_InventoryItem _output_3) (LocalVariables|GetNumTaken)))
            (else
              (Utilities|Array|RemoveIndex (Variables|InventoryComponent_C|GetContents OtherInventory) OtherSlot)))))
      (return (- NumGiven (LocalVariables|GetNumTaken))))))