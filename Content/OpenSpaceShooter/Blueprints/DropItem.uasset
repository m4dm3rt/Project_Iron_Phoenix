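; DropItem is a loot pickup actor that holds items in an inventory and is launched with a mass-scaled impulse at a random offset on spawn.
; Its InputReceiver name lists the item names and counts, refreshed whenever the contents change.
; Locking onto it immediately triggers its input handler, which moves all items into the sender owner's inventory, plays pickup effects and destroys the actor.
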(event HandleInput(InputReceiver)
  (params (Sender :type Input%20Sender%20Object%20Reference) (Input :type String))
  (bind _returnvalue (Components|GetOwner Sender))
  (bind _returnvalue_2 (Actor|GetComponentbyClass _returnvalue "/Game/OpenSpaceShooter/Blueprints/Components/InventoryComponent.InventoryComponent_C"))
  (Utilities|IsValid _returnvalue_2
    (:Is%20Valid
      (Default|TakeAllfrom _returnvalue_2 (Variables|Default|GetInventoryComponent))
      (bind _returnvalue_3 (Effects|SpawnEmitteratLocation "/Game/OpenSpaceShooter/Particles/P_PickUp.P_PickUp" (Transformation|GetActorLocation)))
      (Audio|SpawnSoundAttached "/Game/OpenSpaceShooter/Audio/PickUp_Cue.PickUp_Cue" _returnvalue_3 "None" "0, 0, 0" "0, 0, 0" "KeepRelativeOffset" false 1.0 1.0 0.0 0 0)
      (Actor|DestroyActor))))

(event ContentsChanged(InventoryComponent)
  (CallFunction|UpdateDisplayInfo))

(event OnLocked(InputReceiver)
  (params (InputSender :type Input%20Sender%20Object%20Reference))
  (Default|CallHandleInput (Variables|Default|GetInputReceiver) InputSender))

(event EventBeginPlay
  (bind _mesh (Variables|Default|GetMesh))
  (CallFunction|UpdateDisplayInfo)
  (Physics|AddImpulseatLocation (Variables|Default|GetMesh) (* (Variables|Default|GetLaunchImpulse) (Physics|GetMass _mesh)) (+ (Transformation|GetActorLocation) (* (Math|Random|RandomUnitVector) (* (.SphereRadius (Collision|GetComponentBounds _mesh)) (Math|Random|RandomFloatinRange 0.2 0.4)))) "None"))

(event Collision|EventActorBeginOverlap
  (params (OtherActor :type Actor%20Object%20Reference)))

(event EventTick
  (params (DeltaSeconds :type Float%20%28single-precision%29)))

(fn ConstructionScript)

(fn UpdateDisplayInfo
  (bind _inventorycomponent (Variables|Default|GetInventoryComponent))
  (for _array_element (Variables|/Game/OpenSpaceShooter/Blueprints/Components/InventoryComponent.InventoryComponent_C|GetContents _inventorycomponent)
    (LocalVariables|SetTempText (Utilities|String|Append (LocalVariables|GetTempText) (Utilities|String|Append (.Name (Utilities|Struct|BreakS_ItemDetails (.Details (Default|GetItemDetails _inventorycomponent _array_element)))) " x " (Utilities|String|ToString(Integer) (.Count (Utilities|Struct|BreakS_InventoryItem _array_element))) " 
"))))
  (Variables|/Game/OpenSpaceShooter/Blueprints/Components/InputReceiver.InputReceiver_C|SetName (Variables|Default|GetInputReceiver) (Utilities|String|TrimTrailing (LocalVariables|GetTempText))))