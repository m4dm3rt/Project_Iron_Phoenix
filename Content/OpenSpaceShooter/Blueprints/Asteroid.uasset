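; Destructible asteroid for a space shooter that holds a mineable resource and drops it when destroyed.
; The construction script applies the configured mesh and seeds the inventory with Carbon, Iron or Gold from DT_Items, weighted by repeated array entries.
; The random item count scales with the actor's largest scale axis.
; On health death it spawns a DropItem launched in a random direction, transfers the inventory into it and destroys itself.
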(event OnDeath(HealthComponent)
  (params (Instigator :type Controller%20Object%20Reference) (Causer :type Actor%20Object%20Reference))
  (bind _returnvalue (Game|SpawnActorfromClass "/Game/OpenSpaceShooter/Blueprints/DropItem.DropItem_C" (Transformation|GetActorTransform) "Undefined" "OverrideRootScale" 0 (* (Math|Random|RandomUnitVector) 3e+03) 0))
  (Default|TakeAllfrom (Variables|/Game/OpenSpaceShooter/Blueprints/DropItem.DropItem_C|GetInventoryComponent _returnvalue) (Variables|Default|GetInventoryComponent))
  (Actor|DestroyActor))

(event EventBeginPlay)

(event Collision|EventActorBeginOverlap
  (params (OtherActor :type Actor%20Object%20Reference)))

(event EventTick
  (params (DeltaSeconds :type Float%20%28single-precision%29)))

(fn ConstructionScript
  (bind _returnvalue (Utilities|Name|MakeLiteralName "Gold"))
  (bind _returnvalue_2 (Utilities|Name|MakeLiteralName "Carbon"))
  (bind _returnvalue_3 (Utilities|Name|MakeLiteralName "Iron"))
  (Components|StaticMesh|SetStaticMesh (Variables|Default|GetStaticMesh) (Variables|Default|GetMesh))
  (Default|CreateItem (Variables|Default|GetInventoryComponent) (Utilities|Struct|MakeS_InventoryItem (Utilities|Struct|MakeDataTableRowHandle "/Game/OpenSpaceShooter/Data/DataTables/DT_Items.DT_Items" (Utilities|Array|Get(acopy) (Utilities|Array|MakeArray _returnvalue_2 _returnvalue_2 _returnvalue_2 _returnvalue_2 _returnvalue_2 _returnvalue_3 _returnvalue_3 _returnvalue_3 _returnvalue _returnvalue) (Math|Random|RandomInteger 10))) (Math|Float|Ceil (* (Math|Random|RandomIntegerinRange 1 3) (Math|Vector|GetMaxElement (Transformation|GetActorScale3D)))))))