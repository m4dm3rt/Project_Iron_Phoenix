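; FalconFighter is a fighter Blueprint in OpenSpaceShooter that handles leaving the current level for MainMap.
; Pressing Q casts the game instance to OpenSpaceInst, stores the actor's transform as LastTransform so it outlives the level change, then opens MainMap.
; BeginPlay, overlap and Tick are disabled, and a SpaceStation lookup and an OpenLevel call with test options are left unconnected.
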(event EventBeginPlay
  (|CallParentFunction) ; This node is disabled and will not be called.\nDrag off pins to build functionality.
)

(event Collision|EventActorBeginOverlap
  (params (OtherActor :type Actor%20Object%20Reference))
  (|CallParentFunction OtherActor) ; This node is disabled and will not be called.\nDrag off pins to build functionality.
)

(event EventTick
  (params (DeltaSeconds :type Float%20%28single-precision%29))
  (|CallParentFunction DeltaSeconds) ; This node is disabled and will not be called.\nDrag off pins to build functionality.
)

(event Input|KeyboardEvents|Q
  (params (Key :type Key%20Structure))
  (:Pressed
    (bind _asopen_space_inst (Utilities|Casting|CastToOpenSpaceInst (Game|GetGameInstance)))
    (Variables|/Game/OpenSpaceShooter/Blueprints/Game/OpenSpaceInst.OpenSpaceInst_C|SetLastTransform _asopen_space_inst (Transformation|GetActorTransform))
    (Game|OpenLevel(byName) "MainMap")))

(fn ConstructionScript
  (|CallParentFunction))