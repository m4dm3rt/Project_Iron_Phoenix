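; OpenSpaceController is the controller for the open-space shooter, handling hotkeys for HUD widgets.
; Tab flip-flops the cargo hold widget between expanded and folded, switching the input mode with each state without pausing the game.
; R toggles whether the minimap rotates.
; Both keys look up their widget by class on each press and act on the first valid instance found.
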(event Input|KeyboardEvents|R
  (params (Key :type Key%20Structure :default "None"))
  (:Pressed
    (bind _foundwidgets (Widget|GetAllWidgetsOfClass "/Game/OpenSpaceShooter/Widgets/WBP_Minimap.WBP_Minimap_C" false))
    (Utilities|IsValid (Utilities|Array|Get(acopy) _foundwidgets)
      (:Is%20Valid
        (Variables|/Game/OpenSpaceShooter/Widgets/WBP_Minimap.WBP_Minimap_C|SetMapRotates (Utilities|Array|Get(acopy) _foundwidgets) (not (Variables|/Game/OpenSpaceShooter/Widgets/WBP_Minimap.WBP_Minimap_C|GetMapRotates (Utilities|Array|Get(acopy) _foundwidgets))))))))

(event Input|KeyboardEvents|Tab
  (params (Key :type Key%20Structure :default "None"))
  (:Pressed
    (bind _foundwidgets (Widget|GetAllWidgetsOfClass "/Game/OpenSpaceShooter/Widgets/WBP_CargoHold.WBP_CargoHold_C" false))
    (Utilities|IsValid (Utilities|Array|Get(acopy) _foundwidgets)
      (:Is%20Valid
        (Utilities|FlowControl|FlipFlop
          (:A
            (Default|Expand (Utilities|Array|Get(acopy) _foundwidgets))
            (CallFunction|SetInputMode "NewEnumerator1" false))
          (:B
            (Default|Fold (Utilities|Array|Get(acopy) _foundwidgets))
            (CallFunction|SetInputMode "NewEnumerator0" false)))))))

(fn ConstructionScript)