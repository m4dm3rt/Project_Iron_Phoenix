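; Blueprint function library of shared helpers for the OpenSpaceShooter game.
; Linear searches find the closest location or actor to a reference, starting from the first array element.
; SetInputMode sets pause state, then switches player 0 between game, UI or combined input with matching cursor visibility.
; Lookup helpers return the player pawn's InventoryComponent and a target's child actors filtered by class, optionally including descendants.
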(fn FindClosestLocation
  (params (SelfLocation :type Vector) (OtherLocations :type Array%20of%20Vectors))
  (LocalVariables|SetTempPoint (Utilities|Array|Get(acopy) OtherLocations))
  (for _array_element OtherLocations
    (if (< (Math|Vector|VectorLength (- _array_element SelfLocation)) (Math|Vector|VectorLength (- SelfLocation (LocalVariables|GetTempPoint))))
      (bind _output_get (LocalVariables|SetTempPoint _array_element))))
  (return _output_get))

(fn FindClosestActor
  (params (SelfActor :type Actor%20Object%20Reference) (OtherActors :type Array%20of%20Actor%20Object%20References))
  (LocalVariables|SetTempActor (Utilities|Array|Get(acopy) OtherActors))
  (for _array_element OtherActors
    (if (< (Transformation|GetDistanceTo _array_element SelfActor) (Transformation|GetDistanceTo SelfActor (LocalVariables|GetTempActor)))
      (bind _output_get (LocalVariables|SetTempActor _array_element))))
  (return _output_get))

(fn SetInputMode
  (params (NewMode :type E_InputMode%20Enum :default "NewEnumerator1") (PauseGame :type Boolean))
  (bind _returnvalue (Game|GetPlayerController 0))
  (Game|SetGamePaused 0 PauseGame)
  (switch Utilities|FlowControl|Switch|SwitchonE_InputMode NewMode
    (:NewEnumerator1
      (Input|SetInputModeGameandUI _returnvalue 0 "LockAlways" true false)
      (Variables|/Script/Engine.PlayerController|SetbShowMouseCursor _returnvalue true :!label _label))
    (:NewEnumerator0
      (Input|SetInputModeGameOnly _returnvalue false)
      (Variables|/Script/Engine.PlayerController|SetbShowMouseCursor _returnvalue false))
    (:NewEnumerator2
      (Input|SetInputModeUIOnly _returnvalue 0 "DoNotLock" false)
      (goto _label))))

(fn GetPlayerInventory
  (return (Actor|GetComponentbyClass (Game|Player|GetPlayerPawn 0) "/Game/OpenSpaceShooter/Blueprints/Components/InventoryComponent.InventoryComponent_C")))

(fn GetChildActors
  (params (Target :type Actor%20Object%20Reference) (IncludeDecendants :type Boolean) (FilterClass :type Actor%20Class%20Reference))
  (bind _filteredarray (Utilities|Array|FilterArray (Actor|GetAllChildActors Target IncludeDecendants) FilterClass))
  (return _filteredarray))