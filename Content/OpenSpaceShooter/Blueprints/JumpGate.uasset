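; Jump gate actor that hyper-jumps a ship to a linked Destination gate.
; Input from a ship disables its controls, then a timeline pulls it to the entry point while particles, sound pitch and camera rotation follow the charge.
; Both gates play launch effects, and the destination places the ship at its exit with a forward velocity boost, later restoring controls.
; Construction can make a gate an invisible, collision-free destination with a named marker.
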(event HandleInput(InputReceiver)
  (params (Sender :type Input%20Sender%20Object%20Reference) (Input :type String))
  (bind _returnvalue (Components|GetOwner Sender))
  (bind _asship_base (Utilities|Casting|CastToShipBase _returnvalue))
  (CallFunction|InitiateHyperJump _asship_base)
  (bind _asship_controllable (Utilities|Casting|CastToShipControllable _returnvalue))
  (Default|SetControlsEnabled _asship_controllable false))

(event Custom|Initiate%20Hyper%20Jump
  (params (Passenger :type Ship%20Base%20Object%20Reference))
  (bind _p_hyperjump (Variables|Default|GetP_HyperJump))
  (Variables|Default|GetDestination
    (:then
      (Camera|PlayWorldCameraShake "/Game/OpenSpaceShooter/Blueprints/HyperJumpShake.HyperJumpShake_C" (Math|Vector|SelectVector (Camera|GetCameraLocation (Game|GetPlayerCameraManager 0)) (Transformation|GetActorLocation Passenger) (== Passenger (Game|Player|GetPlayerPawn 0))) 5e+03 5e+03)
      (Components|Timeline|SetPlayRate (Variables|Default|GetHyper%20Jump%20Line) 0.2)
      (Utilities|FlowControl|Sequence
        (:then_0
          (bind _output (Timeline|Hyper%20Jump%20Line PlayFromStart)
            (:Update
              (Default|UpdateManeuver Passenger 0.0 0.0 0.0 0.0 0.0 0.0)
              (Pawn|SetControlRotation (Pawn|GetController Passenger) (Math|Rotator|Lerp(Rotator) (Pawn|GetControlRotation Passenger :!class /Script/Engine.Pawn) (Transformation|GetActorRotation Passenger) 0.05 true))
              (Effects|Components|ParticleSystem|SetVectorParameter _p_hyperjump "Size" (Math|Vector|MakeVector 1e+02 (Math|Float|Lerp 0.0 3e+04 _output) 0.0))
              (Transformation|SetRelativeLocation _p_hyperjump (Math|Vector|MakeVector (* (Math|Float|Lerp 0.0 3e+04 _output) 0.4) 0.0 0.0) false false)
              (Audio|Components|Audio|SetPitchMultiplier (Variables|Default|GetHyperJumpCharge_Cue) (Math|Float|Lerp 0.4 2.0 _output))
              (Transformation|SetActorTransform Passenger (Math|Transform|Lerp(Transform) (Transformation|GetActorTransform Passenger) (Transformation|GetWorldTransform (Variables|Default|GetEntryPoint)) (Math|Float|Power _output 2.0))))
            (:Finished
              (CallFunction|ExitHyperJump (Variables|Default|GetDestination) Passenger true)
              (CallFunction|ExitHyperJump Passenger false))))
        (:then_1
          (Components|Activation|Activate (Variables|Default|GetP_HyperJump) true)
          (Audio|Components|Audio|Play (Variables|Default|GetHyperJumpCharge_Cue) 0.0))))
    (:else)))

(event Custom|Exit%20Hyper%20Jump
  (params (Passenger :type Ship%20Base%20Object%20Reference) (IsDestination :type Boolean))
  (Components|Activation|Deactivate (Variables|Default|GetP_HyperJump))
  (Audio|Components|Audio|FadeOut (Variables|Default|GetHyperJumpCharge_Cue) 1.0 0.0 "Linear" :!class /Script/Engine.AudioComponent)
  (Audio|PlaySoundatLocation "/Game/OpenSpaceShooter/Audio/HyperJumpLaunch_Cue.HyperJumpLaunch_Cue" (Transformation|GetActorLocation) "0, 0, 0" 1.0 1.0 0.0 0 0 0 0)
  (Effects|SpawnEmitterAttached "/Game/OpenSpaceShooter/Particles/P_HyperJumpLaunch.P_HyperJumpLaunch" (Variables|Default|GetHull) "None" "0, 0, 0" "0,180.000000, 0")
  (if IsDestination
    (Transformation|SetActorTransform Passenger (Transformation|GetWorldTransform (Variables|Default|GetExitPoint)))
    (Default|SetVelocity Passenger (* (Transformation|GetActorForwardVector Passenger) (+ (Variables|/Game/OpenSpaceShooter/Blueprints/ShipBase.ShipBase_C|GetMaxSpeed Passenger) 3e+04)))
    (bind _asship_controllable (Utilities|Casting|CastToShipControllable Passenger)
      (:then
        (Utilities|FlowControl|Sequence
          (:then_0
            (Default|TempDisableCameraLag _asship_controllable)
            (Utilities|FlowControl|Delay 0.05)
            (Audio|PlaySoundatLocation "/Game/OpenSpaceShooter/Audio/HyperJumpLaunch_Cue.HyperJumpLaunch_Cue" (Transformation|GetActorLocation) "0, 0, 0" 1.0 1.0 0.0 0 0 0 0 :!label _label))
          (:then_1
            (Utilities|FlowControl|Delay 1.0)
            (Default|SetControlsEnabled _asship_controllable true))))
      (:CastFailed
        (goto _label)))))

(event EventBeginPlay
  (|CallParentFunction) ; This node is disabled and will not be called.\nDrag off pins to build functionality.
)

(event Collision|EventActorBeginOverlap
  (params (OtherActor :type Actor%20Object%20Reference))
  (|CallParentFunction OtherActor) ; This node is disabled and will not be called.\nDrag off pins to build functionality.
)

(event EventTick
  (params (DeltaSeconds :type Float%20%28single-precision%29))
  (|CallParentFunction DeltaSeconds) ; This node is disabled and will not be called.\nDrag off pins to build functionality.
)

(fn ConstructionScript
  (bind _asinvisibledestination (Variables|Default|GetAsInvisibleDestination))
  (bind _returnvalue (not _asinvisibledestination))
  (|CallParentFunction)
  (Rendering|SetVisibility (Variables|Default|GetTargetMarker) _asinvisibledestination true)
  (Rendering|SetVisibility (Variables|Default|GetHull) _returnvalue false)
  (Collision|SetActorEnableCollision _returnvalue)
  (Rendering|Components|TextRender|SetText (Variables|Default|GetMarkerText) (Utilities|Text|ToText(String) (Variables|Default|GetName))))